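; One-shot wind gust ("bourrasque") actor that pushes tagged objects along the view direction of Jojo player characters.
; On BeginPlay it sphere-traces from its Sphere along each BP_PlayerChara_Jojo camera's forward vector, over RangeBourrasque.
; Hit components on "bourrasque"-tagged actors get physics enabled and an impulse scaled by PushesForce.
; The actor then destroys itself without waiting for the in-loop Delay, which only re-enables physics.
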(event `self.ReceiveBeginPlay`
  (bind _sphere (`self.Sphere`))
  (bind _returnvalue (`SceneComponent.K2_GetComponentLocation` _sphere))
  (bind _outactors (`GameplayStatics.GetAllActorsOfClass` "/Game/BP/BP_PlayerChara_Jojo.BP_PlayerChara_Jojo_C"))
  (for _array_element _outactors
    (bind _returnvalue_2 (`SceneComponent.GetForwardVector` (`/Game/BP/BP_PlayerChara_Jojo.Camera` _array_element)))
    (bind (_outhits _returnvalue_3) (`KismetSystemLibrary.SphereTraceMultiForObjects` _returnvalue (+ (* _returnvalue_2 (`self.range Bourrasque`)) _returnvalue) (`SphereComponent.SphereRadius` _sphere) (`|MakeArray` "ObjectTypeQuery1" "ObjectTypeQuery2" "ObjectTypeQuery3" "ObjectTypeQuery4" "ObjectTypeQuery6" "ObjectTypeQuery7" :!type "EObjectTypeQuery Enum") false (`|MakeArray` _array_element :!type "Actor Object Reference")))
    (if _returnvalue_3
      (for _array_element_2 _outhits
        (bind (_bblockinghit _binitialoverlap _time _distance _location _impactpoint _normal _impactnormal _physmat _hitactor _hitcomponent) (`GameplayStatics.BreakHitResult` _array_element_2))
        (for _array_element_3 (`Actor.Tags` _hitactor)
          (if (== _array_element_3 "bourrasque")
            (`PrimitiveComponent.SetSimulatePhysics` _hitcomponent true)
            (`PrimitiveComponent.AddImpulse` _hitcomponent (* _returnvalue_2 (`self.Pushes Force`)) "None" false)
            (`KismetSystemLibrary.Delay` 5.0)
            (`PrimitiveComponent.SetSimulatePhysics` _hitcomponent true))))))
  (`self.K2_DestroyActor`))

(fn `UserConstructionScript`)