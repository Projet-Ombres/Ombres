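; BP_LevelStreamer is a trigger volume that streams sublevels when the player character enters it.
; On overlap with BP_PlayerChara, it loops through SubLevelsToLoad, loading each non-blocking and visible, then loops through SubLevelsToUnload to unload them.
; Both loops use latent stream-level calls chained through a shared index, so each level finishes before the next starts.
; The construction script sizes the Box from BoxScale.
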(event `self.Box.OnComponentBeginOverlap`
  (params (OverlappedComponent :type "PrimitiveComponent Object Reference") (OtherActor :type "Actor Object Reference") (OtherComp :type "PrimitiveComponent Object Reference") (OtherBodyIndex :type Integer) (bFromSweep :type Boolean) (SweepResult :type "HitResult Structure (by ref)"))
  (cast `/Game/BP/BP_PlayerChara` OtherActor)
  (set `self.SubLevelIndex` 0)
  (if (< (`self.SubLevelIndex`) (`KismetArrayLibrary.Array_Length` (`self.SubLevelsToLoad`))) :!label _label
    (`GameplayStatics.LoadStreamLevel` (`|GetArrayItem` (`self.SubLevelsToLoad`) (`self.SubLevelIndex`)) true)
    (`/Engine/EditorBlueprintResources/StandardMacros.IncrementInt` (`self.SubLevelIndex`)
      (:`  `
        (goto _label)))
    (else
      (set `self.SubLevelIndex` 0)
      (if (< (`self.SubLevelIndex`) (`KismetArrayLibrary.Array_Length` (`self.SubLevelsToUnload`))) :!label _label_2
        (`GameplayStatics.UnloadStreamLevel` (`|GetArrayItem` (`self.SubLevelsToUnload`) (`self.SubLevelIndex`)))
        (`/Engine/EditorBlueprintResources/StandardMacros.IncrementInt` (`self.SubLevelIndex`)
          (:`  `
            (goto _label_2)))))))

(fn `UserConstructionScript`
  (`BoxComponent.SetBoxExtent` (`self.Box`) (`KismetMathLibrary.Conv_DoubleToVector` (`self.BoxScale`)) false))