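; Ambient bird flock actor that scatters birds on the ground and sends them flying off when the player approaches.
; BeginPlay spawns a random number of skeletal meshes, aligned by downward traces, each with its own delay and speed.
; Player overlap rerolls flight directions until line traces are clear, changing the cone after repeated failures.
; FlyAway loops by one-frame delay, moving birds with a timeline-eased liftoff, then destroys the actor.
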(event `self.ReceiveBeginPlay`
  ;[1 0 0.6] Beginplay
  (`self.SpawnBirds`))

(event `self.Sphere.OnComponentBeginOverlap`
  (params (OverlappedComponent :type "PrimitiveComponent Object Reference") (OtherActor :type "Actor Object Reference") (OtherComp :type "PrimitiveComponent Object Reference") (OtherBodyIndex :type Integer) (bFromSweep :type Boolean) (SweepResult :type "HitResult Structure (by ref)"))
  ;[1 0 0.8547] Begin overlap
  (if (`.bSuccess` (cast `/Game/BP/BP_PlayerChara` OtherActor :!pure true))
    (`/Engine/EditorBlueprintResources/StandardMacros.DoOnce` false
      (:`Completed`
        (`self.DefineBirdDirection`)))))

(event `self.ReceiveTick`
  (params (DeltaSeconds :type "Float (single-precision)"))
  ;[1 0 0.9627] Event tick
  (set `self.DeltaSec` DeltaSeconds))

(event `SpawnBirds`
  (bind (_minmaxnumberofbirds_x _minmaxnumberofbirds_y) (`KismetMathLibrary.BreakVector2D` (`self.MinMaxNumberOfBirds`)))
  (bind _returnvalue (`SceneComponent.K2_GetComponentLocation` (`self.SpawnedBirdRef`)))
  ;[0 1 0.976] Spawn birds
  ;[1 1 1] Define number of birds
  (bind _output_get (set `self.NumberOfBirds` (`KismetMathLibrary.RandomIntegerInRange` (`KismetMathLibrary.FTrunc` _minmaxnumberofbirds_x) (`KismetMathLibrary.FTrunc` _minmaxnumberofbirds_y))))
  (for _ (range (+ _output_get 1))
    ;[1 1 1] Add skeletal mesh
    (bind _returnvalue_2 (`AddComponent|NODE_AddSkeletalMeshComponent-0` :`RelativeTransform` (`KismetMathLibrary.MakeTransform` (`KismetMathLibrary.RotateAngleAxis` (`KismetMathLibrary.MakeVector` (`KismetMathLibrary.RandomFloatInRange` 0.0 (`self.BirdSpawningRadius`))) (`KismetMathLibrary.RandomFloatInRange` 0.0 360.0) (0.0 0.0 1.0)))))
    (bind _output_get_2 (set `self.SpawnedBirdRef` _returnvalue_2))
    (`KismetArrayLibrary.Array_Add` (`self.BirdsArray`) _output_get_2)
    ;[1 1 1] Tracer down to find ground
    (bind _outhit (`KismetSystemLibrary.LineTraceSingle` _returnvalue (- _returnvalue (0.0 0.0 1000.0)) "TraceTypeQuery1"))
    ;[1 1 1] Positionnement de l'oiseau par rapport au sol
    (`SceneComponent.K2_SetWorldTransform` (`self.SpawnedBirdRef`) (`KismetMathLibrary.MakeTransform` (+ (`.Location` (`GameplayStatics.BreakHitResult` _outhit)) (* (`.Normal` (`GameplayStatics.BreakHitResult` _outhit)) (`self.HalfHeightBirdOffset`))) (`KismetMathLibrary.MakeRotator` (.roll (`KismetMathLibrary.MakeRotFromX` (`.Normal` (`GameplayStatics.BreakHitResult` _outhit)))) (- (.pitch (`KismetMathLibrary.MakeRotFromX` (`.Normal` (`GameplayStatics.BreakHitResult` _outhit)))) 90.0) (.yaw (`KismetMathLibrary.MakeRotFromX` (`.Normal` (`GameplayStatics.BreakHitResult` _outhit)))))) false false)
    ;[1 1 1] Ajout d'une rotation aux oiseaux sur le sol
    (`self.K2_AddActorLocalRotation` (`KismetMathLibrary.MakeRotator` 0.0 0.0 (`KismetMathLibrary.RandomFloatInRange` 0.0 360.0)))
    ;[1 1 1] Define time before bird fly off
    (`KismetArrayLibrary.Array_Add` (`self.FlyingAwayBirdDelayArray`) (`KismetMathLibrary.RandomFloatInRange` 0.0 (`self.MaxTimeBeforeBirdsFlyOff`)))
    ;[1 1 1] Define bird speed
    (`KismetArrayLibrary.Array_Add` (`self.IndividualSpeedBirdArray`) (* 1000.0 (`KismetMathLibrary.RandomFloatInRange` 0.8 1.2)))))

(event `DefineBirdDirection`
  (bind _returnvalue (>= (`self.NombreDe"DefineBirdDirection"Tentative`) 50))
  ;[0 1 0.9418] Define Bird direction
  ;[1 1 1] Waiting 1 frame each x time to avoid infinite loop
  (if (== (mod (`self.NombreDe"DefineBirdDirection"Tentative`) 60) 0)
    (`KismetSystemLibrary.Delay` 0.0))
  (`/Engine/EditorBlueprintResources/StandardMacros.IncrementInt` (`self.NombreDe"DefineBirdDirection"Tentative`)
    (:`  `
      ;[1 0 0.01752] IMPORTANT! rénitialise le tirage de direction
      (`KismetArrayLibrary.Array_Clear` (`self.BirdDirectionValide?Array`))
      (for (_ _array_index) (`self.BirdsArray`)
        ;[1 1 1] tirage d'une direction de debug
        (set `self.Debug direction` (`KismetMathLibrary.RandomUnitVectorInConeInDegrees` (0.0 0.0 1.0) 90.0))
        (bind _returnvalue_2 (* (`KismetMathLibrary.RandomUnitVectorInConeInDegrees` (`KismetMathLibrary.SelectVector` (`self.Debug direction`) (0.0 0.0 1.0) _returnvalue) (`KismetMathLibrary.SelectFloat` 5.0 60.0 _returnvalue)) (`|GetArrayItem` (`self.IndividualSpeedBirdArray`) _array_index)))
        ;[1 1 1] setting du vecteur de déplacement de chaque oiseau
        (`KismetArrayLibrary.Array_Add` (`self.BirdVectorDirectionArray`) _returnvalue_2)
        ;[1 1 1] vérification de la validité de la direction de vol (non valide si collision possible)
        (bind (_outhit _returnvalue_3) (`KismetSystemLibrary.LineTraceSingle` :`Start` (`SceneComponent.K2_GetComponentLocation` (`self.DefaultSceneRoot`)) :`End` (* _returnvalue_2 8000.0) :`TraceChannel` "TraceTypeQuery1" :`DrawTime` 1.0))
        (`KismetArrayLibrary.Array_Add` (`self.BirdDirectionValide?Array`) _returnvalue_3))
      ;[1 1 1] Si direction valide, lance l'envol, sinon relance le tirage de direction
      (if (`KismetArrayLibrary.Array_Contains` (`self.BirdDirectionValide?Array`) true)
        (`self.DefineBirdDirection`)
        (else
          (`self.FlyAway`))))))

(event `FlyAway`
  (bind _flyingawaybirdref (`self.FlyingAwayBirdRef`))
  (bind _flyingawaybirdref_2 (`self.FlyingAwayBirdRef`))
  (bind _returnvalue (`SceneComponent.K2_GetComponentLocation` _flyingawaybirdref_2))
  ;[0 1 0.9404] Fly away
  ;[1 1 1] Delay de 1 frame pour éviter l'infinite loop
  (`KismetSystemLibrary.Delay` 0.0)
  (for (_array_element _array_index) (`self.BirdsArray`)
    (set `self.FlyingAwayBirdRef` _array_element)
    (set `self.FlyingAwayBirdIndex` _array_index)
    ;[1 1 1] Vérification si l'oiseau à attendu son temps de delay
    (if (>= (`self.TimeSinceLastActivation`) (`|GetArrayItem` (`self.FlyingAwayBirdDelayArray`) (`self.FlyingAwayBirdIndex`)))
      (`|ExecutionSequence`
        (:`then_0`
          ;[1 1 1] setting du multiplier de vitesse en fonction d'une courbe pour rendre l'envol plus naturel
          (`/Engine/EditorBlueprintResources/StandardMacros.DoOnce` false
            (:`Completed`
              (bind (_direction _newtrack_0) (`Timeline|Timeline_0` :!via `PlayFromStart`)
                (:`Update`
                  (set `self.lift-off multiplier` (* _newtrack_0 (`self.BirdSpeed`))))))))
        (:`then_1`
          ;[1 1 1] setting de la nouvelle position de l'oiseau
          (`SceneComponent.K2_SetWorldLocation` _flyingawaybirdref (+ (`SceneComponent.K2_GetComponentLocation` _flyingawaybirdref) (* (* (`|GetArrayItem` (`self.BirdVectorDirectionArray`) (`self.FlyingAwayBirdIndex`)) (`self.DeltaSec`)) (`self.lift-off multiplier`))) false false)
          ;[1 1 1] alignement du mesh de l'oiseau avec sa direction de vol
          (`SceneComponent.K2_SetWorldRotation` _flyingawaybirdref_2 (`KismetMathLibrary.FindLookAtRotation` _returnvalue (+ _returnvalue (* (`|GetArrayItem` (`self.BirdVectorDirectionArray`) (`self.FlyingAwayBirdIndex`)) 100.0))) false false)
          ;[1 0 0.07262] ajout d'une rotation suplémentaire car le mesh actuel a été mal produit (forward not= xVector)
          (`SceneComponent.K2_AddLocalRotation` (`self.FlyingAwayBirdRef`) (`KismetMathLibrary.MakeRotator` 0.0 0.0 -90.0) false false)))))
  (`|ExecutionSequence`
    (:`then_0`
      ;[1 1 1] lancement de l'animation des oiseaux
      (`/Engine/EditorBlueprintResources/StandardMacros.DoOnce` false
        (:`Completed`
          (for _array_element_2 (`self.BirdsArray`)
            (`SkeletalMeshComponent.PlayAnimation` _array_element_2 "/Game/art/SM/Birds/Bird_Asset_Anim.Bird_Asset_Anim" true)))))
    (:`then_1`
      ;[1 1 1] update du temps écoulé depuis l'activation
      (set `self.TimeSinceLastActivation` (+ (`self.TimeSinceLastActivation`) (`self.DeltaSec`)))
      ;[1 1 1] destruction de l'acteur après un certain temps après l'activation
      (if (> (`self.TimeSinceLastActivation`) (`KismetMathLibrary.Lerp` 30.0 (`self.TimeBeforeBirdDisappearInSky`) (`self.BirdSpeed`)))
        (`self.K2_DestroyActor`)
        (else
          (`self.FlyAway`))))))

(fn `UserConstructionScript`
  (`SphereComponent.SetSphereRadius` (`self.Sphere`) (`self.TriggerRadius`) true)
  (`SphereComponent.SetSphereRadius` (`self.Sphere1`) (`self.BirdSpawningRadius`) true))