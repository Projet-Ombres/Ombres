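; BP_VideoTuto is a trigger that shows a tutorial video when the player character overlaps its box.
; On overlap it checks through the player's main interface that no cinematic has started, then passes a DoOnce so it fires only once.
; If the player has tutorials enabled, it calls ShowVideo on the tutorial widget with its title, text, media texture and video source.
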(event `self.Box.OnComponentBeginOverlap`
  (params (OverlappedComponent :type "PrimitiveComponent Object Reference") (OtherActor :type "Actor Object Reference") (OtherComp :type "PrimitiveComponent Object Reference") (OtherBodyIndex :type Integer) (bFromSweep :type Boolean) (SweepResult :type "HitResult Structure (by ref)"))
  (bind _asbp_player_chara (cast `/Game/BP/BP_PlayerChara` OtherActor))
  (bind _acinematicisrunning (`/Game/BP/Widgets/Widget_Main_Interface.CheckIfCinematicStarted` (`/Game/BP/BP_PlayerChara.MainInterface` _asbp_player_chara)))
  (if (not _acinematicisrunning)
    (`/Engine/EditorBlueprintResources/StandardMacros.DoOnce` false
      (:`Completed`
        (if (`/Game/BP/BP_PlayerChara.TutoEnabled` _asbp_player_chara)
          (`/Game/BP/Widgets/Widget_Tutorial.ShowVideo` (`/Game/BP/Widgets/Widget_Main_Interface.Widget_Tutorial` (`/Game/BP/BP_PlayerChara.MainInterface` _asbp_player_chara)) (`self.TextToShow`) (`self.VideoTexture`) (`self.Source`) (`self.Title`)))))))

(fn `UserConstructionScript`)