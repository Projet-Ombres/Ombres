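; Transmutation circle actor that starts a drawing minigame when the player overlaps its box, switching the camera and suspending movement and spells.
; Cursor traces convert to UVs, painting render targets and driving the Abadel mesh's hand.
; Three steps confine drawing to successively inner radial zones, each advancing when its ink runs out.
; Completion restores the player, then rotates and grows the circle before playing the Cercle_Quartier2 sequence.
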(event `StopDrawing`
  (bind _returnvalue (`GameplayStatics.GetPlayerController` 0))
  ;[1 1 1] StopDrawing
  (set `self.CircleComplete` true)
  (`SceneComponent.SetVisibility` (`self.AbadelMesh`) false false)
  (`/Game/BP/Widgets/TransmutationCircle/Widget_TransmutationCircle.FadeOutAndRemove` (`self.TransmutationWidget`))
  (`PlayerController.SetViewTargetWithBlend` (`GameplayStatics.GetPlayerController` 0) (`GameplayStatics.GetPlayerCharacter` 0) 1.0 "VTBlend_EaseInOut" 1.5 false)
  (`KismetSystemLibrary.Delay` 1.0)
  (`Controller.ResetIgnoreLookInput` _returnvalue)
  (`Controller.ResetIgnoreMoveInput` _returnvalue)
  (bind _asbp_player_chara (cast `/Game/BP/BP_PlayerChara` (`GameplayStatics.GetPlayerCharacter` 0)))
  (set `/Game/BP/BP_PlayerChara.Drawing` false _asbp_player_chara)
  (set `SkywalkComponent.SpellEnabled` true (`/Game/BP/BP_PlayerChara.Skywalk` _asbp_player_chara))
  (set `/Game/BP/Components/Pouvoirs/BPC_Crystallization.SpellEnabled` true (`/Game/BP/BP_PlayerChara.BPC_Crystallization` _asbp_player_chara))
  (set `/Game/BP/Components/Pouvoirs/BPC_Ping.SpellEnabled` true (`/Game/BP/BP_PlayerChara.BPC_Ping` _asbp_player_chara))
  (set `/Game/BP/Components/CapacitéPhysique/BPC_Jump.CanJump` true (`/Game/BP/BP_PlayerChara.BPC_Jump` _asbp_player_chara))
  (bind _maininterface (`/Game/BP/BP_PlayerChara.MainInterface` _asbp_player_chara))
  (`Widget.SetVisibility` (`/Game/BP/Widgets/Widget_Main_Interface.Widget_Powers` _maininterface) "SelfHitTestInvisible")
  (`Widget.SetVisibility` (`/Game/BP/Widgets/Widget_Main_Interface.Widget_Boussole_Pointeur` _maininterface) "SelfHitTestInvisible")
  (`self.SetActorHiddenInGame` _asbp_player_chara false)
  (`self.OnCircleComplete`)
  (`self.StartRotating`)
  (`self.Grow`))

(event `Grow`
  ;[1 1 1] Grow
  (`GameplayStatics.SpawnEmitterAttached` "/Game/FX_LastShock_2.FX_LastShock_2" (`self.DefaultSceneRoot`))
  (bind _outputvalue (`CustomTimeline.StartCustomTimeline` (/ 1.0 (`self.GrowDuration`)))
    (:`Update`
      (`SceneComponent.SetRelativeScale3D` (`self.StaticMesh`) (`KismetMathLibrary.Conv_DoubleToVector` (`KismetMathLibrary.Lerp` 1.0 (`self.GrowScale`) _outputvalue))))
    (:`Finished`
      (`KismetSystemLibrary.Delay` 2.0)
      (bind (_outactor _returnvalue) (`LevelSequencePlayer.CreateLevelSequencePlayer` "/Game/Cinematique/Cercle_Quartier2.Cercle_Quartier2"))
      (`MovieSceneSequencePlayer.Play` _returnvalue)
      (`KismetSystemLibrary.PrintString` "Hello"))))

(event `StartRotating`
  (bind _rotatingmovement (`self.RotatingMovement`))
  ;[1 1 1] Start rotating
  (`ActorComponent.Activate` _rotatingmovement false)
  (set `RotatingMovementComponent.RotationRate` (`KismetMathLibrary.MakeRotator` 0.0 0.0 (`self.RotationRate`)) _rotatingmovement))

(event `self.ReceiveTick`
  (params (DeltaSeconds :type "Float (single-precision)"))
  (bind _transmutationwidget (`self.TransmutationWidget`))
  (bind _maxink (`self.MaxInk`))
  (bind (_worldposition _worlddirection _returnvalue) (`GameplayStatics.DeprojectScreenToWorld` (`self.PlayerController`) (`self.TargetPosition`)))
  (bind _returnvalue_2 (`SceneComponent.K2_GetComponentLocation` (`self.Camera`)))
  (bind (_locationx _locationy) (`PlayerController.GetMousePosition` (`self.PlayerController`)))
  (bind _returnvalue_3 (/ (`self.InkLeft`) (`self.MaxInk`)))
  (bind _returnvalue_4 (`KismetMathLibrary.MakeVector2D` _locationx _locationy))
  ;[1 0 0.9249] Event tick
  (`/Engine/EditorBlueprintResources/StandardMacros.IsValid` _transmutationwidget
    (:`Is Valid`
      (if (not (== _returnvalue_4 (`self.LastMousePosition`)))
        (bind _output_get (set `self.LastMousePosition` _returnvalue_4))
        (set `self.TargetPosition` (`KismetMathLibrary.MakeVector2D` (`KismetMathLibrary.BreakVector2D` _output_get) (`.Y` (`KismetMathLibrary.BreakVector2D` _output_get)))))
      (`/Game/BP/Widgets/TransmutationCircle/Widget_TransmutationCircle.UpdateCursor` _transmutationwidget (`self.TargetPosition`))
      (if (`self.Drawing`)
        (if _returnvalue
          (bind (_outhit _returnvalue_5) (`KismetSystemLibrary.LineTraceSingle` :`Start` _returnvalue_2 :`End` (+ _returnvalue_2 (* (`KismetMathLibrary.Normal` (- _worldposition _returnvalue_2)) 500.0)) :`TraceChannel` "TraceTypeQuery13" :`bIgnoreSelf` false :`DrawTime` 10.0))
          (if _returnvalue_5
            (cast `/Game/BP/Class/TransmutationCircle/BP_TransmutationCircle` (`.HitActor` (`GameplayStatics.BreakHitResult` _outhit)))
            (bind _uv (`GameplayStatics.FindCollisionUV` _outhit))
            (bind _allowedtodraw (`self.IsAllowedToDraw` _uv))
            (if _allowedtodraw
              (`self.Draw` _uv)
              (bind _returnvalue_6 (`KismetMathLibrary.Distance2D` _uv (`self.PreviousUVTouched`)))
              (set `self.InkLeft` (- (`self.InkLeft`) (* (select `bool` (> _returnvalue_6 0.1) :`false` _returnvalue_6 :`true` 0.01) (`self.InkConsumption`))))
              (`/Game/BP/Widgets/TransmutationCircle/Widget_TransmutationCircle.UpdateJauge` (`self.TransmutationWidget`) (/ (`self.InkLeft`) (`self.MaxInk`)))
              (set `self.PreviousUVTouched` _uv)
              (if (<= (`self.InkLeft`) 0.0)
                (set `self.Drawing` false)
                (`KismetSystemLibrary.Delay` (`self.DelayBetweenSteps`))
                (`/Engine/EditorBlueprintResources/StandardMacros.IncrementInt` (`self.Step`)
                  (:`  `
                    (`self.UpdateBonusDrawings`)
                    (if (< (`self.Step`) 4)
                      (bind _outputvalue (`CustomTimeline.StartCustomTimeline` 2.0)
                        (:`then`
                          (set `self.InkLeft` (select `bool` (== (`self.Step`) 3) :`false` _maxink :`true` (/ _maxink 3.0))))
                        (:`Update`
                          (`/Game/BP/Widgets/TransmutationCircle/Widget_TransmutationCircle.UpdateJauge` (`self.TransmutationWidget`) (* _outputvalue _returnvalue_3)))
                        (:`Finished`
                          (`/Game/BP/Widgets/TransmutationCircle/Widget_TransmutationCircle.UpdateJauge` (`self.TransmutationWidget`) _returnvalue_3)))
                      (else
                        (`self.StopDrawing`)))))))))))))

(event `MoveCursorX`
  (params (AxisValue :type "Float (double-precision)"))
  (bind (_targetposition_x _targetposition_y) (`KismetMathLibrary.BreakVector2D` (`self.TargetPosition`)))
  (set `self.TargetPosition` (`KismetMathLibrary.MakeVector2D` (+ (* (select `bool` (`self.Drawing`) :`false` (* AxisValue (`self.SpeedMultiplierWhenNotDrawing`)) :`true` AxisValue) (select `bool` (`/Game/BP/BP_Controller.PlayingWithKeyboard?` (`self.PlayerController`)) :`false` 3.0 :`true` 1.0 :!type "Float (single-precision)")) _targetposition_x) _targetposition_y)))

(event `UpdateBonusDrawings`
  ;[1 1 1] Update Bonus Drawings count
  (`/Game/BP/Widgets/TransmutationCircle/Widget_TransmutationCircle.UpdateStep` (`self.TransmutationWidget`) (`self.Step`))
  (`MaterialInstanceDynamic.SetScalarParameterValue` (`self.TransmutationCircleMaterialInstance`) "Step" (`KismetMathLibrary.Conv_IntToDouble` (`self.Step`))))

(event `MoveCursorY`
  (params (AxisValue :type "Float (double-precision)"))
  (bind (_targetposition_x _targetposition_y) (`KismetMathLibrary.BreakVector2D` (`self.TargetPosition`)))
  (set `self.TargetPosition` (`KismetMathLibrary.MakeVector2D` _targetposition_x (- _targetposition_y (* (select `bool` (`self.Drawing`) :`false` (* AxisValue (`self.SpeedMultiplierWhenNotDrawing`)) :`true` AxisValue) (select `bool` (`/Game/BP/BP_Controller.PlayingWithKeyboard?` (`self.PlayerController`)) :`false` 3.0 :`true` 1.0 :!type "Float (single-precision)"))))))

(event `self.ReceiveBeginPlay`
  (bind _transmutationcirclematerialinstance (`self.TransmutationCircleMaterialInstance`))
  ;[0.9428 0 1] Begin play
  (bind _asbp_controller (cast `/Game/BP/BP_Controller` (`GameplayStatics.GetPlayerController` 0)))
  (set `self.PlayerController` _asbp_controller)
  (bind _returnvalue (`KismetMaterialLibrary.CreateDynamicMaterialInstance` "/Game/BP/Class/TransmutationCircle/M_Drawing.M_Drawing"))
  (set `self.DrawingMaterialInstance` _returnvalue)
  (bind _returnvalue_2 (`KismetMaterialLibrary.CreateDynamicMaterialInstance` "/Game/BP/Class/TransmutationCircle/M_TransmutationCircle.M_TransmutationCircle"))
  (set `self.TransmutationCircleMaterialInstance` _returnvalue_2)
  (`PrimitiveComponent.SetMaterial` (`self.StaticMesh`) 0 _transmutationcirclematerialinstance)
  (`MaterialInstanceDynamic.SetScalarParameterValue` _transmutationcirclematerialinstance "SmallCircleRadius" (`self.SmallCircleRadius`))
  (`MaterialInstanceDynamic.SetScalarParameterValue` _transmutationcirclematerialinstance "MediumCircleRadius" (`self.MediumCircleRadius`))
  (`MaterialInstanceDynamic.SetScalarParameterValue` _transmutationcirclematerialinstance "LargeCircleRadius" (`self.LargeCircleRadius`))
  (`MaterialInstanceDynamic.SetScalarParameterValue` _transmutationcirclematerialinstance "CircleThickness" (`self.CircleThickness`))
  (bind _asabp_transmutation (cast `/Game/BP/Class/TransmutationCircle/ABP_Transmutation` (`SkeletalMeshComponent.GetAnimInstance` (`self.AbadelMesh`))))
  (set `self.ABPTransmutation` _asabp_transmutation)
  (`SkinnedMeshComponent.HideBoneByName` (`self.AbadelMesh`) "LeftUpLeg" "PBO_None")
  (`SkinnedMeshComponent.HideBoneByName` (`self.AbadelMesh`) "RightUpLeg" "PBO_None")
  (`KismetRenderingLibrary.ClearRenderTarget2D` "/Game/BP/Class/TransmutationCircle/TransmutationStep1.TransmutationStep1")
  (`KismetRenderingLibrary.ClearRenderTarget2D` "/Game/BP/Class/TransmutationCircle/TransmutationStep2.TransmutationStep2")
  (`KismetRenderingLibrary.ClearRenderTarget2D` "/Game/BP/Class/TransmutationCircle/TransmutationStep3.TransmutationStep3"))

(event `Draw`
  (params (Location :type "Vector2D Structure"))
  ;[0 0 0] Draw
  (`MaterialInstanceDynamic.SetVectorParameterValue` (`self.DrawingMaterialInstance`) "DrawingPosition" (`KismetMathLibrary.Conv_VectorToLinearColor` (`KismetMathLibrary.Conv_Vector2DToVector` Location)))
  (set `/Game/BP/Class/TransmutationCircle/ABP_Transmutation.HandPosition` Location (`self.ABPTransmutation`))
  (switch `int` (`self.Step`)
    (:`1`
      (`KismetRenderingLibrary.DrawMaterialToRenderTarget` "/Game/BP/Class/TransmutationCircle/TransmutationStep1.TransmutationStep1" (`self.DrawingMaterialInstance`)))
    (:`2`
      (`KismetRenderingLibrary.DrawMaterialToRenderTarget` "/Game/BP/Class/TransmutationCircle/TransmutationStep2.TransmutationStep2" (`self.DrawingMaterialInstance`)))
    (:`3`
      (`KismetRenderingLibrary.DrawMaterialToRenderTarget` "/Game/BP/Class/TransmutationCircle/TransmutationStep3.TransmutationStep3" (`self.DrawingMaterialInstance`)))))

(event `self.Box.OnComponentBeginOverlap`
  (params (OverlappedComponent :type "PrimitiveComponent Object Reference") (OtherActor :type "Actor Object Reference") (OtherComp :type "PrimitiveComponent Object Reference") (OtherBodyIndex :type Integer) (bFromSweep :type Boolean) (SweepResult :type "HitResult Structure (by ref)"))
  ;[1 1 1] On overlap
  (cast `/Game/BP/BP_PlayerChara` OtherActor)
  (if (not (`self.CircleComplete`))
    (`self.SetupCircle`)))

(event `SetupCircle`
  (bind _returnvalue (`GameplayStatics.GetPlayerController` 0))
  ;[0.3372 0.7857 0.875] Setup for drawing -> move the camera and disable inputs
  (set `self.TargetPosition` (/ (`WidgetLayoutLibrary.GetViewportSize`) 2.0))
  (`Widget.SetVisibility` (`/Game/BP/Widgets/Widget_Main_Interface.Widget_Powers` (`/Game/BP/BP_GameInstance.MainInterface` (cast `/Game/BP/BP_GameInstance` (`GameplayStatics.GetGameInstance`) :!pure true))) "Collapsed")
  (`/Engine/EditorBlueprintResources/StandardMacros.IsValid` (`self.TransmutationWidget`)
    (:`Is Valid`
      _)
    (:`Is Not Valid`
      (bind _returnvalue_2 (`|CreateWidget` "/Game/BP/Widgets/TransmutationCircle/Widget_TransmutationCircle.Widget_TransmutationCircle_C"))
      (set `self.TransmutationWidget` _returnvalue_2)))
  (`KismetRenderingLibrary.ClearRenderTarget2D` "/Game/BP/Class/TransmutationCircle/TransmutationStep1.TransmutationStep1")
  (`KismetRenderingLibrary.ClearRenderTarget2D` "/Game/BP/Class/TransmutationCircle/TransmutationStep2.TransmutationStep2")
  (`KismetRenderingLibrary.ClearRenderTarget2D` "/Game/BP/Class/TransmutationCircle/TransmutationStep3.TransmutationStep3")
  (set `self.InkLeft` (`self.MaxInk`))
  (set `self.Step` 1)
  (`self.UpdateBonusDrawings`)
  (`Controller.SetIgnoreMoveInput` _returnvalue true)
  (`Controller.SetIgnoreLookInput` _returnvalue true)
  (`PlayerController.SetViewTargetWithBlend` (`GameplayStatics.GetPlayerController` 0) self 1.0 "VTBlend_EaseInOut" 1.5 false)
  (`KismetSystemLibrary.Delay` 1.0)
  (`UserWidget.AddToViewport` (`self.TransmutationWidget`) 0)
  (bind _asbp_player_chara (cast `/Game/BP/BP_PlayerChara` (`GameplayStatics.GetPlayerCharacter` 0)))
  (set `/Game/BP/BP_PlayerChara.TransmutationCircle` self _asbp_player_chara)
  (set `/Game/BP/BP_PlayerChara.Drawing` true _asbp_player_chara)
  (`Widget.SetVisibility` (`/Game/BP/Widgets/Widget_Main_Interface.Widget_Boussole_Pointeur` (`/Game/BP/BP_PlayerChara.MainInterface` _asbp_player_chara)) "Collapsed")
  (set `SkywalkComponent.SpellEnabled` false (`/Game/BP/BP_PlayerChara.Skywalk` _asbp_player_chara))
  (set `/Game/BP/Components/Pouvoirs/BPC_Ping.SpellEnabled` false (`/Game/BP/BP_PlayerChara.BPC_Ping` _asbp_player_chara))
  (set `/Game/BP/Components/Pouvoirs/BPC_Crystallization.SpellEnabled` false (`/Game/BP/BP_PlayerChara.BPC_Crystallization` _asbp_player_chara))
  (set `/Game/BP/Components/CapacitéPhysique/BPC_Jump.CanJump` false (`/Game/BP/BP_PlayerChara.BPC_Jump` _asbp_player_chara))
  (`self.SetActorHiddenInGame` _asbp_player_chara true)
  (`SceneComponent.SetVisibility` (`self.AbadelMesh`) true false)
  (`/Game/BP/Widgets/TransmutationCircle/Widget_TransmutationCircle.UpdateJauge` (`self.TransmutationWidget`) 1.0)
  (set `/Game/BP/Class/TransmutationCircle/ABP_Transmutation.HandPosition` (0.5 0.5) (`self.ABPTransmutation`)))

(fn `IsAllowedToDraw`
  (params (Location :type "Vector2D Structure"))
  (returns (AllowedToDraw :type Boolean))
  (locals (ReturnValue :type Boolean))
  (bind _returnvalue (`KismetMathLibrary.Distance2D` Location (0.5 0.5)))
  (switch `int` (`self.Step`)
    (:`1`
      (set `local.ReturnValue` (and (> _returnvalue (`self.MediumCircleRadius`)) (< _returnvalue (`self.LargeCircleRadius`)))))
    (:`2`
      (set `local.ReturnValue` (and (> _returnvalue (`self.SmallCircleRadius`)) (< _returnvalue (`self.MediumCircleRadius`)))))
    (:`3`
      (set `local.ReturnValue` (< _returnvalue (`self.SmallCircleRadius`)))))
  (return (`local.ReturnValue`)))

(fn `UserConstructionScript`)