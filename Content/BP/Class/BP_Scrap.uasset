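; BP_Scrap is a randomly scaled cube that flies into a line of scrap under the player, then falls away.
; StartMovingToTarget chains two timelines with caller-set durations: a lerp to a widely scattered target, then into a slot with downward-cone noise.
; Targets are re-read every update from the player's SkywalkCPP positions, offset by line index, so they follow the player.
; After LifeTime, the cube switches to physics simulation with gravity.
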(event `self.ReceiveBeginPlay`
  (bind _returnvalue (`KismetMathLibrary.RandomFloatInRange` 0.2 0.8))
  ;[1 0 0.6398] Begin play
  (`SceneComponent.SetWorldScale3D` (`self.Cube`) (`KismetMathLibrary.MakeVector` _returnvalue _returnvalue _returnvalue)))

(event `StartMovingToTarget`
  (params (NoiseAmplitude :type "Float (double-precision)") (PlayerRef :type "/Game/BP/BP_PlayerChara Object Reference") (ScrapBringDuration :type "Float (double-precision)") (ScrapUnderDuration :type "Float (double-precision)") (LineIndex :type Integer) (LifeTime :type "Float (double-precision)") (Line :type Integer))
  (bind _returnvalue (== Line 0))
  (bind _cube (`self.Cube`))
  (bind _skywalkcpp (`/Game/BP/BP_PlayerChara.SkywalkCPP` (`self.Player ref`)))
  (bind _scraprightoffset (`SkywalkComponent.ScrapRightOffset` _skywalkcpp))
  ;[1 1 1] Move Scrap in front of camera
  (set `self.LifeTime` LifeTime)
  (set `self.Player ref` PlayerRef)
  (`TimelineComponent.SetPlayRate` (`self.Timeline_1`) (/ 1.0 ScrapBringDuration))
  (`TimelineComponent.SetPlayRate` (`self.Timeline_0`) (/ 1.0 ScrapUnderDuration))
  (set `self.StartPosition` (`self.K2_GetActorLocation`))
  (set `self.NoiseRefPosition` (* (`KismetMathLibrary.RandomUnitVectorInConeInDegrees` (0.0 0.0 -1.0) 45.0) NoiseAmplitude))
  (set `self.BigNoiseRefPosition` (* (`KismetMathLibrary.RandomUnitVector`) (* NoiseAmplitude 3.0)))
  (bind (_direction _scraptargetposition) (`Timeline|Timeline_1` :!via `PlayFromStart`)
    (:`Update`
      (bind _returnvalue_2 (`KismetMathLibrary.VLerp` (`self.StartPosition`) (+ (select `bool` _returnvalue :`false` (`SkywalkComponent.ScrapFinalMiddlePosition2` _skywalkcpp) :`true` (`SkywalkComponent.ScrapMiddlePosition` _skywalkcpp)) (`self.BigNoiseRefPosition`) (* _scraprightoffset LineIndex)) _scraptargetposition))
      (`self.K2_SetActorLocation` self _returnvalue_2 false false))
    (:`Finished`
      ;[1 1 1] Move scrap under the player
      (bind (_direction_2 _scrapfinalposition) (`Timeline|Timeline_0` :!via `PlayFromStart`)
        (:`Update`
          (`self.K2_SetActorLocation` (`KismetMathLibrary.VLerp` _returnvalue_2 (+ (select `bool` _returnvalue :`false` (`SkywalkComponent.ScrapFinalMiddlePosition2` _skywalkcpp) :`true` (`SkywalkComponent.ScrapFinalMiddlePosition` _skywalkcpp)) (* _scraprightoffset LineIndex) (`self.NoiseRefPosition`)) _scrapfinalposition)))
        (:`Finished`
          (`KismetSystemLibrary.Delay` (`self.LifeTime`))
          (`PrimitiveComponent.SetCollisionEnabled` _cube "PhysicsOnly")
          (`PrimitiveComponent.SetSimulatePhysics` _cube true)
          (`PrimitiveComponent.SetEnableGravity` _cube true))))))

(fn `UserConstructionScript`)