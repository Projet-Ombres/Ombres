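; Chimney actor that takes one of three meshes by type, can be highlighted or ping-outlined, and can explode to freeze nearby actors.
; Type 1 adds a timeline-driven piston at random speed, toggling smoke via a FlipFlop.
; Explode hides the chimney, gathers overlapped actors or their parents, excluding chimneys and the player, then lerps their CustomTimeDilation to zero.
; After RootDuration it starts restoring their speed and destroys itself.
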(event `self.ReceiveBeginPlay`
  (bind _particlesystem (`self.ParticleSystem`))
  ;[1 0 0.9467] Being play
  (set `self.BaseMaterial` (`PrimitiveComponent.GetMaterial` (`self.cube`) 0))
  ;[1 1 1] changement du static mesh en fonction du type choisi
  (`StaticMeshComponent.SetStaticMesh` (`self.cube`) (select `int` (- (`self.Cheminee type`) 1) :`0` "/Game/_ART/StaticMesh/Cheminee/SM_cheminee_01_Cylinder003.SM_cheminee_01_Cylinder003" :`1` "/Game/_ART/StaticMesh/Cheminee/SM_cheminee_02.SM_cheminee_02" :`2` "/Game/_ART/StaticMesh/Cheminee/SM_cheminee_03_Cylinder002.SM_cheminee_03_Cylinder002" :!type "StaticMesh Object Reference"))
  (`SceneComponent.SetWorldScale3D` (`self.cube`) (1.0 1.0 1.0))
  ;[1 1 1] vérification que la cheminé et une cheminé mobile
  (if (== (`self.Cheminee type`) 1)
    ;[1 1 1] rajout du mesh du piston et det de ses données
    (bind _returnvalue (`AddComponent|NODE_AddStaticMeshComponent-0`))
    (set `self.piston ref` _returnvalue)
    (`PrimitiveComponent.SetCustomDepthStencilValue` (`self.piston ref`) 1)
    ;[1 1 1] tirage de la vitesse du piston
    (set `self.piston ref position` (`SceneComponent.K2_GetComponentLocation` (`self.piston ref`)))
    (`TimelineComponent.SetPlayRate` (`self.Piston animation`) (`KismetMathLibrary.RandomFloatInRange` 0.8 1.2))
    ;[1 1 1] animation du piston
    (bind (_direction _piston_height) (`Timeline|Piston animation` :!via `PlayFromStart`)
      (:`Update`
        ;;[1 1 1] mouvement du piston
        (`SceneComponent.K2_SetWorldLocation` (`self.piston ref`) (`KismetMathLibrary.MakeVector` (.x (`self.piston ref position`)) (.y (`self.piston ref position`)) (+ (.z (`self.piston ref position`)) _piston_height)) false false))
      (:`smoke activation`
        ;;[1 1 1] Activation de la fumée selement quand le piston et haut
        (`/Engine/EditorBlueprintResources/StandardMacros.FlipFlop`
          (:`A`
            (`ActorComponent.Activate` _particlesystem false))
          (:`B`
            (`ActorComponent.Deactivate` _particlesystem)))))))

(event `hightlight chimney`
  ;[1 1 1] change la couleur de l'objet quand il et sélectioné
  (`PrimitiveComponent.SetMaterial` (`self.cube`) 0 "/Engine/MapTemplates/Materials/BasicAsset01.BasicAsset01"))

(event `Unlight chimney`
  ;[1 1 1] Unlight chimney
  (`PrimitiveComponent.SetMaterial` (`self.cube`) 0 (`self.BaseMaterial`)))

(event `Explode`
  (params (`Player ref` :type "Actor Object Reference"))
  (set `self.Player ref` `Player ref`)
  (`PrimitiveComponent.SetCollisionEnabled` (`self.cube`) "NoCollision")
  (`PrimitiveComponent.SetCollisionEnabled` (`self.piston ref`) "NoCollision")
  ;[1 1 1] Explosion
  (`SceneComponent.SetVisibility` (`self.cube`) false false)
  (`SceneComponent.SetVisibility` (`self.piston ref`) false false)
  (if (`self.As already explode?`)
    _
    (elif (not (`self.IsExploding`))
      (set `self.IsExploding` true)
      (`GameplayStatics.SpawnEmitterAttached` "/Game/StarterContent/Particles/P_Explosion.P_Explosion" (`self.cube`) "None" (0.0 0.0 0.0) (struct) (20.0 20.0 20.0) "SnapToTarget" false)
      (`SceneComponent.SetWorldScale3D` (`self.ParticleSystem`) (30.0 30.0 30.0))
      ;[1 1 1] enregiste tout les objets à portée
      (bind _outactors (`GameplayStatics.GetAllActorsWithTag` "Chimney"))
      (bind _output_get (set `self.AllActorsWithTag` _outactors))
      (`KismetArrayLibrary.Array_Add` _output_get (`self.Player ref`))
      (bind _outactors_2 (`KismetSystemLibrary.SphereOverlapActors` (`SceneComponent.K2_GetComponentLocation` (`self.DefaultSceneRoot`)) (`SphereComponent.SphereRadius` (`self.Area of effect`)) (`|MakeArray` "ObjectTypeQuery2" "ObjectTypeQuery1" "ObjectTypeQuery3" "ObjectTypeQuery4" "ObjectTypeQuery1" :!type "EObjectTypeQuery Enum") null (`self.AllActorsWithTag`)))
      ;[1 1 1] Check if object has a parent actor. If so, add the parent, if not add the already overlapped actor.
      (for _array_element _outactors_2
        (bind _returnvalue (`self.GetParentActor` _array_element))
        (if (== _returnvalue null)
          (`KismetArrayLibrary.Array_Add` (`self.object in range`) _array_element)
          (elif (not (`KismetArrayLibrary.Array_Contains` (`self.object in range`) _returnvalue))
            (`KismetArrayLibrary.Array_Add` (`self.object in range`) _returnvalue))))
      ;[1 1 1] time dilation
      (`self.SlowDownObjectsInRnge`)
      (`KismetSystemLibrary.Delay` (`self.root duration`))
      (`self.RestoreObjectsSpeed`)
      (`self.K2_DestroyActor`))))

(event `SlowDownObjectsInRnge`
  ;[1 1 1] slow down objects in range
  (bind _outputvalue (`CustomTimeline.StartCustomTimeline` 1.0)
    (:`Update`
      (for _array_element (`self.object in range`)
        ;;[1 1 1] set time dilatation(pour bloqué IA et animation)
        (set `Actor.CustomTimeDilation` (`KismetMathLibrary.Lerp` 1.0 0.0 _outputvalue) _array_element)))))

(event `RestoreObjectsSpeed`
  ;[1 1 1] RestoreObjectsSpeed
  (bind _outputvalue (`CustomTimeline.StartCustomTimeline` 1.0)
    (:`Update`
      (for _array_element (`self.object in range`)
        ;;[1 1 1] set time dilatation(pour bloqué IA et animation)
        (set `Actor.CustomTimeDilation` (`KismetMathLibrary.Lerp` 0.0 1.0 _outputvalue) _array_element)))))

(event `ActivatePingOutline`
  ;[1 1 1] Ping outline
  (`PrimitiveComponent.SetRenderCustomDepth` (`self.cube`) true)
  (`PrimitiveComponent.SetRenderCustomDepth` (`self.piston ref`) true))

(event `DeactivatePingOutline`
  ;[1 1 1] Ping outline
  (`PrimitiveComponent.SetRenderCustomDepth` (`self.cube`) false)
  (`PrimitiveComponent.SetRenderCustomDepth` (`self.piston ref`) false))

(fn `UserConstructionScript`)