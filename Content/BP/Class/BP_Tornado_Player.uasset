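; One-shot tornado gust actor that, on BeginPlay, launches the player character away from its origin.
; A sphere trace feeds the first hit to a player cast, stopping wall run or climb before a camera-relative launch with clamped upward lift.
; Walking braking is zeroed, with restoration after a delay, though the actor destroys itself right after the hit loop without waiting for it.
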(event `self.ReceiveBeginPlay`
  ;[0.9169 0 1] Being Play
  (`self.SpawnTornado`))

(event `SpawnTornado`
  (bind _sphere (`self.Sphere`))
  (bind _returnvalue (`SceneComponent.K2_GetComponentLocation` _sphere))
  ;[1 1 1] Spawn Tornado
  (bind (_outhits _returnvalue_2) (`KismetSystemLibrary.SphereTraceMultiForObjects` :`Start` _returnvalue :`End` (+ _returnvalue 0.5) :`Radius` (`SphereComponent.SphereRadius` _sphere) :`ObjectTypes` (`|MakeArray` "ObjectTypeQuery1" "ObjectTypeQuery3" :!type "EObjectTypeQuery Enum") :`DrawTime` 0.5))
  (if _returnvalue_2
    (for _array_element _outhits
      (`/Engine/EditorBlueprintResources/StandardMacros.DoOnce` false
        (:`Completed`
          (bind _output_get (set `self.Character Ref` (cast `/Game/BP/BP_PlayerChara` (`.HitActor` (`GameplayStatics.BreakHitResult` _array_element)) :!pure true)))
          (bind _charactermovement (`Character.CharacterMovement` _output_get))
          (set `self.Current Braking Deceleration` (`CharacterMovementComponent.BrakingDecelerationWalking` _charactermovement))
          (set `CharacterMovementComponent.BrakingDecelerationWalking` 0.0 _charactermovement)
          (bind _bpc_wallrun (`/Game/BP/BP_PlayerChara.BPC_WallRun` _output_get))
          (if (`/Game/BP/Components/BPC_WallRun.IsWallRunning` _bpc_wallrun)
            (`/Game/BP/Components/BPC_WallRun.StopWallRun` _bpc_wallrun))
          (bind _bpc_wallclimb (`/Game/BP/BP_PlayerChara.BPC_WallClimb` _output_get))
          (if (`/Game/BP/Components/BPC_WallClimb.IsEscalatingWall` _bpc_wallclimb)
            (set `/Game/BP/Components/BPC_WallClimb.IsEscalatingWall` false _bpc_wallclimb))
          (`Character.LaunchCharacter` _output_get (* (`KismetMathLibrary.MakeVector` (.x (`KismetMathLibrary.Normal` (- (`SceneComponent.K2_GetComponentLocation` (`/Game/BP/BP_PlayerChara.Camera` _output_get)) (`SceneComponent.K2_GetComponentLocation` (`self.DefaultSceneRoot`))))) (.y (`KismetMathLibrary.Normal` (- (`SceneComponent.K2_GetComponentLocation` (`/Game/BP/BP_PlayerChara.Camera` _output_get)) (`SceneComponent.K2_GetComponentLocation` (`self.DefaultSceneRoot`))))) (`KismetMathLibrary.FClamp` (.z (`KismetMathLibrary.Normal` (- (`SceneComponent.K2_GetComponentLocation` (`/Game/BP/BP_PlayerChara.Camera` _output_get)) (`SceneComponent.K2_GetComponentLocation` (`self.DefaultSceneRoot`))))) 0.15)) (`self.Puissance Bourasque`)) false false)
          (`KismetSystemLibrary.Delay` (`self.Impulse duration`))
          (set `CharacterMovementComponent.BrakingDecelerationWalking` (`self.Current Braking Deceleration`) (`Character.CharacterMovement` _output_get)))))
    (`self.K2_DestroyActor`)))

(fn `UserConstructionScript`)