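; BP_ExtrudeChunk is an actor that builds a flat grid of square tiles from its Lenght, Height and ChunkSize variables.
; The construction script runs LenghtConstruction for a row along X, then HeightConstruction for the full X-Y grid, which overlaps that first row at Y=0.
; Each tile is a separate Cube static mesh component, flattened on Z, spaced by ChunkSize and using M_ExtrudeChunk.
; Event graph logic is empty.
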(event `self.ReceiveBeginPlay`)

(fn `HeightConstruction`
  (bind _chunksize (`self.ChunkSize`))
  (bind _returnvalue (* (`self.ChunkSize`) 100.0))
  (for _index (range (`self.Height`))
    (for _index_2 (range (`self.Lenght`))
      (bind _returnvalue_2 (`AddComponent|NODE_AddStaticMeshComponent-3`))
      (`StaticMeshComponent.SetStaticMesh` _returnvalue_2 "/Engine/BasicShapes/Cube.Cube")
      (`SceneComponent.K2_SetRelativeTransform` _returnvalue_2 (`KismetMathLibrary.MakeTransform` (`KismetMathLibrary.MakeVector` (+ (* _index_2 _returnvalue) 0.0) (+ (* _index _returnvalue) 0.0)) (struct) (`KismetMathLibrary.MakeVector` _chunksize _chunksize 0.001)) false false)
      (`PrimitiveComponent.SetMaterial` _returnvalue_2 0 "/Game/Materials/M_ExtrudeChunk.M_ExtrudeChunk")
      (`KismetSystemLibrary.PrintString` (`KismetStringLibrary.Concat_StrStr` "")))))

(fn `LenghtConstruction`
  (bind _chunksize (`self.ChunkSize`))
  (for _index (range (`self.Lenght`))
    (bind _returnvalue (`AddComponent|NODE_AddStaticMeshComponent-2`))
    (`StaticMeshComponent.SetStaticMesh` _returnvalue "/Engine/BasicShapes/Cube.Cube")
    (`SceneComponent.K2_SetRelativeTransform` _returnvalue (`KismetMathLibrary.MakeTransform` (`KismetMathLibrary.MakeVector` (+ (* (`KismetMathLibrary.Conv_IntToDouble` _index) (* (`self.ChunkSize`) 100.0)) 0.0)) (struct) (`KismetMathLibrary.MakeVector` _chunksize _chunksize 0.001)) false false)
    (`PrimitiveComponent.SetMaterial` _returnvalue 0 "/Game/Materials/M_ExtrudeChunk.M_ExtrudeChunk")))

(fn `UserConstructionScript`
  (`self.LenghtConstruction`)
  (`self.HeightConstruction`))