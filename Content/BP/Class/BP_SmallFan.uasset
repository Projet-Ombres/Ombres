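; BP_SmallFan is a small fan that can be frozen temporarily through its Crystallize event.
; A custom timeline ramps the actor's CustomTimeDilation down to a stop, then Box collision is disabled for the given freeze duration.
; Afterward, collision returns and a second timeline ramps time dilation back to normal.
; IsCrystallized always returns false, even during the freeze.
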(event `/Game/BP/Class/BPI_Cristallizable.Crystallize`
  (params (FreezeDuration :type "Float (single-precision)"))
  (bind _outputvalue (`CustomTimeline.StartCustomTimeline` 1.0)
    (:`Update`
      (set `self.CustomTimeDilation` (- 1.0 _outputvalue)))
    (:`Finished`
      (set `self.CustomTimeDilation` 0.0)
      (`PrimitiveComponent.SetCollisionEnabled` (`self.Box`) "NoCollision")
      (`KismetSystemLibrary.Delay` FreezeDuration)
      (`PrimitiveComponent.SetCollisionEnabled` (`self.Box`) "QueryAndPhysics")
      (bind _outputvalue_2 (`CustomTimeline.StartCustomTimeline` 1.0)
        (:`Update`
          (set `self.CustomTimeDilation` _outputvalue_2))
        (:`Finished`
          (set `self.CustomTimeDilation` 1.0))))))

(fn `IsCrystallized`
  (returns (Crystallized :type Boolean))
  (return false))

(fn `UserConstructionScript`)