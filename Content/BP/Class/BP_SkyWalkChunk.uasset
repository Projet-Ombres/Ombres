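; BP_SkyWalkChunk is one chunk of the player's SkyWalk ability, drawing a scrap piece to the chunk's location.
; On Initialize it claims the nearest unused scrap within range, or spawns a BP_Scrap beside the camera at a fixed low height.
; Chained timelines lerp the scrap to a noise-offset point before the camera, then onto the chunk root.
; SkyWalk's in-use list keeps chunks from sharing scraps.
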(event `Initialize`
  (params (ref :type "/Game/BP/BP_PlayerChara Object Reference") (NewParam :type "Array of Actor Object Reference"))
  (set `self.Player ref` ref)
  (`self.CustomEvent` NewParam)
  (`TimelineComponent.SetPlayRate` (`self.Timeline_3`) 2.0)
  (`TimelineComponent.SetPlayRate` (`self.Timeline_2`) 2.0)
  (`TimelineComponent.SetPlayRate` (`self.Timeline_1`) 2.0)
  (`TimelineComponent.SetPlayRate` (`self.Timeline_0`) 2.0))

(event `CustomEvent`
  (params (`Scrap in World` :type "Array of Actor Object Reference"))
  (bind _closest (`self.Return the nearest Scrap` `Scrap in World`))
  (bind _output_get (set `self.Nearest Scrap` _closest))
  (`KismetArrayLibrary.Array_Add` (`/Game/BP/Components/Pouvoirs/BPC_SkyWalk.Scrap Already in Use` (`/Game/BP/BP_PlayerChara.BPC_SkyWalk` (`self.Player ref`))) _output_get)
  (`self.CustomEvent_0`))

(event `CustomEvent_0`
  (bind _camera (`/Game/BP/BP_PlayerChara.Camera` (`self.Player ref`)))
  (bind _camera_2 (`/Game/BP/BP_PlayerChara.Camera` (`self.Player ref`)))
  (bind _camera_3 (`/Game/BP/BP_PlayerChara.Camera` (`self.Player ref`)))
  (if (`KismetSystemLibrary.IsValid` (stale `CustomEvent` _closest))
    (`KismetSystemLibrary.PrintString` "Hello")
    (bind _output_get (set `self.Scrap starting position` (`SceneComponent.K2_GetComponentLocation` (`Actor.RootComponent` (`self.Nearest Scrap`)))))
    (set `self.Noise ref position` (`KismetMathLibrary.RandomUnitVectorInConeInDegrees` (0.0 0.0 -1.0) 45.0))
    (bind (_direction _newtrack_0) (`Timeline|Timeline_3`)
      (:`Update`
        (bind _returnvalue (`KismetMathLibrary.VLerp` _output_get (+ (`SceneComponent.K2_GetComponentLocation` _camera_3) (+ (* (`SceneComponent.GetForwardVector` _camera_3) (`self.Distance from camera`)) (* (`self.NewVar_0`) (`self.Noise amplitude`)))) _newtrack_0))
        (`SceneComponent.K2_SetWorldLocation` (`Actor.RootComponent` (`self.Nearest Scrap`)) _returnvalue false false))
      (:`Finished`
        (bind (_direction_2 _newtrack_0_2) (`Timeline|Timeline_2`)
          (:`Update`
            (`SceneComponent.K2_SetWorldLocation` (`Actor.RootComponent` (`self.Nearest Scrap`)) (`KismetMathLibrary.VLerp` _returnvalue (`SceneComponent.K2_GetComponentLocation` (`self.DefaultSceneRoot`)) _newtrack_0_2) false false)))))
    (else
      (bind _output_get_2 (set `self.Scrap spawn position` (+ (`SceneComponent.K2_GetComponentLocation` _camera) (* (`SceneComponent.GetRightVector` _camera) (* (`self.spawn distance`) (- (* (`KismetMathLibrary.Conv_IntToDouble` (`KismetMathLibrary.RandomIntegerInRange` 0 1)) 2.0) 1.0))))))
      (bind _returnvalue_2 (`|SpawnActorFromClass` "/Game/BP/Class/BP_Scrap.BP_Scrap_C" (`KismetMathLibrary.MakeTransform` (`KismetMathLibrary.MakeVector` (.x _output_get_2) (.y _output_get_2) -150.0)) "AlwaysSpawn" "OverrideRootScale" null null))
      (bind _output_get_3 (set `self.Scrap ref` _returnvalue_2))
      (`KismetArrayLibrary.Array_Add` (`/Game/BP/Components/Pouvoirs/BPC_SkyWalk.Scrap Already in Use` (`/Game/BP/BP_PlayerChara.BPC_SkyWalk` (`self.Player ref`))) _output_get_3)
      (set `self.Noise ref position` (`KismetMathLibrary.RandomUnitVectorInConeInDegrees` (0.0 0.0 -1.0) 45.0))
      (bind (_direction_3 _newtrack_0_3) (`Timeline|Timeline_0`)
        (:`Update`
          (bind _returnvalue_3 (`KismetMathLibrary.VLerp` (`self.Scrap spawn position`) (+ (`SceneComponent.K2_GetComponentLocation` _camera_2) (+ (* (`SceneComponent.GetForwardVector` _camera_2) (`self.Distance from camera`)) (* (`self.Noise ref position`) (`self.Noise amplitude`)))) _newtrack_0_3))
          (`SceneComponent.K2_SetWorldLocation` (`Actor.RootComponent` (`self.Scrap ref`)) _returnvalue_3 false true))
        (:`Finished`
          (bind _output_get_4 (set `self.Last in view position` _returnvalue_3))
          (bind (_direction_4 _newtrack_0_4) (`Timeline|Timeline_1`)
            (:`Update`
              (`SceneComponent.K2_SetWorldLocation` (`Actor.RootComponent` (`self.Scrap ref`)) (`KismetMathLibrary.VLerp` _output_get_4 (`SceneComponent.K2_GetComponentLocation` (`self.DefaultSceneRoot`)) _newtrack_0_4) false true))))))))

(fn `Return the nearest Scrap`
  (params (`Scrap in World` :type "Array of Actor Object Reference"))
  (returns (closest :type "Actor Object Reference"))
  (locals (Nearest :type "Actor Object Reference") (`Closet Distance Scrap` :type "Float (double-precision)" :default 10000000.0) (`Max distance` :type "Float (double-precision)" :default 200000.0))
  (for _array_element `Scrap in World`
    (if (not (`KismetArrayLibrary.Array_Contains` (`/Game/BP/Components/Pouvoirs/BPC_SkyWalk.Scrap Already in Use` (`/Game/BP/BP_PlayerChara.BPC_SkyWalk` (`self.Player ref`))) _array_element))
      (bind _returnvalue (`self.GetDistanceTo` _array_element))
      (if (and (< _returnvalue (`local.Closet Distance Scrap`)) (< _returnvalue (`local.Max distance`)))
        (set `local.Nearest` _array_element)
        (set `local.Closet Distance Scrap` _returnvalue)
        (else
          (`KismetSystemLibrary.PrintString` "Hello")))))
  (return (`local.Nearest`)))

(fn `UserConstructionScript`)