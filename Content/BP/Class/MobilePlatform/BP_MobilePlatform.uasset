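; Chain-driven moving platform mechanism that carries BP_Platform actors around a looped path over editable gears (rouages).
; Construction builds gear instances, procedural chain strips on external tangents and a spline from the sorted tangent points, curved around the end gears.
; BeginPlay replaces instanced preview platforms with spawned actors and applies speed to the chain material.
; Tick spins each gear inversely to its radius and moves platforms along the spline, wrapping at the end.
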(event `AddRouage`
  (bind _points (`self.Points`))
  ;[0 1 0.3708] Add rouage button
  (`KismetArrayLibrary.Array_Add` _points (+ (`|GetArrayItem` _points (- (`KismetArrayLibrary.Array_Length` _points) 1)) (* (`KismetMathLibrary.Vector_Up`) 20.0)))
  (`KismetArrayLibrary.Array_Add` (`self.Radiuses`) (`self.Radius`)))

(event `self.ReceiveBeginPlay`
  (bind _proceduralmesh (`self.ProceduralMesh`))
  (bind _returnvalue (`InstancedStaticMeshComponent.GetInstanceCount` (`self.Platforms`)))
  ;[1 1 1] Init transforms arrays
  (`KismetArrayLibrary.Array_Resize` (`self.PlatformsActors`) _returnvalue)
  (for _index (range _returnvalue)
    (bind _returnvalue_2 (`|SpawnActorFromClass` "/Game/BP/Class/MobilePlatform/BP_Platform.BP_Platform_C" (`InstancedStaticMeshComponent.GetInstanceTransform` (`self.Platforms`) _index false) "AlwaysSpawn" "OverrideRootScale" null null))
    (`KismetArrayLibrary.Array_Set` (`self.PlatformsActors`) _index _returnvalue_2))
  (`KismetArrayLibrary.Array_Resize` (`self.ExternalNormals`) (`InstancedStaticMeshComponent.GetInstanceCount` (`self.Platforms`)))
  (`KismetArrayLibrary.Array_Resize` (`self.PlatformsTransforms`) (`InstancedStaticMeshComponent.GetInstanceCount` (`self.Platforms`)))
  (for (_ _array_index) (`self.PlatformsTransforms`)
    (`KismetArrayLibrary.Array_Set` (`self.PlatformsTransforms`) _array_index (`InstancedStaticMeshComponent.GetInstanceTransform` (`self.Platforms`) 0 false)))
  (`KismetArrayLibrary.Array_Resize` (`self.Transforms`) (`InstancedStaticMeshComponent.GetInstanceCount` (`self.Rouages`)))
  (for _index_2 (range (`InstancedStaticMeshComponent.GetInstanceCount` (`self.Rouages`)))
    (`KismetArrayLibrary.Array_Set` (`self.Transforms`) _index_2 (`InstancedStaticMeshComponent.GetInstanceTransform` (`self.Rouages`) _index_2 false)))
  (bind _returnvalue_3 (`KismetMaterialLibrary.CreateDynamicMaterialInstance` (`self.ChainMaterial`)))
  (bind _output_get (set `self.MaterialInstance` _returnvalue_3))
  (for _index_3 (range (`ProceduralMeshComponent.GetNumSections` _proceduralmesh))
    (`PrimitiveComponent.SetMaterial` _proceduralmesh _index_3 _output_get))
  (`MaterialInstanceDynamic.SetScalarParameterValue` (`self.MaterialInstance`) "Speed" (* (`self.Speed`) 2.0))
  (`InstancedStaticMeshComponent.ClearInstances` (`self.Platforms`)))

(event `self.ReceiveTick`
  (params (DeltaSeconds :type "Float (single-precision)"))
  ;[1 1 1] Update rouages rotation
  (for _index (range (`InstancedStaticMeshComponent.GetInstanceCount` (`self.Rouages`)))
    (bind _returnvalue (+ (.pitch (.rotation (`|GetArrayItem` (`self.Transforms`) _index))) (* (/ (`self.Speed`) (/ (`|GetArrayItem` (`self.Radiuses`) _index) 2.0)) DeltaSeconds -100.0)))
    (`KismetArrayLibrary.Array_Set` (`self.Transforms`) _index (`KismetMathLibrary.MakeTransform` (.location (`|GetArrayItem` (`self.Transforms`) _index)) (`KismetMathLibrary.MakeRotator` (.roll (.rotation (`|GetArrayItem` (`self.Transforms`) _index))) (select `bool` (<= _returnvalue -90.0) :`false` _returnvalue :`true` (+ _returnvalue 90.0)) (.yaw (.rotation (`|GetArrayItem` (`self.Transforms`) _index)))) (.scale (`|GetArrayItem` (`self.Transforms`) _index)))))
  (`InstancedStaticMeshComponent.BatchUpdateInstancesTransforms` (`self.Rouages`) 0 (`self.Transforms`) false true false)
  (`self.UpdateProgresses` DeltaSeconds))

(event `UpdateProgresses`
  (params (DeltaTime :type "Float (double-precision)"))
  (bind _returnvalue (`SplineComponent.GetSplineLength` (`self.Spline`)))
  ;[1 1 1] Update platforms progress
  (for (_array_element _array_index) (`self.Progresses`)
    (bind _returnvalue_2 (+ _array_element (* (`self.Speed`) DeltaTime 500.0)))
    (`KismetArrayLibrary.Array_Set` (`self.Progresses`) _array_index (select `bool` (> _returnvalue_2 _returnvalue) :`false` _returnvalue_2 :`true` (- _returnvalue_2 _returnvalue)))
    (`self.CalculatePlatformTransform` _array_index DeltaTime)
    (`self.PlacePlatform` _array_index)))

(fn `AddChainWidth`
  (params (Position :type "Vector Structure"))
  (returns (Pos :type "Vector Structure"))
  (return (select `bool` (`self.Décalé`) :`false` Position :`true` (`self.AddOffset` (`self.ChainWidth`) Position))))

(fn `AddOffset`
  (params (Offset :type "Float (double-precision)") (Point :type "Vector Structure"))
  (returns (OffsettedPoint :type "Vector Structure"))
  (return (`KismetMathLibrary.MakeVector` (.x Point) (+ (.y Point) Offset) (.z Point))))

(fn `AddPlatforms`
  (locals (SortedTangentPoints :type "Array of Vector Structure") (Index :type Integer) (Center :type "Vector Structure"))
  (bind _pathpoints (`self.PathPoints`))
  (bind _returnvalue (- (`KismetArrayLibrary.Array_Length` (`self.ExternalTangentPoints`)) 1))
  ;[1 1 1] Sort external tangent points to create the path
  (set `local.Index` 0)
  (`KismetArrayLibrary.Array_Resize` (`local.SortedTangentPoints`) (`KismetArrayLibrary.Array_Length` (`self.ExternalTangentPoints`)))
  (for (_array_element _array_index) (`self.ExternalTangentPoints`)
    (if (== (mod _array_index 2) 0)
      (`KismetArrayLibrary.Array_Set` (`local.SortedTangentPoints`) (`local.Index`) _array_element)
      (`/Engine/EditorBlueprintResources/StandardMacros.IncrementInt` (`local.Index`))))
  (for _index (range (+ _returnvalue 1))
    (bind _returnvalue_2 (- _returnvalue _index))
    (if (== (mod _returnvalue_2 2) 1)
      (`KismetArrayLibrary.Array_Set` (`local.SortedTangentPoints`) (`local.Index`) (`|GetArrayItem` (`self.ExternalTangentPoints`) _returnvalue_2))
      (`/Engine/EditorBlueprintResources/StandardMacros.IncrementInt` (`local.Index`))))
  ;[1 1 1] Set initial progresses
  (bind _output_get (set `self.PathPoints` (`local.SortedTangentPoints`)))
  (if (> (`KismetArrayLibrary.Array_Length` _output_get) 0)
    (`KismetArrayLibrary.Array_Resize` (`self.Progresses`) (`self.PlatformCount`))
    (for (_ _array_index_2) (`self.Progresses`)
      (bind _returnvalue_3 (* (/ (`KismetMathLibrary.Conv_IntToDouble` _array_index_2) (`KismetMathLibrary.Conv_IntToDouble` (`self.PlatformCount`))) (`KismetMathLibrary.Conv_IntToDouble` (`KismetArrayLibrary.Array_Length` (`self.PathPoints`)))))
      (`KismetArrayLibrary.Array_Set` (`self.Progresses`) _array_index_2 _returnvalue_3)
      (bind _returnvalue_4 (`KismetMathLibrary.FTrunc` _returnvalue_3))
      (if (not (`self.IsInCircle` _returnvalue_4))
        (bind _output (`|GetArrayItem` _pathpoints _returnvalue_4))
        (bind _returnvalue_5 (+ _returnvalue_4 1))
        (bind _output_2 (`|GetArrayItem` _pathpoints (select `bool` (< _returnvalue_5 (`KismetArrayLibrary.Array_Length` (`self.PathPoints`))) :`true` _returnvalue_5)))
        (`InstancedStaticMeshComponent.AddInstance` (`self.Platforms`) (`KismetMathLibrary.MakeTransform` (`KismetMathLibrary.VLerp` _output _output_2 (- _returnvalue_3 (`KismetMathLibrary.Conv_IntToDouble` _returnvalue_4))) (struct) (`self.PlatformScale`)))
        (else
          (bind _output_get_2 (set `local.Center` (/ (+ _output _output_2) 2.0))))))))

(fn `AddReverseChainWidth`
  (params (Position :type "Vector Structure"))
  (returns (Pos :type "Vector Structure"))
  (bind _returnvalue (+ Position (`KismetMathLibrary.MakeVector` 0.0 (`self.ChainWidth`))))
  (return (select `bool` (`self.Décalé`) :`false` _returnvalue :`true` (`self.AddOffset` (`self.ChainWidth`) _returnvalue))))

(fn `CalculatePlatformTransform`
  (params (Index :type Integer) (DeltaTime :type "Float (double-precision)"))
  (locals (PrevIndex :type Integer) (NextIndex :type Integer) (Percent :type "Float (double-precision)") (CircleCenter :type "Vector Structure") (AngleToNextPoint :type "Float (double-precision)") (Direction :type "Vector Structure") (Rotation :type "Rotator Structure") (DeltaSeconds :type "Float (double-precision)"))
  (bind _spline (`self.Spline`))
  (bind _output (`|GetArrayItem` (`self.Progresses`) Index))
  (bind (_output_location _output_rotation _output_scale) (`KismetMathLibrary.BreakTransform` (`|GetArrayItem` (`self.PlatformsTransforms`) Index)))
  (`KismetArrayLibrary.Array_Set` (`self.PlatformsTransforms`) Index (`KismetMathLibrary.MakeTransform` (`SplineComponent.GetLocationAtDistanceAlongSpline` _spline _output "Local") (`KismetMathLibrary.MakeRotFromX` (`KismetMathLibrary.GreaterGreater_VectorRotator` (`KismetMathLibrary.GetForwardVector` (`SplineComponent.GetRotationAtDistanceAlongSpline` _spline _output "Local")) (struct :`Pitch` 90.0))) _output_scale)))

(fn `CalculateTotalLength`
  (returns (PathLength :type "Float (double-precision)"))
  (locals (Length :type "Float (double-precision)"))
  (set `local.Length` 0.0)
  (for _index (range (`KismetArrayLibrary.Array_Length` (`self.PathPoints`)))
    (set `local.Length` (+ (`KismetMathLibrary.Vector_Distance` (`|GetArrayItem` (`self.PathPoints`) _index) (`|GetArrayItem` (`self.PathPoints`) (select `bool` (< _index (- (`self.PlatformCount`) 1)) :`true` (+ _index 1)))) (`local.Length`))))
  (return (`local.Length`)))

(fn `GetIndexes`
  (params (Value :type "Float (double-precision)"))
  (returns (PreviousIndex :type Integer) (NextIndex :type Integer))
  (locals (PrevIndex :type Integer) (NextIndex_ :type Integer))
  (bind _output_get (set `local.PrevIndex` (`KismetMathLibrary.FTrunc` Value)))
  (set `local.NextIndex_` (select `bool` (< _output_get (- (`KismetArrayLibrary.Array_Length` (`self.PathPoints`)) 1)) :`true` (+ _output_get 1)))
  (return (`local.PrevIndex`) (`local.NextIndex_`)))

(fn `GetPreviousIndex`
  (params (Index :type Integer))
  (returns (PrevIndex :type Integer))
  (return (select `bool` (> Index 0) :`false` (- (`KismetArrayLibrary.Array_Length` (`self.PathPoints`)) 1) :`true` (- Index 1))))

(fn `GetProgressFromIndex`
  (params (Index :type Integer))
  (returns (Progress :type "Float (double-precision)"))
  (locals (Length :type "Float (double-precision)"))
  (bind _returnvalue (- Index 1))
  (set `local.Length` 0.0)
  (for _index (range (+ _returnvalue 1))
    (set `local.Length` (+ (`KismetMathLibrary.Vector_Distance` (`|GetArrayItem` (`self.PathPoints`) _index) (`|GetArrayItem` (`self.PathPoints`) (select `bool` (< _index _returnvalue) :`true` (+ _index 1)))) (`local.Length`))))
  (return (* (/ (`local.Length`) (`self.CalculateTotalLength`)) (`KismetMathLibrary.Conv_IntToDouble` (`KismetArrayLibrary.Array_Length` (`self.PathPoints`))))))

(fn `GetRouageIndex`
  (params (PathIndex :type Integer))
  (returns (RouageIndex :type Integer))
  (locals (DistanceToExtremity :type Integer))
  (bind _returnvalue (- (/ (`KismetArrayLibrary.Array_Length` (`self.PathPoints`)) 2) 1))
  (bind _output_get (set `local.DistanceToExtremity` (select `bool` (> PathIndex _returnvalue) :`false` PathIndex :`true` (- _returnvalue PathIndex))))
  (return (/ (+ _output_get 1) 2)))

(fn `PlacePlatform`
  (params (Index :type Integer))
  (bind (_returnvalue_roll _returnvalue_pitch _returnvalue_yaw) (`KismetMathLibrary.BreakRotator` (`self.K2_GetActorRotation`)))
  (bind (_output_location _output_rotation _output_scale) (`KismetMathLibrary.BreakTransform` (`|GetArrayItem` (`self.PlatformsTransforms`) Index)))
  (`self.K2_SetActorTransform` (`|GetArrayItem` (`self.PlatformsActors`) Index) (`KismetMathLibrary.MakeTransform` (+ _output_location (`self.K2_GetActorLocation`)) (`KismetMathLibrary.MakeRotator` (+ (.roll _output_rotation) _returnvalue_roll) (+ (.pitch _output_rotation) _returnvalue_pitch) (+ (.yaw _output_rotation) _returnvalue_yaw)) _output_scale) false false))

(fn `SetSplinePoints`
  (locals (PrevIndex :type Integer) (NextIndex :type Integer) (PrevToNextDirection :type "Vector Structure"))
  (bind _returnvalue (`KismetArrayLibrary.Array_Length` (`self.PathPoints`)))
  (bind _returnvalue_2 (/ _returnvalue 2))
  (`SplineComponent.SetSplinePoints` (`self.Spline`) (`self.PathPoints`) "Local" true)
  (for (_ _array_index) (`self.PathPoints`)
    (bind (_previousindex _nextindex) (`self.GetIndexes` (`KismetMathLibrary.Conv_IntToDouble` _array_index)))
    (if (or (== _previousindex (- _returnvalue_2 1)) (== _previousindex (- _returnvalue 1)))
      (bind _returnvalue_3 (* (`self.CalculateRouageRadius` _array_index _nextindex) 4.0))
      (bind _returnvalue_4 (* (`KismetMathLibrary.Normal` (`KismetMathLibrary.GreaterGreater_VectorRotator` (- (`|GetArrayItem` (`self.PathPoints`) _array_index) (`self.CalculateCircleCenter` _array_index _nextindex)) (struct :`Pitch` -90.0))) _returnvalue_3))
      (`SplineComponent.SetTangentsAtSplinePoint` (`self.Spline`) _array_index (* (`KismetMathLibrary.Normal` (- (`|GetArrayItem` (`self.PathPoints`) (`self.GetPreviousIndex` _array_index)) (`|GetArrayItem` (`self.PathPoints`) _array_index))) _returnvalue_3) _returnvalue_4 "Local" true)
      (`SplineComponent.SetTangentsAtSplinePoint` (`self.Spline`) _nextindex (* _returnvalue_4 -1.0) (* (`KismetMathLibrary.Normal` (- (`|GetArrayItem` (`self.PathPoints`) (`.NextIndex` (`self.GetIndexes` (`KismetMathLibrary.Conv_IntToDouble` _nextindex)))) (`|GetArrayItem` (`self.PathPoints`) _nextindex))) _returnvalue_3) "Local" true)
      (elif (!= _previousindex _returnvalue_2)
        (bind _output_get (set `local.PrevToNextDirection` (`KismetMathLibrary.Normal` (- (`|GetArrayItem` (`self.PathPoints`) _nextindex) (`|GetArrayItem` (`self.PathPoints`) _previousindex)))))
        (`SplineComponent.SetTangentsAtSplinePoint` (`self.Spline`) _array_index (* _output_get -1.0) _output_get "Local" true)))))

(fn `UserConstructionScript`
  (locals (CurrentPoint :type "Vector Structure") (NextPoint :type "Vector Structure") (CurrentToNextDirection :type "Vector Structure") (CurrentRadius :type "Float (double-precision)") (NextRadius :type "Float (double-precision)"))
  (bind _externaltangentpoints (`self.ExternalTangentPoints`))
  (bind (_point1 _point2 _point3 _point4) (`self.CalculateTangentExternalPoints` (`local.CurrentPoint`) (`local.NextPoint`) (* (`local.CurrentRadius`) 100.0) (* (`local.NextRadius`) 100.0)))
  (`|ExecutionSequence`
    (:`then_0`
      (set `self.ExternalTangentPoints` (`|MakeArray`))
      (if (== (`KismetArrayLibrary.Array_Length` (`self.Points`)) (`KismetArrayLibrary.Array_Length` (`self.Radiuses`)))
        ;[1 1 1] Update rouages and chains
        (for (_array_element _array_index) (`self.Points`)
          (bind _output (`|GetArrayItem` (`self.Radiuses`) _array_index))
          (`InstancedStaticMeshComponent.AddInstance` (`self.Rouages`) (`KismetMathLibrary.MakeTransform` _array_element (struct) (* (`KismetMathLibrary.Vector_One`) _output)))
          (if (< _array_index (- (`KismetArrayLibrary.Array_Length` (`self.Points`)) 1))
            (set `local.CurrentPoint` _array_element)
            (bind _returnvalue (+ _array_index 1))
            (set `local.NextPoint` (`|GetArrayItem` (`self.Points`) _returnvalue))
            (set `local.CurrentRadius` _output)
            (set `local.NextRadius` (`|GetArrayItem` (`self.Radiuses`) _returnvalue))
            (set `local.CurrentToNextDirection` (`KismetMathLibrary.Normal` (- (`local.NextPoint`) (`local.CurrentPoint`))))
            (`KismetArrayLibrary.Array_AddUnique` _externaltangentpoints _point1)
            (`KismetArrayLibrary.Array_AddUnique` _externaltangentpoints _point2)
            (`KismetArrayLibrary.Array_AddUnique` _externaltangentpoints _point3)
            (`KismetArrayLibrary.Array_AddUnique` _externaltangentpoints _point4)
            (`ProceduralMeshComponent.CreateMeshSection_LinearColor` :`self` (`self.ProceduralMesh`) :`SectionIndex` _array_index :`Vertices` (`|MakeArray` (`self.AddChainWidth` _point1) (`self.AddReverseChainWidth` _point1) (`self.AddChainWidth` _point2) (`self.AddReverseChainWidth` _point2) (`self.AddChainWidth` _point3) (`self.AddReverseChainWidth` _point3) (`self.AddChainWidth` _point4) (`self.AddReverseChainWidth` _point4)) :`Triangles` (`|MakeArray` 2 3 7 7 6 2 0 1 5 5 4 0) :`UV0` (`|MakeArray` (5.0 0.5) (5.0 0.5) (0.5 0.0) (5.0 0.5) (0.0 0.0) (0.0 0.5) (5.0 0.0) (5.0 0.5) :!type "Vector2D Structure"))
            (`PrimitiveComponent.SetMaterial` (`self.ProceduralMesh`) _array_index (`self.ChainMaterial`))
            (set `self.Décalé` (not (`self.Décalé`)))))))
    (:`then_1`
      (`self.AddPlatforms`)
      (`self.SetSplinePoints`))))