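; BP_DeathArea is a fall-recovery volume whose box extent is set from BoxSize in the Construction Script.
; An overlapping player has their portal spawner component spawn a portal at a configurable vertical distance with lowered gravity.
; An overlapping enemy is launched back to its stored pre-fall position using a computed, fixed-duration jump velocity.
; An unconnected alternative that respawns enemies through their spawn reference remains unused.
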(event `self.Box.OnComponentBeginOverlap`
  (params (OverlappedComponent :type "PrimitiveComponent Object Reference") (OtherActor :type "Actor Object Reference") (OtherComp :type "PrimitiveComponent Object Reference") (OtherBodyIndex :type Integer) (bFromSweep :type Boolean) (SweepResult :type "HitResult Structure (by ref)"))
  (bind _asbp_player_chara (cast `/Game/BP/BP_PlayerChara` OtherActor)
    (:`then`
      (`/Game/BP/Components/BPC_PortalSpawner.SpawnPortal` (`/Game/BP/BP_PlayerChara.BPC_PortalSpawner` _asbp_player_chara) (`self.PortalVerticalSpawnDistance`) true -1))
    (:`CastFailed`
      (bind _asbp_enemy (cast `/Game/AI/Blueprints/BP_Enemy` OtherActor))
      (bind _velocity (`/Game/BP/Libraries/BPL_Utilities.CalculateJumpVelocity` (`self.K2_GetActorLocation` _asbp_enemy) (`/Game/AI/Blueprints/BP_Enemy.PositionBeforeFalling` _asbp_enemy) 3.0))
      (set `MovementComponent.Velocity` _velocity (`Character.CharacterMovement` _asbp_enemy)))))

(fn `UserConstructionScript`
  (`BoxComponent.SetBoxExtent` (`self.Box`) (`self.BoxSize`) true))