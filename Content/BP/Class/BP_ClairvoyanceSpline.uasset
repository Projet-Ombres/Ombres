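; BP_ClairvoyanceSpline is a spline path rendered with the Clairvoyance material that can appear, fade out or disappear.
; The construction script builds a spline mesh per segment, each with a stored dynamic material instance and query-only collision blocking a single custom channel.
; Events drive the Opacity parameter on all instances: Appear uses a timeline, FadeOut follows a supplied time value, and Disappear zeroes it instantly.
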(event `FadeOut`
  (params (ValueTime :type "Float (double-precision)"))
  ;[1 1 1] fade out
  (for _array_element (`self.DynamicMaterialInstances`)
    (`MaterialInstanceDynamic.SetScalarParameterValue` _array_element "Opacity" (* (- 1.0 ValueTime) (`self.MaxOpacityValue`)))))

(event `Disappear`
  ;[1 1 1] disappear
  (for _array_element (`self.DynamicMaterialInstances`)
    (`MaterialInstanceDynamic.SetScalarParameterValue` _array_element "Opacity" 0.0)))

(event `Appear`
  ;[1 1 1] appear
  (bind _outputvalue (`CustomTimeline.StartCustomTimeline` 5.0)
    (:`Update`
      (for _array_element (`self.DynamicMaterialInstances`)
        (`MaterialInstanceDynamic.SetScalarParameterValue` _array_element "Opacity" (* _outputvalue (`self.MaxOpacityValue`)))))))

(fn `UserConstructionScript`
  (`KismetArrayLibrary.Array_Clear` (`self.DynamicMaterialInstances`))
  (for _index (range (+ (- (`SplineComponent.GetNumberOfSplinePoints` (`self.Spline`)) 2) 1))
    (bind _returnvalue (`AddComponent|NODE_AddSplineMeshComponent-0`))
    (`StaticMeshComponent.SetStaticMesh` _returnvalue (`self.MeshToSet`))
    (`SplineMeshComponent.SetForwardAxis` _returnvalue (`self.Forward axis`) true)
    (`SceneComponent.K2_AttachToComponent` _returnvalue (`self.Spline`) "None" "KeepRelative" "KeepRelative" "KeepRelative" true)
    (bind _returnvalue_2 (+ _index 1))
    (`SplineMeshComponent.SetStartAndEnd` _returnvalue (`SplineComponent.GetLocationAtSplinePoint` (`self.Spline`) _index "Local") (`SplineComponent.GetTangentAtSplinePoint` (`self.Spline`) _index "Local") (`SplineComponent.GetLocationAtSplinePoint` (`self.Spline`) _returnvalue_2 "Local") (`SplineComponent.GetTangentAtSplinePoint` (`self.Spline`) _returnvalue_2 "Local") true)
    (`PrimitiveComponent.SetCollisionEnabled` _returnvalue "QueryOnly")
    (bind _returnvalue_3 (`PrimitiveComponent.CreateDynamicMaterialInstance` _returnvalue 0 "/Game/Materials/Ping/clairvoyance.clairvoyance" "None"))
    (`KismetArrayLibrary.Array_Add` (`self.DynamicMaterialInstances`) _returnvalue_3)
    (`PrimitiveComponent.SetCollisionResponseToAllChannels` _returnvalue "ECR_Ignore")
    (`PrimitiveComponent.SetCollisionResponseToChannel` _returnvalue "ECC_GameTraceChannel11" "ECR_Block")))