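; BP_FakePortal fakes a portal view by driving a scene capture into a render target that follows the player camera's movement.
; On BeginPlay it stores the capture's start position, disables automatic capturing and assigns the render target.
; Each Tick offsets the capture from that start by the camera's location relative to the portal actor, copies camera pitch and yaw, then captures the scene manually.
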(event `self.ReceiveBeginPlay`
  (bind _capturecomponent2d (`SceneCapture2D.CaptureComponent2D` (`self.TargetCapture`)))
  (set `self.CaptureStartPosition` (`self.K2_GetActorLocation` (`self.TargetCapture`)))
  (set `SceneCaptureComponent.bCaptureEveryFrame` false _capturecomponent2d)
  (set `SceneCaptureComponent.bCaptureOnMovement` false _capturecomponent2d)
  (set `SceneCaptureComponent2D.TextureTarget` "/Game/BP/Class/Portal/FakePortalRenderTarget.FakePortalRenderTarget" _capturecomponent2d))

(event `self.ReceiveTick`
  (params (DeltaSeconds :type "Float (single-precision)"))
  (bind _targetcapture (`self.TargetCapture`))
  (bind (_returnvalue_roll _returnvalue_pitch _returnvalue_yaw) (`KismetMathLibrary.BreakRotator` (`self.K2_GetActorRotation` (`self.PlayerCamera`))))
  (bind _returnvalue_location (`KismetMathLibrary.BreakTransform` (`KismetMathLibrary.MakeRelativeTransform` (`self.GetTransform` (`self.PlayerCamera`)) (`self.GetTransform`))))
  (if (and (`KismetSystemLibrary.IsValid` (`self.TargetCapture`)) (`KismetSystemLibrary.IsValid` (`self.PlayerCamera`)))
    (`self.K2_SetActorLocation` (`self.TargetCapture`) (+ (`self.CaptureStartPosition`) _returnvalue_location) false false)
    (`self.K2_SetActorRotation` _targetcapture (`KismetMathLibrary.MakeRotator` 0.0 _returnvalue_pitch _returnvalue_yaw) false)
    (`SceneCaptureComponent2D.CaptureScene` (`SceneCapture2D.CaptureComponent2D` _targetcapture))))

(fn `UserConstructionScript`)