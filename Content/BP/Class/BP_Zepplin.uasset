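; BP_Zepplin is a zeppelin actor whose static mesh roams along a spline in the world.
; On BeginPlay it plays the Roaming timeline at a rate of one over Temps, so that variable controls travel time.
; Each update samples the spline by time at constant velocity to place and orient the mesh, turning yaw by 180 degrees.
; The construction script sets the mesh's world scale from Taille.
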(event `self.ReceiveBeginPlay`
  (bind _spline (`self.Spline`))
  (`TimelineComponent.SetPlayRate` (`self.Roaming`) (/ 1.0 (`self.Temps`)))
  (bind (_direction _newtrack_0) (`Timeline|Roaming`)
    (:`Update`
      (`SceneComponent.K2_SetWorldLocationAndRotation` (`self.SM_Zepplin`) (`SplineComponent.GetLocationAtTime` _spline _newtrack_0 "World" true) (`KismetMathLibrary.MakeRotator` (.roll (`SplineComponent.GetRotationAtTime` _spline _newtrack_0 "World" true)) (.pitch (`SplineComponent.GetRotationAtTime` _spline _newtrack_0 "World" true)) (- (.yaw (`SplineComponent.GetRotationAtTime` _spline _newtrack_0 "World" true)) 180.0)) false false))))

(fn `UserConstructionScript`
  (`SceneComponent.SetWorldScale3D` (`self.SM_Zepplin`) (`self.Taille`)))