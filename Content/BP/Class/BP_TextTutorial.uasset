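; BP_TextTutorial is an in-world tutorial prompt that shows a controller button hint on a plane and fades with player distance.
; The construction script picks the plane's material and width from TypeOfText (RB, hold RB or B).
; Each Tick, the player's distance minus a hardcoded offset drives the material's Opacity parameter, fading linearly from opaque to invisible at MaxDistancePlayer.
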(event `self.ReceiveTick`
  (params (DeltaSeconds :type "Float (single-precision)"))
  (bind _returnvalue (- (`KismetMathLibrary.Vector_Distance` (`self.K2_GetActorLocation` (`GameplayStatics.GetPlayerCharacter` 0)) (`self.K2_GetActorLocation`)) 1850.0))
  (`MeshComponent.SetScalarParameterValueOnMaterials` (`self.Plane`) "Opacity" (select `bool` (> _returnvalue (`self.MaxDistancePlayer`)) :`false` (`KismetMathLibrary.Lerp` 1.0 0.0 (`KismetMathLibrary.NormalizeToRange` _returnvalue 0.0 (`self.MaxDistancePlayer`))))))

(fn `UserConstructionScript`
  (bind _typeoftext (`self.TypeOfText`))
  (bind _plane (`self.Plane`))
  (`PrimitiveComponent.SetMaterial` _plane 0 (select `/Game/BP/Class/Enum_TypeOfTutoText` _typeoftext :`NewEnumerator0` "/Game/TemporaryAsset/Materials/M_RB_Inst.M_RB_Inst" :`NewEnumerator1` "/Game/TemporaryAsset/Materials/M_RB_Maintenir_Inst.M_RB_Maintenir_Inst" :`NewEnumerator2` "/Game/TemporaryAsset/Materials/M_B_Inst.M_B_Inst" :!type "MaterialInterface Object Reference"))
  (`SceneComponent.SetRelativeScale3D` _plane (`KismetMathLibrary.MakeVector` (select `/Game/BP/Class/Enum_TypeOfTutoText` _typeoftext :`NewEnumerator0` 1.5 :`NewEnumerator1` 2.8 :`NewEnumerator2` 1.5 :!type "Float (single-precision)") 1.1 1.0)))