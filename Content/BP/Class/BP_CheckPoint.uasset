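; BP_CheckPoint is a trigger-box checkpoint that sets which powers the player has when entered.
; Each overlap applies its Skywalk and Crystallization flags and refreshes the powers widget.
; If it differs from the last checkpoint, it notifies the player's handler, plays VFX and sound, and briefly flags activation on the player.
; The Construction Script gives unset checkpoint IDs their array index and positions or sizes the box, scene capture and particles.
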(event `self.Box.OnComponentBeginOverlap`
  (params (OverlappedComponent :type "PrimitiveComponent Object Reference") (OtherActor :type "Actor Object Reference") (OtherComp :type "PrimitiveComponent Object Reference") (OtherBodyIndex :type Integer) (bFromSweep :type Boolean) (SweepResult :type "HitResult Structure (by ref)"))
  (bind _asbp_player_chara (cast `/Game/BP/BP_PlayerChara` OtherActor))
  (bind _gameinstance (`/Game/BP/BP_PlayerChara.GameInstance` _asbp_player_chara))
  (if (`KismetSystemLibrary.IsValid` _gameinstance)
    (`self.EnablePowers`)
    (`/Game/BP/Widgets/MorceauxDeWidgets/MainInterface/Widget_Powers.CheckNumberOfPowers` (`/Game/BP/Widgets/Widget_Main_Interface.Widget_Powers` (`/Game/BP/BP_GameInstance.MainInterface` _gameinstance)))
    (bind _bpc_checkpointhandler (`/Game/BP/BP_PlayerChara.BPC_CheckPointHandler` _asbp_player_chara))
    (if (!= (`/Game/BP/Components/BPC_CheckPointHandler.LastCheckPointReached` _bpc_checkpointhandler) self)
      (`/Game/BP/Components/BPC_CheckPointHandler.OnCheckPointReached` _bpc_checkpointhandler self)
      (`ActorComponent.Activate` (`self.ParticleSystem`) false)
      (`GameplayStatics.PlaySoundAtLocation` "/Game/Sound_Design/Bruitages/Alchimie/Checkpoint_power.Checkpoint_power" (`self.K2_GetActorLocation`) (struct) 1.0 1.0 0.0 "/Game/Sound_Design/SoundAttenuation.SoundAttenuation" null null)
      (bind _asbp_player_chara_2 (cast `/Game/BP/BP_PlayerChara` (`GameplayStatics.GetPlayerCharacter` 0)))
      (set `/Game/BP/BP_PlayerChara.CheckPointBeingActivated` true _asbp_player_chara_2)
      (`KismetSystemLibrary.Delay` 0.5)
      (set `/Game/BP/BP_PlayerChara.CheckPointBeingActivated` false _asbp_player_chara_2))))

(event `EnablePowers`
  (bind _asbp_player_chara (cast `/Game/BP/BP_PlayerChara` (`GameplayStatics.GetPlayerCharacter` 0)))
  (set `SkywalkComponent.SpellEnabled` (`self.SkywalkEnabled`) (`/Game/BP/BP_PlayerChara.Skywalk` _asbp_player_chara))
  (set `/Game/BP/Components/Pouvoirs/BPC_Crystallization.SpellEnabled` (`self.CrystallizationEnabled`) (`/Game/BP/BP_PlayerChara.BPC_Crystallization` _asbp_player_chara)))

(fn `UserConstructionScript`
  (bind _scenecapturecomponent2d (`self.SceneCaptureComponent2D`))
  (bind _particlesystem (`self.ParticleSystem`))
  (bind (_relativelocation_x _relativelocation_y) (`KismetMathLibrary.BreakVector` (`SceneComponent.RelativeLocation` _scenecapturecomponent2d)))
  (`|ExecutionSequence`
    (:`then_0`
      (bind _outactors (`GameplayStatics.GetAllActorsOfClass` "BP_CheckPoint_C"))
      (for (_array_element _array_index) _outactors
        (if (== (`/Game/BP/Class/BP_CheckPoint.ID` _array_element) -1)
          (set `/Game/BP/Class/BP_CheckPoint.ID` _array_index _array_element))))
    (:`then_1`
      (`BoxComponent.SetBoxExtent` (`self.Box`) (`self.BoxSize`) true)
      (`SceneComponent.K2_SetRelativeLocation` _scenecapturecomponent2d (`KismetMathLibrary.MakeVector` _relativelocation_x _relativelocation_y (`self.CameraHeight`)) false false)
      (`SceneComponent.K2_SetRelativeLocationAndRotation` _particlesystem (`self.VFXPosition`) (`self.VFXRotation`) false false)
      (`SceneComponent.SetRelativeScale3D` _particlesystem (`self.VFXScale`)))))