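; Ping spline actor that shows glowing orb emitters flowing along its spline while the game instance's PingActivated flag is on.
; BeginPlay spawns evenly spaced emitters, eases their speed from initial to normal via a timeline, then deactivates them.
; Tick moves each orb by distance along the spline, wrapping at the end, and deactivates orbs both horizontally far from and well below the player for performance.
; ActivateSpline and DeactivateSpline set the flag and toggle the emitters.
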(event `self.ReceiveBeginPlay`
  (`|ExecutionSequence`
    (:`then_0`
      ;[1 1 1] augmentation de la vitesse des sub particule au début
      ;;[1 1 1] setting du temps d'acélération initial
      (`TimelineComponent.SetPlayRate` (`self.Initial speed`) (/ 1.0 (`self.Initial aceleration time`)))
      ;;[1 1 1] lerp de la vitesse initial vers la vitesse normal
      (bind (_direction _initial_speed_learp) (`Timeline|Initial speed` :!via `PlayFromStart`)
        (:`Update`
          (set `self.speed` (`KismetMathLibrary.Lerp` (`self.InitialSpeed`) (`self.NormalSpeed`) _initial_speed_learp)))))
    (:`then_1`
      ;[1 1 1] calcule du nombre de sub particule
      (bind _output_get (set `self.number of sphere` (`.ReturnValue` (`KismetMathLibrary.FMod` (`SplineComponent.GetSplineLength` (`self.Spline`)) (`self.distance between sphere`)))))
      ;[1 1 1] calcule de la distance entre chaque sub particule
      (set `self.Actual distance between sphere` (/ (`SplineComponent.GetSplineLength` (`self.Spline`)) (`KismetMathLibrary.Conv_IntToDouble` _output_get)))
      ;[1 1 1] spawn des sup particule
      (for _index (range (+ _output_get 1))
        (set `self.sphere spawn index` _index)
        (bind _returnvalue (`GameplayStatics.SpawnEmitterAtLocation` "/Game/_ART/Particle/P_OrbGlowLights.P_OrbGlowLights" (0.0 0.0 0.0) (struct) (1.0 1.0 1.0) false))
        (`KismetArrayLibrary.Array_Add` (`self.list of sub particule`) _returnvalue)
        ;[1 1 1] indexation d'une position sur la spline pour chaque sub particule
        (`KismetArrayLibrary.Array_Add` (`self.curent distance`) (* (`self.sphere spawn index`) (`self.Actual distance between sphere`)))))
    (:`then_2`
      (`self.DeactivateSpline`))))

(event `self.ReceiveTick`
  (params (DeltaSeconds :type "Float (single-precision)"))
  (bind (_returnvalue_x _returnvalue_y) (`KismetMathLibrary.BreakVector` (`self.K2_GetActorLocation` (`GameplayStatics.GetPlayerCharacter` 0))))
  (bind (_returnvalue_x_2 _returnvalue_y_2) (`KismetMathLibrary.BreakVector` (`SceneComponent.K2_GetComponentLocation` (`self.Sub Particule ref`))))
  (bind (_returnvalue_x_3 _returnvalue_y_3 _returnvalue_z) (`KismetMathLibrary.BreakVector` (`self.K2_GetActorLocation` (`GameplayStatics.GetPlayerCharacter` 0))))
  (bind (_returnvalue_x_4 _returnvalue_y_4 _returnvalue_z_2) (`KismetMathLibrary.BreakVector` (`SceneComponent.K2_GetComponentLocation` (`self.Sub Particule ref`))))
  ;[1 1 1] récupération du delta time
  (set `self.delta time` DeltaSeconds)
  (for (_array_element _array_index) (`self.list of sub particule`)
    (set `self.Sub Particule ref` _array_element)
    (set `self.sphere move index` _array_index)
    ;[1 1 1] mise a jour de la distance sur la spline de chaque particule
    (`KismetArrayLibrary.Array_Set` (`self.curent distance`) (`self.sphere move index`) (+ (* (`self.speed`) (`self.delta time`)) (`|GetArrayItem` (`self.curent distance`) (`self.sphere move index`))))
    ;[1 1 1] vérification si une sub particule est arrivé au bout de la spline de la spline
    (if (>= (`|GetArrayItem` (`self.curent distance`) (`self.sphere move index`)) (`SplineComponent.GetSplineLength` (`self.Spline`)))
      ;[1 1 1] réinitialisation de la position des sub particule si elle arrive a la fin de la spline
      (`KismetArrayLibrary.Array_Set` (`self.curent distance`) (`self.sphere move index`))
      (`SceneComponent.K2_SetWorldLocation` (`self.Sub Particule ref`) (`SplineComponent.GetLocationAtDistanceAlongSpline` (`self.Spline`) 0.0 "World") false false)
      (else
        ;[1 1 1] mise a jour de la position des sub particule
        (`SceneComponent.K2_SetWorldLocation` (`self.Sub Particule ref`) (`SplineComponent.GetLocationAtDistanceAlongSpline` (`self.Spline`) (`|GetArrayItem` (`self.curent distance`) (`self.sphere move index`)) "World") false false)))
    ;[1 1 1] Pour les fps on fait despawn les particules si trop loin
    (if (and (> (`KismetMathLibrary.Distance2D` (`KismetMathLibrary.MakeVector2D` _returnvalue_x _returnvalue_y) (`KismetMathLibrary.MakeVector2D` _returnvalue_x_2 _returnvalue_y_2)) (`self.distanceAuJoueur`)) (> (- _returnvalue_z _returnvalue_z_2) (/ (`self.distanceAuJoueur`) 3.0)))
      (if (`ActorComponent.IsActive` (`self.Sub Particule ref`))
        (`ActorComponent.Deactivate` (`self.Sub Particule ref`)))
      (elif (`/Game/BP/BP_GameInstance.PingActivated` (cast `/Game/BP/BP_GameInstance` (`GameplayStatics.GetGameInstance`) :!pure true))
        (if (not (`ActorComponent.IsActive` (`self.Sub Particule ref`)))
          (`ActorComponent.Activate` (`self.Sub Particule ref`) false))
        (elif (`ActorComponent.IsActive` (`self.Sub Particule ref`))
          (`ActorComponent.Deactivate` (`self.Sub Particule ref`)))))))

(event `DeactivateSpline`
  ;[1 1 1] desactivate spline
  (set `/Game/BP/BP_GameInstance.PingActivated` false (cast `/Game/BP/BP_GameInstance` (`GameplayStatics.GetGameInstance`) :!pure true))
  (for _array_element (`self.list of sub particule`)
    (`ActorComponent.Deactivate` _array_element)))

(event `ActivateSpline`
  (bind (_returnvalue_x _returnvalue_y) (`KismetMathLibrary.BreakVector` (`self.K2_GetActorLocation` (`GameplayStatics.GetPlayerCharacter` 0))))
  (bind (_returnvalue_x_2 _returnvalue_y_2) (`KismetMathLibrary.BreakVector` (`SceneComponent.K2_GetComponentLocation` (`self.Sub Particule ref`))))
  (bind (_returnvalue_x_3 _returnvalue_y_3 _returnvalue_z) (`KismetMathLibrary.BreakVector` (`self.K2_GetActorLocation` (`GameplayStatics.GetPlayerCharacter` 0))))
  (bind (_returnvalue_x_4 _returnvalue_y_4 _returnvalue_z_2) (`KismetMathLibrary.BreakVector` (`SceneComponent.K2_GetComponentLocation` (`self.Sub Particule ref`))))
  ;[1 1 1] Activate
  (set `/Game/BP/BP_GameInstance.PingActivated` true (cast `/Game/BP/BP_GameInstance` (`GameplayStatics.GetGameInstance`) :!pure true))
  (for _array_element (`self.list of sub particule`)
    (if (and (> (`KismetMathLibrary.Distance2D` (`KismetMathLibrary.MakeVector2D` _returnvalue_x _returnvalue_y) (`KismetMathLibrary.MakeVector2D` _returnvalue_x_2 _returnvalue_y_2)) (`self.distanceAuJoueur`)) (> (- _returnvalue_z _returnvalue_z_2) (/ (`self.distanceAuJoueur`) 3.0)))
      (`ActorComponent.Deactivate` _array_element)
      (else
        (`ActorComponent.Activate` _array_element false)))))

(fn `UserConstructionScript`)