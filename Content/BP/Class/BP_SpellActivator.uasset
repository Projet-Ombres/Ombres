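; BP_SpellActivator is a trigger actor that sets which spells the player character has enabled.
; When a BP_PlayerChara overlaps its Box, it copies its Skywalk, AlchemistEye and CrystalWave flags into the SpellEnabled flag of the player's SkywalkCPP, BPCPing and BPCExplosion components, so it can also disable spells.
; It then prints the resulting spell states as a debug string.
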(event `self.Box.OnComponentBeginOverlap`
  (params (OverlappedComponent :type "PrimitiveComponent Object Reference") (OtherActor :type "Actor Object Reference") (OtherComp :type "PrimitiveComponent Object Reference") (OtherBodyIndex :type Integer) (bFromSweep :type Boolean) (SweepResult :type "HitResult Structure (by ref)"))
  (bind _alchemisteye (`self.AlchemistEye`))
  (bind _asbp_player_chara (cast `/Game/BP/BP_PlayerChara` OtherActor))
  (bind _output_get (set `SkywalkComponent.SpellEnabled` (`self.Skywalk`) (`/Game/BP/BP_PlayerChara.SkywalkCPP` _asbp_player_chara)))
  (set `/Game/BP/Components/Pouvoirs/BPC_Ping.SpellEnabled` _alchemisteye (`/Game/BP/BP_PlayerChara.BPC_Ping` _asbp_player_chara))
  (bind _output_get_2 (set `/Game/BP/Components/Pouvoirs/BPC_Explosion.SpellEnabled` (`self.CrystalWave`) (`/Game/BP/BP_PlayerChara.BPC_Explosion` _asbp_player_chara)))
  (`KismetSystemLibrary.PrintString` (`KismetStringLibrary.Concat_StrStr` "Skywalk " (select `bool` _output_get :`false` "disabled" :`true` "enabled") ", Alchemist eye " (select `bool` _alchemisteye :`false` "disabled" :`true` "enabled") ", Crystal wave " (select `bool` _output_get_2 :`false` "disabled" :`true` "enabled"))))

(fn `UserConstructionScript`)