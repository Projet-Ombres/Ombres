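; Trigger volume that streams sublevels in and out when the player character exits its box.
; The dot product of the LevelDirection forward vector and the player's horizontal velocity selects which list loads and which unloads, reversing them for backward exits.
; Index-driven loops run the non-blocking loads, then the unloads, and the dot value is debug-printed.
; The construction script applies the box size and direction yaw.
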(event `self.Box.OnComponentEndOverlap`
  (params (OverlappedComponent :type "PrimitiveComponent Object Reference") (OtherActor :type "Actor Object Reference") (OtherComp :type "PrimitiveComponent Object Reference") (OtherBodyIndex :type Integer))
  (bind _asbp_player_chara (cast `/Game/BP/BP_PlayerChara` OtherActor))
  (bind _returnvalue (`KismetMathLibrary.Dot_VectorVector` (`KismetMathLibrary.GetForwardVector` (`SceneComponent.K2_GetComponentRotation` (`self.LevelDirection`))) (`KismetMathLibrary.Vector_Normal2D` (`self.GetVelocity` _asbp_player_chara))))
  (`KismetSystemLibrary.PrintString` (`KismetStringLibrary.Concat_StrStr` "dot : " (`KismetStringLibrary.Conv_DoubleToString` _returnvalue)))
  (if (>= _returnvalue 0.0)
    (set `self.PendingSublevelsToLoad` (`self.SubLevelsToLoad`))
    (set `self.PendingSublevelsToUnload` (`self.SubLevelsToUnload`))
    (else
      (set `self.PendingSublevelsToLoad` (`self.SubLevelsToUnload`))
      (set `self.PendingSublevelsToUnload` (`self.SubLevelsToLoad`))))
  (set `self.SubLevelIndex` 0)
  (if (< (`self.SubLevelIndex`) (`KismetArrayLibrary.Array_Length` (`self.PendingSublevelsToLoad`))) :!label _label
    (`GameplayStatics.LoadStreamLevel` (`|GetArrayItem` (`self.PendingSublevelsToLoad`) (`self.SubLevelIndex`)) true)
    (`/Engine/EditorBlueprintResources/StandardMacros.IncrementInt` (`self.SubLevelIndex`)
      (:`  `
        (goto _label)))
    (else
      (set `self.SubLevelIndex` 0)
      (if (< (`self.SubLevelIndex`) (`KismetArrayLibrary.Array_Length` (`self.PendingSublevelsToUnload`))) :!label _label_2
        (`GameplayStatics.UnloadStreamLevel` (`|GetArrayItem` (`self.PendingSublevelsToUnload`) (`self.SubLevelIndex`)))
        (`/Engine/EditorBlueprintResources/StandardMacros.IncrementInt` (`self.SubLevelIndex`)
          (:`  `
            (goto _label_2)))))))

(fn `UserConstructionScript`
  (`BoxComponent.SetBoxExtent` (`self.Box`) (`KismetMathLibrary.Conv_DoubleToVector` (`self.BoxScale`)) false)
  (`SceneComponent.K2_SetRelativeRotation` (`self.LevelDirection`) (`KismetMathLibrary.MakeRotator` 0.0 0.0 (`self.LevelDirectionYaw`)) false false))