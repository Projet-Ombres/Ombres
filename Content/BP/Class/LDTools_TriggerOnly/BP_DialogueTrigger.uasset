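; BP_DialogueTrigger is a level-design trigger box that plays a one-shot dialogue line when the player character overlaps it.
; Before the sound plays attached to the player mesh, StartSound ducks the game instance's loudspeaker sounds and fades out sprint breathing.
; It then flags the player as speaking and shows an optional timed subtitle through the main interface's subtitle widget.
; The construction script sizes the box from TriggerSize.
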(event `self.Box.OnComponentBeginOverlap`
  (params (OverlappedComponent :type "PrimitiveComponent Object Reference") (OtherActor :type "Actor Object Reference") (OtherComp :type "PrimitiveComponent Object Reference") (OtherBodyIndex :type Integer) (bFromSweep :type Boolean) (SweepResult :type "HitResult Structure (by ref)"))
  (bind (_asbp_player_chara _bsuccess) (cast `/Game/BP/BP_PlayerChara` OtherActor :!pure true))
  (if _bsuccess
    (`/Engine/EditorBlueprintResources/StandardMacros.DoOnce` false
      (:`Completed`
        (if (!= (`self.SoundToPlay`) null)
          (`self.StartSound`)
          (`GameplayStatics.SpawnSoundAttached` (`self.SoundToPlay`) (`Character.Mesh` _asbp_player_chara) "None" (0.0 0.0 0.0) (struct) "KeepRelativeOffset" false 1.0 1.0 0.0 null null)
          (set `/Game/BP/BP_PlayerChara.PlayerSpeaking` true (cast `/Game/BP/BP_PlayerChara` (`GameplayStatics.GetPlayerCharacter` 0) :!pure true))
          (if (not (`KismetTextLibrary.TextIsEmpty` (`self.SubtitleText`)))
            (`/Game/BP/Widgets/Widget_Subtitles.SetSubtitle` (`/Game/BP/Widgets/Widget_Main_Interface.Widget_Subtitles` (`/Game/BP/BP_PlayerChara.MainInterface` _asbp_player_chara)) (`self.SubtitleText`) (`self.SubtitleDuration`))))))))

(event `StartSound`
  (bind _hautparleurssounds (`/Game/BP/BP_GameInstance.HautParleursSounds` (cast `/Game/BP/BP_GameInstance` (`GameplayStatics.GetGameInstance`) :!pure true)))
  (bind _breathingsound (`/Game/BP/Components/CapacitéPhysique/BPC_Sprint.BreathingSound` (`/Game/BP/BP_PlayerChara.BPC_Sprint` (cast `/Game/BP/BP_PlayerChara` (`GameplayStatics.GetPlayerCharacter` 0) :!pure true))))
  (if (!= (`KismetArrayLibrary.Array_Length` _hautparleurssounds) 0)
    (for _array_element _hautparleurssounds
      (`AudioComponent.FadeOut` _array_element 0.2 (* (`AudioComponent.VolumeMultiplier` _array_element) 0.2))))
  (if (`KismetSystemLibrary.IsValid` _breathingsound)
    (`AudioComponent.FadeOut` _breathingsound 0.2 0.0)))

(fn `UserConstructionScript`
  (`BoxComponent.SetBoxExtent` (`self.Box`) (`self.TriggerSize`) true))