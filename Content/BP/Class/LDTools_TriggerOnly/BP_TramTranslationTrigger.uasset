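; BP_TramTranslationTrigger is a level-design trigger that relocates the tram when the player enters it.
; On the first box overlap by BP_PlayerChara, a DoOnce gate lets it hide the referenced tram, set its position to LocationToSpawnTram, then reveal it.
; The construction script sizes the box from the TriggerSize variable.
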(event `self.Box.OnComponentBeginOverlap`
  (params (OverlappedComponent :type "PrimitiveComponent Object Reference") (OtherActor :type "Actor Object Reference") (OtherComp :type "PrimitiveComponent Object Reference") (OtherBodyIndex :type Integer) (bFromSweep :type Boolean) (SweepResult :type "HitResult Structure (by ref)"))
  (bind _bp_tram (`self.BP_Tram`))
  (if (`.bSuccess` (cast `/Game/BP/BP_PlayerChara` OtherActor :!pure true))
    (`/Engine/EditorBlueprintResources/StandardMacros.DoOnce` false
      (:`Completed`
        (`/Game/BP/Class/BP_tram.HideTram` _bp_tram)
        (`/Game/BP/Class/BP_tram.SetTramPosition` _bp_tram (`self.LocationToSpawnTram`))
        (`/Game/BP/Class/BP_tram.RevealTram` _bp_tram)))))

(fn `UserConstructionScript`
  (`BoxComponent.SetBoxExtent` (`self.Box`) (`self.TriggerSize`) true))