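; Level trigger Blueprint that updates the on-screen objective text when the player reaches a checkpoint.
; On player character overlap, it reaches the intro target-text widget through the game instance's main interface and hides the current objective.
; After a short delay it sets a hardcoded message to climb through the station, then shows the objective again.
; Nothing disables the trigger, so later overlaps can run the sequence again.
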(event `self.CollisionComponent.OnComponentBeginOverlap`
  (params (OverlappedComponent :type "PrimitiveComponent Object Reference") (OtherActor :type "Actor Object Reference") (OtherComp :type "PrimitiveComponent Object Reference") (OtherBodyIndex :type Integer) (bFromSweep :type Boolean) (SweepResult :type "HitResult Structure (by ref)"))
  (bind _widget_targettextintro (`/Game/BP/Widgets/Widget_Main_Interface.Widget_TargetTextIntro` (`/Game/BP/BP_GameInstance.MainInterface` (cast `/Game/BP/BP_GameInstance` (`GameplayStatics.GetGameInstance`) :!pure true))))
  (if (`.bSuccess` (cast `/Game/BP/BP_PlayerChara` OtherActor :!pure true))
    (`/Game/BP/Widgets/MorceauxDeWidgets/MainInterface/Widget_TargetTextIntro.DisappearObjective` _widget_targettextintro)
    (`KismetSystemLibrary.Delay` 2.0)
    (`TextBlock.SetText` (`/Game/BP/Widgets/MorceauxDeWidgets/MainInterface/Widget_TargetTextIntro.TextBlock_88` _widget_targettextintro) "Find your way up through the station")
    (`/Game/BP/Widgets/MorceauxDeWidgets/MainInterface/Widget_TargetTextIntro.AppearObjective` _widget_targettextintro)))

(fn `UserConstructionScript`)