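; BP_PullBar is a pull bar actor with two mesh variants, selected by the MeshDouble flag.
; Its construction script shows Mechanic2 when the flag is true, and Cylinder1 plus Lanterne when it is false.
; Both visibility and hidden-in-game are set on each component without propagating to children, so editor and game views match.
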(fn `UserConstructionScript`
  (bind _meshdouble (`self.MeshDouble`))
  (`SceneComponent.SetHiddenInGame` (`self.Mechanic2`) (not _meshdouble) false)
  (`SceneComponent.SetVisibility` (`self.Mechanic2`) _meshdouble false)
  (`SceneComponent.SetHiddenInGame` (`self.Cylinder1`) (`self.MeshDouble`) false)
  (`SceneComponent.SetHiddenInGame` (`self.Lanterne`) (`self.MeshDouble`) false)
  (`SceneComponent.SetVisibility` (`self.Cylinder1`) (not (`self.MeshDouble`)) false)
  (`SceneComponent.SetVisibility` (`self.Lanterne`) (not (`self.MeshDouble`)) false))