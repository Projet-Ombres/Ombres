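; Middle car of a tram that responds to a crystallize (freeze) effect.
; Crystallize forwards the freeze duration to the owning Tram, then spawns crystals on the car's static mesh at 30 random points sampled from that mesh.
; The crystal meshes come from the Tram, and the freeze duration is passed to the spawn call.
; IsCrystallized always returns false, so the car never reports itself as crystallized.
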(event `/Game/BP/Class/BPI_Cristallizable.Crystallize`
  (params (FreezeDuration :type "Float (single-precision)"))
  (bind _tram (`self.Tram`))
  (`/Game/BP/Class/BPI_Cristallizable.Crystallize` _tram FreezeDuration)
  (bind _randompoints (`/Game/BP/Libraries/BPL_Utilities.GetRandomPointsInMesh` (`StaticMeshComponent.StaticMesh` (`self.StaticMesh`)) 30))
  (`/Game/BP/Libraries/BP_MacroLibrary.SpawnCrystals` (`self.StaticMesh`) _randompoints (`/Game/BP/Class/BP_tram.CrystalMeshes` _tram) FreezeDuration (`self.SpawnedCrystals`)))

(fn `IsCrystallized`
  (returns (Crystallized :type Boolean))
  (return false))

(fn `UserConstructionScript`)