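; Gust actor ("bourrasque") that knocks a BP_PlayerChara_Jojo away from its origin when it spawns.
; On BeginPlay a sphere trace finds the character and launches it once toward its camera position, with upward direction clamped to a minimum.
; It zeroes walking braking deceleration and schedules a restore after ImpulseDuration.
; On any hit, the actor destroys itself right after the loop, before that delay can finish.
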(event `self.ReceiveBeginPlay`
  ;[0.9169 0 1] Being Play
  (`self.SpawnTornado`))

(event `SpawnTornado`
  (bind _sphere (`self.Sphere`))
  (bind _returnvalue (`SceneComponent.K2_GetComponentLocation` _sphere))
  ;[1 1 1] Spawn Tornado
  (bind (_outhits _returnvalue_2) (`KismetSystemLibrary.SphereTraceMultiForObjects` _returnvalue _returnvalue (`SphereComponent.SphereRadius` _sphere) (`|MakeArray` "ObjectTypeQuery1" "ObjectTypeQuery3" :!type "EObjectTypeQuery Enum")))
  (if _returnvalue_2
    (for _array_element _outhits
      (bind _asbp_player_chara_jojo (cast `/Game/BP/BP_PlayerChara_Jojo` (`.HitActor` (`GameplayStatics.BreakHitResult` _array_element))))
      (`/Engine/EditorBlueprintResources/StandardMacros.DoOnce` false
        (:`Completed`
          (bind _output_get (set `self.Character Ref` _asbp_player_chara_jojo))
          (bind _charactermovement (`Character.CharacterMovement` _output_get))
          (set `self.Current Braking Deceleration` (`CharacterMovementComponent.BrakingDecelerationWalking` _charactermovement))
          (set `CharacterMovementComponent.BrakingDecelerationWalking` 0.0 _charactermovement)
          (`Character.LaunchCharacter` _output_get (* (`KismetMathLibrary.MakeVector` (.x (`KismetMathLibrary.Normal` (- (`SceneComponent.K2_GetComponentLocation` (`/Game/BP/BP_PlayerChara_Jojo.Camera` _output_get)) (`SceneComponent.K2_GetComponentLocation` (`self.DefaultSceneRoot`))))) (.y (`KismetMathLibrary.Normal` (- (`SceneComponent.K2_GetComponentLocation` (`/Game/BP/BP_PlayerChara_Jojo.Camera` _output_get)) (`SceneComponent.K2_GetComponentLocation` (`self.DefaultSceneRoot`))))) (`KismetMathLibrary.FClamp` (.z (`KismetMathLibrary.Normal` (- (`SceneComponent.K2_GetComponentLocation` (`/Game/BP/BP_PlayerChara_Jojo.Camera` _output_get)) (`SceneComponent.K2_GetComponentLocation` (`self.DefaultSceneRoot`))))) 0.15)) (`self.Puissance Bourasque`)) false false)
          (`KismetSystemLibrary.Delay` (`self.Impulse duration`))
          (set `CharacterMovementComponent.BrakingDecelerationWalking` (`self.Current Braking Deceleration`) (`Character.CharacterMovement` _output_get)))))
    (`self.K2_DestroyActor`)))

(fn `UserConstructionScript`)