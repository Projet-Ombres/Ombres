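; BP_CheckpointList is an actor utility that keeps a list of data for the BP_CheckPoint actors found in the world.
; FetchCheckpoints resizes the Checkpoints array to the actor count, refreshing display names and IDs while keeping each index's sublevel fields, so those follow array position rather than ID.
; SelectCheckpoint searches for the actor matching CheckpointIdToSelect, but only exits the loop on a match.
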(event `FetchCheckpoints`
  (bind _checkpoints (`self.Checkpoints`))
  (bind _outactors (`GameplayStatics.GetAllActorsOfClass` "/Game/BP/Class/BP_CheckPoint.BP_CheckPoint_C"))
  (`KismetArrayLibrary.Array_Resize` (`self.Checkpoints`) (`KismetArrayLibrary.Array_Length` _outactors))
  (for (_array_element _array_index) _outactors
    (bind ((`SubLevelName_5_847F41A64A07AD11A4BF109B4B789906` _sublevelname) (`OtherSubLevelsRequired_8_463B1B8C413DAC3151BA62B792681C13` _othersublevelsrequired)) (break `/Game/BP/Class/CheckpointData` (`|GetArrayItem` _checkpoints _array_index)))
    (`KismetArrayLibrary.Array_Set` _checkpoints _array_index (make `/Game/BP/Class/CheckpointData` (`KismetSystemLibrary.GetDisplayName` _array_element) (`/Game/BP/Class/BP_CheckPoint.ID` _array_element) _sublevelname _othersublevelsrequired))))

(event `SelectCheckpoint`
  (bind _outactors (`GameplayStatics.GetAllActorsOfClass` "/Game/BP/Class/BP_CheckPoint.BP_CheckPoint_C"))
  (for _array_element _outactors
    (if (== (`self.CheckpointIdToSelect`) (`/Game/BP/Class/BP_CheckPoint.ID` _array_element))
      (break))))

(fn `UserConstructionScript`)