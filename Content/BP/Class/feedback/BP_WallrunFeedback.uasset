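; BP_WallrunFeedback is a trigger volume that sets up material displacement feedback, apparently for wallrunning, when the player character enters it.
; On overlap it writes path width, displacement amount and six marker world locations into the MCollection_displacement parameter collection, then points its scene capture at a wallrun render target.
; The construction script offsets and scales the trigger box from exposed variables.
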(event `self.Box.OnComponentBeginOverlap`
  (params (OverlappedComponent :type "PrimitiveComponent Object Reference") (OtherActor :type "Actor Object Reference") (OtherComp :type "PrimitiveComponent Object Reference") (OtherBodyIndex :type Integer) (bFromSweep :type Boolean) (SweepResult :type "HitResult Structure (by ref)"))
  (if (== OtherActor "/Game/BP/BP_PlayerChara.BP_PlayerChara")
    (`KismetMaterialLibrary.SetScalarParameterValue` "/Game/_ART/Decals/wallrunfeedback/MCollection_displacement.MCollection_displacement" "Distance" (`self.PathWidth`))
    (`KismetMaterialLibrary.SetScalarParameterValue` "/Game/_ART/Decals/wallrunfeedback/MCollection_displacement.MCollection_displacement" "Displacement" (`self.DisplacementAmount`))
    (`KismetMaterialLibrary.SetVectorParameterValue` "/Game/_ART/Decals/wallrunfeedback/MCollection_displacement.MCollection_displacement" "position1" (`KismetMathLibrary.Conv_VectorToLinearColor` (`SceneComponent.K2_GetComponentLocation` (`TargetPoint.SpriteComponent` (`self.position1`)))))
    (`KismetMaterialLibrary.SetVectorParameterValue` "/Game/_ART/Decals/wallrunfeedback/MCollection_displacement.MCollection_displacement" "position2" (`KismetMathLibrary.Conv_VectorToLinearColor` (`SceneComponent.K2_GetComponentLocation` (`TargetPoint.SpriteComponent` (`self.position2`)))))
    (`KismetMaterialLibrary.SetVectorParameterValue` "/Game/_ART/Decals/wallrunfeedback/MCollection_displacement.MCollection_displacement" "position3" (`KismetMathLibrary.Conv_VectorToLinearColor` (`SceneComponent.K2_GetComponentLocation` (`TargetPoint.SpriteComponent` (`self.position3`)))))
    (`KismetMaterialLibrary.SetVectorParameterValue` "/Game/_ART/Decals/wallrunfeedback/MCollection_displacement.MCollection_displacement" "position4" (`KismetMathLibrary.Conv_VectorToLinearColor` (`SceneComponent.K2_GetComponentLocation` (`TargetPoint.SpriteComponent` (`self.position4`)))))
    (`KismetMaterialLibrary.SetVectorParameterValue` "/Game/_ART/Decals/wallrunfeedback/MCollection_displacement.MCollection_displacement" "position5" (`KismetMathLibrary.Conv_VectorToLinearColor` (`SceneComponent.K2_GetComponentLocation` (`TargetPoint.SpriteComponent` (`self.position5`)))))
    (`KismetMaterialLibrary.SetVectorParameterValue` "/Game/_ART/Decals/wallrunfeedback/MCollection_displacement.MCollection_displacement" "position6" (`KismetMathLibrary.Conv_VectorToLinearColor` (`SceneComponent.K2_GetComponentLocation` (`TargetPoint.SpriteComponent` (`self.position6`)))))
    (set `SceneCaptureComponent2D.TextureTarget` "/Game/BP/Class/feedback/TRT_WallrunFeedback.TRT_WallrunFeedback" (`self.SceneCaptureComponent2D`))))

(fn `UserConstructionScript`
  (bind _box (`self.Box`))
  (`SceneComponent.K2_SetRelativeLocation` _box (`self.colision offset`) false false)
  (`SceneComponent.SetWorldScale3D` _box (`self.colision size`)))