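; BP_Hut is a hut actor that registers itself with BP_Controller while the player overlaps its sphere and releases a Shrek enemy when opened.
; OpenDoor flags the controller, then chains custom timelines to swing the door, turn the Shrek mesh and walk it forward through its AnimBP speed.
; The mesh is then hidden and replaced by a spawned BP_EnemySpawn.
; Reset removes the enemy, restores door and mesh, and clears hut-found and, after a delay, caught flags.
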(event `self.ReceiveBeginPlay`
  (set `self.BaseMeshLocation` (`SceneComponent.RelativeLocation` (`self.ShrekMesh`))))

(event `self.Sphere.OnComponentBeginOverlap`
  (params (OverlappedComponent :type "PrimitiveComponent Object Reference") (OtherActor :type "Actor Object Reference") (OtherComp :type "PrimitiveComponent Object Reference") (OtherBodyIndex :type Integer) (bFromSweep :type Boolean) (SweepResult :type "HitResult Structure (by ref)"))
  (cast `/Game/BP/BP_PlayerChara` OtherActor)
  (bind _asbp_controller (cast `/Game/BP/BP_Controller` (`GameplayStatics.GetPlayerController` 0)))
  (set `/Game/BP/BP_Controller.HutFound` true _asbp_controller)
  (set `/Game/BP/BP_Controller.Hut` self _asbp_controller))

(event `self.Sphere.OnComponentEndOverlap`
  (params (OverlappedComponent :type "PrimitiveComponent Object Reference") (OtherActor :type "Actor Object Reference") (OtherComp :type "PrimitiveComponent Object Reference") (OtherBodyIndex :type Integer))
  (cast `/Game/BP/BP_PlayerChara` OtherActor)
  (bind _asbp_controller (cast `/Game/BP/BP_Controller` (`GameplayStatics.GetPlayerController` 0)))
  (set `/Game/BP/BP_Controller.HutFound` false _asbp_controller))

(event `OpenDoor`
  (bind _shrekmesh (`self.ShrekMesh`))
  (bind (_returnvalue_location _returnvalue_rotation _returnvalue_scale) (`KismetMathLibrary.BreakTransform` (`SceneComponent.K2_GetComponentToWorld` (`self.ShrekMesh`))))
  (bind _asabp_shrek (cast `/Game/AI/Animation/ShrekAnimated/ABP_Shrek` (`SkeletalMeshComponent.GetAnimInstance` _shrekmesh) :!pure true))
  (bind _asbp_controller (cast `/Game/BP/BP_Controller` (`GameplayStatics.GetPlayerController` 0)))
  (set `/Game/BP/BP_Controller.HutTriggered` true _asbp_controller)
  (bind _output_get (set `self.StartRotation` (`SceneComponent.RelativeRotation` (`self.DoorParent`))))
  (set `self.TargetRotation` (`KismetMathLibrary.MakeRotator` (.roll _output_get) (.pitch _output_get) (`self.TargetYaw`)))
  (bind _outputvalue (`CustomTimeline.StartCustomTimeline` (/ 1.0 (`self.DoorOpeningDuration`)))
    (:`Update`
      (`SceneComponent.K2_SetRelativeRotation` (`self.DoorParent`) (`KismetMathLibrary.RLerp` (`self.StartRotation`) (`self.TargetRotation`) _outputvalue true) false false))
    (:`Finished`
      (set `self.StartRotation` (`SceneComponent.RelativeRotation` (`self.ShrekMesh`)))
      (set `self.TargetRotation` (struct :`Yaw` 270.0))
      (bind _outputvalue_2 (`CustomTimeline.StartCustomTimeline` 1.0)
        (:`Update`
          (`SceneComponent.K2_SetRelativeRotation` (`self.ShrekMesh`) (`KismetMathLibrary.RLerp` (`self.StartRotation`) (`self.TargetRotation`) _outputvalue_2 true) false false))
        (:`Finished`
          (bind _outputvalue_3 (`CustomTimeline.StartCustomTimeline` 1.0)
            (:`then`
              (set `/Game/AI/Animation/ShrekAnimated/ABP_Shrek.Speed` 200.0 _asabp_shrek))
            (:`Update`
              (`SceneComponent.K2_SetRelativeLocation` _shrekmesh (+ (`self.BaseMeshLocation`) (* (`self.GetActorForwardVector`) (* _outputvalue_3 100.0))) false false))
            (:`Finished`
              (set `/Game/AI/Animation/ShrekAnimated/ABP_Shrek.Speed` 0.0 _asabp_shrek)
              (bind _returnvalue (`|SpawnActorFromClass` "/Game/AI/Blueprints/BP_EnemySpawn.BP_EnemySpawn_C" (`KismetMathLibrary.MakeTransform` _returnvalue_location (`KismetMathLibrary.MakeRotator` (.roll _returnvalue_rotation) (.pitch _returnvalue_rotation) (+ (.yaw _returnvalue_rotation) 90.0)) _returnvalue_scale) "Undefined" "OverrideRootScale" null "NewEnumerator1" null))
              (bind _output_get_2 (set `self.EnemySpawn` _returnvalue))
              (`/Game/AI/Blueprints/BP_EnemySpawn.SpawnEnemy` _output_get_2)
              (`SceneComponent.SetVisibility` (`self.ShrekMesh`) false false)
              (`KismetSystemLibrary.FlushPersistentDebugLines`))))))))

(event `Reset`
  (bind _enemyspawn (`self.EnemySpawn`))
  (bind _shrekmesh (`self.ShrekMesh`))
  (`SceneComponent.K2_SetRelativeLocation` (`self.ShrekMesh`) (`self.BaseMeshLocation`) false false)
  (`/Game/AI/Blueprints/BP_EnemySpawn.DeleteEnemy` _enemyspawn)
  (`self.K2_DestroyActor` _enemyspawn)
  (`SceneComponent.SetVisibility` _shrekmesh true false)
  (`SceneComponent.K2_SetRelativeRotation` _shrekmesh (struct :`Yaw` 90.0) false false)
  (`SceneComponent.K2_SetRelativeRotation` :`self` (`self.DoorParent`))
  (bind _asbp_controller (cast `/Game/BP/BP_Controller` (`GameplayStatics.GetPlayerController` 0)))
  (set `/Game/BP/BP_Controller.HutFound` false _asbp_controller)
  (`KismetSystemLibrary.Delay` 1.0)
  (bind _asbp_player_chara (cast `/Game/BP/BP_PlayerChara` (`GameplayStatics.GetPlayerCharacter` 0)))
  (set `/Game/BP/BP_PlayerChara.CaughtRecently` false _asbp_player_chara))

(fn `UserConstructionScript`)