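; Tram actor that builds spline-mesh track in construction and runs a looping train of child-actor cars along it, with ambient sound and speed-triggered particles.
; A zero-delay self-calling event advances per-car distances, scaling speed by slope and a position-sampled curve, orienting cars between two spline points.
; At the spline end, cars are destroyed and respawned.
; Crystallize eases the tram to a temporary stop; SetTramPosition re-seats it near a world location.
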(event `self.ReceiveBeginPlay`
  ;[1 0 0.8447] Begin play
  (bind _returnvalue (`GameplayStatics.SpawnSoundAttached` "/Game/Sound_Design/Bruitages/City/Train_city.Train_city" (`self.DefaultSceneRoot`) "None" (0.0 0.0 0.0) (struct) "KeepRelativeOffset" true 5.0 1.0 0.0 null null false))
  (set `self.AmbientSound` _returnvalue)
  (`ActorComponent.K2_DestroyComponent` (`self.SM_metro_locomotive`))
  (`self.start tram`))

(event `self.ReceiveTick`
  (params (DeltaSeconds :type "Float (single-precision)"))
  (bind _particlesystem (`self.ParticleSystem`))
  ;[1 0 0.8225] Event tick
  (set `self.delta time` DeltaSeconds)
  (`self.CheckSound`)
  ;[1 1 1] Activation particule freinage
  (if (> (`self.tram speed`) 30.0)
    (`SceneComponent.SetVisibility` _particlesystem true true)
    (else
      (`SceneComponent.SetVisibility` _particlesystem false true))))

(event `CheckSound`
  (bind _ambientsound (`self.AmbientSound`))
  ;[1 1 1] check sound
  (if (!= _ambientsound null)
    (if (not (`AudioComponent.IsPlaying` _ambientsound))
      (`AudioComponent.Play` _ambientsound 0.0))))

(event `Start tram`
  (bind _spline (`self.Spline`))
  (bind _returnvalue (* (`self.index wagon spawn`) (`self.distance between wagon`)))
  (bind _returnvalue_2 (`KismetMathLibrary.MakeTransform` (`SplineComponent.GetLocationAtDistanceAlongSpline` _spline _returnvalue "World") (`SplineComponent.GetRotationAtDistanceAlongSpline` _spline _returnvalue "World")))
  ;[1 1 1] spawn le wagon de fin
  (bind _returnvalue_3 (`AddComponent|NODE_AddChildActorComponent-0`))
  (bind _asbp_tram_voiture_fin (cast `/Game/BP/Class/BP_Tram_Voiture_Fin` (`ChildActorComponent.ChildActor` _returnvalue_3)))
  (set `/Game/BP/Class/BP_Tram_Voiture_Fin.Tram` self _asbp_tram_voiture_fin)
  (`KismetArrayLibrary.Array_Add` (`self.wagon liste`) _returnvalue_3)
  ;[1 1 1] spawn des wagons
  (for _ (range (+ (- (`self.number of wagon`) 2) 1))
    (bind _returnvalue_4 (`AddComponent|NODE_AddChildActorComponent-1`))
    (bind _asbp_tram_voiture_middle (cast `/Game/BP/Class/BP_Tram_Voiture_Middle` (`ChildActorComponent.ChildActor` _returnvalue_4)))
    (set `/Game/BP/Class/BP_Tram_Voiture_Middle.Tram` self _asbp_tram_voiture_middle)
    (`KismetArrayLibrary.Array_Add` (`self.wagon liste`) _returnvalue_4))
  ;[1 1 1] rajout de la locomotive a la liste des wagon
  (bind _returnvalue_5 (`AddComponent|NODE_AddChildActorComponent-2`))
  (bind _asbp_tram_voiture_first (cast `/Game/BP/Class/BP_Tram_Voiture_First` (`ChildActorComponent.ChildActor` _returnvalue_5)))
  (set `/Game/BP/Class/BP_Tram_Voiture_First.Tram` self _asbp_tram_voiture_first)
  (`KismetArrayLibrary.Array_Add` (`self.wagon liste`) _returnvalue_5)
  ;[1 1 1] setting de la position et rotation initial des wagons
  (for (_array_element _array_index) (`self.wagon liste`)
    (set `self.index wagon spawn` _array_index)
    (`SceneComponent.K2_SetWorldTransform` _array_element _returnvalue_2 false false)
    (`SceneComponent.K2_SetWorldTransform` (`self.Particules`) _returnvalue_2 false false)
    ;[1 1 1] création d'une variable de distance pour chaque wagons
    (`KismetArrayLibrary.Array_Add` (`self.Distance on rail`) (* (`self.index wagon spawn`) (`self.distance between wagon`))))
  ;[1 1 1] lancement de l'event qui bouge les wagons
  (`self.move tram`))

(event `Move tram`
  (bind _next_distance_on_rail (`self.next distance on rail`))
  (bind _returnvalue (select `bool` (`self.customSpline?`) :`false` (`self.Spline`) :`true` (`self.customSpline`)))
  (bind _returnvalue_2 (`SplineComponent.GetLocationAtDistanceAlongSpline` (select `bool` (`self.customSpline?`) :`false` (`self.Spline`) :`true` (`self.customSpline`)) (- (`self.next distance on rail`) (`self.wagon back hangs offset`)) "World"))
  (bind _returnvalue_3 (`SplineComponent.GetLocationAtDistanceAlongSpline` (select `bool` (`self.customSpline?`) :`false` (`self.Spline`) :`true` (`self.customSpline`)) (`self.next distance on rail`) "World"))
  (bind _returnvalue_4 (`KismetMathLibrary.MakeTransform` (`SplineComponent.GetLocationAtDistanceAlongSpline` _returnvalue _next_distance_on_rail "World") (`SplineComponent.GetRotationAtDistanceAlongSpline` _returnvalue _next_distance_on_rail "World")))
  (bind _returnvalue_5 (`KismetMathLibrary.MakeTransform` (`KismetMathLibrary.GetVectorArrayAverage` (`|MakeArray` _returnvalue_3 _returnvalue_2)) (`KismetMathLibrary.FindLookAtRotation` _returnvalue_2 _returnvalue_3)))
  ;[1 1 1] obtention la vitesse
  ;;[1 1 1] permet d'évité un bug d'infiny loop
  (`KismetSystemLibrary.Delay` 0.0)
  (for (_array_element _array_index) (`self.wagon liste`)
    (set `self.wagon ref` _array_element)
    (set `self.index wagon move` _array_index)
    (set `self.tram speed` (* (* (* (* (+ (* (`KismetMathLibrary.Abs` (- (.z (`SplineComponent.GetDirectionAtDistanceAlongSpline` (`self.Spline`) (`|GetArrayItem` (`self.Distance on rail`) (`self.number of wagon`)) "Local")) 1.0)) (`self.tilt speed multiplier`)) (`self.tilt speed offset`)) (`CurveFloat.GetFloatValue` (`self.speed`) (/ (`|GetArrayItem` (`self.Distance on rail`) (`self.number of wagon`)) (`SplineComponent.GetSplineLength` (`self.Spline`))))) (`self.delta time`)) (`self.CustomTimeDilation`)) (`self.SpeedMultiplier`)))
    ;[1 1 1] setting de la prochaine position du wagon qu'on est en train de bouger
    (set `self.next distance on rail` (+ (`self.tram speed`) (`|GetArrayItem` (`self.Distance on rail`) (`self.index wagon move`))))
    ;[1 1 1] setting de la position du wagon qu'on est en train de bouger
    (`KismetArrayLibrary.Array_Set` (`self.Distance on rail`) (`self.index wagon move`) (`self.next distance on rail`))
    ;[1 1 1] vérification que la locomotive a fini de traversé l'entièreté de la spline
    (if (>= (`|GetArrayItem` (`self.Distance on rail`) (- (`KismetArrayLibrary.Array_Length` (`self.wagon liste`)) 1)) (`SplineComponent.GetSplineLength` (`self.Spline`)))
      ;[1 1 1] destruction des wagons
      (for _array_element_2 (`self.wagon liste`)
        (if (!= _array_element_2 null)
          (`ActorComponent.K2_DestroyComponent` _array_element_2)))
      ;[1 1 1] nettoyage des données
      (`KismetArrayLibrary.Array_Clear` (`self.Distance on rail`))
      (`KismetArrayLibrary.Array_Clear` (`self.wagon liste`))
      ;[1 1 1] lance l'event de begin play
      (`self.start tram`)
      (else
        ;[1 1 1] vérification si le wagon bougé est la locomotive
        (if (== (`self.wagon ref`) null)
          ;[1 1 1] setting de la position et rotation de la locomotive en fonction de sa prochaine distance sur la spline
          (`SceneComponent.K2_SetWorldTransform` (`self.wagon ref`) _returnvalue_4 false false)
          (`SceneComponent.K2_SetWorldTransform` (`self.Particules`) _returnvalue_4 false false)
          (else
            ;[1 1 1] setting de la position et rotation des wagons en fonction de sa prochaine distance sur la spline
            (`SceneComponent.K2_SetWorldTransform` (`self.wagon ref`) _returnvalue_5 false false)
            (`SceneComponent.K2_SetWorldTransform` (`self.Particules`) _returnvalue_5 false false)))
        ;[1 1 1] re lance l'event qui fait avancé les wagon
        (`self.move tram`)))))

(event `SetTramPosition`
  (params (WorldPosition :type "Vector Structure"))
  ;[1 1 1] Set tram position
  (bind _distance_on_rail (`self.Find distance and direction along spline closest to world location` WorldPosition (`self.Spline`)))
  (for (_ _array_index) (`self.wagon liste`)
    (`KismetArrayLibrary.Array_Set` (`self.Distance on rail`) _array_index (+ _distance_on_rail (* _array_index (`self.distance between wagon`))))))

(event `/Game/BP/Class/BPI_Cristallizable.Crystallize`
  (params (FreezeDuration :type "Float (single-precision)"))
  (`/Engine/EditorBlueprintResources/StandardMacros.DoOnce` false :!label _label
    (:`Completed`
      (bind _outputvalue (`CustomTimeline.StartCustomTimeline` 1.0)
        (:`Update`
          (set `self.SpeedMultiplier` (- 1.0 _outputvalue)))
        (:`Finished`
          (set `self.SpeedMultiplier` 0.0)
          (`KismetSystemLibrary.Delay` FreezeDuration)
          (bind _outputvalue_2 (`CustomTimeline.StartCustomTimeline` 1.0)
            (:`Update`
              (set `self.SpeedMultiplier` _outputvalue_2))
            (:`Finished`
              (set `self.SpeedMultiplier` 1.0)
              (goto _label :!via `Reset`))))))))

(fn `Find distance and direction along spline closest to world location`
  (params (location :type "Vector Structure") (spline :type "SplineComponent Object Reference"))
  (returns (`distance on rail` :type "Float (double-precision)") (Direction :type "Vector Structure"))
  (return (* (/ (`SplineComponent.FindInputKeyClosestToWorldLocation` spline location) (`KismetMathLibrary.Conv_IntToDouble` (- (`SplineComponent.GetNumberOfSplinePoints` spline) 1))) (`SplineComponent.GetSplineLength` spline)) (`SplineComponent.FindDirectionClosestToWorldLocation` spline location "World")))

(fn `IsCrystallized`
  (returns (Crystallized :type Boolean))
  (return false))

(fn `UserConstructionScript`
  (bind _spline (`self.Spline`))
  (for _index (range (`SplineComponent.GetNumberOfSplinePoints` (`self.Spline`)))
    (bind _returnvalue (`AddComponent|NODE_AddSplineMeshComponent-2`))
    (`SceneComponent.K2_AttachToComponent` _spline (`self.DefaultSceneRoot`) "None" "KeepWorld" "KeepWorld" "KeepRelative" false)
    (bind _returnvalue_2 (- _index 1))
    (`SplineMeshComponent.SetStartAndEnd` _returnvalue (`SplineComponent.GetLocationAtSplinePoint` _spline _index "Local") (* (`SplineComponent.GetTangentAtSplinePoint` _spline _index "Local") (-1.0 -1.0 -1.0)) (`SplineComponent.GetLocationAtSplinePoint` _spline _returnvalue_2 "Local") (* (`SplineComponent.GetTangentAtSplinePoint` _spline _returnvalue_2 "Local") (-1.0 -1.0 -1.0)) true)))