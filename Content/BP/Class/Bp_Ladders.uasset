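; Ladder Blueprint that procedurally places static meshes along a spline in the Construction Script, with no active runtime logic.
; NumLadder sets how many pieces are evenly spaced over the spline length.
; A randomized, looping MultiGate picks one of three mesh component nodes for each piece.
; Each piece is pitched -90 degrees, scaled down to 0.01 and given a random yaw within plus or minus InclinaisonEnDegre.
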(fn `UserConstructionScript`
  (bind _inclinaisonendegre (`self.InclinaisonEnDegre`))
  (bind _returnvalue (`KismetMathLibrary.MakeRotator` 0.0 -90.0 (`KismetMathLibrary.RandomFloatInRange` (* _inclinaisonendegre -1.0) _inclinaisonendegre)))
  (for _index (range 1 (+ (`self.NumLadder`) 1))
    (`|MultiGate` true true 0
      (:`Out 0`
        (bind _returnvalue_2 (`SplineComponent.GetLocationAtDistanceAlongSpline` (`self.Spline`) (* (`KismetMathLibrary.Conv_IntToDouble` _index) (/ (`SplineComponent.GetSplineLength` (`self.Spline`)) (`KismetMathLibrary.Conv_IntToDouble` (`self.NumLadder`)))) "Local"))
        (`AddComponent|NODE_AddStaticMeshComponent-1` :`RelativeTransform` (`KismetMathLibrary.MakeTransform` _returnvalue_2 _returnvalue (0.01 0.01 0.01))))
      (:`Out 1`
        (`AddComponent|NODE_AddStaticMeshComponent-4` :`RelativeTransform` (`KismetMathLibrary.MakeTransform` _returnvalue_2 _returnvalue (0.01 0.01 0.01))))
      (:`Out 2`
        (`AddComponent|NODE_AddStaticMeshComponent-5` :`RelativeTransform` (`KismetMathLibrary.MakeTransform` _returnvalue_2 _returnvalue (0.01 0.01 0.01)))))))