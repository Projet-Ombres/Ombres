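; BP_SpectatorController relays movement requests from the player character's Recorder back into that character's movement functions.
; On BeginPlay it caches player 0's BP_PlayerChara and binds to the Recorder's forward and right move request events.
; Each handler passes the input value to the matching function on the character, and the forward handler also prints it for debugging.
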(event `MoveForward`
  (params (InputValue :type "Float (double-precision)"))
  (`/Game/BP/BP_PlayerChara.MoveForward` (`self.PlayerChara`) InputValue)
  (`KismetSystemLibrary.PrintString` (`KismetStringLibrary.Concat_StrStr` "Move forward : " (`KismetStringLibrary.Conv_DoubleToString` InputValue))))

(event `self.ReceiveBeginPlay`
  (bind _asbp_player_chara (cast `/Game/BP/BP_PlayerChara` (`GameplayStatics.GetPlayerCharacter` 0)))
  (bind _output_get (set `self.PlayerChara` _asbp_player_chara))
  (bind _recorder (`/Game/BP/BP_PlayerChara.Recorder` _output_get))
  (add `RecorderComponent.OnMoveForwardRequest` _recorder (delegate `MoveForward`))
  (add `RecorderComponent.OnMoveRightRequest` _recorder (delegate `MoveRight`)))

(event `MoveRight`
  (params (InputValue :type "Float (double-precision)"))
  (`/Game/BP/BP_PlayerChara.MoveRight` (`self.PlayerChara`) InputValue))

(fn `UserConstructionScript`)