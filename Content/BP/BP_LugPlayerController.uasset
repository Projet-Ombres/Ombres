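; BP_LugPlayerController is the player controller that routes movement, look and jump input to the Lug player character.
; On BeginPlay it casts player character 0 to BP_LugPlayerCharacter and caches it.
; Axis events forward values to that character's movement and look functions, with separate handlers for rate-based and mouse look.
; Pressing Jump calls Jump on the character's BPCJump component, keeping the controller free of gameplay logic.
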(event `self.ReceiveBeginPlay`
  ;[1 0 0.7113] BeginPlay
  ;[1 1 1] Set first person character
  (set `self.PlayerCharacter` (cast `/Game/BP/BP_LugPlayerCharacter` (`GameplayStatics.GetPlayerCharacter` 0) :!pure true)))

(event `InputAxis|TurnRate`
  (params (AxisValue :type "Float (single-precision)"))
  ;[1 0.7991 0.3712] Player character Look around
  (`/Game/BP/BP_LugPlayerCharacter.TurnRateAxis` (`self.PlayerCharacter`) AxisValue))

(event `InputAxis|MoveForward`
  (params (AxisValue :type "Float (single-precision)"))
  ;[1 0.7991 0.3712] Player Character movement
  (`/Game/BP/BP_LugPlayerCharacter.MoveForward` (`self.PlayerCharacter`) AxisValue))

(event `InputAxis|LookUpRate`
  (params (AxisValue :type "Float (single-precision)"))
  ;[1 0.7991 0.3712] Player character Look around
  (`/Game/BP/BP_LugPlayerCharacter.LookUpRate` (`self.PlayerCharacter`) AxisValue))

(event `InputAxis|MoveRight`
  (params (AxisValue :type "Float (single-precision)"))
  ;[1 0.7991 0.3712] Player Character movement
  (`/Game/BP/BP_LugPlayerCharacter.MoveRight` (`self.PlayerCharacter`) AxisValue))

(event `InputAxis|Turn` :overrideparent false
  (params (AxisValue :type "Float (single-precision)"))
  ;[1 0.7991 0.3712] Player character Look around
  (`/Game/BP/BP_LugPlayerCharacter.MouseTurnAxis` (`self.PlayerCharacter`) AxisValue))

(event `InputAxis|LookUp` :overrideparent false
  (params (AxisValue :type "Float (single-precision)"))
  ;[1 0.7991 0.3712] Player character Look around
  (`/Game/BP/BP_LugPlayerCharacter.MouseLookUpAxis` (`self.PlayerCharacter`) AxisValue))

(event `InputAction|Jump`
  (params (Key :type "Key Structure"))
  (:`Pressed`
    (`/Game/BP/Components/CapacitéPhysique/BPC_Jump.Jump` (`/Game/BP/BP_LugPlayerCharacter.BPC_Jump` (`self.PlayerCharacter`)))))

(fn `UserConstructionScript`)