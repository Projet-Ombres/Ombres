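; Player component for a timed skywalk ability that spawns platforms along the player's path.
; SkyWalk sets an active flag for a set duration after Initialize caches the player and mesh.
; While active, Tick spawns a BP_SkywalkPlatform whenever the mesh moves past a distance threshold, then immediately calls Destroy on it.
; Platforms spawn at the mesh, nudged along camera forward, matching camera rotation with clamped pitch.
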(event `Initialize`
  (params (`Player Ref` :type "/Game/BP/BP_PlayerChara Object Reference"))
  (bind _output_get (set `self.Player Ref` `Player Ref`))
  (set `self.Mesh Ref` (`Character.Mesh` _output_get)))

(event `SkyWalk`
  (params (DeltaSeconds :type "Float (double-precision)"))
  (set `self.Sky Walk Is Active?` true)
  (set `self.Last position` (`SceneComponent.K2_GetComponentLocation` (`Character.Mesh` (`self.Player Ref`))))
  (`KismetSystemLibrary.Delay` (`self.Sky Walk Duration`))
  (set `self.Sky Walk Is Active?` false))

(event `self.ReceiveTick`
  (params (DeltaSeconds :type "Float (single-precision)"))
  (bind _camera (`/Game/BP/BP_PlayerChara.Camera` (`self.Player Ref`)))
  (bind (_returnvalue_roll _returnvalue_pitch _returnvalue_yaw) (`KismetMathLibrary.BreakRotator` (`SceneComponent.K2_GetComponentRotation` _camera)))
  (if (`self.Sky Walk Is Active?`)
    (if (> (`KismetMathLibrary.VSize` (- (`self.Last position`) (`SceneComponent.K2_GetComponentLocation` (`Character.Mesh` (`self.Player Ref`))))) 100.0)
      (set `self.Last position` (`SceneComponent.K2_GetComponentLocation` (`Character.Mesh` (`self.Player Ref`))))
      (bind _returnvalue (`|SpawnActorFromClass` "/Game/BP/Skywalk/BP_SkywalkPlatform.BP_SkywalkPlatform_C" (`KismetMathLibrary.MakeTransform` (+ (`SceneComponent.K2_GetComponentLocation` (`self.Mesh Ref`)) (`SceneComponent.GetForwardVector` _camera)) (`KismetMathLibrary.MakeRotator` _returnvalue_roll (`KismetMathLibrary.FClamp` _returnvalue_pitch -40.0 40.0) _returnvalue_yaw)) "Undefined" "OverrideRootScale" null null))
      (`/Game/BP/Skywalk/BP_SkywalkPlatform.Destroy` _returnvalue))))