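; An editor-folder Blueprint that copies window mesh instances from a referenced WindowsEater into its own small, medium and large window components, as hierarchical instances judging by its naming.
; ConvertInstancesToHierarchicalInstances clears all three components, then loops over each matching source component and re-adds every instance using its world-space transform.
; ClearInstances also stands as its own event to empty the three components, and the construction script is empty.
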(event `ClearInstances`
  (`InstancedStaticMeshComponent.ClearInstances` (`self.SmallWindows`))
  (`InstancedStaticMeshComponent.ClearInstances` (`self.MediumWindows`))
  (`InstancedStaticMeshComponent.ClearInstances` (`self.LargeWindows`)))

(event `ConvertInstancesToHierarchicalInstances`
  (bind _windowseater (`self.WindowsEater`))
  (bind _smallwindows (`/Game/BP/Editor/MeshInstacnes/BP_WindowsEater.SmallWindows` _windowseater))
  (bind _mediumwindows (`/Game/BP/Editor/MeshInstacnes/BP_WindowsEater.MediumWindows` _windowseater))
  (bind _largewindows (`/Game/BP/Editor/MeshInstacnes/BP_WindowsEater.LargeWindows` _windowseater))
  (`self.ClearInstances`)
  (`|ExecutionSequence`
    (:`then_0`
      (for _index (range (`InstancedStaticMeshComponent.GetInstanceCount` _smallwindows))
        (`InstancedStaticMeshComponent.AddInstanceWorldSpace` (`self.SmallWindows`) (`InstancedStaticMeshComponent.GetInstanceTransform` _smallwindows _index true))))
    (:`then_1`
      (for _index_2 (range (`InstancedStaticMeshComponent.GetInstanceCount` _mediumwindows))
        (`InstancedStaticMeshComponent.AddInstanceWorldSpace` (`self.MediumWindows`) (`InstancedStaticMeshComponent.GetInstanceTransform` _mediumwindows _index_2 true))))
    (:`then_2`
      (for _index_3 (range (`InstancedStaticMeshComponent.GetInstanceCount` _largewindows))
        (`InstancedStaticMeshComponent.AddInstanceWorldSpace` (`self.LargeWindows`) (`InstancedStaticMeshComponent.GetInstanceTransform` _largewindows _index_3 true))))))

(fn `UserConstructionScript`)