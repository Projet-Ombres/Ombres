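; Window-consolidation actor, apparently an editor tool, that gathers placed windows into six instanced mesh components, covering small, medium and large sizes of two types.
; EatWindows copies window actors' mesh transforms into matching components, then blanks every child actor component using those classes.
; It also converts type 1 window meshes inside M3 actors to instances and blanks the originals.
; ClearInstances empties all six components without restoring blanked sources.
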(event `ClearInstances`
  (`InstancedStaticMeshComponent.ClearInstances` (`self.SmallWindowsType1`))
  (`InstancedStaticMeshComponent.ClearInstances` (`self.MediumWindowsType1`))
  (`InstancedStaticMeshComponent.ClearInstances` (`self.LargeWindowsType1`))
  (`InstancedStaticMeshComponent.ClearInstances` (`self.SmallWindowsType2`))
  (`InstancedStaticMeshComponent.ClearInstances` (`self.MediumWindowsType2`))
  (`InstancedStaticMeshComponent.ClearInstances` (`self.LargeWindowsType2`)))

(event `EatWindows`
  (`|ExecutionSequence`
    (:`then_0`
      (bind _outactors (`GameplayStatics.GetAllActorsOfClass` "/Game/_ART/StaticMesh/Windows/Large_windons_type01.Large_windons_type01_C"))
      (for _array_element _outactors
        (`InstancedStaticMeshComponent.AddInstanceWorldSpace` (`self.LargeWindowsType1`) (`SceneComponent.K2_GetComponentToWorld` (`/Game/_ART/StaticMesh/Windows/Large_windons_type01.SM_Large_Windonw_type01` _array_element)))))
    (:`then_1`
      (bind _outactors_2 (`GameplayStatics.GetAllActorsOfClass` "/Game/_ART/StaticMesh/Windows/medium_windons_type01_2.medium_windons_type01_2_C"))
      (for _array_element_2 _outactors_2
        (`InstancedStaticMeshComponent.AddInstanceWorldSpace` (`self.MediumWindowsType1`) (`SceneComponent.K2_GetComponentToWorld` (`/Game/_ART/StaticMesh/Windows/medium_windons_type01_2.SM_medium_Windonw_type01` _array_element_2)))))
    (:`then_2`
      (bind _outactors_3 (`GameplayStatics.GetAllActorsOfClass` "/Game/_ART/StaticMesh/Windows/small_windons_type01_3.small_windons_type01_3_C"))
      (for _array_element_3 _outactors_3
        (`InstancedStaticMeshComponent.AddInstanceWorldSpace` (`self.SmallWindowsType1`) (`SceneComponent.K2_GetComponentToWorld` (`/Game/_ART/StaticMesh/Windows/small_windons_type01_3.SM_Small_Windonw_type01` _array_element_3)))))
    (:`then_3`
      (bind _outactors_4 (`GameplayStatics.GetAllActorsOfClass` "/Game/_ART/StaticMesh/Windows/large_type2.large_type2_C"))
      (for _array_element_4 _outactors_4
        (`InstancedStaticMeshComponent.AddInstanceWorldSpace` (`self.LargeWindowsType2`) (`SceneComponent.K2_GetComponentToWorld` (`/Game/_ART/StaticMesh/Windows/large_type2.SM_Large_Windonw_type02` _array_element_4)))))
    (:`then_4`
      (bind _outactors_5 (`GameplayStatics.GetAllActorsOfClass` "/Game/_ART/StaticMesh/Windows/medium_type2.medium_type2_C"))
      (for _array_element_5 _outactors_5
        (`InstancedStaticMeshComponent.AddInstanceWorldSpace` (`self.MediumWindowsType2`) (`SceneComponent.K2_GetComponentToWorld` (`/Game/_ART/StaticMesh/Windows/medium_type2.SM_Medium_Windonw_type02` _array_element_5)))))
    (:`then_5`
      (bind _outactors_6 (`GameplayStatics.GetAllActorsOfClass` "/Game/_ART/StaticMesh/Windows/small_type3.small_type3_C"))
      (for _array_element_6 _outactors_6
        (`InstancedStaticMeshComponent.AddInstanceWorldSpace` (`self.SmallWindowsType2`) (`SceneComponent.K2_GetComponentToWorld` (`/Game/_ART/StaticMesh/Windows/small_type3.SM_Small_Windonw_type02` _array_element_6)))))
    (:`then_6`
      (bind _outactors_7 (`GameplayStatics.GetAllActorsOfClass` "/Script/Engine.Actor"))
      (for _array_element_7 _outactors_7
        (for _array_element_8 (`self.K2_GetComponentsByClass` _array_element_7 "/Script/Engine.ChildActorComponent")
          (bind _childactorclass (`ChildActorComponent.ChildActorClass` _array_element_8))
          (if (or (== _childactorclass "/Game/_ART/StaticMesh/Windows/Large_windons_type01.Large_windons_type01_C") (== _childactorclass "/Game/_ART/StaticMesh/Windows/large_type2.large_type2_C") (== _childactorclass "/Game/_ART/StaticMesh/Windows/small_windons_type01_3.small_windons_type01_3_C") (== _childactorclass "/Game/_ART/StaticMesh/Windows/small_type3.small_type3_C") (== _childactorclass "/Game/_ART/StaticMesh/Windows/medium_windons_type01_2.medium_windons_type01_2_C") (== _childactorclass "/Game/_ART/StaticMesh/Windows/medium_type2.medium_type2_C"))
            (`ChildActorComponent.SetChildActorClass` _array_element_8 null)))))
    (:`then_7`
      (bind _outactors_8 (`GameplayStatics.GetAllActorsOfClass` "/Game/Levels/Final_Preprod/Jolie_Maison_preprod/m3.m3_C"))
      (for _array_element_9 _outactors_8
        (for _array_element_10 (`self.K2_GetComponentsByClass` _array_element_9 "/Script/Engine.StaticMeshComponent")
          (bind _staticmesh (`StaticMeshComponent.StaticMesh` _array_element_10))
          (if (== _staticmesh "/Game/_ART/StaticMesh/Windows/SM_Small_Windonw_type01.SM_Small_Windonw_type01")
            (`InstancedStaticMeshComponent.AddInstanceWorldSpace` (`self.SmallWindowsType1`) (`SceneComponent.K2_GetComponentToWorld` _array_element_10))
            (`StaticMeshComponent.SetStaticMesh` _array_element_10 null)
            (elif (== _staticmesh "/Game/_ART/StaticMesh/Windows/SM_medium_Windonw_type01.SM_medium_Windonw_type01")
              (`InstancedStaticMeshComponent.AddInstanceWorldSpace` (`self.MediumWindowsType1`) (`SceneComponent.K2_GetComponentToWorld` _array_element_10))
              (`StaticMeshComponent.SetStaticMesh` _array_element_10 null)
              (elif (== _staticmesh "/Game/_ART/StaticMesh/Windows/SM_Large_Windonw_type01.SM_Large_Windonw_type01")
                (`InstancedStaticMeshComponent.AddInstanceWorldSpace` (`self.LargeWindowsType1`) (`SceneComponent.K2_GetComponentToWorld` _array_element_10))
                (`StaticMeshComponent.SetStaticMesh` _array_element_10 null)))))))))

(fn `UserConstructionScript`)