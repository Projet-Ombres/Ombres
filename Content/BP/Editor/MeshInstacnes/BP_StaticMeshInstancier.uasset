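; Editor utility actor that merges placed copies of a chosen static mesh into one hierarchical instanced static mesh component.
; Convert scans all other actors for components using that mesh, including existing instanced ones, stores their world transforms in Instances and destroys the source components.
; The construction script creates the HISM component and rebuilds its instances from the stored transforms, converted relative to that component.
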(event `Convert`
  (`/Engine/EditorBlueprintResources/StandardMacros.IsValid` (`self.StaticMesh`)
    (:`Is Valid`
      (`KismetArrayLibrary.Array_Clear` (`self.Instances`))
      (bind _outactors (`GameplayStatics.GetAllActorsOfClass` "/Script/Engine.Actor"))
      (for _array_element _outactors
        (if (!= _array_element self)
          (`self.AddStaticMeshInstances` _array_element))))))

(fn `AddStaticMeshInstances`
  (params (Actor :type "Actor Object Reference"))
  (locals (InstancesArray :type "Array of SceneComponent Object Reference"))
  (bind _rootcomponent (`Actor.RootComponent` Actor))
  (`/Engine/EditorBlueprintResources/StandardMacros.IsValid` _rootcomponent
    (:`Is Valid`
      (bind _output_get (set `local.InstancesArray` (`SceneComponent.GetChildrenComponents` _rootcomponent true)))
      (`KismetArrayLibrary.Array_Append` _output_get (`|MakeArray` _rootcomponent))
      (for _array_element _output_get
        (bind _asstatic_mesh_component (cast `StaticMeshComponent` _array_element))
        (if (== (`StaticMeshComponent.StaticMesh` _asstatic_mesh_component) (`self.StaticMesh`))
          (bind _asinstanced_static_mesh_component (cast `InstancedStaticMeshComponent` _asstatic_mesh_component)
            (:`then`
              (for _index (range (`InstancedStaticMeshComponent.GetInstanceCount` _asinstanced_static_mesh_component))
                (`KismetArrayLibrary.Array_Add` (`self.Instances`) (`InstancedStaticMeshComponent.GetInstanceTransform` _asinstanced_static_mesh_component _index true)))
              (`ActorComponent.K2_DestroyComponent` _asinstanced_static_mesh_component))
            (:`CastFailed`
              (`KismetArrayLibrary.Array_Add` (`self.Instances`) (`SceneComponent.K2_GetComponentToWorld` _asstatic_mesh_component))
              (`ActorComponent.K2_DestroyComponent` _asstatic_mesh_component))))))))

(fn `UserConstructionScript`
  (bind _returnvalue (`AddComponent|NODE_AddHierarchicalInstancedStaticMeshComponent-2` :`RelativeTransform` (`KismetMathLibrary.MakeTransform` (0.0 0.0 0.0))))
  (`StaticMeshComponent.SetStaticMesh` _returnvalue (`self.StaticMesh`))
  (for _array_element (`self.Instances`)
    (`InstancedStaticMeshComponent.AddInstance` _returnvalue (`KismetMathLibrary.MakeRelativeTransform` _array_element (`SceneComponent.K2_GetComponentToWorld` _returnvalue)))))