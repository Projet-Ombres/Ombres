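; BP_Instancier is a helper actor that copies placed static mesh actors into hierarchical instanced static mesh instances.
; CreateInstances assigns the chosen StaticMesh to the HISM component, then scans every StaticMeshActor in the level for that same mesh.
; Each match adds an instance at the component's world transform.
; The source actors are left in place, and existing instances are not cleared first.
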(event `CreateInstances`
  (`StaticMeshComponent.SetStaticMesh` (`self.HierarchicalInstancedStaticMesh`) (`self.StaticMesh`))
  (bind _outactors (`GameplayStatics.GetAllActorsOfClass` "/Script/Engine.StaticMeshActor"))
  (for _array_element _outactors
    (bind _staticmeshcomponent (`StaticMeshActor.StaticMeshComponent` _array_element))
    (if (== (`StaticMeshComponent.StaticMesh` _staticmeshcomponent) (`self.StaticMesh`))
      (`InstancedStaticMeshComponent.AddInstanceWorldSpace` (`self.HierarchicalInstancedStaticMesh`) (`SceneComponent.K2_GetComponentToWorld` _staticmeshcomponent)))))

(fn `UserConstructionScript`)