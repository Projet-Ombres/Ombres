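; Editor Blueprint that lays out rotated copies of a static mesh, presumably as source views for creating an imposter.
; The construction script calls GenerateDuplicates, which fills an 8x8 grid on the XZ plane with child StaticMeshActors showing the chosen mesh.
; Offset sets the spacing, and DiffAngle steps roll along each row and yaw from row to row.
; It contains no capture or baking logic.
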(fn `GenerateDuplicates`
  (bind _offset (`self.Offset`))
  (`/Engine/EditorBlueprintResources/StandardMacros.IsValid` (`self.StaticMesh`)
    (:`Is Valid`
      (for _index (range 8)
        (for _index_2 (range 8)
          (bind _returnvalue (`AddComponent|NODE_AddChildActorComponent-1` :`RelativeTransform` (`KismetMathLibrary.MakeTransform` (`KismetMathLibrary.MakeVector` (* _index_2 _offset) 0.0 (* _index _offset)) (`KismetMathLibrary.MakeRotator` (* _index_2 (`self.DiffAngle`)) 0.0 (* _index (`self.DiffAngle`))))))
          (`ChildActorComponent.SetChildActorClass` _returnvalue "/Script/Engine.StaticMeshActor")
          (bind _childactor (`ChildActorComponent.ChildActor` _returnvalue))
          (`self.K2_AttachToComponent` _childactor (`self.RootComponent`) "None" "KeepRelative" "KeepRelative" "KeepRelative" true)
          (bind _asstatic_mesh_actor (cast `StaticMeshActor` _childactor))
          (`StaticMeshComponent.SetStaticMesh` (`StaticMeshActor.StaticMeshComponent` _asstatic_mesh_actor) (`self.StaticMesh`)))))))

(fn `UserConstructionScript`
  (locals (InitialRotation :type "Rotator Structure"))
  (`self.GenerateDuplicates`))