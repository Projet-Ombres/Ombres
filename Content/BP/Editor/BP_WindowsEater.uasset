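; BP_WindowsEater is an editor-folder Blueprint that consolidates window actors in the level into large, medium and small instanced mesh components.
; EatWindows gathers window actors by size and adds a world-space instance at each mesh component's transform.
; It then scans every actor's ChildActorComponents and resets the child class on those matching three classes, apparently removing the original windows.
; ClearInstances empties all three instance components.
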(event `EatWindows`
  (`|ExecutionSequence`
    (:`then_0`
      (bind _outactors (`GameplayStatics.GetAllActorsOfClass` null))
      (for _array_element _outactors
        (`InstancedStaticMeshComponent.AddInstanceWorldSpace` (`self.LargeWindows`) (`SceneComponent.K2_GetComponentToWorld` (`/Game/BP/Editor/BP_WindowsEater.SM_Large_Windonw_type01` _array_element)))))
    (:`then_1`
      (bind _outactors_2 (`GameplayStatics.GetAllActorsOfClass` null))
      (for _array_element_2 _outactors_2
        (`InstancedStaticMeshComponent.AddInstanceWorldSpace` (`self.MediumWindows`) (`SceneComponent.K2_GetComponentToWorld` (`/Game/BP/Editor/BP_WindowsEater.SM_medium_Windonw_type01` _array_element_2)))))
    (:`then_2`
      (bind _outactors_3 (`GameplayStatics.GetAllActorsOfClass` null))
      (for _array_element_3 _outactors_3
        (`InstancedStaticMeshComponent.AddInstanceWorldSpace` (`self.SmallWindows`) (`SceneComponent.K2_GetComponentToWorld` (`/Game/BP/Editor/BP_WindowsEater.SM_Small_Windonw_type01` _array_element_3)))))
    (:`then_3`
      (bind _outactors_4 (`GameplayStatics.GetAllActorsOfClass` "/Script/Engine.Actor"))
      (for _array_element_4 _outactors_4
        (for _array_element_5 (`self.K2_GetComponentsByClass` _array_element_4 "/Script/Engine.ChildActorComponent")
          (bind _childactorclass (`ChildActorComponent.ChildActorClass` _array_element_5))
          (if (or (== _childactorclass null) (== _childactorclass null) (== _childactorclass null))
            (`ChildActorComponent.SetChildActorClass` _array_element_5 null)))))))

(event `ClearInstances`
  (`InstancedStaticMeshComponent.ClearInstances` (`self.SmallWindows`))
  (`InstancedStaticMeshComponent.ClearInstances` (`self.MediumWindows`))
  (`InstancedStaticMeshComponent.ClearInstances` (`self.LargeWindows`)))

(fn `UserConstructionScript`)