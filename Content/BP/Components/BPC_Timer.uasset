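; BPC_Timer is an actor component that keeps a running speedrun time.
; Ticking is disabled at BeginPlay, and StartTimer and StopTimer toggle it along with the TimerStarted flag.
; While ticking, it adds each frame's delta seconds to CurrentSpeedrunTimer, which is never reset here, so restarting resumes from the accumulated value.
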(event `self.ReceiveBeginPlay`
  (`self.SetComponentTickEnabled` false))

(event `StartTimer`
  (set `self.TimerStarted` true)
  (`self.SetComponentTickEnabled` true))

(event `StopTimer`
  (`self.SetComponentTickEnabled` false)
  (set `self.TimerStarted` false))

(event `self.ReceiveTick`
  (params (DeltaSeconds :type "Float (single-precision)"))
  (set `self.CurrentSpeedrunTimer` (+ (`self.CurrentSpeedrunTimer`) DeltaSeconds)))