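; Focus ability component that slows global time while the player spends a Focus resource.
; Focus is gained through events, with a cap check for gain from running.
; Pressing eases time dilation down via a custom timeline, then RemoveFocus loops on timeline completion, decrementing Focus until empty.
; Release restores time at a faster play rate; press also caches every world actor, unused in these graphs.
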(event `Add focus run`
  ;[1 1 1] Add focus while running
  (if (<= (`self.Focus`) (`self.Max focus from running`))
    (set `self.Focus` (+ (`self.Focus`) (`self.Focus gain`)))))

(event `Add focus`
  ;[1 1 1] Add focus (tout court)
  (set `self.Focus` (+ (`self.Focus`) (`self.Focus gain`))))

(event `Focus press`
  ;[1 1 1] Focus press
  (if (> (`self.Focus`) 0)
    (set `self.Focus Is in Use?` true)
    ;;[1 1 1] récupérer tout les actors
    (bind _outactors (`GameplayStatics.GetAllActorsOfClass` "/Script/Engine.Actor"))
    (set `self.Actors in world ` _outactors)
    (bind _outputvalue (`CustomTimeline.StartCustomTimeline` 1.0)
      (:`Update`
        (`GameplayStatics.SetGlobalTimeDilation` (`KismetMathLibrary.FClamp` (- (`self.time dilatation`) _outputvalue) 0.03)))
      (:`Finished`
        (`self.remove focus`)))))

(event `Focus release`
  ;[1 1 1] action quand le focus est release
  (if (`self.Focus Is in Use?`)
    (bind _outputvalue (`CustomTimeline.StartCustomTimeline` 4.0)
      (:`Update`
        (`GameplayStatics.SetGlobalTimeDilation` (`KismetMathLibrary.FClamp` (+ (`self.time dilatation`) _outputvalue) 0.03)))
      (:`Finished`
        (set `self.Focus Is in Use?` false)))))

(event `Remove focus`
  ;[1 1 1] réduit la valeur de focus quand il est utiisé
  ;;[1 1 1] vérification que focus n'est pas en utilisation et/ou égal a zéro
  (if (`self.Focus Is in Use?`)
    (if (> (`self.Focus`) 0)
      (`CustomTimeline.StartCustomTimeline` (/ 1.0 (`self.focus decrease rate`))
        (:`Finished`
          ;;[1 1 1] réduis focus
          (`/Engine/EditorBlueprintResources/StandardMacros.DecrementInt` (`self.Focus`)
            (:`  `
              ;;[1 1 1] fait bouclé la fonction
              (`self.remove focus`)))))
      (else
        ;;[1 1 1] arrète focus si a zéro
        (`self.Focus release`)))))