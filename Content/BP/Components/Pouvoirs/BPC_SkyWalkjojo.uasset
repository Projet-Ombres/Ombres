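; Player power component for a timed SkyWalk ability with a cooldown, laying a path under the player along the camera's aim.
; While active, Tick spawns a pitch-clamped platform every 100 units moved and immediately calls its Destroy.
; It also scatters spaced chunks at tagged points projected onto the camera's plane, passing them the cached "Scrap" actors.
; Scrap is re-cached as the duration ends, then chunks are destroyed after a delay.
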(event `Initialize`
  (params (`Player Ref` :type "/Game/BP/BP_PlayerChara Object Reference"))
  ;[1 1 1] Initialize
  (bind _output_get (set `self.Player Ref` `Player Ref`))
  (set `self.Player ref` _output_get)
  (set `self.Position ref` (`Character.Mesh` _output_get))
  (set `self.Camera ref` (`/Game/BP/BP_PlayerChara.Camera` _output_get))
  (set `self.Position SkyWalk Ref` (`Actor.GetComponentsByTag` _output_get "/Script/Engine.SceneComponent" "PositionSkyWalk")))

(event `SkyWalk`
  (params (DeltaSeconds :type "Float (double-precision)"))
  ;[1 1 1] SkyWalk
  (if (`self.CooldownReay`)
    (set `self.CoolDownValue` 0.0)
    (set `self.CooldownReay` false)
    (set `self.Sky Walk Is Active?` true)
    (set `self.Last position` (`SceneComponent.K2_GetComponentLocation` (`Character.Mesh` (`self.Player Ref`))))
    (`KismetSystemLibrary.Delay` (`self.Sky Walk Duration`))
    (bind _outactors (`GameplayStatics.GetAllActorsWithTag` "Scrap"))
    (set `self.Scrap in World` _outactors)
    (`self.EndskyWalk`)))

(event `self.ReceiveTick`
  (params (DeltaSeconds :type "Float (single-precision)"))
  (bind _camera_ref (`self.Camera ref`))
  (bind _mesh (`Character.Mesh` (`self.Player Ref`)))
  (bind _camera (`/Game/BP/BP_PlayerChara.Camera` (`self.Player Ref`)))
  (bind (_returnvalue_roll _returnvalue_pitch _returnvalue_yaw) (`KismetMathLibrary.BreakRotator` (`SceneComponent.K2_GetComponentRotation` _camera)))
  (bind (_returnvalue_x _returnvalue_y _returnvalue_z) (`KismetMathLibrary.BreakVector` (+ (`SceneComponent.K2_GetComponentLocation` _mesh) (`SceneComponent.GetForwardVector` _camera))))
  ;[0.9197 0 1] Event Tick
  (`|ExecutionSequence`
    (:`then_0`
      (`self.SetCoolDownTimer` DeltaSeconds)
      (if (`self.Sky Walk Is Active?`)
        (if (> (`KismetMathLibrary.VSize` (- (`self.Last position`) (`SceneComponent.K2_GetComponentLocation` (`Character.Mesh` (`self.Player Ref`))))) 100.0)
          (set `self.Last position` (`SceneComponent.K2_GetComponentLocation` _mesh))
          (bind _returnvalue (`|SpawnActorFromClass` "/Game/BP/Class/BP_SkywalkPlatform.BP_SkywalkPlatform_C" (`KismetMathLibrary.MakeTransform` (`KismetMathLibrary.MakeVector` _returnvalue_x _returnvalue_y (- _returnvalue_z 13.0)) (`KismetMathLibrary.MakeRotator` _returnvalue_roll (`KismetMathLibrary.FClamp` _returnvalue_pitch -40.0 40.0) _returnvalue_yaw)) "Undefined" "OverrideRootScale" null null))
          (set `self.LastPlatformSpawned` _returnvalue)
          (`/Game/BP/Class/BP_SkywalkPlatform.Destroy` _returnvalue))))
    (:`then_1`
      (if (`self.Sky Walk Is Active?`)
        (for _array_element (`self.Position SkyWalk Ref`)
          (bind _outactors (`GameplayStatics.GetAllActorsOfClass` "/Game/BP/Class/BP_SkyWalkChunk.BP_SkyWalkChunk_C"))
          (if (<= (`KismetArrayLibrary.Array_Length` _outactors) 0)
            (bind _returnvalue_2 (+ (`KismetMathLibrary.ProjectPointOnToPlane` (`SceneComponent.K2_GetComponentLocation` _array_element) (`SceneComponent.K2_GetComponentLocation` (`Character.Mesh` (`self.Player ref`))) (`KismetMathLibrary.Cross_VectorVector` (`SceneComponent.GetForwardVector` _camera_ref) (`SceneComponent.GetRightVector` _camera_ref))) (* (`KismetMathLibrary.RandomUnitVector`) (`KismetMathLibrary.RandomFloatInRange` 0.0 5.0))))
            (bind _returnvalue_3 (`|SpawnActorFromClass` "/Game/BP/Class/BP_SkyWalkChunk.BP_SkyWalkChunk_C" (`KismetMathLibrary.MakeTransform` _returnvalue_2) "Undefined" "OverrideRootScale" null null :!label _label))
            (set `self.Number of Near Chunk` 0)
            (`/Game/BP/Class/BP_SkyWalkChunk.Initialize` _returnvalue_3 (`self.Player ref`) (`self.Scrap in World`))
            (`KismetSystemLibrary.Delay` 0.1)
            (else
              (for _array_element_2 _outactors
                (if (<= (`KismetMathLibrary.Abs` (`KismetMathLibrary.VSize` (- (`SceneComponent.K2_GetComponentLocation` (`Actor.RootComponent` _array_element_2)) _returnvalue_2))) (`self.Distance Min Between chunk`))
                  (`/Engine/EditorBlueprintResources/StandardMacros.IncrementInt` (`self.Number of Near Chunk`))))
              (if (>= (`self.Number of Near Chunk`) 1)
                (set `self.Number of Near Chunk` 0)
                (`KismetSystemLibrary.Delay` 0.1)
                (else
                  (goto _label))))))
        (set `self.Number of Near Chunk` 0)
        (`KismetSystemLibrary.Delay` 0.1)
        (else
          (`KismetSystemLibrary.Delay` 0.1)
          (set `self.Number of Near Chunk` 0))))))

(event `EndskyWalk`
  (bind _scrap_already_in_use (`self.Scrap Already in Use`))
  ;[1 1 1] End skywalk
  (set `self.Sky Walk Is Active?` false)
  (set `self.OnCoolDown` true)
  (set `self.CooldownReay` false)
  (`KismetSystemLibrary.Delay` 2.0)
  (bind _outactors (`GameplayStatics.GetAllActorsOfClass` "/Game/BP/Class/BP_SkyWalkChunk.BP_SkyWalkChunk_C"))
  (for _array_element _outactors
    (`Actor.K2_DestroyActor` _array_element))
  (for (_array_element_2 _array_index) _scrap_already_in_use
    (`KismetArrayLibrary.Array_RemoveItem` _scrap_already_in_use _array_element_2))
  (`KismetSystemLibrary.PrintString` (`KismetStringLibrary.Conv_IntToString` _array_index)))

(event `SetCoolDownTimer`
  (params (DeltaTime :type "Float (double-precision)"))
  ;[1 1 1] SetCooldown value
  (if (`self.OnCoolDown`)
    (bind _output_get (set `self.CoolDownValue` (+ (`self.CoolDownValue`) DeltaTime)))
    (if (>= _output_get (`self.MaxCooldownNeeded`))
      (set `self.OnCoolDown` false)
      (set `self.CooldownReay` true)
      (else
        (set `self.OnCoolDown` true)
        (set `self.CooldownReay` false)))))