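; Power component for the crystal bump, a shockwave that expands from the player and spawns crystal effects on its surroundings.
; A custom timeline samples a curve to drive the radius in a material parameter collection.
; Once per wave, random line traces in a cone along the player's forward vector store impact points and distances.
; Each update spawns emitters at points the growing radius has reached, then drops them from the arrays.
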(event `CrystalBump`
  (bind _returnvalue (`GameplayStatics.GetPlayerCharacter` 0))
  (bind _emiter_position (`self.emiter position`))
  (bind _emiter_index (`self.emiter index`))
  (bind _emiter_index_2 (`self.emiter index`))
  (bind _returnvalue_2 (`Actor.K2_GetActorLocation` _returnvalue))
  (bind _returnvalue_3 (`CurveFloat.GetFloatValue` (`self.Choc curve`) (`self.timelineValue`)))
  (bind (_outputvalue _realdeltatime _ref) (`CustomTimeline.StartCustomTimeline` 1.5)
    (:`then`
      (set `self.Choc timeline` _ref))
    (:`Update`
      (set `self.timelineValue` _outputvalue)
      (`KismetMaterialLibrary.SetScalarParameterValue` "/Game/Materials/CristalBump/MCollection__cristal_radius.MCollection__cristal_radius" "Radius" _returnvalue_3)
      (`|ExecutionSequence`
        (:`then_0`
          ;[1 1 1] tirage de la position des particule emiter
          (`/Engine/EditorBlueprintResources/StandardMacros.DoOnce` false :!label _label
            (:`Completed`
              (for _ (range (+ (`self.cristal density`) 1))
                (bind _outhit (`KismetSystemLibrary.LineTraceSingle` :`Start` _returnvalue_2 :`End` (+ _returnvalue_2 (* (`KismetMathLibrary.RandomUnitVectorInConeInDegrees` (`Actor.GetActorForwardVector` _returnvalue) (`self.Angle`)) (+ (`self.Max radius`) 200.0))) :`TraceChannel` "TraceTypeQuery2" :`DrawTime` 3.0))
                (bind (_bblockinghit _binitialoverlap _time _distance _location) (`GameplayStatics.BreakHitResult` _outhit))
                (`KismetArrayLibrary.Array_Add` (`self.emiter position`) _location)
                (`KismetArrayLibrary.Array_Add` (`self.emiter distance`) _distance)))))
        (:`then_1`
          ;[1 1 1] calcul et setting du radius de l'onde de choc
          (set `self.actual radius` (* _returnvalue_3 (`self.Max radius`)))
          ;[1 1 1] création d'emiter  le long de l'onde de choc
          (for _index (range (+ (`KismetArrayLibrary.Array_Length` _emiter_position) 1))
            (set `self.emiter index` _index)
            (if (<= (`|GetArrayItem` (`self.emiter distance`) _emiter_index) (`self.actual radius`))
              (`GameplayStatics.SpawnEmitterAtLocation` "/Game/Assets/SM/Cristal/CristalChoc_FX.CristalChoc_FX" (`|GetArrayItem` _emiter_position _emiter_index))
              (`KismetArrayLibrary.Array_Remove` (`self.emiter distance`) _emiter_index_2)
              (`KismetArrayLibrary.Array_Remove` (`self.emiter position`) _emiter_index_2))))))
    (:`Finished`
      (goto _label :!via `Reset`))))