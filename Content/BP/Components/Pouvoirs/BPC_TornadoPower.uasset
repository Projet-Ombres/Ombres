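; BPC_TornadoPower is a component that provides a tornado power with a cooldown, using a camera passed in through Initialize.
; CreateTornado, when the cooldown is ready, spawns both a BP_Tornado_Player and a BP_Tornado_World 200 units behind the camera along its forward vector, then starts the cooldown.
; Tick accumulates elapsed time during the cooldown and re-enables the power once the maximum is reached.
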(event `Initialize`
  (params (Camera :type "CameraComponent Object Reference"))
  ;[0.973 0 1] Initialize
  (set `self.Camera` Camera))

(event `CreateTornado`
  (bind _camera (`self.Camera`))
  (bind _returnvalue (`KismetMathLibrary.MakeTransform` (+ (`SceneComponent.K2_GetComponentLocation` _camera) (* (`SceneComponent.GetForwardVector` _camera) -200.0))))
  ;[1 1 1] Tornado
  (if (`self.CooldownReady`)
    (`KismetSystemLibrary.PrintString` "Create Tornado")
    (set `self.Cooldown value` 0.0)
    (`|SpawnActorFromClass` "/Game/BP/Class/BP_Tornado_Player.BP_Tornado_Player_C" _returnvalue "Undefined" "OverrideRootScale" null null)
    (`|SpawnActorFromClass` "/Game/BP/Class/BP_Tornado_World.BP_Tornado_World_C" _returnvalue "Undefined" "OverrideRootScale" null null)
    (set `self.CooldownReady` false)
    (set `self.OnCooldown` true)))

(event `self.ReceiveTick`
  (params (DeltaSeconds :type "Float (single-precision)"))
  ;[1 1 1] Event tick
  (if (`self.OnCooldown`)
    (bind _output_get (set `self.Cooldown value` (+ DeltaSeconds (`self.Cooldown value`))))
    (if (>= _output_get (`self.MaxCooldwonNeeded`))
      (set `self.CooldownReady` true)
      (set `self.OnCooldown` false)
      (else
        (set `self.CooldownReady` false)
        (set `self.OnCooldown` true)))))