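; Player power component that lets the player aim at chimneys while holding the smoke input and explode them on release, gated by a cooldown.
; While held, Tick box-traces ahead, keeps tagged chimneys passing line-of-sight and 90-degree cone checks, highlights them and draws the cone with debug lines.
; Release explodes a copied target list (a marked hack) after a timeline, with rumble, camera shake and an animation flag.
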(event `Initialize`
  (params (`Player ref` :type "/Game/BP/BP_PlayerChara Object Reference"))
  ;[1 0 0.8839] Initiaize
  (set `self.Player ref` `Player ref`)
  (set `self.Camera` (`/Game/BP/BP_PlayerChara.Camera` `Player ref`))
  (set `self.CurrentCoolDown` (`self.SmokeCooldown`)))

(event `/Game/BP/BPInterface_Power.SetCoolDownTimer`
  (params (DeltaTime :type "Float (single-precision)"))
  ;[1 0.7061 0.1344] Set cool down timer
  (bind _output_get (set `self.CurrentCoolDown` (+ (`self.CurrentCoolDown`) DeltaTime)))
  (if (>= _output_get (`self.SmokeCooldown`))
    (if (`self.OnCoolDown`)
      (set `self.OnCoolDown` false))
    (else
      (set `self.OnCoolDown` true))))

(event `self.ReceiveTick`
  (params (DeltaSeconds :type "Float (single-precision)"))
  (bind _chimneyrefs (`self.ChimneyRefs`))
  (bind _chimneyrefs_2 (`self.ChimneyRefs`))
  (bind _smokeaimdistance (`self.SmokeAimDistance`))
  (bind _returnvalue (`SceneComponent.K2_GetComponentLocation` (`self.Camera`)))
  (bind (_returnvalue_roll _returnvalue_pitch _returnvalue_yaw) (`KismetMathLibrary.BreakRotator` (`Pawn.GetControlRotation` (`self.Player ref`))))
  (bind (_returnvalue_x _returnvalue_y _returnvalue_z) (`KismetMathLibrary.BreakVector` (`KismetMathLibrary.GetForwardVector` (`Pawn.GetControlRotation` (`self.Player ref`)))))
  ;[1 0 0.9066] Event tick
  (`/Game/BP/BPInterface_Power.SetCoolDownTimer` DeltaSeconds)
  (if (`self.Pressed`)
    (`self.Drawcone`)
    ;[1 1 1] Tracers
    (bind _outhits (`KismetSystemLibrary.BoxTraceMulti` :`Start` _returnvalue :`End` (+ _returnvalue (`KismetMathLibrary.MakeVector` (* _returnvalue_x 250.0) (* _returnvalue_y 250.0) _returnvalue_z)) :`HalfSize` (`KismetMathLibrary.MakeVector` _smokeaimdistance _smokeaimdistance 250.0) :`Orientation` (`KismetMathLibrary.MakeRotator` 0.0 0.0 _returnvalue_yaw) :`TraceChannel` "TraceTypeQuery8" :`DrawTime` 0.1))
    (bind _output_get (set `self.MultiSphereTracerHitsArrays` _outhits))
    (for _array_element _output_get
      (bind _tags (`Actor.Tags` (`.HitActor` (`GameplayStatics.BreakHitResult` _array_element))))
      (if (> (`KismetArrayLibrary.Array_Length` _tags) 0)
        (if (== (`|GetArrayItem` _tags) "Chimney")
          (if (not (`/Game/BP/Class/BP_chimney.IsExploding` (cast `/Game/BP/Class/BP_chimney` (`.HitActor` (`GameplayStatics.BreakHitResult` _array_element)) :!pure true)))
            ;[1 1 1] check if chimney is visible
            (bind _outhit (`KismetSystemLibrary.LineTraceSingle` (`Actor.K2_GetActorLocation` (`self.Player ref`)) (`Actor.K2_GetActorLocation` (`.HitActor` (`GameplayStatics.BreakHitResult` _array_element))) "TraceTypeQuery1"))
            (if (== (`.HitActor` (`GameplayStatics.BreakHitResult` _outhit)) (`.HitActor` (`GameplayStatics.BreakHitResult` _array_element)))
              (bind (_returnvalue_roll_2 _returnvalue_pitch_2 _returnvalue_yaw_2) (`KismetMathLibrary.BreakRotator` (`KismetMathLibrary.Conv_VectorToRotator` (`KismetMathLibrary.InverseTransformLocation` (`Actor.GetTransform` (`self.Player ref`)) (`Actor.K2_GetActorLocation` (`.HitActor` (`GameplayStatics.BreakHitResult` _array_element)))))))
              ;[1 1 1] Check if chimney is in sight
              (if (and (<= _returnvalue_yaw_2 45.0) (>= _returnvalue_yaw_2 -45.0))
                ;[1 1 1] Add chimney to exploding array
                (if (not (`KismetArrayLibrary.Array_Contains` (`self.ChimneyRefs`) (`.HitActor` (`GameplayStatics.BreakHitResult` _array_element))))
                  (`KismetArrayLibrary.Array_Add` (`self.ChimneyRefs`) (`.HitActor` (`GameplayStatics.BreakHitResult` _array_element))))
                (else
                  ;[1 1 1] Remove chimney fromù exploding array
                  (`/Game/BP/Class/BP_chimney.Unlight chimney` (cast `/Game/BP/Class/BP_chimney` (`.HitActor` (`GameplayStatics.BreakHitResult` _array_element)) :!pure true))
                  (if (`KismetArrayLibrary.Array_Contains` _chimneyrefs (`.HitActor` (`GameplayStatics.BreakHitResult` _array_element)))
                    (`KismetArrayLibrary.Array_RemoveItem` _chimneyrefs (`.HitActor` (`GameplayStatics.BreakHitResult` _array_element)))))))))))
    (`self.CleanArray`)
    (for _array_element_2 _chimneyrefs_2
      (`/Game/BP/Class/BP_chimney.hightlight chimney` (cast `/Game/BP/Class/BP_chimney` _array_element_2 :!pure true)))
    ;[1 1 1] [HACK] Je copie "chimney refs" parce qu'à ce moment la il est correct (alors qu'après il ne l'est plus mais jsp pk), pour le reutiliser pour faire peter les chimney apres
    (set `self.PendingExplosionChimneys` _chimneyrefs_2)))

(event `/Game/BP/BPInterface_Power.ResetCoolDown`
  ;[1 0.7443 0] reset cool down
  (set `self.CurrentCoolDown` (`self.SmokeCooldown`)))

(event `CleanArray`
  ;[1 1 1] Clear arrays
  ;;[1 1 1] If player isn't touching any chimney, clear chimney array
  (if (> (`KismetArrayLibrary.Array_Length` (`self.MultiSphereTracerHitsArrays`)) 0)
    (for _array_element (`self.ChimneyRefs`)
      (for _array_element_2 (`self.MultiSphereTracerHitsArrays`)
        (if (== (`.HitActor` (`GameplayStatics.BreakHitResult` _array_element_2)) _array_element)
          (set `self.[temporary]IsContained` true)
          (elif (not (`self.[temporary]IsContained`))
            (set `self.[temporary]IsContained` false))))
      (if (`self.[temporary]IsContained`)
        (set `self.[temporary]IsContained` false)
        (else
          (`/Game/BP/Class/BP_chimney.Unlight chimney` (cast `/Game/BP/Class/BP_chimney` _array_element :!pure true))
          (`KismetArrayLibrary.Array_RemoveItem` (`self.ChimneyRefs`) _array_element)
          (set `self.[temporary]IsContained` false))))
    (else
      (for _array_element_3 (`self.ChimneyRefs`)
        (`/Game/BP/Class/BP_chimney.Unlight chimney` (cast `/Game/BP/Class/BP_chimney` _array_element_3 :!pure true)))
      (`KismetArrayLibrary.Array_Clear` (`self.ChimneyRefs`)))))

(event `Drawcone`
  (bind _returnvalue (`Actor.K2_GetActorLocation` (`self.Player ref`)))
  (bind _returnvalue_2 (`Actor.K2_GetActorLocation` (`self.Player ref`)))
  (bind (_returnvalue_x _returnvalue_y) (`KismetMathLibrary.BreakVector` (`KismetMathLibrary.GetForwardVector` (`Pawn.GetControlRotation` (`self.Player ref`)))))
  (bind (_returnvalue_x_2 _returnvalue_y_2) (`KismetMathLibrary.BreakVector` (`KismetMathLibrary.GetForwardVector` (`Pawn.GetControlRotation` (`self.Player ref`)))))
  (bind _returnvalue_3 (+ _returnvalue (* (`KismetMathLibrary.RotateAngleAxis` (`KismetMathLibrary.MakeVector` _returnvalue_x _returnvalue_y) -45.0 (`KismetMathLibrary.Vector_Up`)) (`self.SmokeAimDistance`))))
  (bind _returnvalue_4 (+ _returnvalue_2 (* (`KismetMathLibrary.RotateAngleAxis` (`KismetMathLibrary.MakeVector` _returnvalue_x_2 _returnvalue_y_2) 45.0 (`KismetMathLibrary.Vector_Up`)) (`self.SmokeAimDistance`))))
  ;[1 1 1] Dréaw cone
  (`KismetSystemLibrary.DrawDebugLine` _returnvalue_2 _returnvalue_4 (struct :`R` 0.5625 :`G` 0.089049 :`B` 0.376627 :`A` 1.0) 0.001 2.0)
  (`KismetSystemLibrary.DrawDebugLine` _returnvalue _returnvalue_3 (struct :`R` 0.5625 :`G` 0.089049 :`B` 0.376627 :`A` 1.0) 0.001 2.0)
  (`KismetSystemLibrary.DrawDebugLine` _returnvalue_4 _returnvalue_3 (struct :`R` 0.5625 :`G` 0.089049 :`B` 0.376627 :`A` 1.0) 0.001 5.0))

(event `Smoke press`
  ;[1 1 1] Press
  (if (`self.Pressed`)
    _
    (elif (not (`self.OnCoolDown`))
      (set `self.Pressed` true))))

(event `Smoke release`
  (params (Abort :type Boolean))
  (bind _returnvalue (`GameplayStatics.GetPlayerController` 0))
  (bind _asanim_bp_player_chara (cast `/Game/BP/AnimBP_PlayerChara` (`SkeletalMeshComponent.GetAnimInstance` (`Character.Mesh` (cast `/Game/BP/BP_PlayerChara` (`GameplayStatics.GetPlayerCharacter` 0) :!pure true))) :!pure true))
  ;[1 1 1] lance l'explosion de la cheminée quand la touche est relancée
  (if (`self.Pressed`)
    (set `self.Pressed` false)
    (if (not Abort)
      (if (> (`KismetArrayLibrary.Array_Length` (`self.PendingExplosionChimneys`)) 0)
        (set `self.OnCoolDown` true)
        (set `self.CurrentCoolDown` 0.0)
        (`/Game/BP/BP_Controller.PlayForceFeedback` (cast `/Game/BP/BP_Controller` _returnvalue :!pure true) true false "/Game/BP/FeedbackAssets/Vibrations/Vibration_SmokeExplosion.Vibration_SmokeExplosion")
        (`PlayerController.ClientStartCameraShake` :`self` _returnvalue :`Shake` "/Game/BP/FeedbackAssets/ScreenShakes/BP_CameraShake_SmokeExplosion.BP_CameraShake_SmokeExplosion_C")
        (set `/Game/BP/AnimBP_PlayerChara.ExtrudeSmokeLaunched` true _asanim_bp_player_chara)
        (`CustomTimeline.StartCustomTimeline` 1000.0
          (:`Finished`
            (set `/Game/BP/AnimBP_PlayerChara.ExtrudeSmokeLaunched` false _asanim_bp_player_chara))))
      (for _array_element (`self.PendingExplosionChimneys`)
        (`/Game/BP/Class/BP_chimney.Explode` (cast `/Game/BP/Class/BP_chimney` _array_element :!pure true) (`self.Player ref`))
        (`KismetArrayLibrary.Array_RemoveItem` (`self.ChimneyRefs`) _array_element)))))

(event `DrawVisualCircle`
  ;[0.3615 1 0.6995] Draw view circle PLUS UILISE MAIS LAISSé LA POUR EVE
)