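; Player power component for the smoke ability: hold to aim at an area, release to explode the chimneys inside it.
; While held, a camera line trace places a surface-aligned circle indicator, and a sphere trace there collects and highlights tagged chimneys.
; Release starts the cooldown and, unless aborted, triggers rumble, camera shake and animation, then explodes a cached copy of the chimney list, kept as a noted workaround.
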(event `Initialize`
  (params (`Player ref` :type "/Game/BP/BP_PlayerChara Object Reference"))
  (bind _returnvalue (/ (`self.MultiSphereTracerRadius`) 50.0))
  ;[1 0 0.8839] Initiaize
  (set `self.Player ref` `Player ref`)
  (set `self.Camera` (`/Game/BP/BP_PlayerChara.Camera` `Player ref`))
  ;[1 1 1] Spawn indicator
  (bind _returnvalue_2 (`|SpawnActorFromClass` "/Game/BP/Class/BP_CircleSmokeIndicator.BP_CircleSmokeIndicator_C" (`KismetMathLibrary.MakeTransform` (0.0 0.0 0.0) (struct) (`KismetMathLibrary.MakeVector` _returnvalue _returnvalue 0.01)) "AlwaysSpawn" "OverrideRootScale" null null))
  (bind _output_get (set `self.CircleIndicator` _returnvalue_2))
  (`Actor.SetActorHiddenInGame` _output_get true)
  (set `self.CurrentCoolDown` (`self.SmokeCooldown`)))

(event `self.SetCoolDownTimer`
  (params (DeltaTime :type "Float (single-precision)"))
  ;[1 0.7061 0.1344] Set cool down timer
  (bind _output_get (set `self.CurrentCoolDown` (+ (`self.CurrentCoolDown`) DeltaTime)))
  (if (>= _output_get (`self.SmokeCooldown`))
    (if (`self.OnCoolDown`)
      (set `self.OnCoolDown` false))
    (else
      (set `self.OnCoolDown` true))))

(event `self.ReceiveTick`
  (params (DeltaSeconds :type "Float (single-precision)"))
  (bind _chimneyrefs (`self.ChimneyRefs`))
  (bind _returnvalue (`SceneComponent.K2_GetComponentLocation` (`self.Camera`)))
  ;[1 0 0.9066] Event tick
  (`self.SetCoolDownTimer` DeltaSeconds)
  ;[1 1 1] Tracers
  (if (`self.Pressed`)
    (bind _outhit (`KismetSystemLibrary.LineTraceSingle` :`Start` _returnvalue :`End` (+ _returnvalue (* (`KismetMathLibrary.GetForwardVector` (`Pawn.GetControlRotation` (`self.Player ref`))) (`self.SmokeAimDistance`))) :`TraceChannel` "TraceTypeQuery9" :`bTraceComplex` true :`DrawDebugType` "ForOneFrame" :`DrawTime` 10.0))
    (bind _output_get (set `self.HitLocation` (`.Location` (`GameplayStatics.BreakHitResult` _outhit))))
    (set `self.HitNormal` (`.Normal` (`GameplayStatics.BreakHitResult` _outhit)))
    (set `self.HitActor` (`.HitActor` (`GameplayStatics.BreakHitResult` _outhit)))
    (`self.DrawVisualCircle`)
    (bind _outhits (`KismetSystemLibrary.SphereTraceMulti` _output_get (+ _output_get (* (`KismetMathLibrary.Vector_Up`) 2.0)) (`self.MultiSphereTracerRadius`) "TraceTypeQuery8" true))
    (bind _output_get_2 (set `self.MultiSphereTracerHitsArrays` _outhits))
    (for _array_element _output_get_2
      (bind _tags (`Actor.Tags` (`.HitActor` (`GameplayStatics.BreakHitResult` _array_element))))
      (if (> (`KismetArrayLibrary.Array_Length` _tags) 0)
        (if (== (`|GetArrayItem` _tags) "Chimney")
          (if (not (`/Game/BP/Class/BP_chimney.IsExploding` (cast `/Game/BP/Class/BP_chimney` (`.HitActor` (`GameplayStatics.BreakHitResult` _array_element)) :!pure true)))
            (if (not (`KismetArrayLibrary.Array_Contains` (`self.ChimneyRefs`) (`.HitActor` (`GameplayStatics.BreakHitResult` _array_element))))
              (`KismetArrayLibrary.Array_Add` (`self.ChimneyRefs`) (`.HitActor` (`GameplayStatics.BreakHitResult` _array_element))))))))
    (`self.CleanArray`)
    (for _array_element_2 _chimneyrefs
      (`/Game/BP/Class/BP_chimney.hightlight chimney` (cast `/Game/BP/Class/BP_chimney` _array_element_2 :!pure true)))
    ;;[1 1 1] [HACK] Je copie "chimney refs" parce qu'à ce moment la il est correct (alors qu'après il ne l'est plus mais jsp pk), pour le reutiliser pour faire peter les chimney apres
    (set `self.PendingExplosionChimneys` _chimneyrefs)))

(event `self.ResetCoolDown`
  ;[1 0.7443 0] reset cool down
  (set `self.CurrentCoolDown` (`self.SmokeCooldown`)))

(event `CleanArray`
  ;[1 1 1] Clear arrays
  ;;[1 1 1] If player isn't touching any chimney, clear chimney array
  (if (> (`KismetArrayLibrary.Array_Length` (`self.MultiSphereTracerHitsArrays`)) 0)
    (for _array_element (`self.ChimneyRefs`)
      (for _array_element_2 (`self.MultiSphereTracerHitsArrays`)
        (if (== (`.HitActor` (`GameplayStatics.BreakHitResult` _array_element_2)) _array_element)
          (set `self.[temporary]IsContained` true)
          (elif (not (`self.[temporary]IsContained`))
            (set `self.[temporary]IsContained` false))))
      (if (`self.[temporary]IsContained`)
        (set `self.[temporary]IsContained` false)
        (else
          (`/Game/BP/Class/BP_chimney.Unlight chimney` (cast `/Game/BP/Class/BP_chimney` _array_element :!pure true))
          (`KismetArrayLibrary.Array_RemoveItem` (`self.ChimneyRefs`) _array_element)
          (set `self.[temporary]IsContained` false))))
    (else
      (for _array_element_3 (`self.ChimneyRefs`)
        (`/Game/BP/Class/BP_chimney.Unlight chimney` (cast `/Game/BP/Class/BP_chimney` _array_element_3 :!pure true)))
      (`KismetArrayLibrary.Array_Clear` (`self.ChimneyRefs`)))))

(event `Smoke press`
  ;[1 1 1] Press
  (if (`self.Pressed`)
    _
    (elif (not (`self.OnCoolDown`))
      (set `self.Pressed` true))))

(event `Smoke release`
  (params (Abort :type Boolean))
  (bind _returnvalue (`GameplayStatics.GetPlayerController` 0))
  (bind _asanim_bp_player_chara (cast `/Game/BP/AnimBP_PlayerChara` (`SkeletalMeshComponent.GetAnimInstance` (`Character.Mesh` (cast `/Game/BP/BP_PlayerChara` (`GameplayStatics.GetPlayerCharacter` 0) :!pure true))) :!pure true))
  (if (`self.Pressed`)
    ;[1 1 1] lance l'explosion de la cheminée quand la touche est relancée
    (set `self.OnCoolDown` true)
    (set `self.CurrentCoolDown` 0.0)
    (set `self.Pressed` false)
    (`Actor.SetActorHiddenInGame` (`self.CircleIndicator`) true)
    (if (not Abort)
      (if (> (`KismetArrayLibrary.Array_Length` (`self.PendingExplosionChimneys`)) 0)
        (`/Game/BP/BP_Controller.PlayForceFeedback` (cast `/Game/BP/BP_Controller` _returnvalue :!pure true) true false "/Game/BP/FeedbackAssets/Vibration_SmokeExplosion.Vibration_SmokeExplosion")
        (`PlayerController.ClientStartCameraShake` :`self` _returnvalue :`Shake` "/Game/BP/FeedbackAssets/BP_CameraShake_SmokeExplosion.BP_CameraShake_SmokeExplosion_C")
        (set `/Game/BP/AnimBP_PlayerChara.ExtrudeSmokeLaunched` true _asanim_bp_player_chara)
        (`CustomTimeline.StartCustomTimeline` 1000.0
          (:`Finished`
            (set `/Game/BP/AnimBP_PlayerChara.ExtrudeSmokeLaunched` false _asanim_bp_player_chara))))
      (for _array_element (`self.PendingExplosionChimneys`)
        (`/Game/BP/Class/BP_chimney.Explode` (cast `/Game/BP/Class/BP_chimney` _array_element :!pure true) (`self.Player ref`))
        (`KismetArrayLibrary.Array_RemoveItem` (`self.ChimneyRefs`) _array_element)))))

(event `DrawVisualCircle`
  (bind _circleindicator (`self.CircleIndicator`))
  (bind _hitnormal (`self.HitNormal`))
  (bind _hitnormal_2 (`self.HitNormal`))
  (bind _returnvalue (`KismetMathLibrary.Cross_VectorVector` (`KismetMathLibrary.ProjectVectorOnToPlane` _hitnormal (0.0 0.0 1.0)) _hitnormal))
  (bind (_returnvalue_roll _returnvalue_pitch _returnvalue_yaw) (`KismetMathLibrary.BreakRotator` (`KismetMathLibrary.MakeRotationFromAxes` (`KismetMathLibrary.Vector_Up`) (`KismetMathLibrary.Cross_VectorVector` (`self.HitNormal`) (`KismetMathLibrary.Vector_Up`)) (`self.HitNormal`))))
  (bind (_returnvalue_roll_2 _returnvalue_pitch_2 _returnvalue_yaw_2) (`KismetMathLibrary.BreakRotator` (`KismetMathLibrary.MakeRotationFromAxes` (`KismetMathLibrary.Cross_VectorVector` _returnvalue (`self.HitNormal`)) _returnvalue (`self.HitNormal`))))
  ;[0.3615 1 0.6995] Draw view circle
  (if (and (`KismetMathLibrary.NotEqualExactly_VectorVector` (`self.HitLocation`)) (`KismetMathLibrary.NotEqualExactly_VectorVector` (`self.HitNormal`)) (!= (`self.HitActor`) null))
    (`Actor.SetActorHiddenInGame` _circleindicator false)
    (`Actor.K2_SetActorLocation` _circleindicator (`self.HitLocation`) false true)
    (`Actor.K2_SetActorRotation` (`self.CircleIndicator`) (select `bool` (== (`self.HitNormal`) (0.0 0.0 1.0)) :`false` (select `bool` (== (`KismetMathLibrary.ProjectVectorOnToPlane` _hitnormal_2 (0.0 0.0 1.0)) _hitnormal_2) :`false` (`KismetMathLibrary.MakeRotator` _returnvalue_roll_2 _returnvalue_pitch_2 _returnvalue_yaw_2) :`true` (`KismetMathLibrary.MakeRotator` _returnvalue_roll _returnvalue_pitch _returnvalue_yaw))) false)))