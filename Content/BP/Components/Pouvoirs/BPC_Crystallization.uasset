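; Crystallization power component that finds and outlines crystallisable objects in front of its owner while the power is held.
; Press and release toggle component Tick, which box-traces each frame and keeps BPI_Cristallizable hits within the cone angle.
; Custom depth stencil on their static meshes provides the highlight, reset each tick but not on release.
; The trace end is forward vector times depth, without the owner's location added.
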(event `self.ReceiveBeginPlay`
  (set `self.ConeHalfAngle` (/ (`self.ConeAngle`) 2.0)))

(event `CrystallizePress`
  (`self.SetComponentTickEnabled` true))

(event `CrystallizeRelease`
  (`self.SetComponentTickEnabled` false))

(event `self.ReceiveTick`
  (params (DeltaSeconds :type "Float (single-precision)"))
  (bind _returnvalue (`self.GetOwner`))
  (bind _returnvalue_2 (`self.GetOwner`))
  ;[1 1 1] Unhighlight objects
  (for _array_element (`self.InRangeCrystallisables`)
    (bind _asactor (cast `Actor` _array_element))
    (for _array_element_2 (`Actor.K2_GetComponentsByClass` _asactor "/Script/Engine.StaticMeshComponent")
      (`PrimitiveComponent.SetRenderCustomDepth` _array_element_2 false)
      (`PrimitiveComponent.SetCustomDepthStencilValue` _array_element_2 0)))
  (`KismetArrayLibrary.Array_Clear` (`self.InRangeCrystallisables`))
  (bind _outhits (`KismetSystemLibrary.BoxTraceMulti` :`Start` (`Actor.K2_GetActorLocation` _returnvalue) :`End` (* (`Actor.GetActorForwardVector` _returnvalue) (`self.ConeDepth`)) :`HalfSize` (5.0 5.0 5.0) :`TraceChannel` "TraceTypeQuery8" :`DrawDebugType` "ForOneFrame"))
  (for _array_element_3 _outhits
    (bind (_bblockinghit _binitialoverlap _time _distance _location _impactpoint _normal _impactnormal _physmat _hitactor) (`GameplayStatics.BreakHitResult` _array_element_3))
    (if (<= (`KismetMathLibrary.DegAcos` (`KismetMathLibrary.Dot_VectorVector` (`Actor.GetActorForwardVector` _returnvalue_2) (`KismetMathLibrary.Normal` (- (`Actor.K2_GetActorLocation` _hitactor) (`Actor.K2_GetActorLocation` _returnvalue_2))))) (`self.ConeHalfAngle`))
      (bind _asbpi_cristallizable (cast `/Game/BP/Class/BPI_Cristallizable` _hitactor))
      (`KismetArrayLibrary.Array_Add` (`self.InRangeCrystallisables`) _asbpi_cristallizable)))
  ;[1 1 1] Highlight objects in range
  (for _array_element_4 (`self.InRangeCrystallisables`)
    (bind _asactor_2 (cast `Actor` _array_element_4))
    (for _array_element_5 (`Actor.K2_GetComponentsByClass` _asactor_2 "/Script/Engine.StaticMeshComponent")
      (`PrimitiveComponent.SetRenderCustomDepth` _array_element_5 true)
      (`PrimitiveComponent.SetCustomDepthStencilValue` _array_element_5 2))))