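; Player power component that sends a scan ping outward from the character, highlighting what it touches.
; A custom timeline drives the scan radius in a material parameter collection and a growing sphere trace, enabling chimney outlines, clairvoyance splines or custom-depth stencil on hits.
; Chained timelines then wait, fade post-process scalars and splines, and deactivate highlights.
; The logic to save and restore base scalar values is disconnected, leaving those events empty.
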(event `Initialize`
  (params (ScanEffectPostPro :type "MaterialInstanceDynamic Object Reference"))
  ;[1 0 0.6127] initialize
  (set `self.ScanEffectPostProcess` ScanEffectPostPro)
  (`self.SetPingBaseScalarParameters`))

(event `Ping`
  (bind _returnvalue (`Actor.K2_GetActorLocation` (`GameplayStatics.GetPlayerCharacter` 0)))
  ;[1 1 1] Ping
  (`|ExecutionSequence`
    (:`then_0`
      (`/Engine/EditorBlueprintResources/StandardMacros.DoOnce` false
        (:`Completed`
          (bind _asbp_player_chara (cast `/Game/BP/BP_PlayerChara` (`GameplayStatics.GetPlayerCharacter` 0)))
          (set `self.ScanEffectPostProcess` (`/Game/BP/BP_PlayerChara.ScanEffectPostProcess` _asbp_player_chara)))))
    (:`then_1`
      (`self.DeactivatePingOutlines`)
      (`self.SetScalarParametersBackToBase`)
      (`self.StopTimelines`)
      (bind (_outputvalue _realdeltatime _ref) (`CustomTimeline.StartCustomTimeline` 1.0)
        (:`then`
          (set `self.PingTimeline` _ref))
        (:`Update`
          (`KismetMaterialLibrary.SetScalarParameterValue` "/Game/Materials/Ping/MCollection_ScanEffect_Radius.MCollection_ScanEffect_Radius" "Radius" (`CurveFloat.GetFloatValue` (`self.PingCurve`) _outputvalue))
          (bind _outhits (`KismetSystemLibrary.SphereTraceMulti` _returnvalue (+ _returnvalue (0.0 0.0 1.0)) (* _outputvalue 3000.0) "TraceTypeQuery11"))
          (bind _output_get (set `self.ObjectTouchedByPing` _outhits))
          (for _array_element _output_get
            (bind _asbp_chimney (cast `/Game/BP/Class/BP_chimney` (`.HitActor` (`GameplayStatics.BreakHitResult` _array_element)))
              (:`then`
                (`/Game/BP/Class/BP_chimney.ActivatePingOutline` _asbp_chimney))
              (:`CastFailed`
                (bind _asbp_clairvoyance_spline (cast `/Game/BP/Class/BP_ClairvoyanceSpline` (`.HitActor` (`GameplayStatics.BreakHitResult` _array_element)))
                  (:`then`
                    (`/Game/BP/Class/BP_ClairvoyanceSpline.Appear` _asbp_clairvoyance_spline))
                  (:`CastFailed`
                    (`PrimitiveComponent.SetRenderCustomDepth` (`.HitComponent` (`GameplayStatics.BreakHitResult` _array_element)) true)
                    (`PrimitiveComponent.SetCustomDepthStencilValue` (`.HitComponent` (`GameplayStatics.BreakHitResult` _array_element)) 1)))))))
        (:`Finished`
          (bind (_outputvalue_2 _realdeltatime_2 _ref_2) (`CustomTimeline.StartCustomTimeline` 1.0)
            (:`then`
              (set `self.WaitingBeforeFadeOutPingTimeline` _ref_2))
            (:`Finished`
              (`self.FadeOutPingOutline`))))))))

(event `StopTimelines`
  (bind _pingtimeline (`self.PingTimeline`))
  (bind _fadeoutpingtimeline (`self.FadeOutPingTimeline`))
  (bind _waitingbeforefadeoutpingtimeline (`self.WaitingBeforeFadeOutPingTimeline`))
  ;[1 1 1] Stop timelines
  (if (!= _pingtimeline null)
    (`CustomTimeline.StopCustomTimeline` _pingtimeline))
  (if (!= _fadeoutpingtimeline null)
    (`CustomTimeline.StopCustomTimeline` _fadeoutpingtimeline))
  (if (!= _waitingbeforefadeoutpingtimeline null)
    (`CustomTimeline.StopCustomTimeline` _waitingbeforefadeoutpingtimeline)))

(event `DeactivatePingOutlines`
  ;[1 1 1] Deactivate ping outlines
  (for _array_element (`self.ObjectTouchedByPing`)
    (bind _asbp_chimney (cast `/Game/BP/Class/BP_chimney` (`.HitActor` (`GameplayStatics.BreakHitResult` _array_element)))
      (:`then`
        (`/Game/BP/Class/BP_chimney.DeactivatePingOutline` _asbp_chimney))
      (:`CastFailed`
        (bind _asbp_clairvoyance_spline (cast `/Game/BP/Class/BP_ClairvoyanceSpline` (`.HitActor` (`GameplayStatics.BreakHitResult` _array_element)))
          (:`then`
            (`/Game/BP/Class/BP_ClairvoyanceSpline.Disappear` _asbp_clairvoyance_spline))
          (:`CastFailed`
            (`PrimitiveComponent.SetRenderCustomDepth` (`.HitComponent` (`GameplayStatics.BreakHitResult` _array_element)) false)))))))

(event `FadeOutPingOutline`
  (bind _scaneffectpostprocess (`self.ScanEffectPostProcess`))
  ;[1 1 1] Fade out ping
  (bind (_outputvalue _realdeltatime _ref) (`CustomTimeline.StartCustomTimeline` 0.2)
    (:`then`
      (set `self.FadeOutPingTimeline` _ref))
    (:`Update`
      (bind _returnvalue (`MaterialInstanceDynamic.K2_GetScalarParameterValue` _scaneffectpostprocess "Pow"))
      (`MaterialInstanceDynamic.SetScalarParameterValue` _scaneffectpostprocess "Pow" (+ _returnvalue (* _outputvalue (`self.PingScalarParameter_PowBaseValue`))))
      (`MaterialInstanceDynamic.SetScalarParameterValue` _scaneffectpostprocess "BaseRef" (* (- 1.0 _outputvalue) (`self.PingScalarParameter_BaseRefBaseValue`)))
      (for _array_element (`self.ObjectTouchedByPing`)
        (bind _asbp_clairvoyance_spline (cast `/Game/BP/Class/BP_ClairvoyanceSpline` (`.HitActor` (`GameplayStatics.BreakHitResult` _array_element))))
        (`/Game/BP/Class/BP_ClairvoyanceSpline.FadeOut` _asbp_clairvoyance_spline _outputvalue)))
    (:`Finished`
      (`self.DeactivatePingOutlines`))))

(event `SetScalarParametersBackToBase`
  ;[1 1 1] Set back paramter values ping
)

(event `SetPingBaseScalarParameters`
  ;[1 1 1] Set base scalar parameters values
)