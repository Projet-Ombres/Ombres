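; Player power component for SkyWalk, which lets the player walk through the air on platforms built along the camera's direction.
; While a cooldown-gated custom timeline runs, travelled distance triggers camera-angled platform spawns and lines of scraps.
; Each scrap is the nearest free one in range, or newly spawned, and animates toward shared targets computed once per update.
; The power also changes walk speed and camera pitch limits, restoring them on end.
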(event `SetCoolDownTimer`
  (params (DeltaTime :type "Float (double-precision)"))
  ;[1 1 1] SetCooldown value
  (bind _output_get (set `self.CurrentCoolDown` (+ (`self.CurrentCoolDown`) DeltaTime)))
  (if (>= _output_get (`self.SkyWalkCoolDown`))
    (set `self.OnCoolDown` false)
    (else
      (set `self.OnCoolDown` true))))

(event `self.ReceiveTick`
  (params (DeltaSeconds :type "Float (single-precision)"))
  ;[1 0 0.9792] Event tick
  (`self.SetCoolDownTimer` DeltaSeconds))

(event `Initialize`
  (params (`Player Ref` :type "/Game/BP/BP_PlayerChara Object Reference"))
  ;[1 1 1] Initialize
  (bind _output_get (set `self.Player Ref` `Player Ref`))
  (set `self.Player ref` _output_get)
  (set `self.CurrentCoolDown` (`self.SkyWalkCoolDown`)))

(event `StartSkyWalk`
  (params (DeltaSeconds :type "Float (double-precision)"))
  (bind _returnvalue (`GameplayStatics.GetPlayerCameraManager` 0))
  ;[1 1 1] Start skywalk timeline
  (set `CharacterMovementComponent.MaxWalkSpeed` 500.0 (`Character.CharacterMovement` (`self.Player Ref`)))
  (set `self.Active` true)
  (set `PlayerCameraManager.ViewPitchMin` -45.0 _returnvalue)
  (set `PlayerCameraManager.ViewPitchMax` 45.0 _returnvalue)
  (if (not (`self.OnCoolDown`))
    (set `self.CurrentCoolDown` 0.0)
    (set `self.OnCoolDown` true)
    (set `self.LastPlatformPosition` (`Actor.K2_GetActorLocation` (`self.Player Ref`)))
    (bind (_outputvalue _realdeltatime _ref) (`CustomTimeline.StartCustomTimeline` (/ 1.0 (`self.Sky Walk Duration`)))
      (:`then`
        (set `self.Timeline` _ref))
      (:`Update`
        (`self.UpdateSkywalk`))
      (:`Finished`
        (`self.SpawnPlatform`)
        (`self.ReleaseScraps`)
        (`self.EndskyWalk`)))))

(event `ReleaseScraps`
  (bind _scrap_already_in_use (`self.Scrap Already in Use`))
  ;[1 1 1] Remove scraps from used array
  (`KismetArrayLibrary.Array_Append` (`self.Scrap in World`) _scrap_already_in_use)
  (`KismetArrayLibrary.Array_Clear` _scrap_already_in_use))

(event `MoveScrap`
  (params (LineIndex :type Integer))
  ;[1 1 1] Move scrap
  (`/Game/BP/Class/BP_Scrap.StartMovingToTarget` (`self.Nearest Scrap`) (`self.NoiseAmplitude`) (`self.Player Ref`) (`self.BringScrapDuration`) (`self.PlaceScrapUnderDuration`) (- LineIndex (/ (`self.ScrapsPerLine`) 2)) (`self.ScrapsLevitationDuration`))
  (`KismetArrayLibrary.Array_Add` (`/Game/BP/Components/Pouvoirs/BPC_SkyWalk.Scrap Already in Use` (`/Game/BP/BP_PlayerChara.BPC_SkyWalk` (`self.Player ref`))) (`self.Nearest Scrap`)))

(event `UpdateSkywalk`
  (bind _player_ref (`self.Player ref`))
  (bind _camera (`/Game/BP/BP_PlayerChara.Camera` (`self.Player ref`)))
  ;[1 1 1] Calculate common values for all scraps (optimisation)
  (set `self.ScrapFinalMiddlePosition` (+ (`Actor.K2_GetActorLocation` _player_ref) (* (`SceneComponent.GetForwardVector` (`/Game/BP/BP_PlayerChara.Camera` _player_ref)) 225.0)))
  (set `self.ScrapMiddlePosition` (+ (`SceneComponent.K2_GetComponentLocation` _camera) (* (`SceneComponent.GetForwardVector` _camera) (`self.DistanceFromCamera`))))
  (set `self.ScrapRightOffset` (* (`SceneComponent.GetRightVector` _camera) (`self.SpaceBetweenScraps`)))
  ;[1 1 1] Spawn platform if distance from last platform is enough
  (if (> (`KismetMathLibrary.VSize` (- (`self.LastPlatformPosition`) (`Actor.K2_GetActorLocation` (`self.Player Ref`)))) (`self.DistanceToGrabNewScraps`))
    (`self.SpawnPlatform`)
    (`self.SpawnScrapsLine`)))

(event `SpawnScrapsLine`
  ;[1 1 1] Make a line of scraps
  (for _index (range (+ (`self.ScrapsPerLine`) 1))
    (`self.MoveClosestScrap` _index)))

(event `SpawnPlatform`
  (bind _camera (`/Game/BP/BP_PlayerChara.Camera` (`self.Player Ref`)))
  (bind (_returnvalue_roll _returnvalue_pitch _returnvalue_yaw) (`KismetMathLibrary.BreakRotator` (`SceneComponent.K2_GetComponentRotation` _camera)))
  (bind (_returnvalue_x _returnvalue_y _returnvalue_z) (`KismetMathLibrary.BreakVector` (+ (`Actor.K2_GetActorLocation` (`self.Player Ref`)) (`SceneComponent.GetForwardVector` _camera))))
  ;[1 1 1] Spawn platform under the player
  (set `self.LastPlatformPosition` (`Actor.K2_GetActorLocation` (`self.Player Ref`)))
  (bind _returnvalue (`|SpawnActorFromClass` "/Game/BP/Class/BP_SkywalkPlatform.BP_SkywalkPlatform_C" (`KismetMathLibrary.MakeTransform` (`KismetMathLibrary.MakeVector` _returnvalue_x _returnvalue_y (- _returnvalue_z 100.0)) (`KismetMathLibrary.MakeRotator` _returnvalue_roll (`KismetMathLibrary.FClamp` _returnvalue_pitch -40.0 40.0) _returnvalue_yaw)) "Undefined" "OverrideRootScale" null null))
  (set `/Game/BP/Class/BP_SkywalkPlatform.Fade time` (+ (`self.ScrapsLevitationDuration`) (`self.BringScrapDuration`) (`self.PlaceScrapUnderDuration`)) _returnvalue)
  (set `self.LastPlatformSpawned` _returnvalue))

(event `MoveClosestScrap`
  (params (LineIndex :type Integer))
  (bind _nearest_scrap (`self.Nearest Scrap`))
  (bind _cube (`/Game/BP/Class/BP_Scrap.Cube` _nearest_scrap))
  (bind _camera (`/Game/BP/BP_PlayerChara.Camera` (`self.Player ref`)))
  (bind (_returnvalue_x _returnvalue_y) (`KismetMathLibrary.BreakVector` (+ (`SceneComponent.K2_GetComponentLocation` _camera) (* (`SceneComponent.GetRightVector` _camera) (* (`self.SpawnDistance`) (- (* (`KismetMathLibrary.Conv_IntToDouble` (`KismetMathLibrary.RandomIntegerInRange` 0 1)) 2.0) 1.0))))))
  ;[1 1 1] Get nearest scrap
  (bind _closest (`self.GetClosestScrap`))
  (bind _output_get (set `self.Nearest Scrap` _closest))
  ;[1 1 1] Is scrap available ?
  (`/Engine/EditorBlueprintResources/StandardMacros.IsValid` _output_get
    (:`Is Valid`
      ;[1 1 1] Disable physics
      (`PrimitiveComponent.SetSimulatePhysics` _cube false)
      (`SceneComponent.K2_AttachToComponent` _cube (`Actor.RootComponent` _nearest_scrap) "None" "SnapToTarget" "KeepWorld" "KeepWorld" true) ; Parce que c'est génial UE, quand on simulate physics ça détache le component, du coup il faut le rattacher-> un plaisir vraiment
      (`PrimitiveComponent.SetEnableGravity` _cube false)
      (`PrimitiveComponent.SetCollisionEnabled` _cube "PhysicsOnly")
      (`KismetArrayLibrary.Array_RemoveItem` (`self.Scrap in World`) (`self.Nearest Scrap`))
      (`self.MoveScrap` LineIndex))
    (:`Is Not Valid`
      ;[1 1 1] Spawn new scrap
      (bind _returnvalue (`|SpawnActorFromClass` "/Game/BP/Class/BP_Scrap.BP_Scrap_C" (`KismetMathLibrary.MakeTransform` (`KismetMathLibrary.MakeVector` _returnvalue_x _returnvalue_y -150.0)) "AlwaysSpawn" "OverrideRootScale" null null))
      (set `self.Nearest Scrap` _returnvalue)
      (`self.MoveScrap` LineIndex))))

(event `EndSkyWalk`
  (bind _scrap_already_in_use (`self.Scrap Already in Use`))
  ;[1 1 1] End skywalk
  (set `CharacterMovementComponent.MaxWalkSpeed` 900.0 (`Character.CharacterMovement` (`self.Player Ref`)))
  (set `PlayerCameraManager.ViewPitchMin` -90.0 (`GameplayStatics.GetPlayerCameraManager` 0))
  (set `PlayerCameraManager.ViewPitchMax` 90.0 (`GameplayStatics.GetPlayerCameraManager` 0))
  (set `self.Active` false)
  (set `self.OnCoolDown` true)
  (`CustomTimeline.StopCustomTimeline` (`self.Timeline`))
  (`KismetSystemLibrary.Delay` 2.0)
  (for _array_element _scrap_already_in_use
    (`KismetArrayLibrary.Array_RemoveItem` _scrap_already_in_use _array_element)))

(fn `GetClosestScrap`
  (returns (closest :type "/Game/BP/Class/BP_Scrap Object Reference"))
  (locals (Nearest :type "/Game/BP/Class/BP_Scrap Object Reference") (`Closet Distance Scrap` :type "Float (double-precision)" :default 9999999.0))
  (set `local.Closet Distance Scrap` 999999.0)
  (for _array_element (`self.Scrap in World`)
    (if (not (`KismetArrayLibrary.Array_Contains` (`/Game/BP/Components/Pouvoirs/BPC_SkyWalk.Scrap Already in Use` (`/Game/BP/BP_PlayerChara.BPC_SkyWalk` (`self.Player ref`))) _array_element))
      (bind _returnvalue (`Actor.GetDistanceTo` (`self.Player ref`) _array_element))
      (if (and (< _returnvalue (`local.Closet Distance Scrap`)) (< _returnvalue (`self.MaxRangeToGrabScrap`)))
        (set `local.Nearest` _array_element)
        (set `local.Closet Distance Scrap` _returnvalue))))
  (return (`local.Nearest`)))