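; Player power component that stops time, JoJo "Za Warudo" style, with a sound at the player's location.
; TokiWoTomare ramps global time dilation toward zero while raising the player's post-process effect, then holds the freeze before snapping both back.
; Custom timelines supply real delta time to drive both phases despite the dilation.
; During the freeze, a downward trace records ground contact and position; a flag blocks retriggering.
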(event `self.ReceiveBeginPlay`
  ;[1 0 0.8709] Init player chara
  (set `self.PlayerChara` (cast `/Game/BP/BP_PlayerChara` (`GameplayStatics.GetPlayerCharacter` 0) :!pure true)))

(event `TokiWoTomare`
  ;[1 1 1] Stop time
  (if (not (`self.bStoppingTime`))
    (set `self.bStoppingTime` true)
    (`GameplayStatics.PlaySoundAtLocation` "/Game/TemporaryAsset/Sound/Za_Warudo_Sound_Effect.Za_Warudo_Sound_Effect" (`Actor.K2_GetActorLocation` (`self.PlayerChara`)) (struct) 1.0 1.0 0.0 null null null)
    ;[1 1 1] Transition
    (bind (_outputvalue _realdeltatime) (`CustomTimeline.StartCustomTimeline` (/ 1.0 (`self.TransitionDuration`)))
      (:`Update`
        (set `self.RealDeltaTime` _realdeltatime)
        (`self.SetTimeDilation` (- 1.0 _outputvalue))
        (`/Game/BP/BP_PlayerChara.UpdateZaWarudoPostProcess` (`self.PlayerChara`) (* _outputvalue 1.5)))
      (:`Finished`
        ;[1 1 1] Time stopped
        (`self.SetTimeDilation` 0.0)
        (bind (_outputvalue_2 _realdeltatime_2) (`CustomTimeline.StartCustomTimeline` (/ 1.0 (`self.TimeFreezeDuration`)))
          (:`Update`
            (set `self.RealDeltaTime` _realdeltatime_2)
            ;[1 1 1] Check if grounded
            (bind (_grounded _position) (`self.GetGroundPosition`))
            (set `self.GroundPosition` _position)
            (set `self.bGrounded` _grounded))
          (:`Finished`
            (`self.SetTimeDilation` 1.0)
            (set `self.bStoppingTime` false)
            (`/Game/BP/BP_PlayerChara.UpdateZaWarudoPostProcess` (`self.PlayerChara`) 0.0)))))))

(fn `GetGroundPosition`
  (returns (Grounded :type Boolean) (Position :type "Vector Structure"))
  (bind _returnvalue (`Actor.K2_GetActorLocation` (`self.PlayerChara`)))
  (bind _outhit (`KismetSystemLibrary.LineTraceSingle` _returnvalue (+ _returnvalue (* (`KismetMathLibrary.Vector_Down`) 100.0)) "TraceTypeQuery1"))
  (bind (_bblockinghit _binitialoverlap _time _distance _location _impactpoint) (`GameplayStatics.BreakHitResult` _outhit))
  (return _bblockinghit _impactpoint))

(fn `SetTimeDilation`
  (params (Value :type "Float (double-precision)"))
  (`GameplayStatics.SetGlobalTimeDilation` Value)
  (return))