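; Player power component that extrudes a ramp or pull bar from surfaces tagged ExtrudeChunk, gated by a cooldown.
; While held, Tick sphere-traces from the camera, previewing a pull bar on steep surfaces or a ramp on flatter ones, red when invalid.
; Valid previews snap to the hit component, with ramps aligned to the actor axis nearest the view.
; Release enables query collision, destroys earlier extrusions and restarts cooldown, or discards invalid previews.
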(event `Initialize`
  (params (`Player ref` :type "/Game/BP/BP_PlayerChara Object Reference"))
  ;[1 0 0.8873] initialization
  (set `self.Player ref` `Player ref`)
  (set `self.Camera` (`/Game/BP/BP_PlayerChara.Camera` `Player ref`))
  (set `self.CurrentCoolDown` (`self.ExtrudeCooldown`)))

(event `Rampe press`
  ;[1 1 1] Rampe press
  (if (not (`self.OnCoolDown`))
    (set `self.ExtrudePressed` true)
    (`KismetSystemLibrary.PrintString` "Hello")))

(event `self.SetCoolDownTimer`
  (params (DeltaTime :type "Float (single-precision)"))
  ;[1 0.7379 0] SetCooldown value
  (bind _output_get (set `self.CurrentCoolDown` (+ (`self.CurrentCoolDown`) DeltaTime)))
  (if (>= _output_get (`self.ExtrudeCooldown`))
    (set `self.OnCoolDown` false)
    (else
      (set `self.OnCoolDown` true))))

(event `Rampe release`
  (bind _pendingrampe (`self.PendingRampe`))
  (bind _pendingpullbar (`self.PendingPullBar`))
  (bind _asbp_pull_bar (cast `/Game/BP/Class/BP_PullBar` _pendingpullbar :!pure true))
  ;[1 1 1] Rampe release
  (if (`self.ExtrudePressed`)
    (set `self.ExtrudePressed` false)
    (if (`self.isHittingCorrectObject`)
      (`self.CleanAllOtherObjectsSpawned`)
      (if (!= _pendingrampe null)
        (`PrimitiveComponent.SetCollisionEnabled` (`/Game/BP/Class/BP_Rampe.Cube` (cast `/Game/BP/Class/BP_Rampe` _pendingrampe :!pure true)) "QueryOnly"))
      (if (!= _pendingpullbar null)
        (`PrimitiveComponent.SetCollisionEnabled` (`/Game/BP/Class/BP_PullBar.Box1` _asbp_pull_bar) "QueryOnly")
        (`PrimitiveComponent.SetCollisionEnabled` (`/Game/BP/Class/BP_PullBar.Cylinder` _asbp_pull_bar) "QueryOnly"))
      (set `self.CurrentCoolDown` 0.0)
      (set `self.OnCoolDown` true)
      (else
        (`self.DestroyPendingObjects`)))
    (set `self.PendingRampe` null)
    (set `self.PendingPullBar` null)))

(event `self.ResetCoolDown`
  ;[1 0.7379 0] Reset cooldown
  (set `self.CurrentCoolDown` (`self.ExtrudeCooldown`)))

(event `self.ReceiveTick`
  (params (DeltaSeconds :type "Float (single-precision)"))
  (bind _hit_object_ref (`self.hit object ref`))
  (bind _camera (`self.Camera`))
  (bind _returnvalue (`SceneComponent.K2_GetComponentLocation` _camera))
  (bind _returnvalue_2 (`Actor.GetActorForwardVector` _hit_object_ref))
  (bind _returnvalue_3 (`Actor.GetActorRightVector` _hit_object_ref))
  (bind _returnvalue_4 (`KismetMathLibrary.GetForwardVector` (`SceneComponent.K2_GetComponentRotation` (`self.Camera`))))
  (bind _returnvalue_5 (* _returnvalue_3 -1.0))
  (bind _returnvalue_6 (* _returnvalue_2 -1.0))
  ;[1 0 0.8177] Event tick
  (`self.SetCoolDownTimer` DeltaSeconds)
  (if (`self.ExtrudePressed`)
    ;[1 1 1] ray cast depuis la camera
    (bind (_outhit _returnvalue_7) (`KismetSystemLibrary.SphereTraceSingle` :`Start` _returnvalue :`End` (+ _returnvalue (* (`KismetMathLibrary.GetForwardVector` (`SceneComponent.K2_GetComponentRotation` _camera)) 2000.0)) :`Radius` 5.0 :`TraceChannel` "TraceTypeQuery7" :`DrawDebugType` "ForOneFrame"))
    (if _returnvalue_7
      (bind (_bblockinghit _binitialoverlap _time _distance _location _impactpoint _normal _impactnormal _physmat _hitactor _hitcomponent) (`GameplayStatics.BreakHitResult` _outhit))
      (set `self.hit object location` _location)
      (set `self.hit normal` _normal)
      (set `self.hit object ref` _hitactor)
      (set `self.HitComponentLocation` (`SceneComponent.K2_GetComponentLocation` _hitcomponent))
      (set `self.Rotation Repositioning` (select `int` (`KismetMathLibrary.MaxOfFloatArray` (`|MakeArray` (`KismetMathLibrary.Dot_VectorVector` _returnvalue_2 _returnvalue_4) (`KismetMathLibrary.Dot_VectorVector` _returnvalue_6 _returnvalue_4) (`KismetMathLibrary.Dot_VectorVector` _returnvalue_3 _returnvalue_4) (`KismetMathLibrary.Dot_VectorVector` _returnvalue_5 _returnvalue_4))) :`0` (`KismetMathLibrary.Conv_VectorToRotator` _returnvalue_2) :`1` (`KismetMathLibrary.Conv_VectorToRotator` _returnvalue_6) :`2` (`KismetMathLibrary.Conv_VectorToRotator` _returnvalue_3) :`3` (`KismetMathLibrary.Conv_VectorToRotator` _returnvalue_5)))
      (if (== (`|GetArrayItem` (`Actor.Tags` (`self.hit object ref`))) "ExtrudeChunk")
        ;[1 1 1] Spawn correct texture
        (set `self.isHittingCorrectObject` true)
        (set `self.Extrude is vetical?` (<= (`KismetMathLibrary.Abs` (.z (`self.hit normal`))) 0.45))
        (if (`self.Extrude is vetical?`)
          (if (not (== (`self.PendingRampe`) null))
            (`self.DestroyPendingObjects`))
          (`self.SpawnRightTexture` true)
          (else
            (if (not (== (`self.PendingPullBar`) null))
              (`self.DestroyPendingObjects`))
            (`self.SpawnRightTexture` false)))
        (else
          ;[1 1 1] Spawn red texture
          (set `self.isHittingCorrectObject` false)
          (set `self.Extrude is vetical?` (<= (`KismetMathLibrary.Abs` (.z (`self.hit normal`))) 0.45))
          (if (`self.Extrude is vetical?`)
            (if (not (== (`self.PendingRampe`) null))
              (`self.DestroyPendingObjects`))
            (`self.SpawnTextureRouge` true)
            (else
              (if (not (== (`self.PendingPullBar`) null))
                (`self.DestroyPendingObjects`))
              (`self.SpawnTextureRouge` false)))))
      (else
        (`self.DestroyPendingObjects`)))))

(event `CleanAllOtherObjectsSpawned`
  ;[1 0.2552 0.3694] détruit tout les autres rampe/poutre déja spawn quand une nouvelle rampe/poutre spawn
  (bind _outactors (`GameplayStatics.GetAllActorsWithTag` "ExtrudeSpawn"))
  (for _array_element _outactors
    (if (and (!= _array_element (`self.PendingRampe`)) (!= _array_element (`self.PendingPullBar`)))
      (`Actor.K2_DestroyActor` _array_element))))

(event `DestroyPendingObjects`
  (bind _pendingrampe (`self.PendingRampe`))
  (bind _pendingpullbar (`self.PendingPullBar`))
  ;[1 0.2604 0.2908] Destroy pending objects
  (if (!= _pendingrampe null)
    (`Actor.K2_DestroyActor` _pendingrampe))
  (if (!= _pendingpullbar null)
    (`Actor.K2_DestroyActor` _pendingpullbar))
  (set `self.PendingRampe` null)
  (set `self.PendingPullBar` null))

(event `SpawnTextureRouge`
  (params (SpawnPullBar :type Boolean))
  (bind (_rotation_repositioning_roll _rotation_repositioning_pitch) (`KismetMathLibrary.BreakRotator` (`self.Rotation Repositioning`)))
  (bind (_returnvalue_roll _returnvalue_pitch _returnvalue_yaw) (`KismetMathLibrary.BreakRotator` (`Pawn.GetControlRotation` (`self.Player ref`))))
  ;[1 1 1] Spawn object when NOT HITTING extrude surface
  (if SpawnPullBar
    (if (== (`self.PendingRampe`) null)
      (if (== (`self.PendingPullBar`) null)
        (bind _returnvalue (`|SpawnActorFromClass` "/Game/BP/Class/BP_PullBar.BP_PullBar_C" (`KismetMathLibrary.MakeTransform` (`self.hit object location`) (`self.ProjectVectorOnPlaneAndAddPitch`) (0.5 0.5 7.0)) "AlwaysSpawn" "OverrideRootScale" null null))
        (set `Actor.Tags` (`self.TagArray`) _returnvalue)
        (`PrimitiveComponent.SetMaterial` (`/Game/BP/Class/BP_PullBar.Cylinder` _returnvalue) 0 "/Game/Materials/M_ExtrudeRED.M_ExtrudeRED")
        (set `self.PendingPullBar` _returnvalue)
        (else
          (`self.MovePullBar` false))))
    (elif (== (`self.PendingPullBar`) null)
      (if (== (`self.PendingRampe`) null)
        (bind _returnvalue_2 (`|SpawnActorFromClass` "/Game/BP/Class/BP_Rampe.BP_Rampe_C" (`KismetMathLibrary.MakeTransform` (`self.hit object location`) (`KismetMathLibrary.MakeRotator` _rotation_repositioning_roll _rotation_repositioning_pitch (- _returnvalue_yaw 90.0))) "AlwaysSpawn" "OverrideRootScale" null null))
        (set `Actor.Tags` (`self.TagArray`) _returnvalue_2)
        (`PrimitiveComponent.SetMaterial` (`/Game/BP/Class/BP_Rampe.Cube` _returnvalue_2) 0 "/Game/Materials/M_ExtrudeRED.M_ExtrudeRED")
        (set `self.PendingRampe` _returnvalue_2)
        (else
          (`self.MoveRampe` false))))))

(event `SpawnRightTexture`
  (params (SpawnPullBar :type Boolean))
  ;[1 1 1] Spawn object when HITTING extrude surface
  (if SpawnPullBar
    (if (== (`self.PendingRampe`) null)
      (if (== (`self.PendingPullBar`) null)
        (bind _returnvalue (`|SpawnActorFromClass` "/Game/BP/Class/BP_PullBar.BP_PullBar_C" (`KismetMathLibrary.MakeTransform` (`self.HitComponentLocation`) (`self.ProjectVectorOnPlaneAndAddPitch`) (0.5 0.5 7.0)) "Undefined" "OverrideRootScale" null null))
        (set `Actor.Tags` (`self.TagArray`) _returnvalue)
        (`PrimitiveComponent.SetMaterial` (`/Game/BP/Class/BP_PullBar.Cylinder` _returnvalue) 0 "/Game/Materials/Houdini/Material__26.Material__26")
        (set `self.PendingPullBar` _returnvalue)
        (else
          (`self.MovePullBar` true))))
    (elif (== (`self.PendingPullBar`) null)
      (if (== (`self.PendingRampe`) null)
        (bind _returnvalue_2 (`|SpawnActorFromClass` "/Game/BP/Class/BP_Rampe.BP_Rampe_C" (`KismetMathLibrary.MakeTransform` (`self.HitComponentLocation`) (`self.Rotation Repositioning`)) "Undefined" "OverrideRootScale" null null))
        (set `Actor.Tags` (`self.TagArray`) _returnvalue_2)
        (`PrimitiveComponent.SetMaterial` (`/Game/BP/Class/BP_Rampe.Cube` _returnvalue_2) 0 "/Game/Materials/Houdini/Material__26.Material__26")
        (set `self.PendingRampe` _returnvalue_2)
        (else
          (`self.MoveRampe` true))))))

(event `MoveRampe`
  (params (Righttexture :type Boolean))
  (bind (_rotation_repositioning_roll _rotation_repositioning_pitch _rotation_repositioning_yaw) (`KismetMathLibrary.BreakRotator` (`self.Rotation Repositioning`)))
  (bind (_returnvalue_roll _returnvalue_pitch _returnvalue_yaw) (`KismetMathLibrary.BreakRotator` (`Pawn.GetControlRotation` (`self.Player ref`))))
  ;[1 1 1] Move rampe
  (`Actor.K2_SetActorLocation` (`self.PendingRampe`) (select `bool` Righttexture :`false` (`self.hit object location`) :`true` (`self.HitComponentLocation`)) false true)
  (`Actor.K2_SetActorRotation` (`self.PendingRampe`) (select `bool` Righttexture :`false` (`KismetMathLibrary.MakeRotator` 0.0 0.0 (- _returnvalue_yaw 90.0)) :`true` (`KismetMathLibrary.MakeRotator` _rotation_repositioning_roll _rotation_repositioning_pitch (- _rotation_repositioning_yaw 90.0))) false)
  (if Righttexture
    (`PrimitiveComponent.SetMaterial` (`/Game/BP/Class/BP_Rampe.Cube` (cast `/Game/BP/Class/BP_Rampe` (`self.PendingRampe`) :!pure true)) 0 "/Game/Materials/Houdini/Material__26.Material__26")
    (else
      (`PrimitiveComponent.SetMaterial` (`/Game/BP/Class/BP_Rampe.Cube` (cast `/Game/BP/Class/BP_Rampe` (`self.PendingRampe`) :!pure true)) 0 "/Game/Materials/M_ExtrudeRED.M_ExtrudeRED"))))

(event `MovePullBar`
  (params (RightTexture :type Boolean))
  ;[1 1 1] MovePullBr
  (`Actor.K2_SetActorLocation` (`self.PendingPullBar`) (select `bool` RightTexture :`false` (`self.hit object location`) :`true` (`self.HitComponentLocation`)) false true)
  (`Actor.K2_SetActorRotation` (`self.PendingPullBar`) (`self.ProjectVectorOnPlaneAndAddPitch`) false)
  (if RightTexture
    (`PrimitiveComponent.SetMaterial` (`/Game/BP/Class/BP_PullBar.Cylinder` (cast `/Game/BP/Class/BP_PullBar` (`self.PendingPullBar`) :!pure true)) 0 "/Game/Materials/Houdini/Material__26.Material__26")
    (else
      (`PrimitiveComponent.SetMaterial` (`/Game/BP/Class/BP_PullBar.Cylinder` (cast `/Game/BP/Class/BP_PullBar` (`self.PendingPullBar`) :!pure true)) 0 "/Game/Materials/M_ExtrudeRED.M_ExtrudeRED"))))