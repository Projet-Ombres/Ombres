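; BPC_Jump is a player component that makes jumping forgiving around ledges.
; Each tick, a sphere trace ahead of and below the character stores the last ground hit as the edge and flags void.
; Early jumps at sufficient speed teleport the character to that edge before jumping.
; Late jumps temporarily raise JumpMaxCount for coyote time, using BPCLandingSpeedBoost's airtime, and tick resets the jump state once grounded.
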(event `self.ReceiveBeginPlay`
  ;[1 0 0.5421] Begin play
  (set `self.BP_PlayerChara` (cast `/Game/BP/BP_PlayerChara` (`GameplayStatics.GetPlayerCharacter` 0) :!pure true)))

(event `Jump`
  (bind (_bcandonormaljump _bcandoassistedjump) (`self.CanPlayerJump`))
  ;[1 1 1] Jump event
  ;[1 1 1] Check if is doing an early jump or just a normal jump
  (if _bcandonormaljump
    (if (and (not (`self.IsJumpingClassic`)) (not (`self.IsJumpingTooLate`)))
      (if (and (`self.VoidDetected`) (>= (`KismetMathLibrary.VSizeXY` (`Actor.GetVelocity` (`self.BP_PlayerChara`))) (`self.MinSpeedForEarlyJump`)))
        ;[1 1 1] Too early jump  ->  sets position at the edge and jump
        (`Actor.K2_SetActorLocation` (`self.BP_PlayerChara`) (`self.EdgePosition`) false false)
        (set `self.IsJumpingClassic` true)
        (`Character.Jump` (`self.BP_PlayerChara`))
        (else
          ;[1 1 1] Normal jump
          (set `self.IsJumpingClassic` true)
          (`Character.Jump` (`self.BP_PlayerChara`)))))
    (else
      ;[1 1 1] Too late jump
      (if _bcandoassistedjump
        (if (and (not (`self.IsJumpingClassic`)) (not (`self.IsJumpingTooLate`)))
          (set `Character.JumpMaxCount` 2 (`self.BP_PlayerChara`))
          (set `self.IsJumpingTooLate` true)
          (`Character.Jump` (`self.BP_PlayerChara`)))))))

(event `self.ReceiveTick`
  (params (DeltaSeconds :type "Float (single-precision)"))
  ;[0.9516 0 1] Event tick
  (`self.VoidTracer`)
  ;[1 1 1] Reset IsJumping
  (if (not (`NavMovementComponent.IsFalling` (`Character.CharacterMovement` (`self.BP_PlayerChara`))))
    (if (`self.IsJumpingTooLate`)
      (if (> (`/Game/BP/Components/BPC_LandingSpeedBoost.TimeJumping` (`/Game/BP/BP_PlayerChara.BPC_LandingSpeedBoost` (`self.BP_PlayerChara`))) (`self.TimeGivenToJumpAfterStartingToFall`))
        (set `self.IsJumpingTooLate` false)
        (set `Character.JumpMaxCount` 1 (`self.BP_PlayerChara`)))
      (elif (`self.IsJumpingClassic`)
        (set `self.IsJumpingClassic` false)
        (set `Character.JumpMaxCount` 1 (`self.BP_PlayerChara`))))))

(fn `VoidTracer`
  (bind _bp_playerchara (`self.BP_PlayerChara`))
  (bind _returnvalue (+ (`Actor.K2_GetActorLocation` _bp_playerchara) (* (`Actor.GetActorForwardVector` _bp_playerchara) 150.0)))
  (bind _outhit (`KismetSystemLibrary.SphereTraceSingle` _returnvalue (- _returnvalue (* (`KismetMathLibrary.Vector_Down`) -100.0)) 25.0 "TraceTypeQuery1"))
  (bind (_bblockinghit _binitialoverlap _time _distance _location) (`GameplayStatics.BreakHitResult` _outhit))
  (if _bblockinghit
    (set `self.EdgePosition` _location)
    (set `self.VoidDetected` false)
    (elif (not (`self.VoidDetected`))
      (set `self.VoidDetected` true))))