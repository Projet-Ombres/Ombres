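; Player component for wall climbing: boosts the airborne character up walls, then grabs and climbs ledges.
; Each tick, a forward sphere trace records the wall and a downward trace finds the ledge top, whose height against the pelvis socket selects boost, grab or direct climb.
; Grabbing snaps the capsule to the wall in Flying mode and drives the AnimBP through interface messages; ClimbLedgeI restores Walking.
; Separate events clamp and release camera yaw.
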(event `self.ReceiveTick`
  (params (DeltaSeconds :type "Float (single-precision)"))
  ;[0.8469 0 1] Event Tick
  (if (`self.WasInitialized`)
    ;[1 1 1] PlayerChara Tracers
    (`self.ForwardTracer`)
    (`self.HeightTracer`)))

(event `Initialize`
  (params (BP_PlayerChara :type "/Game/BP/BP_PlayerChara Object Reference"))
  ;[1 1 1] Initialize
  (set `self.BP_PlayerChara` BP_PlayerChara)
  (set `self.WasInitialized` true))

(event `EscalateWall`
  ;[1 1 1] Escalate Wall
  (if (`self.HaveToEscalateWall`)
    (set `self.IsEscalatingWall` true)
    (`/Game/BP/Components/BPC_WallRun.StopWallRun` (`/Game/BP/BP_PlayerChara.BPC_WallRun` (`self.BP_PlayerChara`)))
    (set `MovementComponent.Velocity` (`KismetMathLibrary.MakeVector` 0.0 0.0 (`self.ClimbImpulse`)) (`Character.CharacterMovement` (`self.BP_PlayerChara`))) ; Change Z to change maximum esclating height
  ))

(event `GrabLedge`
  (bind (_returnvalue_roll _returnvalue_pitch _returnvalue_yaw) (`KismetMathLibrary.BreakRotator` (`KismetMathLibrary.Conv_VectorToRotator` (`self.WallNormalOfWallToGrab`))))
  (bind _returnvalue (`SkeletalMeshComponent.GetAnimInstance` (`Character.Mesh` (`self.BP_PlayerChara`))))
  ;[1 1 1] Grab Ledge
  (set `self.IsEscalatingWall` false)
  (set `/Game/TemporaryAsset/Anim/PlayerChara/AnimBP_PlayerChara.ClimbMontageStartTime` 0.0 (cast `/Game/TemporaryAsset/Anim/PlayerChara/AnimBP_PlayerChara` _returnvalue :!pure true))
  (message `/Game/BP/BPInterface_PlayerChara.CanGrab` _returnvalue true)
  (`CharacterMovementComponent.SetMovementMode` (`Character.CharacterMovement` (`self.BP_PlayerChara`)) "MOVE_Flying" 0)
  (set `self.IsHanging` true)
  (`KismetSystemLibrary.MoveComponentTo` (`Character.CapsuleComponent` (`self.BP_PlayerChara`)) (`self.MoveTo`) (`KismetMathLibrary.MakeRotator` _returnvalue_roll _returnvalue_pitch (- _returnvalue_yaw 120.0)) false false 0.13)
  (`MovementComponent.StopMovementImmediately` (`Character.CharacterMovement` (`self.BP_PlayerChara`)))
  (`self.ClimbLedge`))

(event `ClimbLedge`
  ;[1 1 1] Climb Ledge
  (if (not (`self.IsClimbingLedge`))
    (message `/Game/BP/BPInterface_PlayerChara.ClimbLedgeI` (`SkeletalMeshComponent.GetAnimInstance` (`Character.Mesh` (`self.BP_PlayerChara`))) true)
    (`CharacterMovementComponent.SetMovementMode` (`Character.CharacterMovement` (`self.BP_PlayerChara`)) "MOVE_Flying" 0)
    (set `self.IsClimbingLedge` true)
    (set `self.IsHanging` false)))

(event `/Game/BP/BPInterface_PlayerChara.ClimbLedgeI`
  (params (IsClimbing :type Boolean))
  (bind _bp_playerchara (`self.BP_PlayerChara`))
  ;[1 1 1] Climb ledge interface
  (set `self.IsClimbingLedge` IsClimbing)
  (`CharacterMovementComponent.SetMovementMode` (`Character.CharacterMovement` (`self.BP_PlayerChara`)) "MOVE_Walking" 0)
  (`/Game/BP/BP_PlayerChara.SetEverythingAfterLandingOnGround` _bp_playerchara)
  (`KismetSystemLibrary.Delay` (`/Game/BP/BP_PlayerChara.TimerToWaitBeforeCharaNotLandedAnymore` _bp_playerchara))
  (`/Game/BP/BP_PlayerChara.ResetValueAfterDelayLanding` _bp_playerchara))

(event `ClampCamera`
  (bind _returnvalue (`GameplayStatics.GetPlayerController` 0))
  (bind (_returnvalue_roll _returnvalue_pitch _returnvalue_yaw) (`KismetMathLibrary.BreakRotator` (`KismetMathLibrary.Conv_VectorToRotator` (`self.WallNormalOfWallToGrab`))))
  ;[1 1 1] ClampCamera
  (set `Pawn.bUseControllerRotationYaw` false (`self.BP_PlayerChara`))
  (`Controller.SetControlRotation` _returnvalue (`KismetMathLibrary.MakeRotator` (.roll (`Controller.GetControlRotation` _returnvalue)) (.pitch (`Controller.GetControlRotation` _returnvalue)) (+ (`KismetMathLibrary.ClampAngle` (- (.yaw (`Controller.GetControlRotation` _returnvalue)) _returnvalue_yaw) 80.0 -80.0) _returnvalue_yaw))))

(event `UnclampCamera`
  (bind _returnvalue (`GameplayStatics.GetPlayerCameraManager` 0))
  (set `Pawn.bUseControllerRotationYaw` true (`self.BP_PlayerChara`))
  (set `PlayerCameraManager.ViewYawMin` 0.0 _returnvalue)
  (set `PlayerCameraManager.ViewYawMax` 359.98999 _returnvalue))

(fn `ForwardTracer`
  (bind _returnvalue (`Actor.K2_GetActorLocation` (`self.BP_PlayerChara`)))
  (bind (_returnvalue_x _returnvalue_y _returnvalue_z) (`KismetMathLibrary.BreakVector` (`KismetMathLibrary.GetForwardVector` (`Actor.K2_GetActorRotation` (`self.BP_PlayerChara`)))))
  (bind (_velocity_x _velocity_y _velocity_z) (`KismetMathLibrary.BreakVector` (`MovementComponent.Velocity` (`Character.CharacterMovement` (`self.BP_PlayerChara`)))))
  (bind (_outhit _returnvalue_2) (`KismetSystemLibrary.SphereTraceSingle` :`Start` _returnvalue :`End` (+ (`KismetMathLibrary.MakeVector` (* _returnvalue_x 100.0) (* _returnvalue_y 100.0) _returnvalue_z) _returnvalue) :`Radius` 20.0 :`TraceChannel` "TraceTypeQuery3" :`DrawTime` 0.5))
  (if _returnvalue_2
    (set `self.WallLocationOfWallToGrab` (`.Location` (`GameplayStatics.BreakHitResult` _outhit)))
    (set `self.WallNormalOfWallToGrab` (`.Normal` (`GameplayStatics.BreakHitResult` _outhit)))
    (if (!= _velocity_z 0.0)
      (if (`self.IsClimbingLedge`)
        _
        (elif (`self.IsEscalatingWall`)
          _
          (elif (`NavMovementComponent.IsFalling` (`Character.CharacterMovement` (`self.BP_PlayerChara`)))
            (`self.EscalateWall`)))))))

(fn `HeightTracer`
  (bind (_returnvalue_x _returnvalue_y _returnvalue_z) (`KismetMathLibrary.BreakVector` (`self.MoveTo`)))
  (bind (_heightlocationofwalltograb_x _heightlocationofwalltograb_y _heightlocationofwalltograb_z) (`KismetMathLibrary.BreakVector` (`self.HeightLocationOfWallToGrab`)))
  (bind _bp_playerchara (`self.BP_PlayerChara`))
  (bind (_returnvalue_x_2 _returnvalue_y_2 _returnvalue_z_2) (`KismetMathLibrary.BreakVector` (`Actor.K2_GetActorLocation` _bp_playerchara)))
  (bind (_returnvalue_x_3 _returnvalue_y_3 _returnvalue_z_3) (`KismetMathLibrary.BreakVector` (`Actor.K2_GetActorLocation` (`self.BP_PlayerChara`))))
  (bind (_returnvalue_x_4 _returnvalue_y_4 _returnvalue_z_4) (`KismetMathLibrary.BreakVector` (`SceneComponent.GetSocketLocation` (`Character.Mesh` (`self.BP_PlayerChara`)) "pelvisSocket")))
  (bind _returnvalue (+ (`KismetMathLibrary.MakeVector` _returnvalue_x_3 _returnvalue_y_3 (+ _returnvalue_z_3 500.0)) (* (`KismetMathLibrary.GetForwardVector` (`Actor.K2_GetActorRotation` (`self.BP_PlayerChara`))) 70.0)))
  (bind (_outhit _returnvalue_2) (`KismetSystemLibrary.SphereTraceSingle` _returnvalue (`KismetMathLibrary.MakeVector` (.x _returnvalue) (.y _returnvalue) (- (.z _returnvalue) 500.0)) 20.0 "TraceTypeQuery3"))
  (if _returnvalue_2
    (set `self.TracerHorizontalTriggered` true)
    (set `self.HeightLocationOfWallToGrab` (`.ImpactPoint` (`GameplayStatics.BreakHitResult` _outhit)))
    (if (`KismetMathLibrary.InRange_FloatFloat` (- _returnvalue_z_4 _heightlocationofwalltograb_z) -50.0 100.0)
      (set `self.HaveToEscalateWall` false)
      (if (`self.IsClimbingLedge`)
        _
        (elif (`self.IsEscalatingWall`)
          (`self.GrabLedge`)
          (elif (not (`self.IsHanging`))
            (set `/Game/TemporaryAsset/Anim/PlayerChara/AnimBP_PlayerChara.ClimbMontageStartTime` (`KismetMathLibrary.FClamp` (/ (`KismetMathLibrary.Abs` (- _returnvalue_z _returnvalue_z_2)) 200.0)) (cast `/Game/TemporaryAsset/Anim/PlayerChara/AnimBP_PlayerChara` (`SkeletalMeshComponent.GetAnimInstance` (`Character.Mesh` _bp_playerchara)) :!pure true))
            (`self.ClimbLedge`))))
      (else
        (set `self.HaveToEscalateWall` true)))
    (else
      (set `self.HaveToEscalateWall` false)
      (set `self.TracerHorizontalTriggered` false))))