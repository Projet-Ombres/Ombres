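; Player component that lets the character grab overhead BP_PullBar actors, swing like a pendulum and launch off.
; An upward sphere trace each tick triggers the grab, then a timeline squares the player to the bar if the facing angle allows.
; A spawned physics constraint links the simulated capsule to the bar while timed thrusters drive the swing, shortened on fast entry.
; Release destroys the constraint and launches the character along blended actor and camera forward.
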(event `Initialize`
  (params (PlayerChara :type "/Game/BP/BP_PlayerChara Object Reference"))
  (set `self.PlayerChara` PlayerChara))

(event `self.ReceiveTick`
  (params (DeltaSeconds :type "Float (single-precision)"))
  (`self.TracerSearchForPullBar`))

(event `AttachToPullBar`
  ;[0 0.2451 1] Start grabbing
  (set `self.IsHanging` true)
  (`/Game/BP/Components/Pouvoirs/BPC_Focus.Add focus` (`/Game/BP/BP_PlayerChara.BPC_Focus` (`self.PlayerChara`)))
  (`self.CorrectPlayerRotation`)
  (set `Pawn.bUseControllerRotationYaw` false (`self.PlayerChara`)))

(event `CheckForLookingAngle`
  ;[1 0.7768 0.07926] Check For looking angle
  (if (< (`KismetMathLibrary.DegAcos` (`KismetMathLibrary.Dot_VectorVector` (`KismetMathLibrary.Normal` (`Actor.GetActorRightVector` (`self.HitActor`))) (`KismetMathLibrary.Normal` (`KismetMathLibrary.GetForwardVector` (`Actor.K2_GetActorRotation` (`self.PlayerChara`)))))) 70.0)
    (set `self.(Bool)PlayerFacingPullBarRight` (1.0 0.0 0.0))
    (elif (< (`KismetMathLibrary.DegAcos` (`KismetMathLibrary.Dot_VectorVector` (`KismetMathLibrary.Normal` (* (`Actor.GetActorRightVector` (`self.HitActor`)) -1.0)) (`KismetMathLibrary.Normal` (`KismetMathLibrary.GetForwardVector` (`Actor.K2_GetActorRotation` (`self.PlayerChara`)))))) 70.0)
      (set `self.(Bool)PlayerFacingPullBarRight` (0.0 1.0 0.0))
      (else
        (set `self.(Bool)PlayerFacingPullBarRight` (0.0 0.0 1.0))))))

(event `CorrectPlayerRotation`
  (bind (__bool_playerfacingpullbarright_x __bool_playerfacingpullbarright_y __bool_playerfacingpullbarright_z) (`KismetMathLibrary.BreakVector` (`self.(Bool)PlayerFacingPullBarRight`)))
  (bind __bool_playerfacingpullbarright_x_2 (`KismetMathLibrary.BreakVector` (`self.(Bool)PlayerFacingPullBarRight`)))
  (bind (_playerrotationbeforehang_roll _playerrotationbeforehang_pitch) (`KismetMathLibrary.BreakRotator` (`self.PlayerRotationBeforeHang`)))
  (bind (_playerrotationbeforehang_roll_2 _playerrotationbeforehang_pitch_2) (`KismetMathLibrary.BreakRotator` (`self.PlayerRotationBeforeHang`)))
  (bind _returnvalue (* (`Actor.GetActorRightVector` (`self.HitActor`)) 1.0))
  (bind _returnvalue_2 (* (`Actor.GetActorRightVector` (`self.HitActor`)) -1.0))
  (bind _returnvalue_3 (`KismetMathLibrary.ProjectVectorOnToPlane` _returnvalue (0.0 0.0 1.0)))
  (bind _returnvalue_4 (`KismetMathLibrary.ProjectVectorOnToPlane` _returnvalue_2 (0.0 0.0 1.0)))
  (bind (_returnvalue_roll _returnvalue_pitch _returnvalue_yaw) (`KismetMathLibrary.BreakRotator` (`KismetMathLibrary.MakeRotationFromAxes` _returnvalue_3 (`KismetMathLibrary.Cross_VectorVector` _returnvalue_3 _returnvalue) (0.0 0.0 -1.0))))
  (bind (_returnvalue_roll_2 _returnvalue_pitch_2 _returnvalue_yaw_2) (`KismetMathLibrary.BreakRotator` (`KismetMathLibrary.MakeRotationFromAxes` _returnvalue_4 (`KismetMathLibrary.Cross_VectorVector` _returnvalue_4 _returnvalue_2) (0.0 0.0 -1.0))))
  (bind _returnvalue_5 (select `bool` (== __bool_playerfacingpullbarright_x_2 1.0) :`false` (`KismetMathLibrary.MakeRotator` _playerrotationbeforehang_roll_2 _playerrotationbeforehang_pitch_2 _returnvalue_yaw_2) :`true` (`KismetMathLibrary.MakeRotator` _playerrotationbeforehang_roll _playerrotationbeforehang_pitch _returnvalue_yaw)))
  ;[1 1 1] CorrectPlayerRotation
  (`self.CheckForLookingAngle`)
  (if (== __bool_playerfacingpullbarright_z 0.0)
    (bind _outputvalue (`CustomTimeline.StartCustomTimeline` 5.0)
      (:`Update`
        (`Actor.K2_SetActorRotation` (`self.PlayerChara`) (`KismetMathLibrary.RLerp` (`Controller.GetControlRotation` (`GameplayStatics.GetPlayerController` 0)) _returnvalue_5 _outputvalue true) false))
      (:`Finished`
        (set `self.PlayerRotationBeforeHang` _returnvalue_5)
        (`self.CreateConstraints`)))
    (else
      (set `self.IsHanging` false))))

(event `CreateConstraints`
  (bind `_physicsthrusterarrière` (`/Game/BP/BP_PlayerChara.PhysicsThrusterArrière` (`self.PlayerChara`)))
  (bind _capsulecomponent (`Character.CapsuleComponent` (`self.PlayerChara`)))
  (bind _constraintcomp (`PhysicsConstraintActor.ConstraintComp` (`self.ConstraintActor`)))
  ;[1 1 1] Set constraints actor
  (bind _returnvalue (`|SpawnActorFromClass` "/Script/Engine.PhysicsConstraintActor" (`KismetMathLibrary.MakeTransform` (`self.HitLocation`)) "AlwaysSpawn" "OverrideRootScale" null null))
  (set `self.ConstraintActor` _returnvalue)
  (`PhysicsConstraintComponent.SetConstrainedComponents` (`PhysicsConstraintActor.ConstraintComp` (`self.ConstraintActor`)) (`/Game/BP/Class/BP_PullBar.Cylinder` (`self.HitActor`)) "None" _capsulecomponent "None")
  (`PrimitiveComponent.SetSimulatePhysics` _capsulecomponent true)
  (`PhysicsConstraintComponent.SetLinearYLimit` _constraintcomp "LCM_Limited" 2.0)
  (`PhysicsConstraintComponent.SetAngularSwing1Limit` _constraintcomp "ACM_Limited" 45.0)
  (`PhysicsConstraintComponent.SetAngularSwing2Limit` _constraintcomp "ACM_Limited" 0.0)
  (if (< (`KismetMathLibrary.VSizeXY` (`Actor.GetVelocity` (`self.PlayerChara`))) 200.0)
    (`self.StartThrusters`)
    (else
      (`PrimitiveComponent.SetSimulatePhysics` (`Character.CapsuleComponent` (`self.PlayerChara`)) true)
      (`self.ToggleActive` `_physicsthrusterarrière`)
      (`KismetSystemLibrary.Delay` 0.2)
      (`self.ToggleActive` `_physicsthrusterarrière`)
      (`self.JumpOffPullBar`))))

(event `StartThrusters`
  (bind `_physicsthrusterarrière` (`/Game/BP/BP_PlayerChara.PhysicsThrusterArrière` (`self.PlayerChara`)))
  (bind _physicsthrusteravant (`/Game/BP/BP_PlayerChara.PhysicsThrusterAvant` (`self.PlayerChara`)))
  (bind `_physicsthrusterarrière_2` (`/Game/BP/BP_PlayerChara.PhysicsThrusterArrière` (`self.PlayerChara`)))
  ;[0.2838 1 0.2025] Activate thrusters
  (`PrimitiveComponent.SetSimulatePhysics` (`Character.CapsuleComponent` (`self.PlayerChara`)) true)
  (`self.ToggleActive` `_physicsthrusterarrière_2`)
  (`KismetSystemLibrary.Delay` 1.0)
  (`self.ToggleActive` `_physicsthrusterarrière_2`)
  (`self.ToggleActive` _physicsthrusteravant)
  (`KismetSystemLibrary.Delay` 1.0)
  (`self.ToggleActive` _physicsthrusteravant)
  (`self.ToggleActive` `_physicsthrusterarrière`)
  (`KismetSystemLibrary.Delay` 1.0)
  (`self.ToggleActive` `_physicsthrusterarrière`)
  (`self.JumpOffPullBar`))

(event `JumpOffPullBar`
  (bind _playerchara (`self.PlayerChara`))
  (bind (_returnvalue_roll _returnvalue_pitch _returnvalue_yaw) (`KismetMathLibrary.BreakRotator` (`Controller.GetControlRotation` (`GameplayStatics.GetPlayerController` 0))))
  (bind (_returnvalue_x _returnvalue_y) (`KismetMathLibrary.BreakVector` (+ (`KismetMathLibrary.GetForwardVector` (`Actor.K2_GetActorRotation` (`self.PlayerChara`))) (`KismetMathLibrary.GetForwardVector` (`SceneComponent.K2_GetComponentRotation` (`/Game/BP/BP_PlayerChara.Camera` (`self.PlayerChara`)))))))
  (bind (_returnvalue_x_2 _returnvalue_y_2) (`KismetMathLibrary.BreakVector2D` (* (`KismetMathLibrary.MakeVector2D` _returnvalue_x _returnvalue_y) (`self.LongueurJumpOff`))))
  (bind (_returnvalue_x_3 _returnvalue_y_3) (`KismetMathLibrary.BreakVector` (`KismetMathLibrary.ClampVectorSize` (`KismetMathLibrary.MakeVector` _returnvalue_x_2 _returnvalue_y_2) 800.0 801.0)))
  ;[0.4416 1 0.3083] Jump off pull bar
  (`PrimitiveComponent.SetSimulatePhysics` (`Character.CapsuleComponent` (`self.PlayerChara`)) false)
  (set `self.IsHanging` false)
  (set `self.isJumpingOff` true)
  (`Actor.K2_DestroyActor` (`self.ConstraintActor`))
  ;;[1 1 1] Le launch character se fait dans la direction de la cam
  (`PrimitiveComponent.SetSimulatePhysics` (`Character.CapsuleComponent` _playerchara) false)
  (set `Pawn.bUseControllerRotationYaw` true _playerchara)
  (`Actor.K2_SetActorRotation` _playerchara (`KismetMathLibrary.MakeRotator` 0.0 0.0 _returnvalue_yaw) false)
  (`Character.LaunchCharacter` (`self.PlayerChara`) (`KismetMathLibrary.MakeVector` _returnvalue_x_3 _returnvalue_y_3 (`self.HauteurJumpOff`)) true true)
  (`/Game/BP/BP_Controller.PlayForceFeedback` (cast `/Game/BP/BP_Controller` (`GameplayStatics.GetPlayerController` 0) :!pure true) true false "/Game/BP/FeedbackAssets/Vibration_ShortSmall.Vibration_ShortSmall"))

(fn `ClampCamera`
  (params (Value :type "Float (double-precision)"))
  (returns (AllowedToTurn :type Boolean))
  (bind (_relativerotation_roll _relativerotation_pitch _relativerotation_yaw) (`KismetMathLibrary.BreakRotator` (`SceneComponent.RelativeRotation` (`/Game/BP/BP_PlayerChara.Camera` (`self.PlayerChara`)))))
  (bind _returnvalue (+ Value _relativerotation_yaw))
  (return (or (or (and (> Value 0.0) (< _returnvalue (* (`self.CameraAngleAllowed`) 0.5))) (and (< Value 0.0) (>= _returnvalue (* (`self.CameraAngleAllowed`) -0.5)))) (`self.isJumpingOff`))))

(fn `TracerSearchForPullBar`
  (bind _returnvalue (`Actor.K2_GetActorLocation` (`self.PlayerChara`)))
  (bind (_outhit _returnvalue_2) (`KismetSystemLibrary.SphereTraceSingle` _returnvalue (+ _returnvalue (* (`KismetMathLibrary.Vector_Up`) 150.0)) 20.0 "TraceTypeQuery6"))
  (if _returnvalue_2
    (bind (_bblockinghit _binitialoverlap _time _distance _location _impactpoint _normal _impactnormal _physmat _hitactor) (`GameplayStatics.BreakHitResult` _outhit))
    (set `self.HitActor` (cast `/Game/BP/Class/BP_PullBar` _hitactor :!pure true))
    (set `self.HitLocation` _location)
    (set `self.PullBarNormal` _normal)
    (if (not (`self.IsHanging`))
      (`self.AttachToPullBar`))))