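; Player ability component that briefly swings the camera around to look behind, unless the player state check blocks it.
; A custom timeline lerps control rotation to face backward, holds for a set duration, then lerps back, with look input ignored and spring arm adjusted.
; Meanwhile player max speed and time dilation of enemies in halo range are scaled by TimeDilation, then restored.
; The LookingBehind flag clears one second afterward.
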(event `LookBehind`
  (bind _returnvalue (`GameplayStatics.GetPlayerCharacter` 0))
  (bind _returnvalue_2 (`GameplayStatics.GetPlayerCharacter` 0))
  (bind _asbp_player_chara (cast `/Game/BP/BP_PlayerChara` _returnvalue :!pure true))
  (bind _asbp_player_chara_2 (cast `/Game/BP/BP_PlayerChara` _returnvalue_2 :!pure true))
  (bind _isdoingsomething (`/Game/BP/BP_PlayerChara.CheckPlayerStates` (cast `/Game/BP/BP_PlayerChara` (`GameplayStatics.GetPlayerCharacter` 0) :!pure true) true true true true false true true true true true true true))
  (if (not _isdoingsomething)
    (`self.OnLookBehind`)
    (`self.MoveCamera` true)
    (set `self.StartRotation` (`Controller.GetControlRotation` (`GameplayStatics.GetPlayerController` 0)))
    (set `self.TargetRotation` (`KismetMathLibrary.MakeRotFromX` (`KismetMathLibrary.NegateVector` (`Actor.GetActorForwardVector` (`self.GetOwner`)))))
    (`Controller.SetIgnoreLookInput` (`GameplayStatics.GetPlayerController` 0) true)
    (set `Pawn.bUseControllerRotationYaw` false _returnvalue_2)
    (set `CharacterMovementComponent.MaxWalkSpeed` (* (`/Game/BP/Components/CapacitéPhysique/BPC_Sprint.RunningMaxSpeed` (`/Game/BP/BP_PlayerChara.BPC_Sprint` _asbp_player_chara_2)) (`self.TimeDilation`)) (`Character.CharacterMovement` _asbp_player_chara_2))
    (for _array_element (`/Game/BP/BP_PlayerChara.EnemiesInHaloRange` _asbp_player_chara_2)
      (set `Actor.CustomTimeDilation` (`self.TimeDilation`) _array_element))
    (set `self.LookingBehind` true)
    (bind _outputvalue (`CustomTimeline.StartCustomTimeline` 4.0)
      (:`Update`
        (`Controller.SetControlRotation` (`GameplayStatics.GetPlayerController` 0) (`KismetMathLibrary.RLerp` (`self.StartRotation`) (`self.TargetRotation`) _outputvalue true)))
      (:`Finished`
        (`KismetSystemLibrary.Delay` (`self.Duration`))
        (bind _outputvalue_2 (`CustomTimeline.StartCustomTimeline` 4.0)
          (:`Update`
            (bind (_returnvalue_roll _returnvalue_pitch _returnvalue_yaw) (`KismetMathLibrary.BreakRotator` (`KismetMathLibrary.RLerp` (`self.TargetRotation`) (`self.StartRotation`) _outputvalue_2 true)))
            (`Controller.SetControlRotation` (`GameplayStatics.GetPlayerController` 0) (`KismetMathLibrary.MakeRotator` 0.0 _returnvalue_pitch _returnvalue_yaw)))
          (:`Finished`
            (`Controller.SetIgnoreLookInput` (`GameplayStatics.GetPlayerController` 0) false)
            (`self.MoveCamera` false)
            (set `Pawn.bUseControllerRotationYaw` true _returnvalue)
            (for _array_element_2 (`/Game/BP/BP_PlayerChara.EnemiesInHaloRange` _asbp_player_chara)
              (set `Actor.CustomTimeDilation` 1.0 _array_element_2))
            (set `CharacterMovementComponent.MaxWalkSpeed` (`/Game/BP/Components/CapacitéPhysique/BPC_Sprint.RunningMaxSpeed` (`/Game/BP/BP_PlayerChara.BPC_Sprint` _asbp_player_chara)) (`Character.CharacterMovement` _asbp_player_chara))
            (`KismetSystemLibrary.Delay` 1.0)
            (set `self.LookingBehind` false)))))))

(event `MoveCamera`
  (params (`Backward?` :type Boolean))
  ;[1 1 1] move camera to adjsut
  (set `SpringArmComponent.TargetArmLength` (select `bool` `Backward?` :`true` -30.0 :!type "Float (single-precision)") (`/Game/BP/BP_PlayerChara.SpringArm` (cast `/Game/BP/BP_PlayerChara` (`GameplayStatics.GetPlayerCharacter` 0) :!pure true))))