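; Player character component that performs a "thigh jump" vault over obstacles tagged ThighJump, followed by a landing speed boost.
; Each tick, forward and downward sphere traces cache the wall normal, hit point and ledge height.
; JumpThigh disables gravity and WorldStatic collision, then a speed-scaled timeline moves the character along a curve while rolling the camera.
; On finish it restores physics, amplifies velocity and fades max walk speed back to running speed.
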(event `self.ReceiveBeginPlay`
  (bind _ascharacter (cast `Character` (`self.GetOwner`)))
  (bind _output_get (set `self.OwnerCharacter` _ascharacter))
  (set `self.Controller` (`Pawn.GetController` _output_get))
  (bind _asbp_player_chara (cast `/Game/BP/BP_PlayerChara` _ascharacter))
  (set `self.BP_Chara` _asbp_player_chara)
  (bind _output_get_2 (set `self.WasInitialized` true))
  (`self.SetComponentTickEnabled` _output_get_2))

(event `self.ReceiveTick`
  (params (DeltaSeconds :type "Float (single-precision)"))
  ;[1 0 0.7992] Event tick
  (set `self.DeltaSec` DeltaSeconds)
  (if (`self.WasInitialized`)
    (`self.HorizontalTracer`)
    (`self.VerticalTracer`)))

(event `JumpThigh`
  (bind _ownercharacter (`self.OwnerCharacter`))
  (bind _controller (`self.Controller`))
  (bind (_ledge_height_location_x _ledge_height_location_y _ledge_height_location_z) (`KismetMathLibrary.BreakVector` (`self.Ledge height location`)))
  (bind _ownercharacter_2 (`self.OwnerCharacter`))
  (bind (_returnvalue_roll _returnvalue_pitch _returnvalue_yaw) (`KismetMathLibrary.BreakRotator` (`Controller.GetControlRotation` _controller)))
  (bind _charactermovement (`Character.CharacterMovement` (`self.BP_Chara`)))
  (bind _capsulecomponent (`Character.CapsuleComponent` (`self.OwnerCharacter`)))
  (bind _capsulecomponent_2 (`Character.CapsuleComponent` _ownercharacter_2))
  ;[1 1 1] Jump thigh
  (set `self.GroundHeight` (.z (`Actor.K2_GetActorLocation` _ownercharacter_2)))
  (set `self.CharaVelocityBeforeJump` (`Actor.GetVelocity` _ownercharacter_2))
  (set `self.BoostActive` true)
  (set `self.ThighJumping` true)
  (`PrimitiveComponent.SetCollisionResponseToChannel` _capsulecomponent_2 "ECC_WorldStatic" "ECR_Ignore")
  (`PrimitiveComponent.SetEnableGravity` _capsulecomponent_2 false)
  (bind _lerpvaluedistance (`self.ReturnVectorMultiplier(withLerp)XY`))
  (set `self.StartPosition` (`Actor.K2_GetActorLocation` _ownercharacter))
  (bind _output_get (set `self.ThighJumpPlayRate` (`KismetMathLibrary.FClamp` (* 2.0 (/ (`KismetMathLibrary.VSizeXY` (`Actor.GetVelocity` _ownercharacter)) (`CharacterMovementComponent.MaxWalkSpeed` (`Character.CharacterMovement` _ownercharacter)))) 1.2 2.0)))
  (bind _outputvalue (`CustomTimeline.StartCustomTimeline` _output_get)
    (:`Update`
      (bind _returnvalue (`CurveFloat.GetFloatValue` (`self.ThighJumpCurve`) _outputvalue))
      (bind _returnvalue_2 (* _returnvalue (`self.CurveMaxRoll`)))
      (set `self.CurveValue` _returnvalue_2)
      (bind (_returnvalue_x _returnvalue_y) (`KismetMathLibrary.BreakVector` (+ (* (`self.WallNormal`) (* _lerpvaluedistance _outputvalue -1.0)) (`self.StartPosition`))))
      (`Actor.K2_SetActorLocation` (`self.OwnerCharacter`) (`KismetMathLibrary.MakeVector` _returnvalue_x _returnvalue_y (+ (* (* (- _ledge_height_location_z (`self.GroundHeight`)) 1.25) _returnvalue) (`self.GroundHeight`))) false false)
      (`Controller.SetControlRotation` _controller (`KismetMathLibrary.MakeRotator` _returnvalue_2 _returnvalue_pitch _returnvalue_yaw)))
    (:`Finished`
      (set `self.ThighJumping` false)
      (cast `/Game/BP/BP_PlayerChara` (`self.OwnerCharacter`)
        (:`then`
          (`/Game/BP/BP_PlayerChara.ResetValuesAfterLanding` (`self.BP_Chara`))
          (set `MovementComponent.Velocity` (* (`MovementComponent.Velocity` _charactermovement) 5.0) _charactermovement))
        (:`CastFailed`
          _))
      (`PrimitiveComponent.SetCollisionResponseToChannel` _capsulecomponent "ECC_WorldStatic" "ECR_Block")
      (`PrimitiveComponent.SetEnableGravity` _capsulecomponent true)
      (set `Pawn.bUseControllerRotationYaw` true (`self.OwnerCharacter`))
      (`self.Boost`))))

(event `Boost`
  (bind _bp_chara (`self.BP_Chara`))
  ;[1 1 1] Boost
  (if (`self.WasInitialized`)
    (set `CharacterMovementComponent.MaxWalkSpeed` (`self.LandingBoostMaxWalkSpeed`) (`Character.CharacterMovement` (`self.BP_Chara`)))
    (set `self.BoostActive` true)
    (bind _outputvalue (`CustomTimeline.StartCustomTimeline` 1.0)
      (:`Update`
        (`self.LerpWalkSpeed` (- 1.0 _outputvalue)))
      (:`Finished`
        (set `CharacterMovementComponent.MaxWalkSpeed` (`/Game/BP/Components/CapacitéPhysique/BPC_Sprint.RunningMaxSpeed` (`/Game/BP/BP_PlayerChara.BPC_Sprint` _bp_chara)) (`Character.CharacterMovement` _bp_chara))
        (set `self.BoostActive` false)))))

(event `LerpWalkSpeed`
  (params (Value :type "Float (double-precision)"))
  (bind _landingboostmaxwalkspeed (`self.LandingBoostMaxWalkSpeed`))
  (bind _charactermovement (`Character.CharacterMovement` (`self.OwnerCharacter`)))
  (bind _velocity (`MovementComponent.Velocity` _charactermovement))
  ;[1 1 1] Lerp walk speed
  (set `CharacterMovementComponent.MaxWalkSpeed` (`KismetMathLibrary.Lerp` (`/Game/BP/Components/CapacitéPhysique/BPC_Sprint.RunningMaxSpeed` (`/Game/BP/BP_PlayerChara.BPC_Sprint` (`self.BP_Chara`))) (`self.LandingBoostMaxWalkSpeed`) Value) _charactermovement)
  ;;[1 1 1] Correct velocity
  (if (> (`KismetMathLibrary.VSize` _velocity) _landingboostmaxwalkspeed)
    (set `MovementComponent.Velocity` (* (`KismetMathLibrary.Normal` _velocity) _landingboostmaxwalkspeed) _charactermovement)))

(fn `HorizontalTracer`
  (bind _returnvalue (`SceneComponent.K2_GetComponentLocation` (`/Game/BP/BP_PlayerChara.ThighJumpRepère` (`self.BP_Chara`))))
  (bind (_returnvalue_x _returnvalue_y _returnvalue_z) (`KismetMathLibrary.BreakVector` (`KismetMathLibrary.GetForwardVector` (`Actor.K2_GetActorRotation` (`self.BP_Chara`)))))
  (set `self.HorizontalTracerTriggered` false)
  (if (not (`self.ThighJumping`))
    (bind (_outhit _returnvalue_2) (`KismetSystemLibrary.SphereTraceSingle` _returnvalue (+ (`KismetMathLibrary.MakeVector` (* _returnvalue_x 300.0) (* _returnvalue_y 300.0) _returnvalue_z) _returnvalue) 10.0 "TraceTypeQuery5"))
    (if _returnvalue_2
      (if (`KismetSystemLibrary.IsValid` (`.HitActor` (`GameplayStatics.BreakHitResult` _outhit)))
        (if (and (`Actor.ActorHasTag` (`.HitActor` (`GameplayStatics.BreakHitResult` _outhit)) "ThighJump") (not (`NavMovementComponent.IsFalling` (`Character.CharacterMovement` (`self.OwnerCharacter`)))))
          (set `self.HorizontalTracerTriggered` true)
          (set `self.WallNormal` (`.Normal` (`GameplayStatics.BreakHitResult` _outhit)))
          (set `self.WallLocation` (`.Location` (`GameplayStatics.BreakHitResult` _outhit))))))))

(fn `ReturnVectorMultiplier(withLerp)XY`
  (returns (LerpValuedistance :type "Float (double-precision)"))
  (if (> (`KismetMathLibrary.Vector_Distance2D` (`self.WallLocation`) (`SceneComponent.K2_GetComponentLocation` (`Character.CapsuleComponent` (`self.OwnerCharacter`)))) 100.0)
    (return (`KismetMathLibrary.Lerp` 650.0 800.0 (`self.Normalize to range`)))
    (else
      (return (`KismetMathLibrary.Lerp` 370.0 460.0 (`self.Normalize to range`))))))

(fn `VerticalTracer`
  (bind (_walllocation_x _walllocation_y _walllocation_z) (`KismetMathLibrary.BreakVector` (`self.WallLocation`)))
  (bind (_returnvalue_x _returnvalue_y) (`KismetMathLibrary.BreakVector` (* (`KismetMathLibrary.GetForwardVector` (`Actor.K2_GetActorRotation` (`self.BP_Chara`))) 30.0)))
  (bind _returnvalue (+ (`KismetMathLibrary.MakeVector` _walllocation_x _walllocation_y (+ _walllocation_z 100.0)) (`KismetMathLibrary.MakeVector` _returnvalue_x _returnvalue_y)))
  (if (`self.HorizontalTracerTriggered`)
    (if (not (`self.ThighJumping`))
      (bind (_outhit _returnvalue_2) (`KismetSystemLibrary.SphereTraceSingle` :`Start` _returnvalue :`End` (`KismetMathLibrary.MakeVector` (.x _returnvalue) (.y _returnvalue) (- (.z _returnvalue) 100.0)) :`Radius` 10.0 :`TraceChannel` "TraceTypeQuery5" :`TraceHitColor` (struct :`G` 0.79842 :`B` 1.0 :`A` 1.0)))
      (if _returnvalue_2
        (set `self.Ledge height location` (`.Location` (`GameplayStatics.BreakHitResult` _outhit)))))))