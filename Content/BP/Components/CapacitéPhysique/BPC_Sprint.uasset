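; Player sprint component that builds momentum while running forward at full speed and lets sprint input raise walk speed once momentum is maxed.
; Tick accumulates momentum time and clears it when speed drops, firing events with FOV and speedline bonuses.
; Momentum also toggles attached wind particles and timer-repeated breathing sounds, faded during speech, falling or certain player states.
; The node setting Sprinting to true is unconnected here.
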(event `self.ReceiveBeginPlay`
  ;[1 0 0.7767] Being play
  (bind _ascharacter (cast `Character` (`self.GetOwner`)))
  (bind _output_get (set `self.OwnerCharacter` _ascharacter))
  (set `CharacterMovementComponent.MaxWalkSpeed` (`self.RunningMaxSpeed`) (`Character.CharacterMovement` _output_get))
  (bind _returnvalue (`GameplayStatics.SpawnEmitterAttached` "/Game/StarterContent/Particles/P_sprint_V1.P_sprint_V1" (`Actor.RootComponent` (`self.OwnerCharacter`)) "None" (300.0 0.0 60.0) (struct :`Yaw` 180.0) (1.0 1.0 1.0) "KeepRelativeOffset" false))
  (set `self.WindEmitter` _returnvalue)
  (`self.Deactivate` (`self.WindEmitter`)))

(event `StartSprint`
  (params (DeltaSec :type "Float (double-precision)"))
  (bind _ownercharacter (`self.OwnerCharacter`))
  (bind _returnvalue (`Actor.GetVelocity` _ownercharacter))
  (bind _returnvalue_2 (`KismetMathLibrary.VSizeXY` _returnvalue))
  ;[1 1 1] start sprint
  (if (not (`self.MomentumActive`))
    (if (and (`KismetMathLibrary.NearlyEqual_FloatFloat` _returnvalue_2 (`self.RunningMaxSpeed`) 10.0) (> (`KismetMathLibrary.Dot_VectorVector` (`KismetMathLibrary.Normal` _returnvalue) (`Actor.GetActorForwardVector` _ownercharacter)) 0.0))
      (set `self.CurrentMomentumTime` (`KismetMathLibrary.FClamp` (+ (`self.CurrentMomentumTime`) DeltaSec) 0.0 (`self.TimeForMomentumMax`)))
      (if (>= (`self.CurrentMomentumTime`) (`self.TimeForMomentumMax`))
        (if (not (`self.MomentumActive`))
          (set `self.MomentumActive` true)
          (`self.OnMaxMomentumReached` (`self.MomentumSpeedlinesBonusWeight`) (`self.MomentumBonusFOV`) (`self.MomentumMaxSpeed`) (`self.RunningMaxSpeed`))
          (`self.ShowWindParticles` true)
          (`self.BreathingSounds`))))
    (elif (< _returnvalue_2 (`self.RunningMaxSpeed`))
      (set `self.CurrentMomentumTime` 0.0)
      (set `self.MomentumActive` false)
      (`self.OnMomentumExpired`)
      (`AudioComponent.FadeOut` (`self.BreathingSound`) 0.3 0.0)
      (`self.ShowWindParticles` false))))

(event `self.ReceiveTick`
  (params (DeltaSeconds :type "Float (single-precision)"))
  ;[1 0 0.6271] Event tick
  (`self.CheckBreathingSound`)
  (if (not (`self.Sprinting`))
    (`self.StartSprint` DeltaSeconds)
    (elif (not (`KismetMathLibrary.NearlyEqual_FloatFloat` (`KismetMathLibrary.VSizeXY` (`Actor.GetVelocity` (`self.OwnerCharacter`))) (`self.SprintMaxSpeed`) 10.0))
      (`self.StopSprinting`))))

(event `BreathingSounds`
  ;[1 1 1] Breathing sound
  (bind _returnvalue (`GameplayStatics.SpawnSound2D` "/Game/Sound_Design/Voix/InGame/Breathing_Cue.Breathing_Cue" 1.0 1.0 0.0 null false false))
  (bind _output_get (set `self.BreathingSound` _returnvalue))
  (if (`/Game/BP/BP_PlayerChara.PlayerSpeaking` (cast `/Game/BP/BP_PlayerChara` (`self.OwnerCharacter`) :!pure true))
    (set `AudioComponent.VolumeMultiplier` 0.0 _output_get))
  (if (`self.MomentumActive`)
    (`KismetSystemLibrary.K2_SetTimer` null "BreathingSounds" 0.8)))

(event `CheckBreathingSound`
  (bind _returnvalue (`GameplayStatics.GetPlayerCharacter` 0))
  (bind _breathingsound (`self.BreathingSound`))
  ;[1 1 1] Checkbreathingsound
  (if (!= _breathingsound null)
    (if (`AudioComponent.IsPlaying` _breathingsound)
      (bind _isdoingsomething (`/Game/BP/BP_PlayerChara.CheckPlayerStates` (cast `/Game/BP/BP_PlayerChara` _returnvalue :!pure true) true true true true true true true true true true true true false))
      (if (or (`NavMovementComponent.IsFalling` (`Character.CharacterMovement` _returnvalue)) _isdoingsomething (`/Game/BP/BP_PlayerChara.PlayerSpeaking` (cast `/Game/BP/BP_PlayerChara` (`self.OwnerCharacter`) :!pure true)))
        (`AudioComponent.FadeOut` (`self.BreathingSound`) 0.1 0.0)))))

(event `SprintInput`
  ;[1 1 1] Sprint input
  (if (and (`self.MomentumActive`) (not (`self.Sprinting`)) (`/Game/BP/BP_PlayerChara.GoingForward` (cast `/Game/BP/BP_PlayerChara` (`GameplayStatics.GetPlayerCharacter` 0) :!pure true)))
    (set `CharacterMovementComponent.MaxWalkSpeed` (`self.SprintMaxSpeed`) (`Character.CharacterMovement` (`self.OwnerCharacter`)))
    (`self.OnStartSprinting` (`self.SprintSpeedlinesBonusWeight`) (`self.SprintBonusFOV`))))

(event `ShowWindParticles`
  (params (Show :type Boolean))
  (bind _windemitter (`self.WindEmitter`))
  ;[1 1 1] Show/Hide wind particles
  (if Show
    (`self.Activate` _windemitter false)
    (else
      (`self.Deactivate` _windemitter))))

(event `ResetToRunningSpeed`
  ;[1 1 1] reset to running speed
  (set `CharacterMovementComponent.MaxWalkSpeed` (`self.RunningMaxSpeed`) (`Character.CharacterMovement` (`self.OwnerCharacter`)))
  (set `self.Sprinting` false)
  (set `self.CurrentMomentumTime` 0.0)
  (set `self.MomentumActive` false))

(event `StopSprinting`
  ;[1 1 1] stop sprint
  (if (`self.Sprinting`)
    (`self.ResetToRunningSpeed`)
    (`self.OnStopSprinting`)
    (`self.ShowWindParticles` false)))