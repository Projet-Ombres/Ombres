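; Player character component that gives a horizontal launch boost on landing after a long fall or jump.
; SetTimeIntheAir accumulates falling time outside of wall climbing, hanging and wall running, enabling the boost past a time threshold.
; StartSpeedBoostAfterLanding checks that the player just landed and is not hanging, then launches them along their movement direction and clears the boost flag.
; The air timer is never reset within this component.
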(event `Initialize`
  (params (BP_PlayerChara :type "/Game/BP/BP_PlayerChara Object Reference"))
  ;[1 1 1] Initialize
  (set `self.BP_PlayerChara` BP_PlayerChara))

(event `SpeedBoostAfterLanding`
  (bind (_playerdirection_x _playerdirection_y) (`KismetMathLibrary.BreakVector` (`/Game/BP/BP_PlayerChara.Playerdirection` (`self.BP_PlayerChara`))))
  ;[1 1 1] SpeedBoostAfterLanding
  (if (>= (`self.TimeJumping`) 2.0)
    (`Character.LaunchCharacter` (`self.BP_PlayerChara`) (`KismetMathLibrary.MakeVector` (* _playerdirection_x (`self.LandingSpeedBoost`)) (* _playerdirection_y (`self.LandingSpeedBoost`))) false false)
    (set `self.CanBeBoosted` false)))

(event `StartSpeedBoostAfterLanding`
  ;[1 1 1] Start Speed Boost After Landing
  (if (`/Game/BP/Components/CapacitéPhysique/BPC_WallClimb.IsHanging` (`/Game/BP/BP_PlayerChara.BPC_WallClimb` (`self.BP_PlayerChara`)))
    _
    (elif (`self.CanBeBoosted`)
      (if (`/Game/BP/BP_PlayerChara.JustLanded` (`self.BP_PlayerChara`))
        (`self.SpeedBoostAfterLanding`)))))

(fn `SetTimeIntheAir`
  (params (DeltaTime :type "Float (double-precision)"))
  (bind _bp_playerchara (`self.BP_PlayerChara`))
  (bind _bpc_wallclimb (`/Game/BP/BP_PlayerChara.BPC_WallClimb` _bp_playerchara))
  (if (and (not (`/Game/BP/Components/CapacitéPhysique/BPC_WallClimb.IsHanging` _bpc_wallclimb)) (not (`/Game/BP/Components/CapacitéPhysique/BPC_WallClimb.IsClimbingLedge` _bpc_wallclimb)) (not (`/Game/BP/Components/CapacitéPhysique/BPC_WallClimb.IsEscalatingWall` _bpc_wallclimb)) (not (`/Game/BP/Components/CapacitéPhysique/BPC_WallRun.IsWallRunning` (`/Game/BP/BP_PlayerChara.BPC_WallRun` _bp_playerchara))))
    (if (`NavMovementComponent.IsFalling` (`Character.CharacterMovement` (`self.BP_PlayerChara`)))
      (set `self.TimeJumping` (+ (`self.TimeJumping`) DeltaTime))
      (if (> (`self.TimeJumping`) 2.0)
        (set `self.CanBeBoosted` true)
        (else
          (set `self.CanBeBoosted` false))))))