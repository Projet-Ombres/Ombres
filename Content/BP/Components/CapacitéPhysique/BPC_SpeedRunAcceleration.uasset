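; Player physical-ability component that widens the camera field of view during sustained movement to convey running speed.
; Initialize caches the player, base FOV and base walk speed, though only the camera FOV is ever changed.
; Each tick, a clamped timer rises while horizontal speed passes a threshold outside wall-climb states, and otherwise drains ten times faster.
; That timer drives a clamped lerp from base to maximum FOV.
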(event `LerpFOV`
  ;[1 1 1] LERPFOV
  (`CameraComponent.SetFieldOfView` (`/Game/BP/BP_PlayerChara.Camera` (`self.Playerchara`)) (`KismetMathLibrary.FClamp` (`KismetMathLibrary.Lerp` (`self.FOVBase`) (`self.MaxFOV`) (`KismetMathLibrary.FClamp` (/ (`self.TimerFOV`) (`self.FOVScaleDuration`)))) 102.0 (`self.MaxFOV`))))

(event `Initialize`
  (params (Player :type "/Game/BP/BP_PlayerChara Object Reference"))
  ;[1 1 1] Initialize
  (bind _output_get (set `self.Playerchara` Player))
  (set `self.MaxWalkSpeedBase` (`CharacterMovementComponent.MaxWalkSpeed` (`Character.CharacterMovement` _output_get)))
  (set `self.FOVBase` (`CameraComponent.FieldOfView` (`/Game/BP/BP_PlayerChara.Camera` _output_get))))

(event `self.ReceiveTick`
  (params (DeltaSeconds :type "Float (single-precision)"))
  (bind _playerchara (`self.Playerchara`))
  (bind _bpc_wallclimb (`/Game/BP/BP_PlayerChara.BPC_WallClimb` _playerchara))
  (set `self.DeltaSec` DeltaSeconds)
  ;[1 1 1] Event tick
  (`self.LerpFOV`)
  (bind _output_get (set `self.PlayerSpeed` (`KismetMathLibrary.VSizeXY` (`MovementComponent.Velocity` (`Character.CharacterMovement` _playerchara)))))
  (if (and (> _output_get 100.0) (not (`/Game/BP/Components/CapacitéPhysique/BPC_WallClimb.IsHanging` _bpc_wallclimb)) (not (`/Game/BP/Components/CapacitéPhysique/BPC_WallClimb.IsEscalatingWall` _bpc_wallclimb)) (not (`/Game/BP/Components/CapacitéPhysique/BPC_WallClimb.IsClimbingLedge` _bpc_wallclimb)))
    (set `self.TimerFOV` (`KismetMathLibrary.FClamp` (+ (`self.TimerFOV`) (`self.DeltaSec`)) 0.0 (`self.FOVScaleDuration`)))
    (else
      (set `self.TimerFOV` (`KismetMathLibrary.FClamp` (- (`self.TimerFOV`) (* (`self.DeltaSec`) 10.0)) 0.0 (`self.FOVScaleDuration`))))))