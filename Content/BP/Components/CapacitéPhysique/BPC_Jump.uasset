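; Player jump component that adds optional jump assistance for early and late presses near ledges, plus a boosted jump from BP_Rampe ramps.
; Tick traces for void ahead, caching the last edge; early jumps slide the player there at current speed before jumping.
; Late jumps after leaving ground temporarily raise JumpMaxCount to two.
; Each jump drives GravityScale from a curve through a custom timeline.
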(event `self.ReceiveBeginPlay`
  ;[1 0 0.5421] Begin play
  (set `self.BP_PlayerChara` (cast `/Game/BP/BP_PlayerChara` (`GameplayStatics.GetPlayerCharacter` 0) :!pure true)))

(event `Jump`
  (bind (_bcandonormaljump _bcandoassistedjump) (`self.CanPlayerJump`))
  (bind _bp_playerchara (`self.BP_PlayerChara`))
  (bind _returnvalue (+ (`self.EdgePosition`) (* (`KismetMathLibrary.Vector_Up`) 60.0)))
  ;[1 1 1] Jump event
  (if (`self.JumpAssistEnabled`)
    ;[1 1 1] Check if is doing an early jump or just a normal jump
    (if _bcandonormaljump
      (if (and (not (`self.IsJumpingClassic`)) (not (`self.IsJumpingTooLate`)))
        (if (and (`self.VoidDetected`) (>= (`KismetMathLibrary.VSizeXY` (`Actor.GetVelocity` (`self.BP_PlayerChara`))) (`self.MinSpeedForEarlyJump`)))
          (set `self.EdgePosition` (+ (* (`KismetMathLibrary.Normal` (- (`Actor.K2_GetActorLocation` (`self.BP_PlayerChara`)) _returnvalue)) 30.0) _returnvalue))
          (set `self.LerpStartPosition` (`Actor.K2_GetActorLocation` (`self.BP_PlayerChara`)))
          (set `self.LerpingPosition` true)
          ;[1 1 1] Lerp position with timeline
          (bind _outputvalue (`CustomTimeline.StartCustomTimeline` (/ 1.0 (/ (`KismetMathLibrary.Vector_Distance2D` (`self.EdgePosition`) (`Actor.K2_GetActorLocation` _bp_playerchara)) (`KismetMathLibrary.VSizeXY` (`Actor.GetVelocity` _bp_playerchara)))))
            (:`Update`
              (`Actor.K2_SetActorLocation` (`self.BP_PlayerChara`) (`KismetMathLibrary.VLerp` (`self.LerpStartPosition`) (`self.EdgePosition`) _outputvalue) false false))
            (:`Finished`
              (set `self.IsJumpingClassic` true)
              (set `self.LerpingPosition` false)
              (`self.PerformJump`)))
          (else
            ;[1 1 1] Normal jump
            (set `self.IsJumpingClassic` true)
            (set `self.IsJumpingTooLate` false)
            (`self.PerformJump`))))
      (else
        ;[1 1 1] Too late jump
        (if _bcandoassistedjump
          (if (and (not (`self.IsJumpingClassic`)) (not (`self.IsJumpingTooLate`)))
            (set `Character.JumpMaxCount` 2 (`self.BP_PlayerChara`))
            (set `self.IsJumpingTooLate` true)
            (`self.PerformJump`)))))
    (else
      (`self.PerformJump`))))

(event `self.ReceiveTick`
  (params (DeltaSeconds :type "Float (single-precision)"))
  ;[0.9516 0 1] Event tick
  (`self.DownTracer`)
  (`self.VoidTracer`)
  ;[1 1 1] Reset IsJumping
  (if (not (`NavMovementComponent.IsFalling` (`Character.CharacterMovement` (`self.BP_PlayerChara`))))
    (if (`self.IsJumpingTooLate`)
      (if (> (`/Game/BP/BP_PlayerChara.TimeInTheAirTimer` (`self.BP_PlayerChara`)) (`self.TimeGivenToJumpAfterStartingToFall`))
        (set `self.IsJumpingTooLate` false)
        (set `Character.JumpMaxCount` 1 (`self.BP_PlayerChara`)))
      (elif (`self.IsJumpingClassic`)
        (set `self.IsJumpingClassic` false)
        (set `Character.JumpMaxCount` 1 (`self.BP_PlayerChara`))
        ;[1 0.2304 0.8781] Reset jump velocity
        (set `CharacterMovementComponent.JumpZVelocity` (`self.Jump Z Velocity `) (`Character.CharacterMovement` (`self.BP_PlayerChara`)))))))

(event `PerformJump`
  (bind _lasttimeline (`self.LastTimeline`))
  (bind _lasttimeline_2 (`self.LastTimeline`))
  (bind _charactermovement (`Character.CharacterMovement` (`self.BP_PlayerChara`)))
  ;[1 0.6162 0.08689] Perform jump (with ramp check)
  (`/Engine/EditorBlueprintResources/StandardMacros.IsValid` _lasttimeline_2
    (:`Is Valid`
      (if (`CustomTimeline.IsRunning` _lasttimeline_2)
        (`CustomTimeline.StopCustomTimeline` _lasttimeline _lasttimeline)))
    (:`Is Not Valid`
      _))
  (cast `/Game/BP/Class/BP_Rampe` (`.HitActor` (`GameplayStatics.BreakHitResult` (`.HitResult` (break `FindFloorResult` (`CharacterMovementComponent.CurrentFloor` _charactermovement)))))
    (:`then`
      (set `CharacterMovementComponent.JumpZVelocity` (`self.RampJumpVelocity`) _charactermovement))
    (:`CastFailed`
      _))
  (`Character.Jump` (`self.BP_PlayerChara`))
  (`self.ApplyGravityCurve`))

(event `ApplyGravityCurve`
  ;[1 1 1] GravityCurve
  (bind (_outputvalue _realdeltatime _ref) (`CustomTimeline.StartCustomTimeline` 1.0)
    (:`then`
      (set `self.LastTimeline` _ref))
    (:`Update`
      (set `CharacterMovementComponent.GravityScale` (`CurveFloat.GetFloatValue` (`self.GravityScale`) _outputvalue) (`Character.CharacterMovement` (`self.BP_PlayerChara`))))))

(event `SetJumpAssistEnabled`
  (params (JumpAssist :type Boolean))
  (set `self.JumpAssistEnabled` JumpAssist))

(event `StopGravityCurve`
  (bind _lasttimeline (`self.LastTimeline`))
  ;[1 1 1] StopGravity curve
  (`/Engine/EditorBlueprintResources/StandardMacros.IsValid` _lasttimeline
    (:`Is Valid`
      (if (`CustomTimeline.IsRunning` _lasttimeline)
        (`CustomTimeline.StopCustomTimeline` (`self.LastTimeline`))))
    (:`Is Not Valid`
      _))
  (set `CharacterMovementComponent.GravityScale` 1.0 (`Character.CharacterMovement` (`self.BP_PlayerChara`))))

(fn `DownTracer`
  (bind _returnvalue (`Actor.K2_GetActorLocation` (`self.BP_PlayerChara`)))
  (bind (_outhit _returnvalue_2) (`KismetSystemLibrary.LineTraceSingle` _returnvalue (+ _returnvalue (* (`KismetMathLibrary.Vector_Down`) 1000.0)) "TraceTypeQuery1"))
  (if _returnvalue_2
    (set `self.PlayerGroundPosition` (`.ImpactPoint` (`GameplayStatics.BreakHitResult` _outhit)))))

(fn `VoidTracer`
  (bind _bp_playerchara (`self.BP_PlayerChara`))
  (bind _earlyjumpdetectionrange (`self.EarlyJumpDetectionRange`))
  (bind _returnvalue (`Actor.K2_GetActorLocation` _bp_playerchara))
  (bind _returnvalue_2 (`KismetMathLibrary.Normal` (`Actor.GetVelocity` _bp_playerchara)))
  (if (not (`self.LerpingPosition`))
    (bind _outhit (`KismetSystemLibrary.SphereTraceSingle` :`Start` (+ _returnvalue (* _returnvalue_2 (* _earlyjumpdetectionrange 0.666667))) :`End` (- (+ _returnvalue (* _returnvalue_2 _earlyjumpdetectionrange)) (* (`KismetMathLibrary.Vector_Down`) -200.0)) :`Radius` 25.0 :`TraceChannel` "TraceTypeQuery1" :`bTraceComplex` true :`TraceColor` (struct :`G` 1.0 :`B` 0.815809 :`A` 1.0)))
    (bind (_bblockinghit _binitialoverlap _time _distance _location _impactpoint) (`GameplayStatics.BreakHitResult` _outhit))
    (if _bblockinghit
      (set `self.EdgePosition` _impactpoint)
      (set `self.VoidDetected` false)
      (elif (not (`self.VoidDetected`))
        (set `self.VoidDetected` true)))))