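; Player slide component: a forward-only slide that crouches the character, lowers the spring arm and plays camera shake and force feedback.
; Custom timelines drive decaying velocity, while Tick checks floor slope to sustain a faster downhill slide or end timed-out flat and uphill ones.
; Exiting retries with forward impulses while an overhead sphere trace hits, then uncrouches, raises the camera and triggers BPCJump's PerformJump.
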(event `MoveCameraDown`
  (bind _cameradowntimeline (`self.CameraDownTimeline`))
  (bind _camerauptimeline (`self.CameraUpTimeline`))
  (bind (_relativelocation_x _relativelocation_y _relativelocation_z) (`KismetMathLibrary.BreakVector` (`SceneComponent.RelativeLocation` (`/Game/BP/BP_PlayerChara.SpringArm` (`self.BP_PlayerChara`)))))
  (bind (_relativelocation_x_2 _relativelocation_y_2) (`KismetMathLibrary.BreakVector` (`SceneComponent.RelativeLocation` (`/Game/BP/BP_PlayerChara.SpringArm` (`self.BP_PlayerChara`)))))
  (bind (_relativelocation_x_3 _relativelocation_y_3) (`KismetMathLibrary.BreakVector` (`SceneComponent.RelativeLocation` (`/Game/BP/BP_PlayerChara.SpringArm` (`self.BP_PlayerChara`)))))
  ;[0.04638 1 0.9003] MoveCameraDown
  (`/Engine/EditorBlueprintResources/StandardMacros.IsValid` (`self.CameraDownTimeline`)
    (:`Is Valid`
      (if (`CustomTimeline.IsRunning` _cameradowntimeline)
        (`CustomTimeline.StopCustomTimeline` _cameradowntimeline _cameradowntimeline)))
    (:`Is Not Valid`
      _))
  (`/Engine/EditorBlueprintResources/StandardMacros.IsValid` (`self.CameraUpTimeline`)
    (:`Is Valid`
      (if (`CustomTimeline.IsRunning` _camerauptimeline)
        (`CustomTimeline.StopCustomTimeline` _camerauptimeline)))
    (:`Is Not Valid`
      _))
  (set `Pawn.bUseControllerRotationYaw` false (`self.BP_PlayerChara`))
  (set `self.[TEMPORARY]CamZPosition` _relativelocation_z)
  (bind (_outputvalue _realdeltatime _ref) (`CustomTimeline.StartCustomTimeline` 10.0)
    (:`Update`
      (set `self.CameraDownTimeline` _ref)
      (`SceneComponent.K2_SetRelativeLocation` (`/Game/BP/BP_PlayerChara.SpringArm` (`self.BP_PlayerChara`)) (`KismetMathLibrary.MakeVector` _relativelocation_x_2 _relativelocation_y_2 (`KismetMathLibrary.Lerp` (`self.[TEMPORARY]CamZPosition`) 10.0 _outputvalue)) false false))
    (:`Finished`
      (`SceneComponent.K2_SetRelativeLocation` (`/Game/BP/BP_PlayerChara.SpringArm` (`self.BP_PlayerChara`)) (`KismetMathLibrary.MakeVector` _relativelocation_x_3 _relativelocation_y_3 10.0) false false))))

(event `MoveCameraUp`
  (bind _cameradowntimeline (`self.CameraDownTimeline`))
  (bind _camerauptimeline (`self.CameraUpTimeline`))
  (bind (_relativelocation_x _relativelocation_y) (`KismetMathLibrary.BreakVector` (`SceneComponent.RelativeLocation` (`/Game/BP/BP_PlayerChara.SpringArm` (`self.BP_PlayerChara`)))))
  (bind (_relativelocation_x_2 _relativelocation_y_2) (`KismetMathLibrary.BreakVector` (`SceneComponent.RelativeLocation` (`/Game/BP/BP_PlayerChara.SpringArm` (`self.BP_PlayerChara`)))))
  ;[0.04638 1 0.9003] Move Camera Up
  (`/Engine/EditorBlueprintResources/StandardMacros.IsValid` (`self.CameraDownTimeline`)
    (:`Is Valid`
      (if (`CustomTimeline.IsRunning` _cameradowntimeline)
        (`CustomTimeline.StopCustomTimeline` _cameradowntimeline _cameradowntimeline)))
    (:`Is Not Valid`
      _))
  (`/Engine/EditorBlueprintResources/StandardMacros.IsValid` (`self.CameraUpTimeline`)
    (:`Is Valid`
      (if (`CustomTimeline.IsRunning` _camerauptimeline)
        (`CustomTimeline.StopCustomTimeline` _camerauptimeline)))
    (:`Is Not Valid`
      _))
  (if (or (`self.IsSliding`) (`self.isSlidingEnPente`))
    (set `Pawn.bUseControllerRotationYaw` false (`self.BP_PlayerChara`)))
  (bind (_outputvalue _realdeltatime _ref) (`CustomTimeline.StartCustomTimeline` 7.0)
    (:`then`
      (`KismetSystemLibrary.Delay` 0.0)
      (`/Game/BP/Components/CapacitéPhysique/BPC_Jump.PerformJump` (`/Game/BP/BP_PlayerChara.BPC_Jump` (`self.BP_PlayerChara`))))
    (:`Update`
      (set `self.CameraUpTimeline` _ref)
      (`SceneComponent.K2_SetRelativeLocation` (`/Game/BP/BP_PlayerChara.SpringArm` (`self.BP_PlayerChara`)) (`KismetMathLibrary.MakeVector` _relativelocation_x_2 _relativelocation_y_2 (`KismetMathLibrary.Lerp` 10.0 (`self.[TEMPORARY]CamZPosition`) _outputvalue)) false false))
    (:`Finished`
      (set `Pawn.bUseControllerRotationYaw` true (`self.BP_PlayerChara`))
      (`SceneComponent.K2_SetRelativeLocation` (`/Game/BP/BP_PlayerChara.SpringArm` (`self.BP_PlayerChara`)) (`KismetMathLibrary.MakeVector` _relativelocation_x _relativelocation_y 56.0) false false)
      (set `self.Uncrouching` false))))

(event `Initialize`
  (params (BP_Chara :type "/Game/BP/BP_PlayerChara Object Reference"))
  ;[0.9973 0 1] Initialize
  (bind _output_get (set `self.BP_PlayerChara` BP_Chara))
  (set `self.FOVBase` (`CameraComponent.FieldOfView` (`/Game/BP/BP_PlayerChara.Camera` _output_get))))

(event `LerpFOV`
  ;[1 0.1015 0] No need de ca si on change la fov en courant
  ;;[1 1 1] Lerp fov
  (bind _outputvalue (`CustomTimeline.StartCustomTimeline` 10.0)
    (:`Update`
      (`CameraComponent.SetFieldOfView` (`/Game/BP/BP_PlayerChara.Camera` (`self.BP_PlayerChara`)) (`KismetMathLibrary.Lerp` (`self.FOVBase`) (`self.MaxFOV`) _outputvalue)))))

(event `self.ReceiveTick`
  (params (DeltaSeconds :type "Float (single-precision)"))
  ;[1 0 0.8165] Event tick
  (`self.CameraTilt`)
  (`self.SetSlidingTimer` DeltaSeconds)
  ;[1 1 1] check slope
  (`self.CheckForSlope`)
  (`self.CheckIfSlideIsTooSlow`))

(event `SetSlidingTimer`
  (params (DeltaSec :type "Float (double-precision)"))
  ;[1 1 1] Set sliding timer for if too much uncrouch
  (if (`self.IsSliding`)
    (set `self.SlideTimelineTimer` (+ (`self.SlideTimelineTimer`) DeltaSec))))

(event `UnlerpFOV`
  ;[1 0.1015 0] No need de ca si on change la fov en courant
  ;;[1 1 1] Unlerp fov
  (bind _outputvalue (`CustomTimeline.StartCustomTimeline` 10.0)
    (:`Update`
      (`CameraComponent.SetFieldOfView` (`/Game/BP/BP_PlayerChara.Camera` (`self.BP_PlayerChara`)) (`KismetMathLibrary.Lerp` (`self.MaxFOV`) (`self.FOVBase`) _outputvalue)))))

(event `CheckForSlope`
  (bind (_playerdirection_x _playerdirection_y _playerdirection_z) (`KismetMathLibrary.BreakVector` (`self.PlayerDirection`)))
  (bind _slidetimelineref (`self.SlideTimelineREF`))
  (bind _charactermovement (`Character.CharacterMovement` (`self.BP_PlayerChara`)))
  (bind _returnvalue (* (`/Game/BP/BP_PlayerChara.MaxSpeed` (`self.BP_PlayerChara`)) 2.0))
  ;[1 1 1] Check for slope
  (`self.ReturnSlopCorrectDirection`)
  (if (`self.SlopeIsUnderPlayer`)
    (if (and (not (`self.UpwaySlope`)) (`self.IsSliding`))
      (if (`KismetSystemLibrary.IsValid` _slidetimelineref)
        (if (`CustomTimeline.IsRunning` _slidetimelineref)
          (`CustomTimeline.StopCustomTimeline` _slidetimelineref)))
      (set `self.IsSliding` true)
      (set `self.isSlidingEnPente` true)
      (set `CharacterMovementComponent.MaxWalkSpeed` 1800.0 _charactermovement)
      (set `MovementComponent.Velocity` (`KismetMathLibrary.MakeVector` (* _playerdirection_x _returnvalue) (* _playerdirection_y _returnvalue) _playerdirection_z) _charactermovement)
      (`self.CorrectSlopeSlideTrajectoire`)
      (`self.SetMeshRotation`))
    (else
      (bind _somethingunder (`self.DownTracer`))
      (if _somethingunder
        (if (`self.isSlidingEnPente`)
          (set `self.isSlidingEnPente` false)
          (`self.HalfSlideAfterSlope`))
        (else
          (`self.UnCrouchAndMoveCamUp`))))))

(event `Slide`
  (params (isPressed :type Boolean))
  ;[1 0.7166 0] On slide pressed
  (if isPressed
    (if (`/Game/BP/BP_PlayerChara.GoingForward` (`self.BP_PlayerChara`))
      (set `self.IsSliding` true)
      (`self.ReducedSlide`)
      (`/Game/BP/BP_Controller.PlayForceFeedback` (cast `/Game/BP/BP_Controller` (`GameplayStatics.GetPlayerController` 0) :!pure true) true false "/Game/BP/FeedbackAssets/Vibrations/Vibration_Slide.Vibration_Slide"))
    (else
      (`self.UnCrouchAndMoveCamUp`)
      (set `self.isSlidingEnPente` false))))

(event `ReducedSlide`
  (bind (_playerdirection_x _playerdirection_y _playerdirection_z) (`KismetMathLibrary.BreakVector` (`self.PlayerDirection`)))
  (bind _bp_playerchara (`self.BP_PlayerChara`))
  (bind _charactermovement (`Character.CharacterMovement` _bp_playerchara))
  (bind (_velocity_x _velocity_y _velocity_z) (`KismetMathLibrary.BreakVector` (`MovementComponent.Velocity` _charactermovement)))
  ;[1 0.7166 0] Half slide
  (`self.CrouchAndMoveDownCam` true)
  (set `self.FullSlide` false)
  (bind (_outputvalue _realdeltatime _ref) (`CustomTimeline.StartCustomTimeline` (/ 1.0 (`self.SlideDuration`)))
    (:`Update`
      (if (`self.IsSliding`)
        (set `self.SlideTimelineREF` _ref)
        (bind _returnvalue (* (- 1.0 _outputvalue) (`self.MaxSlideSpeed`)))
        (set `MovementComponent.Velocity` (`KismetMathLibrary.MakeVector` (* (* _returnvalue _playerdirection_x) 1.3) (* (* _returnvalue _playerdirection_y) 1.3) _playerdirection_z) (`Character.CharacterMovement` (`self.BP_PlayerChara`)))
        (if (`/Game/BP/BP_PlayerChara.MovingUp` (`self.BP_PlayerChara`))
          (set `MovementComponent.Velocity` (`KismetMathLibrary.MakeVector` _velocity_x _velocity_y (+ _velocity_z (`/Game/BP/BP_PlayerChara.UpZTracerPosition` _bp_playerchara))) _charactermovement))))))

(event `CorrectSlopeSlideTrajectoire`
  ;[1 1 1] Correct Slope Slide Trajectoir
  (`/Engine/EditorBlueprintResources/StandardMacros.IsValid` (`self.(SlopeCorrection)SlideTimelineREF`)
    (:`Is Valid`
      (if (not (`CustomTimeline.IsRunning` (`self.(SlopeCorrection)SlideTimelineREF`)))
        (`KismetSystemLibrary.Delay` 0.2 :!label _label)
        (bind (_outputvalue _realdeltatime _ref) (`CustomTimeline.StartCustomTimeline` 0.1)
          (:`Update`
            (set `self.(SlopeCorrection)SlideTimelineREF` _ref)
            (set `self.PlayerDirection` (`KismetMathLibrary.VLerp` (`self.PlayerDirection`) (`KismetMathLibrary.Normal` (`KismetMathLibrary.ProjectVectorOnToPlane` (`.Normal` (`GameplayStatics.BreakHitResult` (`.HitResult` (break `FindFloorResult` (`CharacterMovementComponent.CurrentFloor` (`Character.CharacterMovement` (`self.BP_PlayerChara`))))))) (0.0 0.0 1.0))) (/ _outputvalue 3.0)))))))
    (:`Is Not Valid`
      (goto _label))))

(event `SetMeshRotation`
  (bind _returnvalue (`KismetMathLibrary.ProjectVectorOnToPlane` (`/Game/BP/BP_PlayerChara.Playerdirection` (`self.BP_PlayerChara`)) (0.0 0.0 1.0)))
  ;[1 1 1] Set Mesh rotation
  (`SceneComponent.K2_SetWorldRotation` (`Character.CapsuleComponent` (`self.BP_PlayerChara`)) (`KismetMathLibrary.MakeRotationFromAxes` _returnvalue (`KismetMathLibrary.Cross_VectorVector` _returnvalue (0.0 0.0 -1.0)) (0.0 0.0 1.0)) false false))

(event `HalfSlideAfterSlope`
  (bind _bp_playerchara (`self.BP_PlayerChara`))
  (bind _charactermovement (`Character.CharacterMovement` _bp_playerchara))
  (bind (_returnvalue_x _returnvalue_y) (`KismetMathLibrary.BreakVector` (`KismetMathLibrary.Normal` (`Actor.GetVelocity` (`self.BP_PlayerChara`)))))
  (bind (_velocity_x _velocity_y _velocity_z) (`KismetMathLibrary.BreakVector` (`MovementComponent.Velocity` _charactermovement)))
  ;[1 0.7166 0] Half slide after slope (same as before but player idrection isnt reset)
  (`Character.Crouch` (`self.BP_PlayerChara`))
  (set `self.FullSlide` false)
  (bind (_outputvalue _realdeltatime _ref) (`CustomTimeline.StartCustomTimeline` (/ 1.0 (`self.SlideDuration`)))
    (:`Update`
      (if (`self.IsSliding`)
        (set `self.(SlopeLanding)SlideTimelineREF` _ref)
        (bind _returnvalue (* (- 1.0 _outputvalue) (`self.MaxSlideSpeed`)))
        (set `MovementComponent.Velocity` (`KismetMathLibrary.MakeVector` (* (* _returnvalue _returnvalue_x) 1.3) (* (* _returnvalue _returnvalue_y) 1.3)) (`Character.CharacterMovement` (`self.BP_PlayerChara`)))
        (if (`/Game/BP/BP_PlayerChara.MovingUp` (`self.BP_PlayerChara`))
          (set `MovementComponent.Velocity` (`KismetMathLibrary.MakeVector` _velocity_x _velocity_y (+ _velocity_z (`/Game/BP/BP_PlayerChara.UpZTracerPosition` _bp_playerchara))) _charactermovement))))
    (:`Finished`
      (if (`self.IsSliding`)
        (`self.UnCrouchAndMoveCamUp`)))))

(event `ReturnSlopCorrectDirection`
  (bind (_returnvalue_x _returnvalue_y _returnvalue_z) (`KismetMathLibrary.BreakVector` (`Actor.K2_GetActorLocation` (`self.BP_PlayerChara`))))
  ;[1 1 1] Return if player takes the slope down
  (set `self.ZPlayerPosition` _returnvalue_z)
  (bind _somethingunder (`self.DownTracer`))
  (if _somethingunder
    (if (> (`KismetMathLibrary.DegAcos` (`KismetMathLibrary.Dot_VectorVector` (`KismetMathLibrary.Vector_Up`) (`.Normal` (`GameplayStatics.BreakHitResult` (`.HitResult` (break `FindFloorResult` (`CharacterMovementComponent.CurrentFloor` (`Character.CharacterMovement` (`self.BP_PlayerChara`))))))))) 9.5)
      (if (`/Game/BP/BP_PlayerChara.MovingUp` (`self.BP_PlayerChara`))
        (set `self.UpwaySlope` true)
        (set `self.SlopeIsUnderPlayer` true)
        (else
          (set `self.SlopeIsUnderPlayer` true)
          (set `self.UpwaySlope` false)))
      (else
        (set `self.SlopeIsUnderPlayer` false :!label _label_2)
        (set `self.UpwaySlope` false)))
    (else
      (goto _label_2))))

(event `PrintEveruthing`
  ;[1 1 1] Print everything DEBUg
)

(event `CameraTilt`
  ;[1 1 1] SlideCameraTilting
  (if (`self.IsSliding`)
    (`PlayerController.ClientStartCameraShake` :`self` (`GameplayStatics.GetPlayerController` 0) :`Shake` "/Game/BP/FeedbackAssets/ScreenShakes/BP_CameraShake_Slide.BP_CameraShake_Slide_C" :`Scale` (/ (`KismetMathLibrary.VSizeXY` (`Actor.GetVelocity` (`self.BP_PlayerChara`))) 100.0))))

(event `CrouchAndMoveDownCam`
  (params (SetPlayerDirection :type Boolean))
  ;[1 0.3656 0.6776] Crouch and Move down cam
  (`Character.Crouch` (`self.BP_PlayerChara`))
  (`self.MoveCameraDown`)
  (if SetPlayerDirection
    (set `self.PlayerDirection` (`/Game/BP/BP_PlayerChara.Playerdirection` (`self.BP_PlayerChara`)))))

(event `UnCrouchAndMoveCamUp`
  (bind __slopecorrection_slidetimelineref (`self.(SlopeCorrection)SlideTimelineREF`))
  (bind _slidetimelineref (`self.SlideTimelineREF`))
  (bind _bp_playerchara (`self.BP_PlayerChara`))
  (bind __slopelanding_slidetimelineref (`self.(SlopeLanding)SlideTimelineREF`))
  (bind (_returnvalue_x _returnvalue_y) (`KismetMathLibrary.BreakVector` (`KismetMathLibrary.GetForwardVector` (`Pawn.GetControlRotation` (`self.BP_PlayerChara`)))))
  ;[1 0.3656 0.6776] Uncrouch and move up cam
  (bind _returnvalue (`self.UpTracer`))
  (if _returnvalue
    (if (`self.IsSliding`)
      ;;[1 1 1] Si ya un obstacle ua dessus du joueur il continue de lside un peu
      (`CharacterMovementComponent.AddImpulse` (`Character.CharacterMovement` (`self.BP_PlayerChara`)) (`KismetMathLibrary.MakeVector` (* _returnvalue_x 250.0) (* _returnvalue_y 250.0)) false)
      (`KismetSystemLibrary.Delay` 0.1)
      (`self.UnCrouchAndMoveCamUp`))
    (elif (`self.IsSliding`)
      (set `self.Uncrouching` true)
      (`PlayerController.ClientStopForceFeedback` (`GameplayStatics.GetPlayerController` 0) "/Game/BP/FeedbackAssets/Vibrations/Vibration_Slide.Vibration_Slide" "None")
      (`Character.UnCrouch` (`self.BP_PlayerChara`))
      (`self.MoveCameraUp`)
      (set `CharacterMovementComponent.MaxWalkSpeed` (`/Game/BP/BP_PlayerChara.MaxSpeed` _bp_playerchara) (`Character.CharacterMovement` _bp_playerchara))
      (set `self.IsSliding` false)
      (set `self.isSlidingEnPente` false)
      (set `self.SlideTimelineTimer` 0.0)
      (`/Engine/EditorBlueprintResources/StandardMacros.IsValid` __slopelanding_slidetimelineref
        (:`Is Valid`
          (if (`CustomTimeline.IsRunning` __slopelanding_slidetimelineref)
            (`CustomTimeline.StopCustomTimeline` __slopelanding_slidetimelineref)))
        (:`Is Not Valid`
          _))
      (`/Engine/EditorBlueprintResources/StandardMacros.IsValid` _slidetimelineref
        (:`Is Valid`
          (if (`CustomTimeline.IsRunning` _slidetimelineref)
            (`CustomTimeline.StopCustomTimeline` _slidetimelineref)))
        (:`Is Not Valid`
          _))
      (`/Engine/EditorBlueprintResources/StandardMacros.IsValid` (`self.(SlopeCorrection)SlideTimelineREF`)
        (:`Is Valid`
          (if (`CustomTimeline.IsRunning` __slopecorrection_slidetimelineref)
            (`CustomTimeline.StopCustomTimeline` __slopecorrection_slidetimelineref)))
        (:`Is Not Valid`
          _))
      (if (`self.FullSlide`)
        (set `self.CooldownSlideReady` false)
        (set `self.FullSlide` false)
        (`KismetSystemLibrary.Delay` (`self.CooldownSlide`))
        (set `self.CooldownSlideReady` true)))))

(event `CheckIfSlideIsTooSlow`
  ;[1 1 1] Check if sliding too much and should uncrouch
  (if (`self.IsSliding`)
    (if (> (`self.SlideTimelineTimer`) 0.5)
      (if (not (`self.SlopeIsUnderPlayer`))
        (`self.UnCrouchAndMoveCamUp`)
        (elif (`self.UpwaySlope`)
          (`self.UnCrouchAndMoveCamUp`))))))

(fn `DownTracer`
  (returns (SomethingUnder :type Boolean))
  (bind (_returnvalue_x _returnvalue_y _returnvalue_z) (`KismetMathLibrary.BreakVector` (`SceneComponent.K2_GetComponentLocation` (`/Game/BP/BP_PlayerChara.FeetRepère` (`self.BP_PlayerChara`)))))
  (bind (_outhit _returnvalue) (`KismetSystemLibrary.SphereTraceSingle` (`SceneComponent.K2_GetComponentLocation` (`/Game/BP/BP_PlayerChara.FeetRepère` (`self.BP_PlayerChara`))) (`KismetMathLibrary.MakeVector` _returnvalue_x _returnvalue_y (+ _returnvalue_z 100.0)) 20.0 "TraceTypeQuery1"))
  (return _returnvalue))

(fn `UpTracer`
  (returns (ReturnValue :type Boolean))
  (bind _returnvalue (`Actor.K2_GetActorLocation` (`self.BP_PlayerChara`)))
  (bind (_outhit _returnvalue_2) (`KismetSystemLibrary.SphereTraceSingle` _returnvalue (+ _returnvalue (* (`KismetMathLibrary.Vector_Up`) 300.0)) 50.0 "TraceTypeQuery1"))
  (return _returnvalue_2))