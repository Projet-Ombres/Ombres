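; Player camera component that turns the camera 180 degrees to look behind while slowing global time, then swings it back.
; StartRotation detaches the camera from pawn control rotation, applies slow motion and uses a custom timeline to lerp yaw around, keeping control pitch and roll.
; EndRotation restores normal time, reverses the yaw and flips the camera's X offset, re-enabling pawn control rotation when finished.
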(event `Initialize`
  (params (PlayerChara :type "/Game/BP/BP_PlayerChara Object Reference"))
  ;[1 1 1] Initialize
  (bind _output_get (set `self.PlayerChara` PlayerChara))
  (set `self.CameraInitialPosition` (`SceneComponent.RelativeLocation` (`/Game/BP/BP_PlayerChara.Camera` _output_get))))

(event `StartRotation`
  (bind (_returnvalue_roll _returnvalue_pitch) (`KismetMathLibrary.BreakRotator` (`Pawn.GetControlRotation` (`self.PlayerChara`))))
  (bind _camera (`/Game/BP/BP_PlayerChara.Camera` (`self.PlayerChara`)))
  ;[1 1 1] Start rotation
  (set `CameraComponent.bUsePawnControlRotation` false (`/Game/BP/BP_PlayerChara.Camera` (`self.PlayerChara`)))
  (set `self.IsRotating` true)
  (`GameplayStatics.SetGlobalTimeDilation` 0.1)
  (bind _outputvalue (`CustomTimeline.StartCustomTimeline` 4.0)
    (:`Update`
      (`SceneComponent.K2_SetRelativeRotation` _camera (`KismetMathLibrary.MakeRotator` _returnvalue_roll _returnvalue_pitch (`KismetMathLibrary.FClamp` (`KismetMathLibrary.Lerp` 0.0 180.0 (* _outputvalue 1.1)) 0.0 180.0)) false false)
      (`SceneComponent.K2_SetRelativeLocation` _camera (-28.0 0.0 78.0) false false))))

(event `EndRotation`
  (bind (_returnvalue_roll _returnvalue_pitch) (`KismetMathLibrary.BreakRotator` (`Pawn.GetControlRotation` (`self.PlayerChara`))))
  (bind _camera (`/Game/BP/BP_PlayerChara.Camera` (`self.PlayerChara`)))
  ;[1 1 1] end rotation
  (`GameplayStatics.SetGlobalTimeDilation` 1.0)
  (bind _outputvalue (`CustomTimeline.StartCustomTimeline` 2.0)
    (:`Update`
      (`SceneComponent.K2_SetRelativeRotation` _camera (`KismetMathLibrary.MakeRotator` _returnvalue_roll _returnvalue_pitch (`KismetMathLibrary.FClamp` (`KismetMathLibrary.Lerp` 180.0 0.0 (* _outputvalue 1.1)) 0.0 180.0)) false false)
      (`SceneComponent.K2_SetRelativeLocation` _camera (28.0 0.0 78.0) false false))
    (:`Finished`
      (set `CameraComponent.bUsePawnControlRotation` true (`/Game/BP/BP_PlayerChara.Camera` (`self.PlayerChara`)))
      (set `self.IsRotating` false))))