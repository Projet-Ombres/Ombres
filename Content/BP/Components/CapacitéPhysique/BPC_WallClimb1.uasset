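; Player character component for wall climbing: scaling walls, grabbing and climbing ledges, and propelling off walls.
; Each tick, forward and two downward hand sphere traces locate wall and ledge, triggering an upward velocity boost or a ledge climb based on pelvis height.
; Grabbing moves the capsule to the wall in Flying mode and feeds slope-corrected hand spots to the AnimBP.
; Wall propulsion applies an impulse along the wall normal and lerps control rotation.
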(event `self.ReceiveTick`
  (params (DeltaSeconds :type "Float (single-precision)"))
  ;[0.8469 0 1] Event Tick
  (if (`self.WasInitialized`)
    ;[1 1 1] PlayerChara Tracers
    (`self.ForwardTracer`)
    (`self.HeightTracer`)
    (`self.LerpControllerRotation` DeltaSeconds)))

(event `Initialize`
  (params (BP_PlayerChara :type "/Game/BP/BP_PlayerChara Object Reference"))
  ;[1 1 1] Initialize
  (bind _output_get (set `self.BP_PlayerChara` BP_PlayerChara))
  (set `self.WasInitialized` true)
  (set `self.AnimBP` (cast `/Game/TemporaryAsset/Anim/PlayerChara/AnimBP_PlayerChara` (`SkeletalMeshComponent.GetAnimInstance` (`Character.Mesh` _output_get)) :!pure true)))

(event `GrabLedge`
  (bind _animbp (`self.AnimBP`))
  (bind (_returnvalue_roll _returnvalue_pitch _returnvalue_yaw) (`KismetMathLibrary.BreakRotator` (`KismetMathLibrary.Conv_VectorToRotator` (`self.WallNormalOfWallToGrab`))))
  (bind (_returnvalue_roll_2 _returnvalue_pitch_2 _returnvalue_yaw_2) (`KismetMathLibrary.BreakRotator` (`Controller.GetControlRotation` (`GameplayStatics.GetPlayerController` 0))))
  ;[1 1 1] Grab Ledge
  (set `self.PlayerYaw` _returnvalue_yaw_2)
  (set `self.IsEscalatingWall` false)
  (set `/Game/TemporaryAsset/Anim/PlayerChara/AnimBP_PlayerChara.ClimbMontageStartTime` 0.0 _animbp)
  (message `/Game/BP/BPInterface_PlayerChara.CanGrab` _animbp true)
  (`CharacterMovementComponent.SetMovementMode` (`Character.CharacterMovement` (`self.BP_PlayerChara`)) "MOVE_Flying" 0)
  (set `self.IsHanging` true)
  (`KismetSystemLibrary.MoveComponentTo` (`Character.CapsuleComponent` (`self.BP_PlayerChara`)) (`self.MoveTo`) (`KismetMathLibrary.MakeRotator` _returnvalue_roll _returnvalue_pitch (- _returnvalue_yaw 180.0)) false false 0.13)
  (`MovementComponent.StopMovementImmediately` (`Character.CharacterMovement` (`self.BP_PlayerChara`)))
  (`self.ClimbLedge`))

(event `EscalateWall`
  (bind _bp_playerchara (`self.BP_PlayerChara`))
  (bind (_returnvalue_x _returnvalue_y _returnvalue_z) (`KismetMathLibrary.BreakVector` (`Actor.K2_GetActorLocation` (`self.BP_PlayerChara`))))
  (bind _bpc_skywalk (`/Game/BP/BP_PlayerChara.BPC_SkyWalk` _bp_playerchara))
  (bind _bpc_wallrun (`/Game/BP/BP_PlayerChara.BPC_WallRun` _bp_playerchara))
  (bind _charactermovement (`Character.CharacterMovement` (`self.BP_PlayerChara`)))
  (bind _lastplatformspawned (`/Game/BP/Components/Pouvoirs/BPC_SkyWalk.LastPlatformSpawned` _bpc_skywalk))
  ;[1 1 1] Escalate Wall
  (set `Pawn.bUseControllerRotationYaw` false (`self.BP_PlayerChara`))
  (if (`self.HaveToEscalateWall`)
    (if (not (`self.IsPropulsed`))
      (set `self.ClimbStartHeight` _returnvalue_z)
      (set `self.IsEscalatingWall` true)
      (if (`/Game/BP/Components/CapacitéPhysique/BPC_WallRun.IsWallRunning` _bpc_wallrun)
        (`/Game/BP/Components/CapacitéPhysique/BPC_WallRun.StopWallRun` _bpc_wallrun))
      (`/Game/BP/Components/Pouvoirs/BPC_SkyWalk.EndskyWalk` _bpc_skywalk)
      (`/Engine/EditorBlueprintResources/StandardMacros.IsValid` _lastplatformspawned
        (:`Is Valid`
          (`Actor.K2_DestroyActor` _lastplatformspawned))
        (:`Is Not Valid`
          _))
      (set `MovementComponent.Velocity` (0.0 0.0 0.0) _charactermovement)
      (set `MovementComponent.Velocity` (`KismetMathLibrary.MakeVector` 0.0 0.0 (`self.EscalateImpulse`)) _charactermovement))))

(event `ClimbLedge`
  ;[1 1 1] Climb Ledge
  (if (not (`self.IsClimbingLedge`))
    (message `/Game/BP/BPInterface_PlayerChara.ClimbLedgeI` (`SkeletalMeshComponent.GetAnimInstance` (`Character.Mesh` (`self.BP_PlayerChara`))) true)
    (`CharacterMovementComponent.SetMovementMode` (`Character.CharacterMovement` (`self.BP_PlayerChara`)) "MOVE_Flying" 0)
    (set `self.IsClimbingLedge` true)
    (set `self.IsHanging` false)))

(event `/Game/BP/BPInterface_PlayerChara.ClimbLedgeI`
  (params (IsClimbing :type Boolean))
  ;[1 1 1] Climb ledge interface
  (set `self.IsClimbingLedge` IsClimbing)
  (`CharacterMovementComponent.SetMovementMode` (`Character.CharacterMovement` (`self.BP_PlayerChara`)) "MOVE_Walking" 0)
  (`/Game/BP/BP_PlayerChara.ResetValuesAfterLanding` (`self.BP_PlayerChara`)))

(event `WallPropulsion`
  ;[1 1 1] WallPropulsion
  (set `Pawn.bUseControllerRotationYaw` true (`self.BP_PlayerChara`))
  (set `self.IsClimbingLedge` false)
  (set `self.IsEscalatingWall` false)
  (set `self.IsPropulsed` true)
  (`CharacterMovementComponent.AddImpulse` (`Character.CharacterMovement` (`self.BP_PlayerChara`)) (+ (* (`self.WallNormalOfWallToGrab`) (`self.HorizontalPropulsionPower`)) (* (`KismetMathLibrary.Vector_Up`) (`self.UpPropulsionPower`))) false)
  (set `self.SetControllerLerpRotation` true)
  (`KismetSystemLibrary.Delay` (`self.LerpRotationMeshDurationMAX`))
  (set `self.SetControllerLerpRotation` false)
  (set `self.IsPropulsed` false))

(event `LerpControllerRotation`
  (params (DeltaTick :type "Float (double-precision)"))
  ;[1 1 1] Set Controller rotation
  (if (`self.SetControllerLerpRotation`)
    (set `self.LerpRotationMeshDuration` (+ (`self.LerpRotationMeshDuration`) DeltaTick))
    (`Controller.SetControlRotation` (`GameplayStatics.GetPlayerController` 0) (`KismetMathLibrary.RLerp` (`Actor.K2_GetActorRotation` (`GameplayStatics.GetPlayerController` 0)) (`KismetMathLibrary.FindLookAtRotation` (`KismetMathLibrary.Vector_Zero`) (`self.WallNormalOfWallToGrab`)) (/ (`self.LerpRotationMeshDuration`) (`self.LerpRotationMeshDurationMAX`)) true))
    (else
      (set `self.LerpRotationMeshDuration` 0.0))))

(fn `CalculateHandRotations`
  (returns (LeftHandRotY :type "Float (double-precision)") (RightHandRotY :type "Float (double-precision)"))
  (bind _bp_playerchara (`self.BP_PlayerChara`))
  (bind _lefthandnormal (`self.LeftHandNormal`))
  (bind _righthandnormal (`self.RightHandNormal`))
  (return (* (`KismetMathLibrary.DegAcos` (`KismetMathLibrary.Dot_VectorVector` (`KismetMathLibrary.Vector_Up`) _lefthandnormal)) (* (`KismetMathLibrary.SignOfFloat` (`KismetMathLibrary.Dot_VectorVector` _lefthandnormal (`Actor.GetActorRightVector` _bp_playerchara))) -1.0)) (* (`KismetMathLibrary.DegAcos` (`KismetMathLibrary.Dot_VectorVector` (`KismetMathLibrary.Vector_Up`) _righthandnormal)) (`KismetMathLibrary.SignOfFloat` (`KismetMathLibrary.Dot_VectorVector` (`Actor.GetActorRightVector` _bp_playerchara) _righthandnormal)))))

(fn `ClampCamera`
  (params (Value :type "Float (double-precision)"))
  (returns (AllowedToTurn :type Boolean))
  (bind (_relativerotation_roll _relativerotation_pitch _relativerotation_yaw) (`KismetMathLibrary.BreakRotator` (`SceneComponent.RelativeRotation` (`/Game/BP/BP_PlayerChara.Camera` (`self.BP_PlayerChara`)))))
  (bind _returnvalue (+ Value _relativerotation_yaw))
  (return (or (or (and (> Value 0.0) (< _returnvalue (* (`self.CameraAngleAllowed`) 0.5))) (and (< Value 0.0) (>= _returnvalue (* (`self.CameraAngleAllowed`) -0.5)))) (not (`self.IsEscalatingWall`)))))

(fn `CorrectHandPosition`
  (params (LeftHandRotY :type "Float (double-precision)") (RightHandRotY :type "Float (double-precision)"))
  (returns (LeftHandPos :type "Vector Structure") (RightHandPos :type "Vector Structure"))
  (locals (LHP :type "Vector Structure") (RHP :type "Vector Structure"))
  (set `local.LHP` (`self.LeftHandSpotToGrab`))
  (set `local.RHP` (`self.RightHandSpotToGrab`))
  (if (>= LeftHandRotY 0.0)
    (set `local.LHP` (- (`self.LeftHandSpotToGrab`) (`KismetMathLibrary.MakeVector` 0.0 0.0 (* (`KismetMathLibrary.Abs` LeftHandRotY) (`self.HandPositionCorrectionMultiplier`))))))
  (if (>= RightHandRotY 0.0)
    (set `local.RHP` (- (`self.RightHandSpotToGrab`) (`KismetMathLibrary.MakeVector` 0.0 0.0 (* (`KismetMathLibrary.Abs` RightHandRotY) (`self.HandPositionCorrectionMultiplier`))))))
  (return (`local.LHP`) (`local.RHP`)))

(fn `ForwardTracer`
  (bind _returnvalue (`SceneComponent.K2_GetComponentLocation` (`/Game/BP/BP_PlayerChara.HorizontalTracerRepère` (`self.BP_PlayerChara`))))
  (bind (_velocity_x _velocity_y _velocity_z) (`KismetMathLibrary.BreakVector` (`MovementComponent.Velocity` (`Character.CharacterMovement` (`self.BP_PlayerChara`)))))
  (bind (_outhit _returnvalue_2) (`KismetSystemLibrary.SphereTraceSingle` :`Start` _returnvalue :`End` (+ (* (`KismetMathLibrary.GetForwardVector` (`Actor.K2_GetActorRotation` (`self.BP_PlayerChara`))) 85.0) _returnvalue) :`Radius` 20.0 :`TraceChannel` "TraceTypeQuery3" :`DrawDebugType` "ForOneFrame" :`DrawTime` 0.5))
  (if _returnvalue_2
    (set `self.TracerHorizontallyTriggered` true)
    (set `self.WallLocationOfWallToGrab` (`.Location` (`GameplayStatics.BreakHitResult` _outhit)))
    (set `self.WallNormalOfWallToGrab` (`.Normal` (`GameplayStatics.BreakHitResult` _outhit)))
    (if (!= _velocity_z 0.0)
      (if (`self.IsClimbingLedge`)
        _
        (elif (`self.IsEscalatingWall`)
          _
          (elif (`NavMovementComponent.IsFalling` (`Character.CharacterMovement` (`self.BP_PlayerChara`)))
            (if (`self.IsPropulsed`)
              _
              (elif (and (`self.LeftHandTracerTriggered`) (`self.RightHandTracerTriggered`))
                (`self.EscalateWall`)))))))
    (else
      (set `self.TracerHorizontallyTriggered` false))))

(fn `HeightTracer`
  (locals (StartTracePoint :type "Vector Structure") (EndTracePoint :type "Vector Structure") (TempVector :type "Vector Structure"))
  (bind (_returnvalue_x _returnvalue_y _returnvalue_z) (`KismetMathLibrary.BreakVector` (`self.MoveTo`)))
  (bind (_lefthandspottograb_x _lefthandspottograb_y _lefthandspottograb_z) (`KismetMathLibrary.BreakVector` (`self.LeftHandSpotToGrab`)))
  (bind (_righthandspottograb_x _righthandspottograb_y _righthandspottograb_z) (`KismetMathLibrary.BreakVector` (`self.RightHandSpotToGrab`)))
  (bind (_returnvalue_x_2 _returnvalue_y_2 _returnvalue_z_2) (`KismetMathLibrary.BreakVector` (`Actor.K2_GetActorLocation` (`self.BP_PlayerChara`))))
  (bind (_returnvalue_x_3 _returnvalue_y_3 _returnvalue_z_3) (`KismetMathLibrary.BreakVector` (`Actor.K2_GetActorLocation` (`self.BP_PlayerChara`))))
  (bind (_returnvalue_x_4 _returnvalue_y_4 _returnvalue_z_4) (`KismetMathLibrary.BreakVector` (`SceneComponent.GetSocketLocation` (`Character.Mesh` (`self.BP_PlayerChara`)) "pelvisSocket")))
  (bind _returnvalue (+ (`KismetMathLibrary.MakeVector` _returnvalue_x_3 _returnvalue_y_3 (+ _returnvalue_z_3 470.0)) (* (`KismetMathLibrary.GetForwardVector` (`Actor.K2_GetActorRotation` (`self.BP_PlayerChara`))) 85.0)))
  (set `local.StartTracePoint` _returnvalue)
  (set `local.EndTracePoint` (`KismetMathLibrary.MakeVector` (.x _returnvalue) (.y _returnvalue) (- (.z _returnvalue) 470.0)))
  (`|ExecutionSequence`
    (:`then_0`
      (bind _output_get (set `local.TempVector` (* (`Actor.GetActorRightVector` (`self.BP_PlayerChara`)) (`self.SideTracersOffset`))))
      (bind (_outhit _returnvalue_2) (`KismetSystemLibrary.SphereTraceSingle` :`Start` (+ _output_get (`local.StartTracePoint`)) :`End` (+ (`local.EndTracePoint`) (`local.TempVector`)) :`Radius` 15.0 :`TraceChannel` "TraceTypeQuery3" :`DrawDebugType` "ForOneFrame" :`TraceColor` (struct :`R` 0.007688 :`B` 1.0 :`A` 1.0))) ; Right tracer
      (bind _output_get_2 (set `self.RightHandTracerTriggered` _returnvalue_2))
      (if _output_get_2
        (set `self.RightHandSpotToGrab` (`.ImpactPoint` (`GameplayStatics.BreakHitResult` _outhit)))
        (set `self.RightHandNormal` (`.ImpactNormal` (`GameplayStatics.BreakHitResult` _outhit)))))
    (:`then_1`
      (bind (_outhit_2 _returnvalue_3) (`KismetSystemLibrary.SphereTraceSingle` :`Start` (- (`local.StartTracePoint`) (`local.TempVector`)) :`End` (- (`local.EndTracePoint`) (`local.TempVector`)) :`Radius` 15.0 :`TraceChannel` "TraceTypeQuery3" :`DrawDebugType` "ForOneFrame" :`TraceColor` (struct :`G` 0.797142 :`B` 1.0 :`A` 1.0))) ; left tracer
      (bind _output_get_3 (set `self.LeftHandTracerTriggered` _returnvalue_3))
      (if _output_get_3
        (bind _output_get_4 (set `self.LeftHandSpotToGrab` (`.ImpactPoint` (`GameplayStatics.BreakHitResult` _outhit_2))))
        (set `self.LeftHandNormal` (`.ImpactNormal` (`GameplayStatics.BreakHitResult` _outhit_2)))
        (set `self.HeightLocationOfWallToGrab` (/ (+ _output_get_4 (`self.RightHandSpotToGrab`)) 2.0))
        (if (or (`KismetMathLibrary.InRange_FloatFloat` (- _returnvalue_z_4 _lefthandspottograb_z) -50.0 100.0) (`KismetMathLibrary.InRange_FloatFloat` (- _returnvalue_z_4 _righthandspottograb_z) -50.0 100.0))
          (set `self.HaveToEscalateWall` false)
          (if (not (`self.IsClimbingLedge`))
            (bind (_lefthandroty _righthandroty) (`self.CalculateHandRotations`))
            (bind (_lefthandpos _righthandpos) (`self.CorrectHandPosition` _lefthandroty _righthandroty))
            (`/Game/TemporaryAsset/Anim/PlayerChara/AnimBP_PlayerChara.UpdateHandSpots` (`self.AnimBP`) _lefthandpos _righthandpos (`KismetMathLibrary.MakeRotator` 0.0 _lefthandroty) (`KismetMathLibrary.MakeRotator` 0.0 _righthandroty))
            (if (`self.IsEscalatingWall`)
              (`self.GrabLedge`)
              (elif (`self.IsHanging`)
                _
                (elif (`/Game/BP/BP_PlayerChara.JumpButtonWasPressed` (`self.BP_PlayerChara`))
                  (set `/Game/TemporaryAsset/Anim/PlayerChara/AnimBP_PlayerChara.ClimbMontageStartTime` (`KismetMathLibrary.FClamp` (/ (`KismetMathLibrary.Abs` (- _returnvalue_z _returnvalue_z_2)) 200.0)) (`self.AnimBP`))
                  (set `self.IsEscalatingWall` false)
                  (set `self.IsHanging` true)
                  (`self.ClimbLedge`)))))
          (else
            (set `self.HaveToEscalateWall` true)))))))