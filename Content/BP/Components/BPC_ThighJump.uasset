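; Character component for a "thigh jump", a vault over obstacles tagged ThighJump that grants a landing speed boost.
; Each tick after initialization, a forward sphere trace finds the wall and toggles the jump-assist UI, and a downward trace finds ledge height.
; JumpThigh moves the capsule up, then across by a distance-scaled offset, and restores clamped pre-jump velocity.
; Tick then lerps boosted walk speed back to normal on a timer.
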(event `Initialize`
  (params (BP_chara :type "/Game/BP/BP_PlayerChara Object Reference"))
  ;[1 1 1] Initialize
  (set `self.BP_Chara` BP_chara)
  (set `self.WasInitialized` true))

(event `self.ReceiveTick`
  (params (DeltaSeconds :type "Float (single-precision)"))
  ;[1 0 0.7992] Event tick
  (set `self.DeltaSec` DeltaSeconds)
  (if (`self.WasInitialized`)
    (`self.HorizontalTracer`)
    (`self.VerticalTracer`)
    ;[1 1 1] Lerp Walk speed after boost
    (if (> (`CharacterMovementComponent.MaxWalkSpeed` (`Character.CharacterMovement` (`self.BP_Chara`))) 900.0)
      (set `self.Timer` (- (`self.Timer`) (`self.DeltaSec`)))
      (`self.LerpWalkSpeed`)
      (else
        (set `self.Timer` (`self.TimerMax`))))))

(event `JumpThigh`
  (bind _bp_chara (`self.BP_Chara`))
  (bind _bp_chara_2 (`self.BP_Chara`))
  (bind _bp_chara_3 (`self.BP_Chara`))
  (bind (_ledge_height_location_x _ledge_height_location_y _ledge_height_location_z) (`KismetMathLibrary.BreakVector` (`self.Ledge height location`)))
  (bind _bp_chara_4 (`self.BP_Chara`))
  (bind _returnvalue (+ _ledge_height_location_z 5.0))
  (bind (_returnvalue_x _returnvalue_y) (`KismetMathLibrary.BreakVector` (`SceneComponent.K2_GetComponentLocation` (`Character.CapsuleComponent` (`self.BP_Chara`)))))
  ;[1 1 1] Jump thigh
  (set `self.CharaVelocityBeforeJump` (`Actor.GetVelocity` (`self.BP_Chara`)))
  (set `self.ThighJumping` true)
  (`KismetSystemLibrary.MoveComponentTo` (`Character.CapsuleComponent` _bp_chara_2) (`KismetMathLibrary.MakeVector` _returnvalue_x _returnvalue_y _returnvalue) (`Actor.K2_GetActorRotation` _bp_chara_2) false false 0.05 true)
  (bind _lerpvaluedistance (`self.ReturnVectorMultiplier(withLerp)XY`))
  (bind (_returnvalue_x_2 _returnvalue_y_2) (`KismetMathLibrary.BreakVector` (+ (* (* (`self.WallNormal`) _lerpvaluedistance) -1.0) (`SceneComponent.K2_GetComponentLocation` (`Character.CapsuleComponent` (`self.BP_Chara`))))))
  (`KismetSystemLibrary.MoveComponentTo` (`Character.CapsuleComponent` _bp_chara_4) (`KismetMathLibrary.MakeVector` _returnvalue_x_2 _returnvalue_y_2 _returnvalue) (`Actor.K2_GetActorRotation` _bp_chara_4) false false 0.4 true)
  (set `self.ThighJumping` false)
  (set `MovementComponent.Velocity` (`KismetMathLibrary.ClampVectorSize` (`self.CharaVelocityBeforeJump`) 0.0 900.0) (`Character.CharacterMovement` _bp_chara))
  (`/Game/BP/BP_PlayerChara.ResetValuesAfterLanding` _bp_chara)
  (set `CharacterMovementComponent.MaxWalkSpeed` (`self.LandingBoostMaxWalkSpeed`) (`Character.CharacterMovement` _bp_chara_3))
  (set `/Game/BP/BP_PlayerChara.SpeedMultiplier` 100.0 _bp_chara_3)
  (set `/Game/BP/BP_PlayerChara.SpeedMultiplier` 1.0 (`self.BP_Chara`)))

(event `LerpWalkSpeed`
  (bind _landingboostmaxwalkspeed (`self.LandingBoostMaxWalkSpeed`))
  ;[1 1 1] Lerp walk speed
  (set `CharacterMovementComponent.MaxWalkSpeed` (`KismetMathLibrary.FClamp` (`KismetMathLibrary.Lerp` 900.0 _landingboostmaxwalkspeed (`KismetMathLibrary.FClamp` (/ (`self.Timer`) (`self.TimerMax`)))) 900.0 _landingboostmaxwalkspeed) (`Character.CharacterMovement` (`self.BP_Chara`))))

(fn `HorizontalTracer`
  (bind _returnvalue (`SceneComponent.K2_GetComponentLocation` (`/Game/BP/BP_PlayerChara.ThighJumpRepère` (`self.BP_Chara`))))
  (bind (_returnvalue_x _returnvalue_y _returnvalue_z) (`KismetMathLibrary.BreakVector` (`KismetMathLibrary.GetForwardVector` (`Actor.K2_GetActorRotation` (`self.BP_Chara`)))))
  (set `self.HorizontalTracerTriggered` false)
  (`/Game/BP/Widgets/Widget_MainInterface.ToggleJumpAssist` (`/Game/BP/BP_GameInstance.MainInterface` (cast `/Game/BP/BP_GameInstance` (`GameplayStatics.GetGameInstance`) :!pure true)) false)
  (if (not (`self.ThighJumping`))
    (bind (_outhit _returnvalue_2) (`KismetSystemLibrary.SphereTraceSingle` _returnvalue (+ (`KismetMathLibrary.MakeVector` (* _returnvalue_x 300.0) (* _returnvalue_y 300.0) _returnvalue_z) _returnvalue) 10.0 "TraceTypeQuery5"))
    (if _returnvalue_2
      (if (`Actor.ActorHasTag` (`.HitActor` (`GameplayStatics.BreakHitResult` _outhit)) "ThighJump")
        (set `self.HorizontalTracerTriggered` true)
        (set `self.WallNormal` (`.Normal` (`GameplayStatics.BreakHitResult` _outhit)))
        (set `self.WallLocation` (`.Location` (`GameplayStatics.BreakHitResult` _outhit)))
        (if (> (`KismetMathLibrary.VSize` (`Actor.GetVelocity` (`self.BP_Chara`))) 100.0)
          (`/Game/BP/Widgets/Widget_MainInterface.ToggleJumpAssist` (`/Game/BP/BP_GameInstance.MainInterface` (cast `/Game/BP/BP_GameInstance` (`GameplayStatics.GetGameInstance`) :!pure true)) true))))))

(fn `ReturnVectorMultiplier(withLerp)XY`
  (returns (LerpValuedistance :type "Float (double-precision)"))
  (if (> (`KismetMathLibrary.Vector_Distance2D` (`self.WallLocation`) (`SceneComponent.K2_GetComponentLocation` (`Character.CapsuleComponent` (`self.BP_Chara`)))) 100.0)
    (return (`KismetMathLibrary.Lerp` 650.0 800.0 (`self.Normalize to range`)))
    (else
      (return (`KismetMathLibrary.Lerp` 370.0 460.0 (`self.Normalize to range`))))))

(fn `VerticalTracer`
  (bind (_walllocation_x _walllocation_y _walllocation_z) (`KismetMathLibrary.BreakVector` (`self.WallLocation`)))
  (bind (_returnvalue_x _returnvalue_y) (`KismetMathLibrary.BreakVector` (* (`KismetMathLibrary.GetForwardVector` (`Actor.K2_GetActorRotation` (`self.BP_Chara`))) 30.0)))
  (bind _returnvalue (+ (`KismetMathLibrary.MakeVector` _walllocation_x _walllocation_y (+ _walllocation_z 100.0)) (`KismetMathLibrary.MakeVector` _returnvalue_x _returnvalue_y)))
  (if (`self.HorizontalTracerTriggered`)
    (if (not (`self.ThighJumping`))
      (bind (_outhit _returnvalue_2) (`KismetSystemLibrary.SphereTraceSingle` :`Start` _returnvalue :`End` (`KismetMathLibrary.MakeVector` (.x _returnvalue) (.y _returnvalue) (- (.z _returnvalue) 100.0)) :`Radius` 10.0 :`TraceChannel` "TraceTypeQuery5" :`TraceHitColor` (struct :`G` 0.79842 :`B` 1.0 :`A` 1.0)))
      (if _returnvalue_2
        (set `self.Ledge height location` (`.Location` (`GameplayStatics.BreakHitResult` _outhit)))))))