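; Skywalk ability component that lays platforms along the player's path for a timed duration, then enters cooldown.
; While active, Tick spawns a BP_SkywalkPlatform just below the mesh location whenever it moves over 100 units, oriented to the camera with clamped pitch.
; Each platform has Destroy called right after spawning.
; Tick also accumulates the cooldown timer, re-arming the ability and printing a ready message at the maximum.
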(event `Initialize`
  (params (`Player Ref` :type "/Game/BP/BP_PlayerChara Object Reference"))
  ;[1 1 1] Initialize
  (set `self.Player Ref` `Player Ref`))

(event `SkyWalk`
  (params (DeltaSeconds :type "Float (double-precision)"))
  ;[1 1 1] SkyWalk
  (if (`self.CooldownReay`)
    (set `self.CoolDownValue` 0.0)
    (set `self.CooldownReay` false)
    (set `self.Sky Walk Is Active?` true)
    (set `self.Last position` (`SceneComponent.K2_GetComponentLocation` (`Character.Mesh` (`self.Player Ref`))))
    (`KismetSystemLibrary.Delay` (`self.Sky Walk Duration`))
    (`self.EndskyWalk`)))

(event `self.ReceiveTick`
  (params (DeltaSeconds :type "Float (single-precision)"))
  (bind _camera (`/Game/BP/BP_PlayerChara.Camera` (`self.Player Ref`)))
  (bind _mesh (`Character.Mesh` (`self.Player Ref`)))
  (bind (_returnvalue_roll _returnvalue_pitch _returnvalue_yaw) (`KismetMathLibrary.BreakRotator` (`SceneComponent.K2_GetComponentRotation` _camera)))
  (bind (_returnvalue_x _returnvalue_y _returnvalue_z) (`KismetMathLibrary.BreakVector` (+ (`SceneComponent.K2_GetComponentLocation` _mesh) (`SceneComponent.GetForwardVector` _camera))))
  ;[0.9197 0 1] Event Tick
  (`self.SetCoolDownTimer` DeltaSeconds)
  (if (`self.Sky Walk Is Active?`)
    (if (> (`KismetMathLibrary.VSize` (- (`self.Last position`) (`SceneComponent.K2_GetComponentLocation` (`Character.Mesh` (`self.Player Ref`))))) 100.0)
      (set `self.Last position` (`SceneComponent.K2_GetComponentLocation` _mesh))
      (bind _returnvalue (`|SpawnActorFromClass` "/Game/BP/Class/BP_SkywalkPlatform.BP_SkywalkPlatform_C" (`KismetMathLibrary.MakeTransform` (`KismetMathLibrary.MakeVector` _returnvalue_x _returnvalue_y (- _returnvalue_z 13.0)) (`KismetMathLibrary.MakeRotator` _returnvalue_roll (`KismetMathLibrary.FClamp` _returnvalue_pitch -40.0 40.0) _returnvalue_yaw)) "Undefined" "OverrideRootScale" null null))
      (set `self.LastPlatformSpawned` _returnvalue)
      (`/Game/BP/Class/BP_SkywalkPlatform.Destroy` _returnvalue))))

(event `EndskyWalk`
  ;[1 1 1] End skywalk
  (set `self.Sky Walk Is Active?` false)
  (set `self.OnCoolDown` true)
  (set `self.CooldownReay` false))

(event `SetCoolDownTimer`
  (params (DeltaTime :type "Float (double-precision)"))
  ;[1 1 1] SetCooldown value
  (if (`self.OnCoolDown`)
    (bind _output_get (set `self.CoolDownValue` (+ (`self.CoolDownValue`) DeltaTime)))
    (if (>= _output_get (`self.MaxCooldownNeeded`))
      (set `self.OnCoolDown` false)
      (set `self.CooldownReay` true)
      (`KismetSystemLibrary.PrintString` "Skywalk Ready")
      (else
        (set `self.OnCoolDown` true)
        (set `self.CooldownReay` false)))))