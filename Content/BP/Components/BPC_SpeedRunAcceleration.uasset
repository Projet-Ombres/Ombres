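; Player component that grants a speed-run boost after sustained running and widens the camera FOV with speed.
; Initialize stores the player reference along with its base walk speed and FOV.
; Tick lerps FOV by current velocity and times how long speed stays above a threshold.
; Passing the required time raises MaxWalkSpeed; dropping below the threshold resets the timer and restores base speed, with debug prints on both transitions.
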(event `LerpFOV`
  ;[1 1 1] LERPFOV
  (`CameraComponent.SetFieldOfView` (`/Game/BP/BP_PlayerChara.Camera` (`self.Playerchara`)) (`KismetMathLibrary.Lerp` (`self.FOVBase`) (`self.MaxFOV`) (/ (`self.PlayerSpeed`) 1500.0))))

(event `Initialize`
  (params (Player :type "/Game/BP/BP_PlayerChara Object Reference"))
  ;[1 1 1] Initialize
  (bind _output_get (set `self.Playerchara` Player))
  (set `self.MaxWalkSpeedBase` (`CharacterMovementComponent.MaxWalkSpeed` (`Character.CharacterMovement` _output_get)))
  (set `self.FOVBase` (`CameraComponent.FieldOfView` (`/Game/BP/BP_PlayerChara.Camera` _output_get))))

(event `StartAcceleration`
  ;[1 1 1] Start acceleration
  (set `self.AccelerationStarted` true)
  (set `CharacterMovementComponent.MaxWalkSpeed` 900.0 (`Character.CharacterMovement` (`self.Playerchara`)))
  (`KismetSystemLibrary.PrintString` "AccelerationStarted"))

(event `StopAcceleration`
  ;[1 1 1] End acceleration
  (set `self.AccelerationStarted` false)
  (set `CharacterMovementComponent.MaxWalkSpeed` (`self.MaxWalkSpeedBase`) (`Character.CharacterMovement` (`self.Playerchara`)))
  (`KismetSystemLibrary.PrintString` "Acceleration Stopped"))

(event `self.ReceiveTick`
  (params (DeltaSeconds :type "Float (single-precision)"))
  ;[1 1 1] Event tick
  (bind _output_get (set `self.PlayerSpeed` (`KismetMathLibrary.VSize` (`MovementComponent.Velocity` (`Character.CharacterMovement` (`self.Playerchara`))))))
  (`self.LerpFOV`)
  (if (>= _output_get 800.0)
    (bind _output_get_2 (set `self.RunningTime` (+ (`self.RunningTime`) DeltaSeconds)))
    (if (>= _output_get_2 (`self.TimeRunninBeforeAcceleration`))
      (if (not (`self.AccelerationStarted`))
        (`self.StartAcceleration`)))
    (else
      (set `self.RunningTime` 0.0)
      (if (`self.AccelerationStarted`)
        (`self.StopAcceleration`)))))