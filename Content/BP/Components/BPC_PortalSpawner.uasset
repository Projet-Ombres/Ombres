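; BPC_PortalSpawner is a component for BP_PlayerChara that spawns and opens a BP_Portal beneath the player.
; SpawnPortal places the portal a given distance below the player's location, guarded by a check on the stored portal reference.
; It sets the portal's box to overlap all channels, calls OpenPortal, and briefly raises the player's PortalOpen flag, clearing it after a short delay.
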(event `self.ReceiveBeginPlay`
  (bind _asbp_player_chara (cast `/Game/BP/BP_PlayerChara` (`self.GetOwner`)))
  (set `self.PlayerChara` _asbp_player_chara))

(event `SpawnPortal`
  (params (SpawnDistance :type "Float (double-precision)"))
  (if (== (`self.SpawnedPortal`) null)
    (bind _returnvalue (`|SpawnActorFromClass` "/Game/BP/Class/Portal/BP_Portal.BP_Portal_C" (`KismetMathLibrary.MakeTransform` (`KismetMathLibrary.MakeVector` (.x (`Actor.K2_GetActorLocation` (`self.PlayerChara`))) (.y (`Actor.K2_GetActorLocation` (`self.PlayerChara`))) (- (.z (`Actor.K2_GetActorLocation` (`self.PlayerChara`))) SpawnDistance))) "AlwaysSpawn" "OverrideRootScale" null null))
    (bind _output_get (set `self.SpawnedPortal` _returnvalue))
    (bind _box (`/Game/BP/Class/Portal/BP_Portal.Box` _output_get))
    (`PrimitiveComponent.SetCollisionEnabled` _box "QueryAndPhysics")
    (`PrimitiveComponent.SetCollisionResponseToAllChannels` _box "ECR_Overlap")
    (set `/Game/BP/BP_PlayerChara.PortalOpen` true (`self.PlayerChara`))
    (`/Game/BP/Class/Portal/BP_Portal.OpenPortal` _output_get)
    (`KismetSystemLibrary.Delay` 0.2)
    (set `/Game/BP/BP_PlayerChara.PortalOpen` false (`self.PlayerChara`))))