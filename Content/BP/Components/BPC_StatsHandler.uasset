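; Component that tracks the player's speedrun time and per-level gameplay stats, such as movement, ability usage and speed.
; Tick runs the timer only between StartTimer and StopTimer, while a looping one-second timer samples player velocity into a running average and maximum.
; ArchiveStats stores current stats in a map keyed by level name, which GetTotalSessionTime sums with the current timer.
; SaveStats and LoadStats copy everything to and from the GameInstance's SaveGame object.
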(event `RegisterCurrentSpeed`
  (bind _returnvalue (`KismetMathLibrary.VSize` (`Actor.GetVelocity` (`GameplayStatics.GetPlayerCharacter` 0))))
  (`/Engine/EditorBlueprintResources/StandardMacros.IncrementInt` (`self.SpeedsRegistered`)
    (:`  `
      (set `self.AverageSpeed` (/ (+ (* (`self.AverageSpeed`) (`KismetMathLibrary.Conv_IntToDouble` (- (`self.SpeedsRegistered`) 1))) _returnvalue) (`KismetMathLibrary.Conv_IntToDouble` (`self.SpeedsRegistered`))))
      (if (> _returnvalue (`self.MaxSpeedReached`))
        (set `self.MaxSpeedReached` _returnvalue)))))

(event `self.ReceiveBeginPlay`
  (`self.SetComponentTickEnabled` false)
  (`KismetSystemLibrary.K2_SetTimerDelegate` (delegate `RegisterCurrentSpeed`) 1.0 true))

(event `StartTimer`
  (set `self.CurrentSpeedrunTimer` 0.0)
  (set `self.TimerStarted` true)
  (`self.SetComponentTickEnabled` true))

(event `StopTimer`
  (`self.SetComponentTickEnabled` false)
  (set `self.TimerStarted` false))

(event `self.ReceiveTick`
  (params (DeltaSeconds :type "Float (single-precision)"))
  (set `self.CurrentSpeedrunTimer` (+ (`self.CurrentSpeedrunTimer`) DeltaSeconds)))

(event `ArchiveStats`
  (params (Level :type "/Game/BP/Components/ELevelsNames Enum" :default "NewEnumerator0"))
  (set `self.SessionStatsPerLevel` (`/Game/BP/Libraries/BPL_Utilities.SetMapElement` (`self.SessionStatsPerLevel`) (`|GetEnumeratorNameAsString` Level) (make `/Game/BP/Class/PlayerLevelStats` (`self.CurrentSpeedrunTimer`) (`self.PortalsUsed`) (`self.RobotCatches`) (`self.SkywalksUsed`) (`self.CristallisationsUsed`) (`self.PingsUsed`) (`self.JumpsUsed`) (`self.SlidesUsed`) (`self.TotalSlideDuration`) (`self.WallrunsUsed`) (`self.TotalWallrunDuration`) (`self.MaxSpeedReached`) (`self.AverageSpeed`) (`self.LedgesClimbed`) (`self.PullbarsGrabbed`) (`self.WallJumps`) (`self.MechanismsParalysed`) (`self.SpellsUsed`)))))

(event `ResetCurrentLevelStats`
  (set `self.CurrentSpeedrunTimer` 0.0)
  (set `self.PortalsUsed` 0)
  (set `self.RobotCatches` 0)
  (set `self.SkywalksUsed` 0)
  (set `self.CristallisationsUsed` 0)
  (set `self.PingsUsed` 0)
  (set `self.JumpsUsed` 0)
  (set `self.SlidesUsed` 0)
  (set `self.TotalSlideDuration` 0.0)
  (set `self.WallrunsUsed` 0)
  (set `self.TotalWallrunDuration` 0.0)
  (set `self.MaxSpeedReached` 0.0)
  (set `self.AverageSpeed` 0.0)
  (set `self.LedgesClimbed` 0)
  (set `self.PullbarsGrabbed` 0)
  (set `self.WallJumps` 0)
  (set `self.MechanismsParalysed` 0)
  (set `self.SpellsUsed` 0)
  (set `self.SpeedsRegistered` 0))

(fn `GetTotalSessionTime`
  (returns (Time :type "Float (double-precision)"))
  (locals (Total :type "Float (double-precision)"))
  (bind _values (`BlueprintMapLibrary.Map_Values` (`self.SessionStatsPerLevel`)))
  (for _array_element _values
    (set `local.Total` (+ (`.Time_2_7E7EC9D24B627E3A676216884A253355` (break `/Game/BP/Class/PlayerLevelStats` _array_element)) (`local.Total`))))
  (return (+ (`local.Total`) (`self.CurrentSpeedrunTimer`))))

(fn `LoadStats`
  (locals (SaveGame :type "/Game/BP/Class/BP_SaveGame Object Reference"))
  (bind _asbp_game_instance (cast `/Game/BP/BP_GameInstance` (`GameplayStatics.GetGameInstance`)))
  (set `local.SaveGame` (`/Game/BP/BP_GameInstance.SaveGame` _asbp_game_instance))
  (set `self.CurrentSpeedrunTimer` (`/Game/BP/Class/BP_SaveGame.CurrentTimer` (`local.SaveGame`)))
  (set `self.SessionStatsPerLevel` (`/Game/BP/Class/BP_SaveGame.SessionTimes` (`local.SaveGame`)))
  (set `self.PortalsUsed` (`/Game/BP/Class/BP_SaveGame.PortalsUsed` (`local.SaveGame`)))
  (set `self.RobotCatches` (`/Game/BP/Class/BP_SaveGame.RobotCatches` (`local.SaveGame`)))
  (set `self.SkywalksUsed` (`/Game/BP/Class/BP_SaveGame.SkywalksUsed` (`local.SaveGame`)))
  (set `self.CristallisationsUsed` (`/Game/BP/Class/BP_SaveGame.CristallisationsUsed` (`local.SaveGame`)))
  (set `self.PingsUsed` (`/Game/BP/Class/BP_SaveGame.PingsUsed` (`local.SaveGame`)))
  (set `self.JumpsUsed` (`/Game/BP/Class/BP_SaveGame.JumpsUsed` (`local.SaveGame`)))
  (set `self.SlidesUsed` (`/Game/BP/Class/BP_SaveGame.SlidesUsed` (`local.SaveGame`)))
  (set `self.TotalSlideDuration` (`/Game/BP/Class/BP_SaveGame.TotalSlideDuration` (`local.SaveGame`)))
  (set `self.WallrunsUsed` (`/Game/BP/Class/BP_SaveGame.WallrunsUsed` (`local.SaveGame`)))
  (set `self.TotalWallrunDuration` (`/Game/BP/Class/BP_SaveGame.TotalWallrunDuration` (`local.SaveGame`)))
  (set `self.MaxSpeedReached` (`/Game/BP/Class/BP_SaveGame.MaxSpeedReached` (`local.SaveGame`)))
  (set `self.AverageSpeed` (`/Game/BP/Class/BP_SaveGame.AverageSpeed` (`local.SaveGame`)))
  (set `self.LedgesClimbed` (`/Game/BP/Class/BP_SaveGame.LedgesClimbed` (`local.SaveGame`)))
  (set `self.PullbarsGrabbed` (`/Game/BP/Class/BP_SaveGame.PullbarsGrabbed` (`local.SaveGame`)))
  (set `self.WallJumps` (`/Game/BP/Class/BP_SaveGame.WallJumps` (`local.SaveGame`)))
  (set `self.MechanismsParalysed` (`/Game/BP/Class/BP_SaveGame.MechanismsParalysed` (`local.SaveGame`)))
  (set `self.SpellsUsed` (`/Game/BP/Class/BP_SaveGame.SpellsUsed` (`local.SaveGame`)))
  (set `self.SpeedsRegistered` (`/Game/BP/Class/BP_SaveGame.SpeedsRegistered` (`local.SaveGame`))))

(fn `SaveStats`
  (locals (SaveGame :type "/Game/BP/Class/BP_SaveGame Object Reference"))
  (bind _asbp_game_instance (cast `/Game/BP/BP_GameInstance` (`GameplayStatics.GetGameInstance`)))
  (bind _output_get (set `local.SaveGame` (`/Game/BP/BP_GameInstance.SaveGame` _asbp_game_instance)))
  (set `/Game/BP/Class/BP_SaveGame.CurrentTimer` (`self.CurrentSpeedrunTimer`) _output_get)
  (set `/Game/BP/Class/BP_SaveGame.SessionTimes` (`self.SessionStatsPerLevel`) (`local.SaveGame`))
  (set `/Game/BP/Class/BP_SaveGame.PortalsUsed` (`self.PortalsUsed`) (`local.SaveGame`))
  (set `/Game/BP/Class/BP_SaveGame.RobotCatches` (`self.RobotCatches`) (`local.SaveGame`))
  (set `/Game/BP/Class/BP_SaveGame.SkywalksUsed` (`self.SkywalksUsed`) (`local.SaveGame`))
  (set `/Game/BP/Class/BP_SaveGame.CristallisationsUsed` (`self.CristallisationsUsed`) (`local.SaveGame`))
  (set `/Game/BP/Class/BP_SaveGame.PingsUsed` (`self.PingsUsed`) (`local.SaveGame`))
  (set `/Game/BP/Class/BP_SaveGame.JumpsUsed` (`self.JumpsUsed`) (`local.SaveGame`))
  (set `/Game/BP/Class/BP_SaveGame.SlidesUsed` (`self.SlidesUsed`) (`local.SaveGame`))
  (set `/Game/BP/Class/BP_SaveGame.TotalSlideDuration` (`self.TotalSlideDuration`) (`local.SaveGame`))
  (set `/Game/BP/Class/BP_SaveGame.WallrunsUsed` (`self.WallrunsUsed`) (`local.SaveGame`))
  (set `/Game/BP/Class/BP_SaveGame.TotalWallrunDuration` (`self.TotalWallrunDuration`) (`local.SaveGame`))
  (set `/Game/BP/Class/BP_SaveGame.MaxSpeedReached` (`self.MaxSpeedReached`) (`local.SaveGame`))
  (set `/Game/BP/Class/BP_SaveGame.AverageSpeed` (`self.AverageSpeed`) (`local.SaveGame`))
  (set `/Game/BP/Class/BP_SaveGame.LedgesClimbed` (`self.LedgesClimbed`) (`local.SaveGame`))
  (set `/Game/BP/Class/BP_SaveGame.PullbarsGrabbed` (`self.PullbarsGrabbed`) (`local.SaveGame`))
  (set `/Game/BP/Class/BP_SaveGame.WallJumps` (`self.WallJumps`) (`local.SaveGame`))
  (set `/Game/BP/Class/BP_SaveGame.MechanismsParalysed` (`self.MechanismsParalysed`) (`local.SaveGame`))
  (set `/Game/BP/Class/BP_SaveGame.SpellsUsed` (`self.SpellsUsed`) (`local.SaveGame`))
  (set `/Game/BP/Class/BP_SaveGame.SpeedsRegistered` (`self.SpeedsRegistered`) (`local.SaveGame`)))