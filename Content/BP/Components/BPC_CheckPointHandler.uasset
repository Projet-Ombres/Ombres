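; Checkpoint handler component that records progress and triggers a save when a checkpoint is reached.
; On the reached event it stores the checkpoint and snapshots every BP_Enemy's location and spawn ID into an enemy data array.
; It then has the player character save the checkpoint, notifies the player's main interface, and calls SaveData on the game instance.
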(event `OnCheckPointReached`
  (params (CheckPoint :type "/Game/BP/Class/BP_CheckPoint Object Reference"))
  (bind _asbp_player_chara (cast `/Game/BP/BP_PlayerChara` (`GameplayStatics.GetPlayerCharacter` 0) :!pure true))
  (`KismetSystemLibrary.PrintString` (`KismetStringLibrary.Concat_StrStr` "Checkpoint " (`KismetStringLibrary.Conv_IntToString` (`/Game/BP/Class/BP_CheckPoint.ID` CheckPoint)) " reached."))
  (set `self.LastCheckPointReached` CheckPoint)
  (bind _outactors (`GameplayStatics.GetAllActorsOfClass` "/Game/AI/Blueprints/BP_Enemy.BP_Enemy_C"))
  (`KismetArrayLibrary.Array_Resize` (`self.EnemiesData`) (`KismetArrayLibrary.Array_Length` _outactors))
  (for (_array_element _array_index) _outactors
    (`KismetArrayLibrary.Array_Set` (`self.EnemiesData`) _array_index (make `/Game/BP/Class/EnemyData` (`Actor.K2_GetActorLocation` _array_element) (`/Game/AI/Blueprints/BP_EnemySpawn.ID` (`/Game/AI/Blueprints/BP_Enemy.SpawnRef` _array_element)))))
  (`/Game/BP/BP_PlayerChara.SaveCheckpoint` _asbp_player_chara)
  (`/Game/BP/Widgets/Widget_Main_Interface.CheckpointReached` (`/Game/BP/BP_PlayerChara.MainInterface` _asbp_player_chara))
  (bind _asbp_game_instance (cast `/Game/BP/BP_GameInstance` (`GameplayStatics.GetGameInstance`)))
  (`/Game/BP/BP_GameInstance.SaveData` _asbp_game_instance))