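; Example actor that previews a Skywalk cooldown material effect on a Plane mesh when the G key is pressed.
; Three chained timelines drive the spawn, cooldown and opacity scalar parameters in turn.
; When the last timeline finishes, all three parameters are set from a Reset value, with opacity offset.
; Input is enabled for the first player controller on BeginPlay.
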(event `Key|G`
  (params (Key :type "Key Structure"))
  (bind _plane (`self.Plane`))
  (bind _reset (`self.reset`))
  (:`Pressed`
    (`KismetSystemLibrary.PrintString` "")
    (bind (_direction _spawn) (`Timeline|Timeline_0`)
      (:`Update`
        (`MeshComponent.SetScalarParameterValueOnMaterials` _plane "Skywalk_spawn" _spawn))
      (:`Finished`
        (bind (_direction_2 _cooldown) (`Timeline|Timeline_1`)
          (:`Update`
            (`MeshComponent.SetScalarParameterValueOnMaterials` _plane "Skywalk_Cooldown" _cooldown))
          (:`Finished`
            (bind (_direction_3 _kill) (`Timeline|Timeline_2`)
              (:`Update`
                (`MeshComponent.SetScalarParameterValueOnMaterials` _plane "Skywalk_opac" _kill))
              (:`Finished`
                (`MeshComponent.SetScalarParameterValueOnMaterials` _plane "Skywalk_spawn" _reset)
                (`MeshComponent.SetScalarParameterValueOnMaterials` _plane "Skywalk_Cooldown" _reset)
                (`MeshComponent.SetScalarParameterValueOnMaterials` _plane "Skywalk_opac" (+ _reset 10.0))))))))))

(event `self.ReceiveBeginPlay`
  (`self.EnableInput` (`GameplayStatics.GetPlayerController` 0)))

(event `Key|C`
  (params (Key :type "Key Structure")))

(event `Key|P`
  (params (Key :type "Key Structure")))

(fn `UserConstructionScript`)