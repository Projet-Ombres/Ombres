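; Standalone gear ("Rouage Seul") actor that plays an attached gear sound and can be covered in crystals.
; BeginPlay attaches the attenuated Gear_city sound to the root.
; Crystallize clears the spawned crystal list, then calls SpawnCrystals to place crystal meshes at preset points on the static mesh, passing along the freeze duration.
; IsCrystallized always returns false, and the construction script is empty.
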(event `/Game/BP/Class/BPI_Cristallizable.Crystallize`
  (params (FreezeDuration :type "Float (single-precision)"))
  (bind _spawnedcrystals (`self.SpawnedCrystals`))
  (`KismetArrayLibrary.Array_Clear` _spawnedcrystals)
  (`/Game/BP/Libraries/BP_MacroLibrary.SpawnCrystals` (`self.StaticMesh`) (`self.CrystalPoints`) (`self.CrystalMeshes`) FreezeDuration _spawnedcrystals))

(event `self.ReceiveBeginPlay`
  (`GameplayStatics.SpawnSoundAttached` "/Game/Sound_Design/Bruitages/City/Gear_city.Gear_city" (`self.DefaultSceneRoot`) "None" (0.0 0.0 0.0) (struct) "KeepRelativeOffset" true 1.0 1.0 0.0 "/Game/Sound_Design/SoundAttenuation.SoundAttenuation" null false))

(fn `IsCrystallized`
  (returns (Crystallized :type Boolean))
  (return false))

(fn `UserConstructionScript`)