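; Crystal collectible that increments the player's EnergyBallsCollected stat when BP_PlayerChara overlaps its Box.
; The overlap also plays a 2D sound and starts a timeline that compounds the main render component's scale each update.
; Each update also sets emissive, color and opacity material parameters on four render components and shows CristalTakeFX, hiding it after a delay.
; The graph never destroys the actor or disables the overlap.
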(event `self.ReceiveBeginPlay`)

(event `self.Box.OnComponentBeginOverlap`
  (params (OverlappedComponent :type "PrimitiveComponent Object Reference") (OtherActor :type "Actor Object Reference") (OtherComp :type "PrimitiveComponent Object Reference") (OtherBodyIndex :type Integer) (bFromSweep :type Boolean) (SweepResult :type "HitResult Structure (by ref)"))
  (bind _rendercomponent (`self.RenderComponent`))
  (bind _rendercomponent1 (`self.RenderComponent1`))
  (bind _rendercomponent2 (`self.RenderComponent2`))
  (bind _rendercomponent3 (`self.RenderComponent3`))
  (bind _cristal_take_fx (`self.Cristal_take_FX`))
  (bind _color (`self.color`))
  (bind _emi (`self.emi`))
  (bind _opac (`self.opac`))
  (bind _asbp_player_chara (cast `/Game/BP/BP_PlayerChara` OtherActor))
  (`/Engine/EditorBlueprintResources/StandardMacros.IncrementInt` (`/Game/BP/Components/BPC_StatsHandler.EnergyBallsCollected` (`/Game/BP/BP_PlayerChara.BPC_StatsHandler` _asbp_player_chara))
    (:`  `
      ;[1 1 1] sfx
      (`GameplayStatics.PlaySound2D` "/Game/_ART/Shader/Materials/VFX/1591.1591" 1.0 1.0 0.0 null null)
      ;[1 1 1] scale
      (bind (_direction _size) (`Timeline|Timeline_0` :`NewTime` 1.0)
        (:`Update`
          (`SceneComponent.SetRelativeScale3D` _rendercomponent (* (`SceneComponent.RelativeScale3D` _rendercomponent) _size))
          ;[1 1 1] mat
          (`MeshComponent.SetScalarParameterValueOnMaterials` _rendercomponent "emi" _emi)
          (`MeshComponent.SetVectorParameterValueOnMaterials` _rendercomponent "color" _color)
          (`MeshComponent.SetScalarParameterValueOnMaterials` _rendercomponent "opac" _opac)
          (`MeshComponent.SetScalarParameterValueOnMaterials` _rendercomponent1 "emi" _emi)
          (`MeshComponent.SetVectorParameterValueOnMaterials` _rendercomponent1 "color" _color)
          (`MeshComponent.SetScalarParameterValueOnMaterials` _rendercomponent1 "opac" _opac)
          (`MeshComponent.SetScalarParameterValueOnMaterials` _rendercomponent2 "emi" _emi)
          (`MeshComponent.SetVectorParameterValueOnMaterials` _rendercomponent2 "color" _color)
          (`MeshComponent.SetScalarParameterValueOnMaterials` _rendercomponent2 "opac" _opac)
          (`MeshComponent.SetScalarParameterValueOnMaterials` _rendercomponent3 "emi" _emi)
          (`MeshComponent.SetVectorParameterValueOnMaterials` _rendercomponent3 "color" _color)
          (`MeshComponent.SetScalarParameterValueOnMaterials` _rendercomponent3 "opac" _opac)
          ;[1 1 1] vfx
          (`SceneComponent.SetVisibility` _cristal_take_fx true false)
          (`KismetSystemLibrary.Delay` 1.0)
          (`SceneComponent.SetVisibility` _cristal_take_fx false false))))))

(fn `UserConstructionScript`)