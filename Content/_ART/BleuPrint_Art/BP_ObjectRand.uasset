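; BP_ObjectRand is an art placement actor that randomizes its look to add variety to props.
; Its Construction Script assigns a random mesh from an array to its static mesh component, then applies slight independent scale jitter per axis and a random yaw.
; The randomness is unseeded, so results can change whenever construction reruns.
; The Event Graph holds no runtime logic.
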(fn `UserConstructionScript`
  (bind _returnvalue (`KismetMathLibrary.RandomFloatInRange` 0.9 1.1))
  (`StaticMeshComponent.SetStaticMesh` (`self.teypdfgpa_11`) (`|GetArrayItem` (`self.NewVar_0`) (`KismetMathLibrary.RandomInteger` 7)))
  (`self.SetActorScale3D` (`KismetMathLibrary.MakeVector` _returnvalue _returnvalue _returnvalue))
  (`self.K2_SetActorRotation` (`KismetMathLibrary.MakeRotator` 0.0 0.0 (`KismetMathLibrary.RandomFloatInRange` -180.0 180.0))))