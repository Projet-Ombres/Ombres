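; BP_Rail is a construction-script-only art Blueprint that builds a rail along an editable spline.
; For each point, it adds a spline mesh running back to the previous index, using negated tangents to suit the reversed direction.
; A nested loop repeatedly stacks pairs of scaled static meshes at each point, all rotated to match the last point.
; The event graph has no logic.
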(fn `UserConstructionScript`
  (bind _spline (`self.Spline`))
  (bind _returnvalue (- (`SplineComponent.GetNumberOfSplinePoints` (`self.Spline`)) 1))
  (bind _returnvalue_2 (`SplineComponent.GetRotationAtSplinePoint` (`self.Spline`) _returnvalue "Local"))
  (for _index (range (+ _returnvalue 1))
    (bind _returnvalue_3 (`AddComponent|NODE_AddSplineMeshComponent-0`))
    (`SceneComponent.K2_AttachToComponent` (`self.Spline`) (`self.Scene`) "None" "KeepWorld" "KeepWorld" "KeepRelative" false)
    (bind _returnvalue_4 (`SplineComponent.GetLocationAtSplinePoint` _spline _index "Local"))
    (bind _returnvalue_5 (- _index 1))
    (`SplineMeshComponent.SetStartAndEnd` _returnvalue_3 _returnvalue_4 (* (`SplineComponent.GetTangentAtSplinePoint` _spline _index "Local") (-1.0 -1.0 -1.0)) (`SplineComponent.GetLocationAtSplinePoint` _spline _returnvalue_5 "Local") (* (`SplineComponent.GetTangentAtSplinePoint` _spline _returnvalue_5 "Local") (-1.0 -1.0 -1.0)) true)
    (for _ (range 1 (+ _returnvalue 1))
      (`AddComponent|NODE_AddStaticMeshComponent-4` :`RelativeTransform` (`KismetMathLibrary.MakeTransform` _returnvalue_4 _returnvalue_2 (10.0 10.0 10.0)))
      (`AddComponent|NODE_AddStaticMeshComponent-3` :`RelativeTransform` (`KismetMathLibrary.MakeTransform` _returnvalue_4 _returnvalue_2 (10.0 10.0 10.0))))))