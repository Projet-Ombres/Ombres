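; BP_ElevatorPlatform is a one-shot elevator that raises its static mesh when the player character enters its trigger box.
; The overlap blocks move input and disables the Skywalk and Crystallization spells, then calls MovePlatformUp, guarded by a DoOnce.
; A custom timeline adds its output times Speed to the mesh's Z on each update, restoring input and spells when finished.
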(event `self.Box.OnComponentBeginOverlap`
  (params (OverlappedComponent :type "PrimitiveComponent Object Reference") (OtherActor :type "Actor Object Reference") (OtherComp :type "PrimitiveComponent Object Reference") (OtherBodyIndex :type Integer) (bFromSweep :type Boolean) (SweepResult :type "HitResult Structure (by ref)"))
  (bind (_asbp_player_chara _bsuccess) (cast `/Game/BP/BP_PlayerChara` OtherActor :!pure true))
  (if _bsuccess
    (`Controller.SetIgnoreMoveInput` (`GameplayStatics.GetPlayerController` 0) true)
    (set `SkywalkComponent.SpellEnabled` false (`/Game/BP/BP_PlayerChara.Skywalk` _asbp_player_chara))
    (set `/Game/BP/Components/Pouvoirs/BPC_Crystallization.SpellEnabled` false (`/Game/BP/BP_PlayerChara.BPC_Crystallization` _asbp_player_chara))
    (`self.MovePlatformUp`)))

(event `MovePlatformUp`
  (bind _staticmeshcomponent (`self.StaticMeshComponent`))
  (bind (_returnvalue_x _returnvalue_y _returnvalue_z) (`KismetMathLibrary.BreakVector` (`SceneComponent.K2_GetComponentLocation` _staticmeshcomponent)))
  (`/Engine/EditorBlueprintResources/StandardMacros.DoOnce` false
    (:`Completed`
      (bind _outputvalue (`CustomTimeline.StartCustomTimeline` (`self.MovingUpDurationTimeline`))
        (:`Update`
          (`SceneComponent.K2_SetWorldLocation` _staticmeshcomponent (`KismetMathLibrary.MakeVector` _returnvalue_x _returnvalue_y (+ _returnvalue_z (* _outputvalue (`self.Speed`)))) false false))
        (:`Finished`
          (`Controller.ResetIgnoreMoveInput` (`GameplayStatics.GetPlayerController` 0))
          (bind (_asbp_player_chara _bsuccess) (cast `/Game/BP/BP_PlayerChara` (stale `self.Box.OnComponentBeginOverlap` OtherActor) :!pure true))
          (set `SkywalkComponent.SpellEnabled` true (`/Game/BP/BP_PlayerChara.Skywalk` _asbp_player_chara))
          (set `/Game/BP/Components/Pouvoirs/BPC_Crystallization.SpellEnabled` true (`/Game/BP/BP_PlayerChara.BPC_Crystallization` _asbp_player_chara)))))))

(fn `UserConstructionScript`)