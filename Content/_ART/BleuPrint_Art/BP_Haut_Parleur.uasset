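; Loudspeaker actor that plays random voice announcements framed by start and end cues while the player is inside its detection sphere.
; A self-rescheduling Speak timer rolls for each announcement and holds off while the pause menu is open.
; Tick detects the voice's end and fades speaker audio down while the player speaks.
; Active sounds register in BP_GameInstance, and the construction script sets sphere radius and swaps meshes.
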(event `self.ReceiveBeginPlay`
  (`self.Speak`))

(event `CheckEndSpeaker`
  (bind _currentspeakingvoice (`self.currentSpeakingVoice`))
  ;[1 1 1] check for end voice speaker
  (if (!= _currentspeakingvoice null)
    (if (not (`AudioComponent.IsPlaying` _currentspeakingvoice))
      (`KismetArrayLibrary.Array_RemoveItem` (`/Game/BP/BP_GameInstance.HautParleursSounds` (cast `/Game/BP/BP_GameInstance` (`GameplayStatics.GetGameInstance`) :!pure true)) _currentspeakingvoice)
      (set `self.currentSpeakingVoice` null)
      (`KismetSystemLibrary.Delay` 0.5)
      (bind _returnvalue (`GameplayStatics.SpawnSoundAttached` "/Game/Sound_Design/Bruitages/City/speakers/SpeakersEnd_Cue.SpeakersEnd_Cue" (`self.StaticMesh`) "None" (0.0 0.0 0.0) (struct) "KeepRelativeOffset" false 1.0 1.0 0.0 "/Game/Sound_Design/SoundAttenuation.SoundAttenuation" null false))
      (set `self.SpeakersSounds` _returnvalue)
      (`KismetArrayLibrary.Array_Add` (`/Game/BP/BP_GameInstance.HautParleursSounds` (cast `/Game/BP/BP_GameInstance` (`GameplayStatics.GetGameInstance`) :!pure true)) _returnvalue)
      (`KismetSystemLibrary.Delay` 3.0)
      (set `self.SpeakersSounds` null)
      (`KismetArrayLibrary.Array_RemoveItem` (`/Game/BP/BP_GameInstance.HautParleursSounds` (cast `/Game/BP/BP_GameInstance` (`GameplayStatics.GetGameInstance`) :!pure true)) _returnvalue)
      (`KismetSystemLibrary.K2_SetTimer` null "Speak" (`KismetMathLibrary.RandomFloatInRange` 5.0 12.0)))))

(event `Speak`
  ;[1 1 1] speak
  (if (`self.PlayerInRange`)
    (if (== (`KismetMathLibrary.RandomInteger` 2) 0)
      (if (`/Game/BP/Widgets/Widget_Main_Interface.PauseMenuOpened` (`/Game/BP/BP_GameInstance.MainInterface` (cast `/Game/BP/BP_GameInstance` (`GameplayStatics.GetGameInstance`) :!pure true)))
        (`KismetSystemLibrary.K2_SetTimer` null "Speak" (`KismetMathLibrary.RandomFloatInRange` 1.0 2.0) :!label _label)
        (else
          (bind _returnvalue (`GameplayStatics.SpawnSoundAttached` "/Game/Sound_Design/Bruitages/City/speakers/SpeakersStart_Cue.SpeakersStart_Cue" (`self.StaticMesh`) "None" (0.0 0.0 0.0) (struct) "KeepRelativeOffset" false 1.0 1.0 0.0 "/Game/Sound_Design/SoundAttenuation.SoundAttenuation" null false))
          (set `self.SpeakersSounds` _returnvalue)
          (`KismetArrayLibrary.Array_Add` (`/Game/BP/BP_GameInstance.HautParleursSounds` (cast `/Game/BP/BP_GameInstance` (`GameplayStatics.GetGameInstance`) :!pure true)) _returnvalue)
          (`KismetSystemLibrary.Delay` 2.5)
          (set `self.SpeakersSounds` null)
          (`KismetArrayLibrary.Array_RemoveItem` (`/Game/BP/BP_GameInstance.HautParleursSounds` (cast `/Game/BP/BP_GameInstance` (`GameplayStatics.GetGameInstance`) :!pure true)) _returnvalue)
          (bind _returnvalue_2 (`GameplayStatics.SpawnSoundAttached` "/Game/Sound_Design/Voix/Voice_Speaker/HautParleurs_cue.HautParleurs_cue" (`self.StaticMesh`) "None" (0.0 0.0 0.0) (struct) "KeepRelativeOffset" false 1.0 1.0 0.0 "/Game/Sound_Design/SoundAttenuation.SoundAttenuation" null false))
          (bind _output_get (set `self.currentSpeakingVoice` _returnvalue_2))
          (`KismetArrayLibrary.Array_Add` (`/Game/BP/BP_GameInstance.HautParleursSounds` (cast `/Game/BP/BP_GameInstance` (`GameplayStatics.GetGameInstance`) :!pure true)) _output_get)))
      (else
        (`KismetSystemLibrary.K2_SetTimer` null "Speak" (`KismetMathLibrary.RandomFloatInRange` 8.0 15.0))))
    (else
      (goto _label))))

(event `self.Sphere.OnComponentBeginOverlap`
  (params (OverlappedComponent :type "PrimitiveComponent Object Reference") (OtherActor :type "Actor Object Reference") (OtherComp :type "PrimitiveComponent Object Reference") (OtherBodyIndex :type Integer) (bFromSweep :type Boolean) (SweepResult :type "HitResult Structure (by ref)"))
  ;[1 1 1] End begin overlap
  (if (`.bSuccess` (cast `/Game/BP/BP_PlayerChara` OtherActor :!pure true))
    (set `self.PlayerInRange` true)))

(event `self.ReceiveTick`
  (params (DeltaSeconds :type "Float (single-precision)"))
  ;[1 1 1] event tick
  (`self.CheckEndSpeaker`)
  (`self.AdjustSoundAbadelSpeaking`))

(event `AdjustSoundAbadelSpeaking`
  (bind _currentspeakingvoice (`self.currentSpeakingVoice`))
  (bind _speakerssounds (`self.SpeakersSounds`))
  (bind (_asbp_player_chara _bsuccess) (cast `/Game/BP/BP_PlayerChara` (`GameplayStatics.GetPlayerCharacter` 0) :!pure true))
  ;[1 1 1] adjust sound if abadel speaking
  (if _bsuccess
    (if (`/Game/BP/BP_PlayerChara.PlayerSpeaking` _asbp_player_chara)
      (if (!= _currentspeakingvoice null)
        (`AudioComponent.FadeOut` _currentspeakingvoice 0.2 (* (`AudioComponent.VolumeMultiplier` _currentspeakingvoice) 0.2))
        (else
          (if (!= _speakerssounds null) :!label _label_2
            (`AudioComponent.FadeOut` _speakerssounds 0.2 (* (`AudioComponent.VolumeMultiplier` _speakerssounds) 0.2)))))
      (else
        (goto _label_2)))))

(event `self.Sphere.OnComponentEndOverlap`
  (params (OverlappedComponent :type "PrimitiveComponent Object Reference") (OtherActor :type "Actor Object Reference") (OtherComp :type "PrimitiveComponent Object Reference") (OtherBodyIndex :type Integer))
  ;[1 1 1] End begin overlap
  (if (`.bSuccess` (cast `/Game/BP/BP_PlayerChara` OtherActor :!pure true))
    (set `self.PlayerInRange` false)))

(fn `UserConstructionScript`
  (`SphereComponent.SetSphereRadius` (`self.Sphere`) (`self.DetectionRadius`) true)
  (if (`self.Visible`)
    (`SceneComponent.SetHiddenInGame` (`self.StaticMesh`) false false)
    (`SceneComponent.SetHiddenInGame` (`self.StaticMesh1`) true false)
    (else
      (`SceneComponent.SetHiddenInGame` (`self.StaticMesh`) true false)
      (`SceneComponent.SetHiddenInGame` (`self.StaticMesh1`) false false))))