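; Art prop actor that randomizes its look, with no active gameplay logic.
; The construction script assigns its static mesh component a random pick from the first seven entries of a mesh array.
; It then sets the actor rotation to a random moderate roll with zero pitch and yaw, overriding any placed rotation.
; Both choices re-roll whenever the construction script reruns.
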(fn `UserConstructionScript`
  (`StaticMeshComponent.SetStaticMesh` (`self.teypdfgpa_11`) (`|GetArrayItem` (`self.NewVar_0`) (`KismetMathLibrary.RandomInteger` 7)))
  (`self.K2_SetActorRotation` (`KismetMathLibrary.MakeRotator` (`KismetMathLibrary.RandomFloatInRange` -25.0 25.0))))