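; BP_DebugPingSpline is a debug actor that displays ping particle effects along a spline.
; On BeginPlay it spawns FX_PingSpline emitters at evenly spaced normalized times along the spline, matching its position and rotation.
; Each Tick it moves and orients ScrollingEmitter along the spline in a loop at SpeedScroll.
; Spline transforms are sampled in local space but applied as world values.
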(event `self.ReceiveBeginPlay`
  (bind _maxparticles (`self.maxParticles`))
  (bind _spline (`self.Spline`))
  (for _index (range (+ _maxparticles 1))
    (bind _returnvalue (/ (`KismetMathLibrary.Conv_IntToDouble` _index) (`KismetMathLibrary.Conv_IntToDouble` _maxparticles)))
    (`GameplayStatics.SpawnEmitterAtLocation` "/Game/Ombres/VFX/PingSpline/FX_PingSpline.FX_PingSpline" (`SplineComponent.GetLocationAtTime` _spline _returnvalue "Local" false) (`SplineComponent.GetRotationAtTime` _spline _returnvalue "Local" false))))

(event `self.ReceiveTick`
  (params (DeltaSeconds :type "Float (single-precision)"))
  (bind _spline (`self.Spline`))
  (bind _scrollingemitter (`self.ScrollingEmitter`))
  (bind _output_get (set `self.time` (+ (`self.time`) (* DeltaSeconds (`self.speedScroll`)))))
  (bind _returnvalue (`KismetMathLibrary.Fraction` _output_get))
  (`SceneComponent.K2_SetWorldLocation` _scrollingemitter (`SplineComponent.GetLocationAtTime` _spline _returnvalue "Local" false) false false)
  (`SceneComponent.K2_SetWorldRotation` _scrollingemitter (`SplineComponent.GetRotationAtTime` _spline _returnvalue "Local" false) false false))

(fn `UserConstructionScript`)