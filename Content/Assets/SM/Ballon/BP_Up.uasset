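; BP_Up is an actor that builds a string of randomly colored balloons along a spline.
; The construction script adds 85 scaled static mesh components at fixed distances along the spline, each with a dynamic MI_Ballon material given a random color.
; It then attaches them to the root, keeping world transforms.
; An ascension timeline that would raise the actor exists but is never triggered.
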(fn `UserConstructionScript`
  (for _index (range 85)
    (bind _returnvalue (`AddComponent|NODE_AddStaticMeshComponent-0` :`bManualAttachment` true :`RelativeTransform` (`KismetMathLibrary.MakeTransform` (`SplineComponent.GetLocationAtDistanceAlongSpline` (`self.Spline`) (* _index 450.0) "World") (struct) (3.0 3.0 3.0))))
    (`KismetArrayLibrary.Array_Add` (`self.Ballon`) _returnvalue)
    (bind _returnvalue_2 (`PrimitiveComponent.CreateDynamicMaterialInstance` _returnvalue 0 "/Game/Assets/SM/Ballon/MI_Ballon.MI_Ballon" "None"))
    (`MaterialInstanceDynamic.SetVectorParameterValue` _returnvalue_2 "Color" (`KismetMathLibrary.MakeColor` (`KismetMathLibrary.RandomFloatInRange` 0.0 1.0) (`KismetMathLibrary.RandomFloatInRange` 0.0 1.0) (`KismetMathLibrary.RandomFloatInRange` 0.0 1.0))))
  (for _array_element (`self.Ballon`)
    (`SceneComponent.K2_AttachToComponent` _array_element (`self.DefaultSceneRoot`) "None" "KeepWorld" "KeepWorld" "KeepWorld" true)))