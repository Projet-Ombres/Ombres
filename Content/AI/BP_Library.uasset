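; AI Blueprint library with one function that calculates the launch velocity for a jump from a start to an end position in a given duration.
; Horizontal components are displacement divided by duration, while the vertical component adds compensation for gravity using the projectile motion equation.
; Gravity is hard-coded to Earth's value in centimeters rather than read from the world, and a zero duration is not guarded.
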(fn `CalculateJumpVelocity`
  (params (StartPosition :type "Vector Structure") (EndPosition :type "Vector Structure") (JumpDuration :type "Float (double-precision)"))
  (returns (Velocity :type "Vector Structure"))
  (return (`KismetMathLibrary.MakeVector` (/ (- (.x EndPosition) (.x StartPosition)) JumpDuration) (/ (- (.y EndPosition) (.y StartPosition)) JumpDuration) (/ (- (.z EndPosition) (+ (.z StartPosition) (* (`KismetMathLibrary.Square` JumpDuration) -0.5 981.0))) JumpDuration))))