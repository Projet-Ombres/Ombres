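; Enemy character Blueprint that senses the player, turns toward targets and shoots bullets.
; A one-second timer and perception updates write player distance and sight to the Blackboard, both paused while IsRoot is set.
; LookTowards stops movement and rotates yaw, but when rooted only records the yaw once.
; ShootOnPlayer requires sight, firing from the right-hand socket toward the player's feet with random spread scaled by BulletImpactRange.
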(event `self.ReceiveBeginPlay`
  (`KismetSystemLibrary.K2_SetTimerDelegate` (delegate `UpdateDistanceToPlayer`) 1.0 true)
  (bind _asbp_player_chara (cast `/Game/BP/BP_PlayerChara` (`GameplayStatics.GetPlayerCharacter` 0)))
  (set `self.PlayerChara` _asbp_player_chara))

(event `UpdateDistanceToPlayer`
  ;[1 1 1] Update distance to player every second (to avoid event tick)
  (if (not (`self.IsRoot?`))
    (`BlackboardComponent.SetValueAsFloat` (`AIBlueprintHelperLibrary.GetBlackboard` null) "DistanceToPlayer" (`KismetMathLibrary.Vector_Distance2D` (`self.K2_GetActorLocation`) (`self.K2_GetActorLocation` (`GameplayStatics.GetPlayerCharacter` 0))))))

(event `self.AIPerception.OnTargetPerceptionUpdated`
  (params (Actor :type "Actor Object Reference") (Stimulus :type "AIStimulus Structure"))
  (bind _returnvalue (`AIBlueprintHelperLibrary.GetBlackboard` null))
  ;[1 1 1] Detect player
  (if (not (`self.IsRoot?`))
    (cast `/Game/BP/BP_PlayerChara` Actor)
    (`/Engine/EditorBlueprintResources/StandardMacros.IsValid` _returnvalue
      (:`Is Valid`
        (`BlackboardComponent.SetValueAsBool` _returnvalue "PlayerInSight" (`.bSuccessfullySensed` (break `AIStimulus` Stimulus))))
      (:`Is Not Valid`
        (`KismetSystemLibrary.PrintString` "Tu as placé un BP_Enemy directement dans le level : utilise plutôt un BP_EnemySpawn" true false (struct :`R` 1.0 :`G` 0.853144 :`A` 1.0) 5.0)))))

(event `LookTowards`
  (params (Target :type "Vector Structure"))
  (bind (_returnvalue_roll _returnvalue_pitch) (`KismetMathLibrary.BreakRotator` (`self.K2_GetActorRotation`)))
  (bind (_returnvalue_roll_2 _returnvalue_pitch_2 _returnvalue_yaw) (`KismetMathLibrary.BreakRotator` (`KismetMathLibrary.FindLookAtRotation` (`self.K2_GetActorLocation`) Target)))
  ;[1 1 1] Look towards
  (if (`self.IsRoot?`)
    (`/Engine/EditorBlueprintResources/StandardMacros.DoOnce` false :!label _label
      (:`Completed`
        (set `self.rotation when root` _returnvalue_yaw)))
    (else
      (`|ExecutionSequence`
        (:`then_0`
          (goto _label :!via `Reset`))
        (:`then_1`
          (`MovementComponent.StopMovementImmediately` (`self.CharacterMovement`))
          (`self.K2_SetActorRotation` (`KismetMathLibrary.MakeRotator` _returnvalue_roll _returnvalue_pitch (select `bool` (`self.IsRoot?`) :`false` _returnvalue_yaw :`true` (`self.rotation when root`)))))))))

(event `ShootOnPlayer`
  (bind _playerchara (`self.PlayerChara`))
  (bind (_returnvalue_x _returnvalue_y _returnvalue_z) (`KismetMathLibrary.BreakVector` (`self.K2_GetActorLocation` _playerchara)))
  ;[1 1 1] Shoot on player
  (if (`BlackboardComponent.GetValueAsBool` (`AIBlueprintHelperLibrary.GetBlackboard` null) "PlayerInSight")
    (`|SpawnActorFromClass` "/Game/AI/BP_Bullet.BP_Bullet_C" (`KismetMathLibrary.MakeTransform` (`SceneComponent.GetSocketLocation` (`self.Mesh`) "RightHand") (`KismetMathLibrary.FindLookAtRotation` (`self.K2_GetActorLocation`) (+ (`KismetMathLibrary.MakeVector` _returnvalue_x _returnvalue_y (- _returnvalue_z (`CapsuleComponent.GetScaledCapsuleHalfHeight` (`Character.CapsuleComponent` _playerchara)))) (* (`KismetMathLibrary.MakeVector` (`KismetMathLibrary.RandomFloat`) (`KismetMathLibrary.RandomFloat`)) (`self.BulletImpactRange`))))) "Undefined" "OverrideRootScale" null null)))

(fn `UserConstructionScript`
  (locals (TimerHandle :type "TimerHandle Structure")))