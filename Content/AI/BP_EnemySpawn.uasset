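; BP_EnemySpawn is a placed spawn point that spawns and despawns an enemy based on player proximity.
; A one-second looping timer checks 2D distance to the player, spawning BP_Enemy with BT_Enemy inside EnemySpawnRange and destroying it outside.
; A Spawned flag prevents duplicates while that range holds.
; The construction script sets a preview skeletal mesh from EnemyType, which is hidden upon spawning.
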(event `self.ReceiveBeginPlay`
  ;[1 0 0.8111] Begin play
  (bind _asbp_player_chara (cast `/Game/BP/BP_PlayerChara` (`GameplayStatics.GetPlayerCharacter` 0)))
  (set `self.PlayerChara` _asbp_player_chara)
  (bind _returnvalue (`KismetSystemLibrary.K2_SetTimerDelegate` (delegate `CheckDistanceToPlayer`) 1.0 true))
  (set `self.CheckDistanceTimerHandle` _returnvalue)
  (`self.CheckDistanceToPlayer`))

(event `CheckDistanceToPlayer`
  ;[1 1 1] Check distance to player every second
  (if (< (`KismetMathLibrary.Vector_Distance2D` (`self.K2_GetActorLocation` (`self.PlayerChara`)) (`self.K2_GetActorLocation`)) (`self.EnemySpawnRange`))
    (if (not (`self.Spawned`))
      (`self.SpawnEnemy`)
      (set `self.Spawned` true))
    (elif (`self.Spawned`)
      (`self.K2_DestroyActor` (`self.EnemySpawned`))
      (set `self.Spawned` false))))

(fn `SpawnEnemy`
  (`SceneComponent.SetVisibility` (`self.MeshPreview`) false false)
  (bind _returnvalue (`AIBlueprintHelperLibrary.SpawnAIFromClass` "/Game/AI/BP_Enemy.BP_Enemy_C" "/Game/AI/BT_Enemy.BT_Enemy" (`self.K2_GetActorLocation`) (`self.K2_GetActorRotation`)))
  (set `self.EnemySpawned` _returnvalue)
  (return))

(fn `UserConstructionScript`
  (locals (EnemyMesh :type "SkeletalMesh Object Reference"))
  (switch `/Game/AI/EEnemyType` (`self.EnemyType`)
    (:`NewEnumerator0`
      (set `local.EnemyMesh` "/Game/AI/Animation/SK_Enemy.SK_Enemy")
      (`SkinnedMeshComponent.SetSkinnedAssetAndUpdate` (`self.MeshPreview`) (`local.EnemyMesh`) true))))