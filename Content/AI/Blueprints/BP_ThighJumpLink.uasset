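; BP_ThighJumpLink is a smart nav link that triggers a thigh jump for enemy AI that reaches it.
; It passes the destination as wall location, a normal pointing from it toward the agent, and its actor-relative ledge point to the enemy's BPCThighJump component.
; It then sets the enemy Anim Blueprint's state and calls JumpThigh on that component.
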(event `self.ReceiveSmartLinkReached`
  (params (Agent :type "Actor Object Reference") (Destination :type "Vector Structure (by ref)"))
  (bind _asbp_enemy (cast `/Game/AI/Blueprints/BP_Enemy` Agent))
  (bind _bpc_thighjump (`/Game/AI/Blueprints/BP_Enemy.BPC_ThighJump` _asbp_enemy))
  (set `/Game/BP/Components/CapacitéPhysique/BPC_ThighJump.WallLocation` Destination _bpc_thighjump)
  (set `/Game/BP/Components/CapacitéPhysique/BPC_ThighJump.WallNormal` (`KismetMathLibrary.Normal` (- (`self.K2_GetActorLocation` Agent) Destination)) _bpc_thighjump)
  (set `/Game/BP/Components/CapacitéPhysique/BPC_ThighJump.Ledge height location` (+ (`self.LedgeLocation`) (`self.K2_GetActorLocation`)) _bpc_thighjump)
  (bind _asabp_enemy (cast `/Game/AI/Animation/Robot_OLD/ABP_Enemy` (`SkeletalMeshComponent.GetAnimInstance` (`Character.Mesh` _asbp_enemy))))
  (set `/Game/AI/Animation/Robot_OLD/ABP_Enemy.State` "NewEnumerator3" _asabp_enemy)
  (`/Game/BP/Components/CapacitéPhysique/BPC_ThighJump.JumpThigh` _bpc_thighjump))

(fn `UserConstructionScript`)