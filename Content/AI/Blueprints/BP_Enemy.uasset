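; Enemy AI character that shoots at the player and triggers game over on contact, with walk speed scaled by difficulty.
; Perception and a one-second timer, used instead of Tick, feed sight and distance to the Blackboard unless IsRoot is set.
; ShootOnPlayer fires randomly offset bullets toward the player's feet when in sight.
; LookTowards handles facing, and jump-link events toggle pawn collision during jumps.
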(event `self.ReceiveHit`
  (params (MyComp :type "PrimitiveComponent Object Reference") (Other :type "Actor Object Reference") (OtherComp :type "PrimitiveComponent Object Reference") (bSelfMoved :type Boolean) (HitLocation :type "Vector Structure") (HitNormal :type "Vector Structure") (NormalImpulse :type "Vector Structure") (Hit :type "HitResult Structure (by ref)"))
  (bind _returnvalue (`GameplayStatics.GetPlayerController` 0))
  ;[1 1 1] On player touch
  (cast `/Game/BP/BP_PlayerChara` Other)
  (`/Game/BP/Widgets/Widget_Main_Interface.ToggleGameOverPanel` (`/Game/BP/BP_GameInstance.MainInterface` (cast `/Game/BP/BP_GameInstance` (`GameplayStatics.GetGameInstance`) :!pure true)) true)
  (`MovementComponent.StopMovementImmediately` (`Character.CharacterMovement` (`self.PlayerChara`)))
  (`Controller.SetIgnoreMoveInput` _returnvalue true)
  (`Controller.SetIgnoreLookInput` _returnvalue true))

(event `self.ReceiveBeginPlay`
  (bind _maxwalkspeed (`CharacterMovementComponent.MaxWalkSpeed` (`self.CharacterMovement`)))
  ;[1 0 0.8583] Begin play
  (`KismetSystemLibrary.K2_SetTimerDelegate` (delegate `UpdateDistanceToPlayer`) 1.0 true)
  (bind _asbp_player_chara (cast `/Game/BP/BP_PlayerChara` (`GameplayStatics.GetPlayerCharacter` 0)))
  (set `self.PlayerChara` _asbp_player_chara)
  ;[1 1 1] Set movement speed from difficulty
  (set `CharacterMovementComponent.MaxWalkSpeed` (select `int` (`/Game/BP/Class/BP_SaveGame.Difficulty` (`/Game/BP/BP_GameInstance.SaveGame` (cast `/Game/BP/BP_GameInstance` (`GameplayStatics.GetGameInstance`) :!pure true))) :`0` (* _maxwalkspeed 0.9) :`1` _maxwalkspeed :`2` (* _maxwalkspeed 1.1)) (`self.CharacterMovement`)))

(event `UpdateDistanceToPlayer`
  ;[1 1 1] Update distance to player every second (to avoid event tick)
  (if (not (`self.bIsRoot`))
    (`BlackboardComponent.SetValueAsFloat` (`AIBlueprintHelperLibrary.GetBlackboard` null) "DistanceToPlayer" (`KismetMathLibrary.Vector_Distance2D` (`self.K2_GetActorLocation`) (`self.K2_GetActorLocation` (`GameplayStatics.GetPlayerCharacter` 0))))))

(event `self.AIPerception.OnTargetPerceptionUpdated`
  (params (Actor :type "Actor Object Reference") (Stimulus :type "AIStimulus Structure"))
  (bind _returnvalue (`AIBlueprintHelperLibrary.GetBlackboard` null))
  ;[1 1 1] Detect player
  (if (not (`self.bIsRoot`))
    (cast `/Game/BP/BP_PlayerChara` Actor)
    (`/Engine/EditorBlueprintResources/StandardMacros.IsValid` _returnvalue
      (:`Is Valid`
        (`BlackboardComponent.SetValueAsBool` _returnvalue "PlayerInSight" (`.bSuccessfullySensed` (break `AIStimulus` Stimulus))))
      (:`Is Not Valid`
        (`KismetSystemLibrary.PrintString` "Tu as placé un BP_Enemy directement dans le level : utilise plutôt un BP_EnemySpawn" true false (struct :`R` 1.0 :`G` 0.853144 :`A` 1.0) 5.0)))))

(event `LookTowards`
  (params (Target :type "Vector Structure"))
  (bind (_returnvalue_roll _returnvalue_pitch) (`KismetMathLibrary.BreakRotator` (`self.K2_GetActorRotation`)))
  (bind (_returnvalue_roll_2 _returnvalue_pitch_2 _returnvalue_yaw) (`KismetMathLibrary.BreakRotator` (`KismetMathLibrary.FindLookAtRotation` (`self.K2_GetActorLocation`) Target)))
  ;[1 1 1] Look towards
  (if (`self.bIsRoot`)
    (`/Engine/EditorBlueprintResources/StandardMacros.DoOnce` false :!label _label
      (:`Completed`
        (set `self.rootYaw` _returnvalue_yaw)))
    (else
      (`|ExecutionSequence`
        (:`then_0`
          (goto _label :!via `Reset`))
        (:`then_1`
          (`MovementComponent.StopMovementImmediately` (`self.CharacterMovement`))
          (`self.K2_SetActorRotation` (`KismetMathLibrary.MakeRotator` _returnvalue_roll _returnvalue_pitch (select `bool` (`self.bIsRoot`) :`false` _returnvalue_yaw :`true` (`self.rootYaw`)))))))))

(event `ShootOnPlayer`
  (bind _playerchara (`self.PlayerChara`))
  (bind (_returnvalue_x _returnvalue_y _returnvalue_z) (`KismetMathLibrary.BreakVector` (`self.K2_GetActorLocation` _playerchara)))
  ;[1 1 1] Shoot on player
  (if (`BlackboardComponent.GetValueAsBool` (`AIBlueprintHelperLibrary.GetBlackboard` null) "PlayerInSight")
    (`|SpawnActorFromClass` "/Game/AI/Blueprints/BP_Bullet.BP_Bullet_C" (`KismetMathLibrary.MakeTransform` (`SceneComponent.GetSocketLocation` (`self.Mesh`) "RightHand") (`KismetMathLibrary.FindLookAtRotation` (`self.K2_GetActorLocation`) (+ (`KismetMathLibrary.MakeVector` _returnvalue_x _returnvalue_y (- _returnvalue_z (`CapsuleComponent.GetScaledCapsuleHalfHeight` (`Character.CapsuleComponent` _playerchara)))) (* (`KismetMathLibrary.MakeVector` (`KismetMathLibrary.RandomFloat`) (`KismetMathLibrary.RandomFloat`)) (`self.BulletImpactRange`))))) "Undefined" "OverrideRootScale" null null)))

(event `self.OnLanded`
  (params (Hit :type "HitResult Structure (by ref)"))
  ;[1 1 1] On landed
  (`PrimitiveComponent.SetCollisionResponseToChannel` (`self.CapsuleComponent`) "ECC_Pawn" "ECR_Block")
  (`/Engine/EditorBlueprintResources/StandardMacros.IsValid` (`self.LastJumpedLink`)
    (:`Is Valid`
      (`KismetSystemLibrary.Delay` 0.75)
      (set `self.LastJumpedLink` null))))

(event `OnJumpLink`
  ;[1 1 1] On jumped
  (`PrimitiveComponent.SetCollisionResponseToChannel` (`self.CapsuleComponent`) "ECC_Pawn" "ECR_Ignore"))

(fn `UserConstructionScript`
  (locals (TimerHandle :type "TimerHandle Structure")))