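; BP_Bullet is a bullet actor that handles the visual impact and cleanup when it hits something.
; Its Hit event spawns a bullet decal and an enlarged impact particle effect at the hit location, both oriented along the surface normal.
; It then destroys its Sphere component if valid, and destroys the whole actor after a delay equal to the decal's lifetime.
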(event `self.ReceiveHit`
  (params (MyComp :type "PrimitiveComponent Object Reference") (Other :type "Actor Object Reference") (OtherComp :type "PrimitiveComponent Object Reference") (bSelfMoved :type Boolean) (HitLocation :type "Vector Structure") (HitNormal :type "Vector Structure") (NormalImpulse :type "Vector Structure") (Hit :type "HitResult Structure (by ref)"))
  (bind _returnvalue (`KismetMathLibrary.Conv_VectorToRotator` HitNormal))
  (bind _sphere (`self.Sphere`))
  (`GameplayStatics.SpawnDecalAtLocation` "/Game/AI/Materials/M_BulletDecal.M_BulletDecal" (5.0 5.0 5.0) HitLocation _returnvalue (`self.DecalLifeTime`))
  (`GameplayStatics.SpawnEmitterAtLocation` "/Game/AI/ParticleSystems/P_BulletImpact.P_BulletImpact" HitLocation _returnvalue (2.0 2.0 2.0))
  (`/Engine/EditorBlueprintResources/StandardMacros.IsValid` _sphere
    (:`Is Valid`
      (`ActorComponent.K2_DestroyComponent` _sphere))
    (:`Is Not Valid`
      _))
  (`KismetSystemLibrary.Delay` (`self.DecalLifeTime`))
  (`self.K2_DestroyActor`))

(fn `UserConstructionScript`
  (`parent.UserConstructionScript`))