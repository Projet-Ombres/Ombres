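; Patrolling searchlight that detects the player and, after enough exposure, ejects them through a spawned portal.
; Tick sweeps the spotlight back and forth along PathPoints by rotating or moving it, pausing at points.
; Inside the Range sphere, a cone test and line trace drive a catch timer that reddens light and scene, then blocks movement input and spawns the portal.
; Construction script configures the light and range and draws a debug path preview.
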(event `self.ReceiveBeginPlay`
  ;[1 0 0.7658] Begin play
  (set `self.Progress` 0.0)
  ;[1 1 1] Remove preview
  (`KismetSystemLibrary.FlushPersistentDebugLines`))

(event `self.ReceiveTick`
  (params (DeltaSeconds :type "Float (single-precision)"))
  (bind (_targetedposition_x _targetedposition_y _targetedposition_z) (`KismetMathLibrary.BreakVector` (`self.TargetedPosition`)))
  (bind _progress (`self.Progress`))
  (bind _pathpoints (`self.PathPoints`))
  (bind _returnvalue (< _progress 0.0))
  (bind _returnvalue_2 (`KismetMathLibrary.FTrunc` (`self.Progress`)))
  (bind _returnvalue_3 (`KismetMathLibrary.Conv_IntToDouble` (`KismetArrayLibrary.Array_Length` (`self.PathPoints`))))
  ;[1 0 0.9121] Event tick
  (if (`self.PlayerCaught`)
    (`self.SetActorTickEnabled` false)
    (elif (not (`self.Stopping`))
      (if (`self.Overlapping`)
        (`self.CheckVisibility`)
        (if (`self.PlayerIsVisible`)
          (bind _output_get (set `self.CurrentCatchDuration` (+ (`self.CurrentCatchDuration`) DeltaSeconds)))
          ;[1 1 1] Calculate progression percent
          (`self.UpdateCatchTime` _output_get)
          (else
            (`self.ResetCatchTime`))))
      (bind _output_get_2 (set `self.Progress` (+ (* (* DeltaSeconds (`self.MovementSpeed`)) (select `bool` (`self.GoingForward`) :`false` -1.0 :`true` 1.0 :!type "Float (single-precision)")) (`self.Progress`))))
      (if (> _output_get_2 _returnvalue_3)
        (if (not (`self.PlayerCaught`))
          (set `self.Progress` (- _progress _returnvalue_3))
          (if (or (and (!= _returnvalue_2 (`self.PrevIndex`)) (!= _returnvalue_2 (- (`KismetArrayLibrary.Array_Length` (`self.PathPoints`)) 1))) (and _returnvalue (not (`self.GoingForward`)))) :!label _label
            (set `self.Stopping` true)
            (if _returnvalue
              (set `self.Progress` -1e-06))
            (`KismetSystemLibrary.Delay` (`self.StopDuration`))
            (set `self.Stopping` false))
          (bind _output_get_3 (set `self.PrevIndex` _returnvalue_2))
          (bind _output_get_4 (set `self.NextIndex` (+ _output_get_3 1)))
          (if (or (>= _output_get_4 (`KismetArrayLibrary.Array_Length` (`self.PathPoints`))) (< (`self.Progress`) 0.0))
            (set `self.GoingForward` (not (`self.GoingForward`)))
            (else
              (set `self.Percent` (- (`self.Progress`) (`KismetMathLibrary.Conv_IntToDouble` (`self.PrevIndex`))))
              (set `self.TargetedPosition` (`KismetMathLibrary.VLerp` (`|GetArrayItem` _pathpoints (`self.PrevIndex`)) (`|GetArrayItem` _pathpoints (`self.NextIndex`)) (`self.Percent`)))
              (switch `/Game/AI/Blueprints/EProjectorType` (`self.ProjectorType`)
                (:`NewEnumerator0`
                  ;[1 1 1] Set spotlight rotation
                  (`SceneComponent.K2_SetRelativeRotation` (`self.SpotLight`) (`KismetMathLibrary.FindLookAtRotation` (`SceneComponent.RelativeLocation` (`self.SpotLight`)) (`self.TargetedPosition`)) false false))
                (:`NewEnumerator1`
                  ;[1 1 1] Set spotligh position
                  (`SceneComponent.K2_SetRelativeLocation` (`self.SpotLight`) (`KismetMathLibrary.MakeVector` _targetedposition_x _targetedposition_y (+ _targetedposition_z (`self.ProjectorHeight`))) false false)))))
          (else
            (`self.SetActorTickEnabled` false)))
        (else
          (goto _label))))))

(event `self.Range.OnComponentBeginOverlap`
  (params (OverlappedComponent :type "PrimitiveComponent Object Reference") (OtherActor :type "Actor Object Reference") (OtherComp :type "PrimitiveComponent Object Reference") (OtherBodyIndex :type Integer) (bFromSweep :type Boolean) (SweepResult :type "HitResult Structure (by ref)"))
  ;[1 1 1] Overlap
  (cast `/Game/BP/BP_PlayerChara` OtherActor)
  (set `self.Overlapping` true))

(event `UpdateCatchTime`
  (params (CatchTime :type "Float (double-precision)"))
  (bind _timetogoaway (`self.TimeToGoAway`))
  (bind _returnvalue (`KismetMathLibrary.LinearColorLerp` (`self.LightStartColor`) (`self.LightGameOverColor`) (/ CatchTime _timetogoaway)))
  ;[1 1 1] Turn to red on overlap
  (if (< CatchTime _timetogoaway)
    (`LightComponent.SetLightColor` (`self.SpotLight`) _returnvalue true)
    (`/Game/BP/BP_PlayerChara.SetSceneTintToRed` (cast `/Game/BP/BP_PlayerChara` (`GameplayStatics.GetPlayerCharacter` 0) :!pure true) _returnvalue)
    (else
      (`Controller.SetIgnoreMoveInput` (`GameplayStatics.GetPlayerController` 0) true)
      (set `self.PlayerCaught` true)
      (`KismetSystemLibrary.Delay` 0.5)
      (`self.SpawnPortalUnderPlayer`))))

(event `self.Range.OnComponentEndOverlap`
  (params (OverlappedComponent :type "PrimitiveComponent Object Reference") (OtherActor :type "Actor Object Reference") (OtherComp :type "PrimitiveComponent Object Reference") (OtherBodyIndex :type Integer))
  ;[1 1 1] Overlap
  (cast `/Game/BP/BP_PlayerChara` OtherActor)
  (set `self.Overlapping` false))

(event `FocusPosition`
  (params (StartPosition :type "Vector Structure") (TargetPosition :type "Vector Structure"))
  ;[1 1 1] TO DO : ramener tous les projecteurs sur le perso
  (set `self.PlayerCaught` true))

(event `ResetCatchTime`
  ;[1 1 1] Set color back to normal
  (set `self.CurrentCatchDuration` 0.0)
  (`LightComponent.SetLightColor` (`self.SpotLight`) (`self.LightStartColor`) true)
  (`/Game/BP/BP_PlayerChara.SetSceneTintToWhite` (cast `/Game/BP/BP_PlayerChara` (`GameplayStatics.GetPlayerCharacter` 0) :!pure true))
  (`self.SetActorTickEnabled` true))

(event `SpawnPortalUnderPlayer`
  (bind _asbp_player_chara (cast `/Game/BP/BP_PlayerChara` (`GameplayStatics.GetPlayerCharacter` 0)))
  (bind _charactermovement (`Character.CharacterMovement` _asbp_player_chara))
  (`MovementComponent.StopMovementImmediately` _charactermovement)
  (`CharacterMovementComponent.AddImpulse` _charactermovement (0.0 0.0 1000.0) true)
  (`/Game/BP/Components/BPC_PortalSpawner.SpawnPortal` (`/Game/BP/BP_PlayerChara.BPC_PortalSpawner` _asbp_player_chara) (* (`KismetMathLibrary.Vector_Distance` (`self.K2_GetActorLocation` _asbp_player_chara) (`.ImpactPoint` (`GameplayStatics.BreakHitResult` (`.HitResult` (break `FindFloorResult` (`CharacterMovementComponent.CurrentFloor` _charactermovement)))))) 1.5) false)
  (`KismetSystemLibrary.Delay` 0.5)
  (set `self.PlayerCaught` false)
  (`self.ResetCatchTime`))

(event `CheckVisibility`
  (bind _returnvalue (`GameplayStatics.GetPlayerCharacter` 0))
  (bind _returnvalue_2 (`SceneComponent.K2_GetComponentLocation` (`self.SpotLight`)))
  (bind _returnvalue_3 (`self.K2_GetActorLocation` (`GameplayStatics.GetPlayerCharacter` 0)))
  ;[1 1 1] Raycast from the player to the spotlight
  (if (and (< (`KismetMathLibrary.DegAcos` (`KismetMathLibrary.Dot_VectorVector` (`KismetMathLibrary.Normal` (- _returnvalue_3 _returnvalue_2)) (`SceneComponent.GetForwardVector` (`self.SpotLight`)))) (`self.ProjectorAngle`)) (< (`KismetMathLibrary.Vector_Distance` _returnvalue_3 _returnvalue_2) (`self.LightRange`)))
    (bind (_outhit _returnvalue_4) (`KismetSystemLibrary.LineTraceSingle` (`self.K2_GetActorLocation` _returnvalue) (`SceneComponent.K2_GetComponentLocation` (`self.SpotLight`)) "TraceTypeQuery10" true (`|MakeArray` _returnvalue :!type "Actor Object Reference") "None" false))
    (set `self.PlayerIsVisible` (and _returnvalue_4 (== (`.HitActor` (`GameplayStatics.BreakHitResult` _outhit)) self)))
    (else
      (set `self.PlayerIsVisible` false))))

(fn `GetMaxDistance`
  (returns (Distance :type "Float (double-precision)"))
  (locals (MaxDistance :type "Float (double-precision)"))
  (for _array_element (`self.PathPoints`)
    (bind _returnvalue (`KismetMathLibrary.VSize` _array_element))
    (if (> _returnvalue (`local.MaxDistance`))
      (set `local.MaxDistance` _returnvalue)))
  (return (`local.MaxDistance`)))

(fn `UserConstructionScript`
  (locals (PathMaxIndex :type Integer) (ActorLocation :type "Vector Structure") (CurrentPoint :type "Vector Structure") (PreviousPoint :type "Vector Structure") (Direction :type "Vector Structure") (RightOffset :type "Vector Structure") (CurrentGroundRadius :type "Float (double-precision)") (PreviousGroundRadius :type "Float (double-precision)"))
  (bind (_returnvalue_x _returnvalue_y _returnvalue_z) (`KismetMathLibrary.BreakVector` (`self.K2_GetActorLocation`)))
  (bind (_returnvalue_x_2 _returnvalue_y_2 _returnvalue_z_2) (`KismetMathLibrary.BreakVector` (`self.K2_GetActorLocation`)))
  (bind _spotlight (`self.SpotLight`))
  (bind (_currentpoint_x _currentpoint_y _currentpoint_z) (`KismetMathLibrary.BreakVector` (`local.CurrentPoint`)))
  (bind _actorlocation (`local.ActorLocation`))
  (bind (_previouspoint_x _previouspoint_y _previouspoint_z) (`KismetMathLibrary.BreakVector` (`local.PreviousPoint`)))
  (bind _projectorangle (`self.ProjectorAngle`))
  (bind (_relativelocation_x _relativelocation_y) (`KismetMathLibrary.BreakVector` (`SceneComponent.RelativeLocation` (`self.SpotLight`))))
  (`SceneComponent.SetVisibility` (`self.Range`) (`self.DrawPreview`) false)
  (`SphereComponent.SetSphereRadius` (`self.Range`) (select `bool` (`self.UseCustomRange`) :`false` (+ (`self.GetMaxDistance`) 500.0) :`true` (`self.CustomRange`)) false)
  (`LocalLightComponent.SetAttenuationRadius` _spotlight (`self.LightRange`))
  (`LightComponent.SetLightColor` _spotlight (`self.LightStartColor`) true)
  (`LocalLightComponent.SetIntensityUnits` (`self.SpotLight`) (`self.LightUnits`))
  (`LightComponent.SetIntensity` (`self.SpotLight`) (`self.LightIntensity`))
  (`SpotLightComponent.SetOuterConeAngle` (`self.SpotLight`) (`self.ProjectorAngle`))
  (`SceneComponent.K2_SetRelativeLocation` (`self.SpotLight`) (`KismetMathLibrary.MakeVector` _relativelocation_x _relativelocation_y (`self.ProjectorHeight`)) false false)
  (`KismetSystemLibrary.FlushPersistentDebugLines`)
  (set `local.ActorLocation` (`self.K2_GetActorLocation`))
  (if (`self.DrawPreview`)
    (bind _output_get (set `local.PathMaxIndex` (- (`KismetArrayLibrary.Array_Length` (`self.PathPoints`)) 1)))
    (for _index (range (+ _output_get 1))
      ;[1 1 1] Calculate points
      (if (!= _index 0)
        (set `local.CurrentPoint` (+ _actorlocation (`|GetArrayItem` (`self.PathPoints`) _index)))
        (set `local.PreviousPoint` (+ (`|GetArrayItem` (`self.PathPoints`) (- _index 1)) _actorlocation))
        (set `local.CurrentGroundRadius` (* (`KismetMathLibrary.DegTan` _projectorangle) (- (+ (`self.ProjectorHeight`) _returnvalue_z) _currentpoint_z)))
        ;[1 1 1] Draw lines
        (set `local.PreviousGroundRadius` (* (`KismetMathLibrary.DegTan` _projectorangle) (- (+ (`self.ProjectorHeight`) _returnvalue_z_2) _previouspoint_z)))
        (bind _output_get_2 (set `local.Direction` (`KismetMathLibrary.Normal` (- (`local.CurrentPoint`) (`local.PreviousPoint`)))))
        (bind _returnvalue (`KismetMathLibrary.RotateAngleAxis` _output_get_2 90.0 (0.0 0.0 1.0)))
        (bind _returnvalue_2 (* _returnvalue (`local.CurrentGroundRadius`)))
        (`KismetSystemLibrary.DrawDebugLine` (+ (`local.PreviousPoint`) _returnvalue_2) (+ (`local.CurrentPoint`) _returnvalue_2) (`self.PreviewColor`) (`self.PreviewDuration`) (`self.PreviewThickness`))
        (bind _returnvalue_3 (* _returnvalue (`local.PreviousGroundRadius`)))
        (`KismetSystemLibrary.DrawDebugLine` (- (`local.PreviousPoint`) _returnvalue_3) (- (`local.CurrentPoint`) _returnvalue_3) (`self.PreviewColor`) (`self.PreviewDuration`) (`self.PreviewThickness`))))))