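; BP_ClassicJumpLink is a smart nav link that launches AI enemies toward the link destination.
; If IsDestinationAbove passes, AIJump computes velocity and flags charged jumps, which lock the link and set a blackboard flag during the delay before launch.
; Otherwise the enemy gets a fixed forward hop with slight lift.
; Enemies arriving while it is locked join a de-duplicated queue, served after charged jumps and hops.
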(event `self.ReceiveSmartLinkReached`
  (params (Agent :type "Actor Object Reference") (Destination :type "Vector Structure (by ref)"))
  ;[1 1 1] AI reaches link
  (set `self.Destination` Destination)
  (bind _asbp_enemy (cast `/Game/AI/Blueprints/BP_Enemy` Agent))
  (if (`self.Available`)
    (`self.PerformJump` _asbp_enemy)
    (elif (!= _asbp_enemy (`self.JumpingEnemy`))
      (`self.AddToQueue` _asbp_enemy))))

(event `PerformJump`
  (params (Enemy :type "/Game/AI/Blueprints/BP_Enemy Object Reference"))
  (bind _returnvalue (`AIBlueprintHelperLibrary.GetBlackboard` Enemy))
  (bind (_returnvalue_x _returnvalue_y _returnvalue_z) (`KismetMathLibrary.BreakVector` (`self.K2_GetActorLocation` Enemy)))
  (bind _destination (`self.Destination`))
  (bind _z (.z _destination))
  (bind _returnvalue_2 (- _returnvalue_z (`CapsuleComponent.GetScaledCapsuleHalfHeight` (`Character.CapsuleComponent` Enemy))))
  (set `self.JumpingEnemy` Enemy)
  (if (and (not (`/Game/AI/Blueprints/BP_Enemy.ChargingJump` Enemy)) (not (`NavMovementComponent.IsFalling` (`Character.CharacterMovement` Enemy))))
    ;[1 1 1] Orienter le perso dans la direction du saut
    (`/Game/AI/Blueprints/BP_Enemy.LookTowards` Enemy _destination)
    (if (or (< _returnvalue_2 _z) (< (`KismetMathLibrary.Abs` (- _returnvalue_2 _z)) (* (`KismetMathLibrary.Vector_Distance2D` (`self.K2_GetActorLocation` Enemy) _destination) 0.15)))
      ;[1 1 1] La destination est plus haute que le personnage ou suffisamment loin
      (bind (_needtocharge _velocity) (`/Game/BP/Libraries/BPL_Utilities.AIJump` Enemy _destination (`/Game/AI/Blueprints/BP_Enemy.ChargedJumpDistance` Enemy)))
      (if _needtocharge
        (set `self.Available` false)
        (bind _output_get (set `/Game/AI/Blueprints/BP_Enemy.ChargingJump` true Enemy))
        (`BlackboardComponent.SetValueAsBool` _returnvalue "ChargingJump" _output_get)
        (`KismetSystemLibrary.Delay` (`/Game/AI/Blueprints/BP_Enemy.ChargeDuration` Enemy))
        (`BlackboardComponent.SetValueAsBool` _returnvalue "ChargingJump" false)
        (`Character.LaunchCharacter` Enemy _velocity true true)
        (set `/Game/AI/Blueprints/BP_Enemy.ChargingJump` false Enemy)
        (set `self.Available` true)
        (`self.Next`))
      (else
        ;[1 1 1] L'inverse
        (`Character.LaunchCharacter` Enemy (+ (* (`KismetMathLibrary.Vector_Normal2D` (- _destination (`self.K2_GetActorLocation` Enemy))) 500.0) (* (`KismetMathLibrary.Vector_Up`) 100.0)) true true)
        (`KismetSystemLibrary.Delay` 0.2)
        (`self.Next`)))))

(event `Next`
  ;[1 1 1] Next enemy in queue
  (if (> (`KismetArrayLibrary.Array_Length` (`self.WaitingEnemies`)) 0)
    (`self.PerformJump` (`|GetArrayItem` (`self.WaitingEnemies`)))
    (`KismetArrayLibrary.Array_Remove` (`self.WaitingEnemies`))))

(event `AddToQueue`
  (params (Enemy :type "/Game/AI/Blueprints/BP_Enemy Object Reference"))
  ;[1 1 1] Add to queue
  (if (not (`KismetArrayLibrary.Array_Contains` (`self.WaitingEnemies`) Enemy))
    (`KismetArrayLibrary.Array_Add` (`self.WaitingEnemies`) Enemy)))

(fn `UserConstructionScript`)