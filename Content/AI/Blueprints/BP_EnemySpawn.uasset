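; Enemy spawn point that streams its chosen enemy type in and out by player proximity.
; When active, a one-second timer spawns the AI with configured vision within range and destroys it beyond range.
; The timer also writes player distance to the enemy's blackboard and updates the player's halo-range enemy list for nearby enemies.
; The construction script previews the mesh and vision cone in-editor and re-indexes all spawner IDs.
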(event `self.ReceiveBeginPlay`
  ;[1 0 0.8111] Begin play
  (bind _asbp_player_chara (cast `/Game/BP/BP_PlayerChara` (`GameplayStatics.GetPlayerCharacter` 0)))
  (set `self.PlayerChara` _asbp_player_chara)
  (`SceneComponent.SetVisibility` (`self.MeshPreview`) false false)
  (if (`self.Active`)
    (bind _returnvalue (`KismetSystemLibrary.K2_SetTimerDelegate` (delegate `CheckDistanceToPlayer`) 1.0 true))
    (set `self.CheckDistanceTimerHandle` _returnvalue)))

(event `CheckDistanceToPlayer`
  (bind _postprocesshalorange (`self.PostProcessHaloRange`))
  (bind _enemyspawned (`self.EnemySpawned`))
  (bind _returnvalue (`KismetMathLibrary.Vector_Distance` (`self.K2_GetActorLocation` _enemyspawned) (`self.K2_GetActorLocation` (`self.PlayerChara`))))
  ;[1 1 1] Check distance to player every second
  (if (`self.Spawned`)
    ;[1 1 1] Check distance between player and enemy
    (`BlackboardComponent.SetValueAsFloat` (`AIBlueprintHelperLibrary.GetBlackboard` _enemyspawned) "DistanceToPlayer" _returnvalue)
    (if (> _returnvalue (`self.EnemySpawnRange`))
      (`self.DeleteEnemy`)
      (if (`KismetArrayLibrary.Array_Contains` (`/Game/BP/BP_PlayerChara.EnemiesInHaloRange` (`self.PlayerChara`)) (`self.EnemySpawned`)) :!label _label
        (`KismetArrayLibrary.Array_RemoveItem` (`/Game/BP/BP_PlayerChara.EnemiesInHaloRange` (`self.PlayerChara`)) (`self.EnemySpawned`)))
      (elif (and (!= _returnvalue 0.0) (<= _returnvalue _postprocesshalorange))
        (if (not (`KismetArrayLibrary.Array_Contains` (`/Game/BP/BP_PlayerChara.EnemiesInHaloRange` (`self.PlayerChara`)) (`self.EnemySpawned`)))
          (`KismetArrayLibrary.Array_Add` (`/Game/BP/BP_PlayerChara.EnemiesInHaloRange` (`self.PlayerChara`)) (`self.EnemySpawned`)))
        (elif (> _returnvalue _postprocesshalorange)
          (goto _label))))
    (elif (< (`KismetMathLibrary.Vector_Distance` (`self.K2_GetActorLocation` (`self.PlayerChara`)) (`self.K2_GetActorLocation`)) (`self.EnemySpawnRange`))
      (`self.SpawnEnemy`))))

(event `self.ReceiveEndPlay`
  (params (EndPlayReason :type "EEndPlayReason Enum" :default "Destroyed"))
  ;[1 1 1] Destroy enemy on end play
  (if (`self.Spawned`)
    (`self.K2_DestroyActor` (`self.EnemySpawned`))))

(fn `DeleteEnemy`
  (`self.K2_DestroyActor` (`self.EnemySpawned`))
  (set `self.Spawned` false))

(fn `SpawnEnemy`
  (`KismetSystemLibrary.PrintString` "Enemy spawned")
  (bind _returnvalue (`AIBlueprintHelperLibrary.SpawnAIFromClass` (select `/Game/AI/Blueprints/EEnemyType` (`self.EnemyType`) :`NewEnumerator0` "/Game/AI/Blueprints/BP_Enemy.BP_Enemy_C" :`NewEnumerator2` "/Game/AI/Blueprints/BP_Enemy.BP_Enemy_C" :`NewEnumerator1` "/Game/AI/Blueprints/BP_Shrek.BP_Shrek_C" :!type "Pawn Class Reference") "/Game/AI/BT_Enemy.BT_Enemy" (`self.K2_GetActorLocation`) (`self.K2_GetActorRotation`) true))
  (bind _asbp_enemy (cast `/Game/AI/Blueprints/BP_Enemy` _returnvalue))
  (if (`|EnumEquality` (`self.EnemyType`) "NewEnumerator2")
    (`/Game/AI/Blueprints/BP_Enemy.SetBroken` _asbp_enemy))
  (bind _output_get (set `self.EnemySpawned` _asbp_enemy))
  (set `/Game/AI/Blueprints/BP_Enemy.SpawnRef` self _output_get)
  (bind _pawnsensing (`/Game/AI/Blueprints/BP_Enemy.PawnSensing` _output_get))
  (`PawnSensingComponent.SetPeripheralVisionAngle` _pawnsensing (`self.VisionAngle`))
  (set `PawnSensingComponent.SightRadius` (`self.VisionRadius`) _pawnsensing)
  (set `self.Spawned` true)
  (return))

(fn `UserConstructionScript`
  (locals (EnemyMesh :type "SkeletalMesh Object Reference"))
  (`KismetSystemLibrary.FlushPersistentDebugLines`)
  (`KismetSystemLibrary.DrawDebugConeInDegrees` (`SceneComponent.GetSocketLocation` (`self.MeshPreview`) "Head") (`self.GetActorForwardVector`) (`self.VisionRadius`) (`self.VisionAngle`) 90.0 12 (struct :`G` 0.121957 :`B` 0.713542 :`A` 1.0) 10.0 10.0)
  (set `local.EnemyMesh` (select `/Game/AI/Blueprints/EEnemyType` (`self.EnemyType`) :`NewEnumerator0` "/Game/Character/Robot/SK_Mesh/SK_Robot_Mesh.SK_Robot_Mesh" :`NewEnumerator2` "/Game/Character/Robot/SK_Mesh/SK_Robot_Mesh.SK_Robot_Mesh" :`NewEnumerator1` "/Game/AI/Animation/ShrekAnimated/CHARACTER_Shrek.CHARACTER_Shrek" :!type "SkeletalMesh Object Reference"))
  (`SkinnedMeshComponent.SetSkinnedAssetAndUpdate` (`self.MeshPreview`) (`local.EnemyMesh`) true)
  (bind _outactors (`GameplayStatics.GetAllActorsOfClass` "BP_EnemySpawn_C"))
  (for (_array_element _array_index) _outactors
    (set `/Game/AI/Blueprints/BP_EnemySpawn.ID` _array_index _array_element)))