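; BP_Shrek is an AI enemy, derived from a parent class, that detects and catches the player.
; It destroys its SpotLight at start, and detection marks it awake with the player in sight in both blackboard and variables.
; On a catch it runs the parent logic, then after a delay shrinks its mesh and crystallizes.
; A second delay clears the player's CaughtRecently flag.
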(event `self.ReceiveBeginPlay`
  (`ActorComponent.K2_DestroyComponent` (`self.SpotLight`))
  (`parent.ReceiveBeginPlay`))

(event `self.DetectPlayer`
  (`BlackboardComponent.SetValueAsBool` (`AIBlueprintHelperLibrary.GetBlackboard` null) "PlayerInSight" true)
  (`BlackboardComponent.SetValueAsBool` (`AIBlueprintHelperLibrary.GetBlackboard` null) "Awake" true)
  (`BlackboardComponent.SetValueAsBool` (`AIBlueprintHelperLibrary.GetBlackboard` null) "InSleepMode" false)
  (set `self.InSleepMode` false)
  (set `self.Awake` true)
  (set `self.PlayerInSight` true))

(event `self.CatchPlayer`
  (`parent.CatchPlayer`)
  (`KismetSystemLibrary.Delay` 1.0)
  (`SceneComponent.SetRelativeScale3D` (`self.Mesh`) (0.1 0.1 0.1))
  (`self.Crystallize` 1.0)
  (`KismetSystemLibrary.Delay` 2.0)
  (set `/Game/BP/BP_PlayerChara.CaughtRecently` false (`self.PlayerChara`)))

(fn `UserConstructionScript`
  (`parent.UserConstructionScript`))